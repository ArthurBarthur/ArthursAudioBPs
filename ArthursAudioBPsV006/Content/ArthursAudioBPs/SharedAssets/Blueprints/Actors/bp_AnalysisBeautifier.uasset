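; Actor that turns raw magnitudes from a referenced SubmixAnalyzer into smoothed 0–1 values per analyzed frequency.
; Each Tick it records peak magnitudes, normalizes against them (per frequency or against the overall top peak), then interpolates with separate attack and release speeds.
; A looping one-second timer re-arms a DoOnce that decays the stored peaks by five percent, so normalization adapts to changing loudness.
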(event `self.ReceiveBeginPlay`
  ;[1 1 1] beginplay
  (`|ExecutionSequence`
    (:`then_0`
      ;[1 1 1] get frequencies to analyze from SubmixAnalyzer
      (set `self.FrequenciesToAnalyze` (`/Game/ArthursAudioBPs/SharedAssets/Blueprints/Actors/bp_SubmixAnalyzer.FrequenciesToAnalyze` (`self.SubmixAnalyzerRef`))))
    (:`then_1`
      ;[1 1 1] initialize array of max magnitudes
      (for (_ _array_index) (`self.FrequenciesToAnalyze`)
        (`KismetArrayLibrary.Array_Set` (`self.MaxMagnitudes`) _array_index 0.0 true)))
    (:`then_2`
      ;[1 1 1] Enable Tick
      (`self.SetActorTickEnabled` true))
    (:`then_3`
      ;[1 1 1] Set up looping timer for DecreaseMaxValuesEvent
      (`KismetSystemLibrary.K2_SetTimerDelegate` (`|CreateDelegate` :!event `DecreaseMaxValues`) 1.0 true))))

(event `self.ReceiveTick`
  (params (DeltaSeconds :type "Float (single-precision)"))
  ;[1 1 1] Tick
  (set `self.DeltaTick` DeltaSeconds)
  (`|ExecutionSequence`
    (:`then_0`
      ;[1 1 1] get latest central analysis
      (set `self.LatestMagnitudes` (`/Game/ArthursAudioBPs/SharedAssets/Blueprints/Actors/bp_SubmixAnalyzer.LatestMagnitudes` (`self.SubmixAnalyzerRef`))))
    (:`then_1`
      ;[1 1 1] store max recorded magnitudes
      (`self.StoreMaxMagnitudes`))
    (:`then_2`
      ;[1 1 1] normalize. (magnitudes to 0-1)
      (`self.NormalizeMagnitudes`))
    (:`then_3`
      ;[1 1 1] smoothing.
      (`|ExecutionSequence`
        (:`then_0`
          (`/Engine/EditorBlueprintResources/StandardMacros.DoOnce` false
            (:`Completed`
              (`self.InitSmoothing`))))
        (:`then_1`
          ;;[1 1 1] smoothen values
          (`self.Smoothing`))))
    (:`then_4`
      ;[1 1 1] DecreaseHistoricMaxValues
      (`/Engine/EditorBlueprintResources/StandardMacros.DoOnce` true :!label _label
        (:`Completed`
          (`self.DecreaseHistoricMaxMagnitudes`))))))

(event `DecreaseMaxValues`
  ;[1 1 1] DecreaseHistoricMaxValues
  (goto _label :!via `Reset`))

(fn `DecreaseHistoricMaxMagnitudes`
  (for (_array_element _array_index) (`self.MaxMagnitudes`)
    (`KismetArrayLibrary.Array_Set` (`self.MaxMagnitudes`) _array_index (* _array_element 0.95))))

(fn `InitSmoothing`
  ;[1 1 1] fill smoothed values array with the correct amount of zeroes
  (for (_ _array_index) (`self.NormalizedValues`)
    (`KismetArrayLibrary.Array_Set` (`self.SmoothedValues`) _array_index 0.0 true)))

(fn `NormalizeMagnitudes`
  (locals (_currentIndex :type Integer))
  ;[1 1 1] Normalize all freqs independently?
  (if (not (`self.NormalizeEachFrequencyIndependently`))
    (`self.UseOnlyTopMagnitudeForMax`))
  ;[1 1 1] loop through latest magnitudes
  (for (_array_element _array_index) (`self.LatestMagnitudes`)
    (set `local._currentIndex` _array_index)
    ;[1 1 1] Store Normalized magnitudes
    (`KismetArrayLibrary.Array_Set` (`self.NormalizedValues`) (`local._currentIndex`) (`KismetMathLibrary.MapRangeClamped` _array_element 0.0 (`|GetArrayItem` (`self.MaxMagnitudes`) (`local._currentIndex`)) 0.0 1.0) true)))

(fn `Smoothing`
  (locals (_latestNormalizedValue :type "Float (double-precision)") (_currentIndex :type Integer) (_latestSmoothValue :type "Float (double-precision)" :default 0.0))
  ;[1 1 1] loop through normalized values
  (for (_array_element _array_index) (`self.NormalizedValues`)
    (set `local._latestNormalizedValue` _array_element)
    (set `local._currentIndex` _array_index)
    ;[1 1 1] store smoothed values
    (`KismetArrayLibrary.Array_Set` (`self.SmoothedValues`) (`local._currentIndex`) (`KismetMathLibrary.FInterpTo` (`|GetArrayItem` (`self.SmoothedValues`) (`local._currentIndex`)) (`local._latestNormalizedValue`) (`self.DeltaTick`) (select `bool` (> (`local._latestNormalizedValue`) (`|GetArrayItem` (`self.SmoothedValues`) (`local._currentIndex`))) :`false` (`self.Release`) :`true` (`self.Attack`))) true)))

(fn `StoreMaxMagnitudes`
  (locals (_latestMagnitude :type "Float (double-precision)") (_currentIndex :type Integer))
  ;[1 1 1] loop through latest magnitudes
  (for (_array_element _array_index) (`self.LatestMagnitudes`)
    (set `local._latestMagnitude` _array_element)
    (set `local._currentIndex` _array_index)
    ;[1 1 1] store if current is an historic max value
    (if (> (`local._latestMagnitude`) (`|GetArrayItem` (`self.MaxMagnitudes`) (`local._currentIndex`)))
      (`KismetArrayLibrary.Array_Set` (`self.MaxMagnitudes`) (`local._currentIndex`) (`local._latestMagnitude`) true))))

(fn `UseOnlyTopMagnitudeForMax`
  (locals (_TopMagnitude :type "Float (double-precision)" :default 0.0))
  ;[1 1 1] get top magnitude of all
  (set `local._TopMagnitude` (`.MaxValue` (`KismetMathLibrary.MaxOfFloatArray` (`self.MaxMagnitudes`))))
  ;[1 1 1] write top value to all records
  (for (_ _array_index) (`self.MaxMagnitudes`)
    (`KismetArrayLibrary.Array_Set` (`self.MaxMagnitudes`) _array_index (`local._TopMagnitude`) true)))

(fn `UserConstructionScript`)