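; SoundPlayer is an actor that plays a sound wave through a granular synth component, configured from a preset.
; On BeginPlay it copies the GranularPreset's envelope, playhead and grain settings onto the synth, then assigns the Sound wave.
; After a short delay it activates and starts the synth and triggers a single note-on, with no further control after startup.
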(event `self.ReceiveBeginPlay`
  (bind _granularsynth (`self.GranularSynth`))
  (bind (_attackmsec _releasemsec _decaymsec _sustaingain _playheadpossec _playheadlerpsec _playheadseektype _playheadspeedrate _grainspersecond _grainprobability _volumebase _volumerange _durationbasemsec _durationrange _panbase _panrange _pitchbase _pitchrange _scrubmode _envelopetype) (break `/Game/ArthursAudioBPs/Examples/GranularSynth/GranularBPs/granularPreset` (`self.GranularPreset`)))
  (`|ExecutionSequence`
    (:`then_0`
      (`|ExecutionSequence`
        (:`then_0`
          ;[1 1 1] ADSR
          (`GranularSynth.SetAttackTime` _granularsynth _attackmsec))
        (:`then_1`
          (`GranularSynth.SetReleaseTimeMsec` _granularsynth _releasemsec))
        (:`then_2`
          (`GranularSynth.SetDecayTime` _granularsynth _decaymsec))
        (:`then_3`
          (`GranularSynth.SetSustainGain` _granularsynth _sustaingain))
        (:`then_4`
          (`GranularSynth.SetPlayheadTime` _granularsynth _playheadpossec _playheadlerpsec _playheadseektype))
        (:`then_5`
          (`GranularSynth.SetPlaybackSpeed` _granularsynth _playheadspeedrate))
        (:`then_6`
          (`GranularSynth.SetGrainsPerSecond` _granularsynth _grainspersecond))
        (:`then_7`
          (`GranularSynth.SetGrainProbability` _granularsynth _grainprobability))
        (:`then_8`
          (`GranularSynth.SetGrainVolume` _granularsynth _volumebase _volumerange))
        (:`then_9`
          (`GranularSynth.SetGrainDuration` _granularsynth _durationbasemsec _durationrange))
        (:`then_10`
          (`GranularSynth.SetGrainPan` _granularsynth _panbase _panrange))
        (:`then_11`
          (`GranularSynth.SetGrainPitch` _granularsynth _pitchbase _pitchrange))
        (:`then_12`
          (`GranularSynth.SetScrubMode` _granularsynth _scrubmode))
        (:`then_13`
          (`GranularSynth.SetGrainEnvelopeType` _granularsynth _envelopetype))))
    (:`then_1`
      (`GranularSynth.SetSoundWave` (`self.GranularSynth`) (`self.Sound`)))
    (:`then_2`
      (`KismetSystemLibrary.Delay` 0.2)
      (`ActorComponent.Activate` (`self.GranularSynth`) false)
      (`SynthComponent.Start` (`self.GranularSynth`))
      (`GranularSynth.NoteOn` (`self.GranularSynth`) 60.0 100 -1.0))))

(fn `UserConstructionScript`)