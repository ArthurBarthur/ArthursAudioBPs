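; Actor that endlessly plays random notes or chords on a Modular Synth with randomized presets, while its cube glows with the audio.
; Each cycle rolls seed, note, velocity and timings, gets a preset from RandomizerType, plays, fades out, then repeats.
; A waveshaper source effect's output gain serves as volume, ducking preset swaps and driving the timeline fade.
; The peak-normalized envelope drives emissive brightness, and SavePreset stores the current preset in a bank.
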(event `self.ReceiveBeginPlay`
  ;[1 1 1] create dynamic material(MID)
  (bind _returnvalue (`PrimitiveComponent.CreateDynamicMaterialInstance` (`self.Cube`) 0 "/Game/ArthursAudioBPs/SharedAssets/Materials/m_SimpleMat_Inst1.m_SimpleMat_Inst1" "None"))
  (set `self.MID` _returnvalue)
  ;[1 1 1] init synth
  (`self.InitSynth`)
  (`KismetSystemLibrary.Delay` 0.2)
  ;[1 1 1] trigger first note
  (`self.PlayRandomNote`))

(event `self.ModularSynth.OnAudioEnvelopeValue`
  (params (EnvelopeValue :type "Float (single-precision)"))
  ;[1 1 1] latest envelope
  (set `self.EnvLatest` EnvelopeValue)
  ;[1 1 1] normalize
  (if (> (`self.EnvLatest`) (`self.EnvMax`))
    (set `self.EnvMax` (`self.EnvLatest`)))
  (set `self.EnvNormalized` (`KismetMathLibrary.MapRangeClamped` (`self.EnvLatest`) 0.0 (`self.EnvMax`) 0.0 1.0))
  ;[1 1 1] mod MID emissive
  (`MaterialInstanceDynamic.SetScalarParameterValue` (`self.MID`) "Emissive Multiplier" (* (`self.EnvNormalized`) 30.0)))

(event `PlayRandomNote`
  ;[1 1 1] Trigger note
  ;[1 1 1] set current randomizer parameters
  (set `self.CurrentRandomSeed` (`KismetMathLibrary.RandomIntegerInRange` (`self.RandomSeedMin`) (`self.RandomSeedMax`)))
  (set `self.CurrentNote` (`KismetMathLibrary.Conv_IntToDouble` (`KismetMathLibrary.RandomIntegerInRange` (`self.NoteMin`) (`self.NoteMax`))))
  (set `self.CurrentVelocity` (`KismetMathLibrary.RandomIntegerInRange` (`self.VelocityMin`) (`self.VelocityMax`)))
  (set `self.CurrentDuration` (`KismetMathLibrary.RandomFloatInRange` (`self.NoteDurationMin(seconds)`) (`self.NoteDurationMax(seconds)`)))
  (set `self.CurrentTailDuration` (`KismetMathLibrary.RandomFloatInRange` (`self.TailDurationMin(seconds)`) (`self.TailDurationMax(seconds)`)))
  ;[1 1 1] change preset + note
  ;;[1 1 1] turn down volume on source effect
  (`self.ModSourceEffectWaveshaper` -60.0)
  ;;[1 1 1] get new preset
  (`self.GetNewRandomPreset` (`self.CurrentRandomSeed`))
  (`ModularSynthComponent.SetSynthPreset` (`self.ModularSynth`) (`self.CurrentSynthPreset`))
  ;;[1 1 1] turn up volume on source effect
  (`self.ModSourceEffectWaveshaper` 0.0)
  (if (`self.PlayChordInsteadOfNote`)
    ;;[1 1 1] play chord instead
    (bind _midinotes (`/Game/ArthursAudioBPs/SharedAssets/Blueprints/Components/ChordComponent/ChordComponent.BuildChord` (`self.bpc_chords`) (`self.ChordSettings`)))
    (bind _output_get (set `self.MidiNotes` _midinotes))
    (for _array_element _output_get
      (`ModularSynthComponent.NoteOn` (`self.ModularSynth`) _array_element (`self.CurrentVelocity`) (`self.CurrentDuration`)))
    (else
      ;;[1 1 1] Play random note
      (`ModularSynthComponent.NoteOn` (`self.ModularSynth`) (`self.CurrentNote`) (`self.CurrentVelocity`) (`self.CurrentDuration`))))
  ;;[1 1 1] Wait for note duration
  (`KismetSystemLibrary.Delay` (`self.CurrentDuration`))
  ;;[1 1 1] update tail/fadeout time
  (`TimelineComponent.SetPlayRate` (`self.SoundFade 1sec`) (/ 1.0 (`self.CurrentTailDuration`)))
  ;[1 1 1] tail/fade out audio via source effect
  (bind (_direction _1_0) (`Timeline|SoundFade 1sec` :!via `PlayFromStart`)
    (:`Update`
      (`self.ModSourceEffectWaveshaper` (`KismetMathLibrary.MapRangeClamped` _1_0 1.0 0.0 0.0 -60.0)))
    (:`Finished`
      ;[1 1 1] all notes off
      (`ModularSynthComponent.NoteOff` (`self.ModularSynth`) 0.0 true true)
      ;[1 1 1] return to start and go again
      (`self.PlayRandomNote`))))

(event `SavePreset`
  ;[1 1 1] save preset to bank
  (`ModularSynthLibrary.AddModularSynthPresetToBankAsset` (`self.CustomSavesPresetBank`) (`self.CurrentSynthPreset`) "SavedCustomPreset"))

(fn `GetNewRandomPreset`
  (params (RandomSeed :type Integer))
  ;[1 1 1] get randomized preset(run randomize function in randomizer data blueprint)
  (bind _synthpresetfinal (`/Game/ArthursAudioBPs/SharedAssets/Blueprints/RandomPresetGenerators/DataAssets/DataPrimary_RandomPresets.RandomizePresetFull` (`self.RandomizerType`) RandomSeed))
  (set `self.CurrentSynthPreset` _synthpresetfinal))

(fn `InitSynth`
  ;[1 1 1] GetARandomPreset
  (`self.GetNewRandomPreset` 0)
  ;[1 1 1] init base preset
  (`ModularSynthComponent.SetSynthPreset` (`self.ModularSynth`) (`self.CurrentSynthPreset`))
  ;[1 1 1] activate synth
  (`ActorComponent.Activate` (`self.ModularSynth`) false))

(fn `ModSourceEffectWaveshaper`
  (params (OutputGainDb :type "Float (double-precision)"))
  (`SourceEffectWaveShaperPreset.SetSettings` (`self.SourceEffectWaveshaper`) (make `SourceEffectWaveShaperSettings` (`.Amount` (break `SourceEffectWaveShaperSettings` (`SourceEffectWaveShaperPreset.Settings` (`self.SourceEffectWaveshaper`)))) OutputGainDb)))

(fn `UserConstructionScript`)