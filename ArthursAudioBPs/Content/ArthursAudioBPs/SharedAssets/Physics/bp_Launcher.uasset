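; Launcher actor that periodically spawns an actor of a configurable class and fires it along the launcher's up vector.
; After an initial delay it starts a looping timer and launches immediately.
; Shortly after each spawn, it enables CCD, gravity and physics on the first static mesh and applies a mass-independent impulse.
; A self-destruct component then limits lifetime to the launch interval or an override.
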(event `self.ReceiveBeginPlay`
  (`KismetSystemLibrary.Delay` (`self.InitialDelay`))
  ;[1 1 1] LaunchTimer
  (`KismetSystemLibrary.K2_SetTimerDelegate` (`|CreateDelegate` :!event `Launch`) (`self.LaunchInterval`) true)
  (`self.Launch`))

(event `Launch`
  ;[1 1 1] Spawn thing to be launched
  (bind _returnvalue (`|SpawnActorFromClass` (`self.ClassToSpawn`) (`self.GetTransform`) "DontSpawnIfColliding" "OverrideRootScale" null null))
  (set `self.LatestSpawnedActor` _returnvalue)
  (`KismetSystemLibrary.Delay` 0.2)
  ;[1 1 1] add impulse to launched obj
  (`self.AddImpulse`)
  ;[1 1 1] add time to live selfdestruct component to actor
  (`AddComponent|NODE_Addbpc_timeToLive-2` :`self` (`self.LatestSpawnedActor`) :`TimeToLive` (select `bool` (`self.OverrideBallTTL`) :`false` (`self.LaunchInterval`) :`true` (`self.TTL(override)`))))

(fn `AddImpulse`
  (locals (_MeshComponent :type "StaticMeshComponent Object Reference"))
  ;[1 1 1] Add impulse to first mesh in launchd obj
  (set `local._MeshComponent` (`self.GetComponentByClass` (`self.LatestSpawnedActor`) "/Script/Engine.StaticMeshComponent"))
  (`PrimitiveComponent.SetUseCCD` (`local._MeshComponent`) true "None")
  (`PrimitiveComponent.SetEnableGravity` (`local._MeshComponent`) true)
  (`PrimitiveComponent.SetSimulatePhysics` (`local._MeshComponent`) true)
  (`PrimitiveComponent.AddImpulse` (`local._MeshComponent`) (* (`self.GetActorUpVector`) (`self.LaunchImpulseMP`)) "None" true))

(fn `UserConstructionScript`)