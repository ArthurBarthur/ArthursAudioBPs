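; Component that normalizes and smooths an incoming envelope value, likely from audio, into a 0–1 signal.
; Beautify tracks the highest value seen, remaps input against it, then interpolates at constant speed using Tick's delta time.
; A looping timer is set to decay that maximum, so normalization adapts over time.
; Smoothing speed depends on direction, with the release time applied to rising values and attack to falling ones.
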(event `self.ReceiveBeginPlay`
  ;[1 1 1] Set up looping timer for DecreaseMaxValuesEvent
  (`KismetSystemLibrary.K2_SetTimerDelegate` (`|CreateDelegate` :!event `CustomEventDecreaseMaxValues`) 0.5 true))

(event `self.ReceiveTick`
  (params (DeltaSeconds :type "Float (single-precision)"))
  (set `self.DeltaTick` DeltaSeconds))

(event `CustomEventDecreaseMaxValues`
  ;[1 1 1] DecreaseHistoricMaxValue
  (bind _output_get (set `self.EnvMax` (* (stale _output_get) 0.95))))

(fn `Beautify`
  (params (EnvLatest :type "Float (double-precision)") (`Attack(in milliseconds)` :type "Float (double-precision)" :default 100.0) (`Release(in milliseconds)` :type "Float (double-precision)" :default 500.0))
  (returns (EnvSmoothed :type "Float (double-precision)"))
  (set `self.EnvLatest` EnvLatest)
  (set `self.Attack(in milliseconds)` `Attack(in milliseconds)`)
  (set `self.Release(in milliseconds)` `Release(in milliseconds)`)
  ;[1 1 1] store if current is an historic max value
  (if (> (`self.EnvLatest`) (`self.EnvMax`))
    (set `self.EnvMax` (`self.EnvLatest`)))
  ;[1 1 1] normalize
  ;;[1 1 1] Store Normalized value
  (set `self.EnvNormalized` (`KismetMathLibrary.MapRangeClamped` (`self.EnvLatest`) 0.0 (`self.EnvMax`) 0.0 1.0))
  ;[1 1 1] smoothing
  (set `self.EnvSmoothed` (`KismetMathLibrary.FInterpTo_Constant` (`self.EnvSmoothed`) (`self.EnvNormalized`) (`self.DeltaTick`) (select `bool` (> (`self.EnvNormalized`) (`self.EnvSmoothed`)) :`false` (/ 1.0 (/ (`self.Attack(in milliseconds)`) 1000.0)) :`true` (/ 1.0 (/ (`self.Release(in milliseconds)`) 1000.0)))))
  (return (`self.EnvSmoothed`)))