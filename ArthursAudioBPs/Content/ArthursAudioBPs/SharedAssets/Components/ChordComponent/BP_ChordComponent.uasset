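; Actor component that builds a chord as an array of MIDI note numbers for its parent actor.
; BuildChord takes root note, chord type, octave and extra octaves, then offsets the chord type's intervals from ChordTypeStruct by root and octave.
; Extra octaves add unique transposed copies after the base chord, with out-of-range MIDI notes dropped.
; The EventGraph holds only an unconnected example call.
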(fn `BuildChord`
  (params (ChordSettings :type "/Game/ArthursAudioBPs/SharedAssets/Components/ChordComponent/FChordSettings Structure"))
  (returns (MidiNotes :type "Array of Float (double-precision)"))
  (locals (_currentNote :type "Float (double-precision)" :default 0.0) (_extraOctavesMidiNotes :type "Array of Float (double-precision)") (_localChordSettings :type "/Game/ArthursAudioBPs/SharedAssets/Components/ChordComponent/FChordSettings Structure") (_MidiNotes :type "Array of Float (double-precision)") (_ChordTypeStruct :type "/Game/ArthursAudioBPs/SharedAssets/Components/ChordComponent/FChordTypes Structure"))
  (bind (_major _minor _7th _major7th _minor7th _augmented _diminished) (break `/Game/ArthursAudioBPs/SharedAssets/Components/ChordComponent/FChordTypes` (`local._ChordTypeStruct`)))
  ;[1 1 1] input
  (set `local._localChordSettings` ChordSettings)
  (`KismetArrayLibrary.Array_Clear` (`local._MidiNotes`))
  (`KismetArrayLibrary.Array_Clear` (`local._extraOctavesMidiNotes`))
  ;[1 1 1] make chord notes
  (for _array_element (select `/Game/ArthursAudioBPs/SharedAssets/Components/ChordComponent/EChordType` (`.ChordType_10_2FE802A14ABB2A0197E9C0B96E6A6BBE` (break `/Game/ArthursAudioBPs/SharedAssets/Components/ChordComponent/FChordSettings` (`local._localChordSettings`))) :`NewEnumerator1` _major :`NewEnumerator0` _minor :`NewEnumerator4` _7th :`NewEnumerator2` _major7th :`NewEnumerator3` _minor7th :`NewEnumerator5` _augmented :`NewEnumerator6` _diminished)
    ;;[1 1 1] current note
    (set `local._currentNote` (+ (+ _array_element (`KismetMathLibrary.Conv_IntToDouble` (select `/Game/ArthursAudioBPs/SharedAssets/Components/ChordComponent/ERootNotes` (`.RootNote_8_1B9983E34417FE94FF044984B6F48F2F` (break `/Game/ArthursAudioBPs/SharedAssets/Components/ChordComponent/FChordSettings` (`local._localChordSettings`))) :`NewEnumerator1` 1 :`NewEnumerator2` 2 :`NewEnumerator3` 3 :`NewEnumerator4` 4 :`NewEnumerator5` 5 :`NewEnumerator6` 6 :`NewEnumerator7` 7 :`NewEnumerator8` 8 :`NewEnumerator9` 9 :`NewEnumerator10` 10 :`NewEnumerator11` 11))) (`KismetMathLibrary.Conv_IntToDouble` (* 12 (`.Octave_11_31CCB5444832592EF6E4A0AE992BB897` (break `/Game/ArthursAudioBPs/SharedAssets/Components/ChordComponent/FChordSettings` (`local._localChordSettings`)))))))
    ;;[1 1 1] in midi note range?
    (if (`KismetMathLibrary.InRange_FloatFloat` (`local._currentNote`) 0.0 127.0)
      ;;[1 1 1] add to array
      (`KismetArrayLibrary.Array_Add` (`local._MidiNotes`) (`local._currentNote`))))
  ;[1 1 1] add any extra octaves
  ;;[1 1 1] add octaves if non-zero
  (for _index (range (+ (`.ExtraOctaves_12_4AEB15524D235AC20A0190B67EA16A7A` (break `/Game/ArthursAudioBPs/SharedAssets/Components/ChordComponent/FChordSettings` (`local._localChordSettings`))) 1))
    (if (not (== _index 0))
      ;;[1 1 1] add extra notes to array if in range and unique
      (for _array_element_2 (`local._MidiNotes`)
        (bind _returnvalue (+ _array_element_2 (`KismetMathLibrary.Conv_IntToDouble` (* _index 12))))
        (if (`KismetMathLibrary.InRange_FloatFloat` _returnvalue 1.0 127.0)
          (`KismetArrayLibrary.Array_AddUnique` (`local._extraOctavesMidiNotes`) _returnvalue)))))
  ;;[1 1 1] Combine base chord and octaved chord arrays
  (`KismetArrayLibrary.Array_Append` (`local._MidiNotes`) (`local._extraOctavesMidiNotes`))
  ;[1 1 1] output
  (return (`local._MidiNotes`)))