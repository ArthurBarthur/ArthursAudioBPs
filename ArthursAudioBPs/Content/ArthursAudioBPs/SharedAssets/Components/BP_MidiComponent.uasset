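; BP_MidiComponent is an actor component that finds MIDI input and output devices by partial name for its parent actor.
; FindMidiDevice lists all devices on screen, keeps the last name match that can receive or send, and creates a controller for each.
; It returns found flags and controller variables, but the created output controller is never stored.
; The EventGraph holds only an unconnected example call, so the parent must call the function.
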(fn `FindMidiDevice`
  (params (MidiDeviceInputNameContains :type String) (MidiDeviceOutputNameContains :type String))
  (returns (FoundValidMidiInputDevice :type Boolean) (MidiDeviceInputController :type "MIDIDeviceInputController Object Reference") (FoundMidiOutputDevice :type Boolean) (MidiDeviceOutputController :type "MIDIDeviceOutputController Object Reference"))
  (bind _selectedmidiinputdeviceid (`self.SelectedMidiInputDeviceID`))
  (bind _selectedmidioutputdeviceid (`self.SelectedMidiOutputDeviceID`))
  ;[1 1 1] input
  (`|ExecutionSequence`
    (:`then_0`
      ;[1 1 1] set midi name to search for
      (set `self.MidiInputDeviceNameContainsThis` MidiDeviceInputNameContains)
      (set `self.MidiOutputDeviceNameContainsThis` MidiDeviceOutputNameContains)
      ;[1 1 1] reset any previous results
      (set `self.SelectedMidiInputDeviceID` -1)
      (set `self.SelectedMidiOutputDeviceID` -1)
      (`KismetArrayLibrary.Array_Clear` (`self.AllDevices`)))
    (:`then_1`
      ;[1 1 1] store all midi devices
      (bind _outmididevices (`MIDIDeviceManager.FindMIDIDevices`))
      (set `self.MidiDevices` _outmididevices))
    (:`then_2`
      ;[1 1 1] add all device names to list
      (for _array_element (`self.MidiDevices`)
        (`KismetArrayLibrary.Array_Add` (`self.AllDevices`) (`.DeviceName` (break `FoundMIDIDevice` _array_element))))
      ;[1 1 1] print list of all devices
      (`KismetSystemLibrary.PrintString` (`KismetStringLibrary.Concat_StrStr` " \nAll midi devices: \n" (`KismetStringLibrary.JoinStringArray` (`self.AllDevices`) "  \n") " \n") true true (struct :`G` 0.66 :`B` 1.0 :`A` 1.0) 10.0))
    (:`then_3`
      ;[1 1 1] Find input device
      (for _array_element_2 (`self.MidiDevices`)
        (bind (_deviceid _devicename _bcanreceivefrom) (break `FoundMIDIDevice` _array_element_2))
        ;[1 1 1] store input device
        (if (and (`KismetStringLibrary.Contains` _devicename (`self.MidiInputDeviceNameContainsThis`)) _bcanreceivefrom)
          (set `self.SelectedMidiInputDeviceID` _deviceid))))
    (:`then_4`
      ;[1 1 1] Find output device
      (for _array_element_3 (`self.MidiDevices`)
        (bind (_deviceid_2 _devicename_2 _bcanreceivefrom_2 _bcansendto) (break `FoundMIDIDevice` _array_element_3))
        ;[1 1 1] store output device
        (if (and (`KismetStringLibrary.Contains` _devicename_2 (`self.MidiOutputDeviceNameContainsThis`)) _bcansendto)
          (set `self.SelectedMidiOutputDeviceID` _deviceid_2))))
    (:`then_5`
      ;[1 1 1] print name of found input device
      (bind _output_get (set `self.FoundMidiInputDevice` (> (`self.SelectedMidiInputDeviceID`) -1)))
      (if _output_get
        (`KismetSystemLibrary.PrintString` (`KismetStringLibrary.Concat_StrStr` "Selected Input Device: " (`.DeviceName` (break `FoundMIDIDevice` (`|GetArrayItem` (`self.MidiDevices`) _selectedmidiinputdeviceid))) (`KismetStringLibrary.Conv_IntToString` _selectedmidiinputdeviceid)) true true (struct :`G` 0.66 :`B` 1.0 :`A` 1.0) 10.0)
        ;[1 1 1] create midi input controller from found device id
        (bind _returnvalue (`MIDIDeviceManager.CreateMIDIDeviceInputController` (`self.SelectedMidiInputDeviceID`)))
        (set `self.MidiDeviceInputController` _returnvalue)
        (else
          ;[1 1 1] print could not find
          (`KismetSystemLibrary.PrintString` (`KismetStringLibrary.Concat_StrStr` "Could not find midi input device containing " "\"" (`self.MidiInputDeviceNameContainsThis`) "\"") true true (struct :`G` 0.66 :`B` 1.0 :`A` 1.0) 10.0))))
    (:`then_6`
      ;[1 1 1] print name of found output device
      (bind _output_get_2 (set `self.FoundMidiOutputDevice` (> (`self.SelectedMidiOutputDeviceID`) -1)))
      (if _output_get_2
        (`KismetSystemLibrary.PrintString` (`KismetStringLibrary.Concat_StrStr` "Selected Output Device: " (`.DeviceName` (break `FoundMIDIDevice` (`|GetArrayItem` (`self.MidiDevices`) _selectedmidioutputdeviceid))) (`KismetStringLibrary.Conv_IntToString` _selectedmidioutputdeviceid)) true true (struct :`G` 0.66 :`B` 1.0 :`A` 1.0) 10.0)
        ;[1 1 1] create midi output controller from found device id
        (`MIDIDeviceManager.CreateMIDIDeviceOutputController` (`self.SelectedMidiOutputDeviceID`))
        (else
          ;[1 1 1] print could not find
          (`KismetSystemLibrary.PrintString` (`KismetStringLibrary.Concat_StrStr` "Could not find midi output device containing " "\"" (`self.MidiOutputDeviceNameContainsThis`) "\"") true true (struct :`G` 0.66 :`B` 1.0 :`A` 1.0) 10.0))))
    (:`then_7`
      ;[1 1 1] function output
      (return (`self.FoundMidiInputDevice`) (`self.MidiDeviceInputController`) (`self.FoundMidiOutputDevice`) (`self.MidiDeviceOutputController`)))))