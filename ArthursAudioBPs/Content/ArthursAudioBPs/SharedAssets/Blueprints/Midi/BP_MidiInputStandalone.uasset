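; Standalone MIDI input Blueprint that plays a modular synth component from the default MIDI input device.
; On BeginPlay it creates a controller for that device, binds its note on and note off events, and applies the synth preset.
; Note on prints note and velocity to screen and starts the synth note with no fixed duration, leaving note off to release it.
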(event `self.ReceiveBeginPlay`
  ;[1 1 1] set up default midi device
  (bind _deviceid (`MIDIDeviceManager.GetDefaultIMIDIInputDeviceID`))
  (bind _returnvalue (`MIDIDeviceManager.CreateMIDIDeviceInputController` _deviceid))
  (bind _output_get (set `self.MidiController` _returnvalue))
  ;[1 1 1] set up midi events
  (add `MIDIDeviceInputController.OnMIDINoteOn` _output_get (delegate `OnMIDINoteOn_Event_0`))
  (add `MIDIDeviceInputController.OnMIDINoteOff` _output_get (delegate `OnMIDINoteOff_Event_0`))
  ;[1 1 1] set up synth component
  (`ModularSynthComponent.SetSynthPreset` (`self.ModularSynth`) (`self.SynthPreset`)))

(event `OnMIDINoteOn_Event_0`
  (params (MIDIDeviceController :type "MIDIDeviceInputController Object Reference") (Timestamp :type Integer) (Channel :type Integer) (Note :type Integer) (Velocity :type Integer))
  ;[1 1 1] midi events
  (`KismetSystemLibrary.PrintString` (`KismetStringLibrary.Concat_StrStr` "Note: " (`KismetStringLibrary.Conv_IntToString` Note) " Velocity: " (`KismetStringLibrary.Conv_IntToString` Velocity)))
  (`ModularSynthComponent.NoteOn` (`self.ModularSynth`) (`KismetMathLibrary.Conv_IntToDouble` Note) Velocity -1.0))

(event `OnMIDINoteOff_Event_0`
  (params (MIDIDeviceController :type "MIDIDeviceInputController Object Reference") (Timestamp :type Integer) (Channel :type Integer) (Note :type Integer) (Velocity :type Integer))
  ;[1 1 1] midi events
  (`ModularSynthComponent.NoteOff` (`self.ModularSynth`) (`KismetMathLibrary.Conv_IntToDouble` Note) false false))

(fn `UserConstructionScript`)