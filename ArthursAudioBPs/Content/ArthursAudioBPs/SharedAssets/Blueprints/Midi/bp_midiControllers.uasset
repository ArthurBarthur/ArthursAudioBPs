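; Blueprint actor that demonstrates MIDI device input and output, playing a modular synth from an external MIDI controller.
; On BeginPlay it applies a synth preset and finds input and output devices by name through a MIDI component.
; Incoming note on/off events on all channels drive the synth.
; If an output device is found, a delay loop endlessly sends a repeating test note on channel 1.
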(event `OnMidiNoteON`
  (params (MIDIDeviceController :type "MIDIDeviceInputController Object Reference") (Timestamp :type Integer) (Channel :type Integer) (Note :type Integer) (Velocity :type Integer))
  ;[1 1 1] midi INPUT (currently receiving on all channels)
  ;;[1 1 1] synth note on
  (`ModularSynthComponent.NoteOn` (`self.ModularSynth`) (`KismetMathLibrary.Conv_IntToDouble` Note) Velocity -1.0))

(event `OnMIDINoteOff_Event_0`
  (params (MIDIDeviceController :type "MIDIDeviceInputController Object Reference") (Timestamp :type Integer) (Channel :type Integer) (Note :type Integer) (Velocity :type Integer))
  ;[1 1 1] midi INPUT (currently receiving on all channels)
  ;;[1 1 1] synth note off
  (`ModularSynthComponent.NoteOff` (`self.ModularSynth`) (`KismetMathLibrary.Conv_IntToDouble` Note) false false))

(event `self.ReceiveBeginPlay`
  (bind _midideviceoutputcontroller (`self.MidiDeviceOutputController`))
  (`KismetSystemLibrary.Delay` 0.2)
  ;[1 1 1] set synth preset
  (`ModularSynthComponent.SetSynthPreset` (`self.ModularSynth`) (`self.SynthPreset`))
  ;[1 1 1] get midi device controller
  (bind (_foundvalidmidiinputdevice _midideviceinputcontroller _foundmidioutputdevice _midideviceoutputcontroller_2) (`/Game/ArthursAudioBPs/SharedAssets/Components/BP_MidiComponent.FindMidiDevice` (`self.MidiComponent`) (`self.MidiDeviceInputNameContains:`) (`self.MidiDeviceOutputNameContains:`)))
  (`|ExecutionSequence`
    (:`then_0`
      (if _foundvalidmidiinputdevice
        (set `self.MidiDeviceInputController` _midideviceinputcontroller)
        ;[1 1 1] midi INPUT (currently receiving on all channels)
        ;;[1 1 1] bind event midi note on
        (add `MIDIDeviceInputController.OnMIDINoteOn` (`self.MidiDeviceInputController`) (`|CreateDelegate` :!event `OnMidiNoteON`))
        ;;[1 1 1] bind event midi note off
        (add `MIDIDeviceInputController.OnMIDINoteOff` (`self.MidiDeviceInputController`) (`|CreateDelegate` :!event `OnMIDINoteOff_Event_0`))))
    (:`then_1`
      (if _foundmidioutputdevice
        (set `self.MidiDeviceOutputController` _midideviceoutputcontroller_2)
        ;[1 1 1] midi OUTPUT (currently sending on channel 1)
        ;;[1 1 1] Send infinite stream of midi notes
        (`KismetSystemLibrary.Delay` 1.0 :!label _label)
        (`MIDIDeviceOutputController.SendMIDINoteOn` _midideviceoutputcontroller 1 62 100)
        (`KismetSystemLibrary.Delay` 0.2)
        (`MIDIDeviceOutputController.SendMIDIEvent` _midideviceoutputcontroller "NoteOff" 1 62 100)
        (goto _label)))))

(fn `UserConstructionScript`)