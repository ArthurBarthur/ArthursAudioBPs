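; BP_ModulationActor1 is an actor that applies modulation settings to the audio component of a linked actor at the start of play.
; After a short delay on BeginPlay it finds the AudioComponent on ActorWithAudioComp, stops it, assigns ModulationSettings and plays it again from the start.
; It prints a warning if no audio component is found.
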(event `self.ReceiveBeginPlay`
  (bind _returnvalue (`self.GetComponentByClass` (`self.ActorWithAudioComp`) "/Script/Engine.AudioComponent"))
  (`KismetSystemLibrary.Delay` 0.5)
  ;[1 1 1] find hooked-up audio comp
  (`/Engine/EditorBlueprintResources/StandardMacros.IsValid` _returnvalue
    (:`Is Valid`
      (set `self.FoundAudioComp` _returnvalue)
      ;[1 1 1] stop audio
      (`AudioComponent.Stop` (`self.FoundAudioComp`))
      ;[1 1 1] put modulation on audio comp
      (set `AudioComponent.Modulation` (`self.ModulationSettings`) (`self.FoundAudioComp`))
      ;[1 1 1] start audio
      (`AudioComponent.Play` (`self.FoundAudioComp`) 0.0))
    (:`Is Not Valid`
      (`KismetSystemLibrary.PrintString` "bp_ModulationActor not connected to an actor with audio comp"))))

(fn `UserConstructionScript`)