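; BP_NiagaraFun is an audio-reactive Blueprint that drives a referenced Niagara actor's particles from submix analysis.
; Each Tick it reads one frequency slot's smoothed, normalized envelope from AnalysisBeautifierRef.
; That value scales SpawnRate and blends ParticleColor between low and high colors.
; VelocityMin and VelocityMax are also set from it, but their identical output bounds keep velocity constant.
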(event `self.ReceiveBeginPlay`)

(event `self.ReceiveTick`
  (params (DeltaSeconds :type "Float (single-precision)"))
  (bind _returnvalue (`KismetMathLibrary.MapRangeClamped` (`self.Envelope0-1Live`) 0.0 1.0 400.0 400.0))
  ;[1 1 1] tick
  (set `self.TickDelta` DeltaSeconds)
  ;[1 1 1] store latest env
  (set `self.Envelope0-1Live` (`|GetArrayItem` (`/Game/ArthursAudioBPs/SharedAssets/Blueprints/AudioVisualisation/bp_AnalysisBeautifier.FinalEnvelopeSmoothedNormalizedOutputValuesFromAnalysis` (`self.AnalysisBeautifierRef`)) (`self.FreqSlot(from submix analyzers array of freqs)`)))
  ;[1 1 1] control niagara actor/system
  (`|ExecutionSequence`
    (:`then_1`
      (`FXSystemComponent.SetFloatParameter` (`NiagaraActor.NiagaraComponent` (`self.NiagaraActor`)) "VelocityMin" _returnvalue))
    (:`then_2`
      (`FXSystemComponent.SetFloatParameter` (`NiagaraActor.NiagaraComponent` (`self.NiagaraActor`)) "VelocityMax" _returnvalue))
    (:`then_3`
      (`FXSystemComponent.SetFloatParameter` (`NiagaraActor.NiagaraComponent` (`self.NiagaraActor`)) "SpawnRate" (`KismetMathLibrary.MapRangeClamped` (`self.Envelope0-1Live`) 0.0 1.0 0.0 400.0)))
    (:`then_4`
      (`FXSystemComponent.SetColorParameter` (`NiagaraActor.NiagaraComponent` (`self.NiagaraActor`)) "ParticleColor" (`KismetMathLibrary.LinearColorLerp` (`self.ColorLow`) (`self.ColorHigh`) (`self.Envelope0-1Live`))))))

(fn `UserConstructionScript`)