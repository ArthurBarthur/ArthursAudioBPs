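; Audio-reactive actor that builds a row of Niagara systems, one per analyzed frequency.
; Construction script lays out spaced arrow previews from the Analyzer's frequencies and picks two random HSV-range colors for each.
; BeginPlay spawns inactive systems at those locations, and the first Tick activates them.
; Each Tick feeds Beautifier's smoothed envelopes into color, mesh Z scale and glow; spawn rate, velocity and sprite size map to constants.
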(event `self.ReceiveBeginPlay`
  ;[1 1 1] add niagara systems at each arrow
  (for _array_element (`self.ArrowTransforms`)
    (bind _returnvalue (`NiagaraFunctionLibrary.SpawnSystemAtLocation` (`self.NiagaraSystem`) (`KismetMathLibrary.TransformLocation` (`SceneComponent.GetRelativeTransform` (`self.DefaultSceneRoot`)) (.location _array_element)) (struct) (1.0 1.0 1.0) true false))
    (`KismetArrayLibrary.Array_Add` (`self.NiagaraSystems`) _returnvalue)))

(event `self.ReceiveTick`
  (params (DeltaSeconds :type "Float (single-precision)"))
  ;[1 1 1] get latest freq envelopes
  (set `self.LatestFreqs` (`/Game/ArthursAudioBPs/SharedAssets/Blueprints/AudioVisualisation/bp_AnalysisBeautifier.FinalEnvelopeSmoothedNormalizedOutputValuesFromAnalysis` (`self.Beautifier`)))
  (for (_array_element _array_index) (`self.LatestFreqs`)
    (bind _output (`|GetArrayItem` (`self.NiagaraSystems`) _array_index))
    ;[1 1 1] rate
    (`NiagaraComponent.SetVariableFloat` _output "SpawnRate" (`KismetMathLibrary.MapRangeClamped` _array_element 0.0 1.0 30.0 30.0))
    (bind _returnvalue (`KismetMathLibrary.MapRangeClamped` _array_element 0.0 1.0 8000.0 8000.0))
    ;[1 1 1] velocity min max
    (`NiagaraComponent.SetVariableFloat` _output "VelocityMin" _returnvalue)
    (`NiagaraComponent.SetVariableFloat` _output "VelocityMax" _returnvalue)
    ;[1 1 1] color
    (`NiagaraComponent.SetVariableLinearColor` _output "ParticleColor" (`KismetMathLibrary.LinearColorLerp` (`|GetArrayItem` (`self.Colors1`) _array_index) (`|GetArrayItem` (`self.Colors2`) _array_index) _array_element))
    (bind (_returnvalue_x _returnvalue_y) (`KismetMathLibrary.BreakVector` (`KismetMathLibrary.VLerp` (10.0 10.0 0.0) (10.0 10.0 0.0) _array_element)))
    ;[1 1 1] sprite size
    (`NiagaraComponent.SetVariableVec2` _output "SpriteSize" (`KismetMathLibrary.MakeVector2D` _returnvalue_x _returnvalue_y))
    ;[1 1 1] mesh scale
    (`NiagaraComponent.SetVariableVec3` _output "MeshScale" (`KismetMathLibrary.VLerp` (1.0 1.0 1.0) (1.0 1.0 30.0) _array_element))
    ;[1 1 1] glow!
    (`NiagaraComponent.SetVariableFloat` _output "User.Glow" (`KismetMathLibrary.MapRangeClamped` _array_element 0.0 1.0 0.0 50.0)))
  ;[1 1 1] once: activate niagara systems when things are ready
  (`/Engine/EditorBlueprintResources/StandardMacros.DoOnce` false
    (:`Completed`
      (for _array_element_2 (`self.NiagaraSystems`)
        (`ActorComponent.Activate` _array_element_2 false)))))

(fn `UserConstructionScript`
  (bind _analyzer (`self.Analyzer`))
  (bind (_h _s _v) (`KismetMathLibrary.RGBToHSV` (`self.ColorMax2`)))
  (bind (_h_2 _s_2 _v_2) (`KismetMathLibrary.RGBToHSV` (`self.ColorMin2`)))
  (bind (_h_3 _s_3 _v_3) (`KismetMathLibrary.RGBToHSV` (`self.ColorMin1`)))
  (bind (_h_4 _s_4 _v_4) (`KismetMathLibrary.RGBToHSV` (`self.ColorMax1`)))
  ;[1 1 1] Create locations and arrow visualizers from Beautifier freqs
  (`KismetArrayLibrary.Array_Clear` (`self.ArrowTransforms`))
  (`/Engine/EditorBlueprintResources/StandardMacros.IsValid` _analyzer
    (:`Is Valid`
      (`KismetArrayLibrary.Array_Clear` (`self.Arrows`))
      (for (_ _array_index) (`/Game/ArthursAudioBPs/SharedAssets/Blueprints/AudioVisualisation/bp_SubmixAnalyzer.FrequenciesToAnalyze` _analyzer)
        (bind _returnvalue (`KismetArrayLibrary.Array_Add` (`self.ArrowTransforms`) (`KismetMathLibrary.MakeTransform` (`KismetMathLibrary.MakeVector` 0.0 (* _array_index (`self.Spacing`))))))
        (bind _returnvalue_2 (`AddComponent|NODE_AddArrowComponent-0` :`RelativeTransform` (`|GetArrayItem` (`self.ArrowTransforms`) _returnvalue)))
        (`KismetArrayLibrary.Array_Add` (`self.Arrows`) _returnvalue_2))
      ;[1 1 1] colors 1
      (`KismetArrayLibrary.Array_Clear` (`self.Colors1`))
      (for _ (`/Game/ArthursAudioBPs/SharedAssets/Blueprints/AudioVisualisation/bp_SubmixAnalyzer.FrequenciesToAnalyze` (`self.Analyzer`))
        (`KismetArrayLibrary.Array_Add` (`self.Colors1`) (`KismetMathLibrary.HSVToRGB` (`KismetMathLibrary.RandomFloatInRange` _h_3 _h_4) (`KismetMathLibrary.RandomFloatInRange` _s_3 _s_4) (`KismetMathLibrary.RandomFloatInRange` _v_3 _v_4))))
      ;[1 1 1] colors2
      (`KismetArrayLibrary.Array_Clear` (`self.Colors2`))
      (for _ (`/Game/ArthursAudioBPs/SharedAssets/Blueprints/AudioVisualisation/bp_SubmixAnalyzer.FrequenciesToAnalyze` (`self.Analyzer`))
        (`KismetArrayLibrary.Array_Add` (`self.Colors2`) (`KismetMathLibrary.HSVToRGB` (`KismetMathLibrary.RandomFloatInRange` _h_2 _h) (`KismetMathLibrary.RandomFloatInRange` _s_2 _s) (`KismetMathLibrary.RandomFloatInRange` _v_2 _v))))
      (for (_array_element _array_index_2) (`self.Arrows`)
        (`ArrowComponent.SetArrowColor` _array_element (`|GetArrayItem` (`self.Colors2`) _array_index_2))))))