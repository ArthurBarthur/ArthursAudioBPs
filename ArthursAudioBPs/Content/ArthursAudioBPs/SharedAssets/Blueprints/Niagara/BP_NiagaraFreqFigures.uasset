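; Audio-reactive Blueprint that drives the noise strength of a referenced Niagara actor from analyzed frequency volumes.
; Each Tick it reads the smoothed, normalized analysis output from a beautifier reference and averages the frequency slots it is set to listen to.
; That average is range-mapped with clamping and written to the Niagara User.NoiseStrength parameter, so louder selected frequencies produce stronger noise.
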(event `self.ReceiveBeginPlay`)

(event `self.ReceiveTick`
  (params (DeltaSeconds :type "Float (single-precision)"))
  ;[1 1 1] get latest freq volumes from beautifier
  (set `self.latestFreqVolumesFromBeautifier` (`/Game/ArthursAudioBPs/SharedAssets/Blueprints/AudioVisualisation/bp_AnalysisBeautifier.FinalEnvelopeSmoothedNormalizedOutputValuesFromAnalysis` (`self.BeautifierRef`)))
  (`|ExecutionSequence`
    (:`then_0`
      ;[1 1 1] AverageTheFreqsWeAreListeningTo
      (set `self.AverageVolumeOverFreqs` 0.0)
      (for _array_element (`self.FreqSlotsToListenTo`)
        (bind _output_get (set `self.AverageVolumeOverFreqs` (+ (stale _output_get) (`|GetArrayItem` (`self.latestFreqVolumesFromBeautifier`) _array_element)))))
      (bind _output_get_2 (set `self.AverageVolumeOverFreqs` (/ (stale _output_get_2) (`KismetMathLibrary.Conv_IntToDouble` (`KismetArrayLibrary.Array_Length` (`self.FreqSlotsToListenTo`)))))))
    (:`then_1`
      ;[1 1 1] UpdateNoiseStrength
      (`FXSystemComponent.SetFloatParameter` (`NiagaraActor.NiagaraComponent` (`self.NiagaraActor`)) "User.NoiseStrength" (`KismetMathLibrary.MapRangeClamped` (`self.AverageVolumeOverFreqs`) 0.0 1.0 0.0 200.0)))))

(fn `UserConstructionScript`)