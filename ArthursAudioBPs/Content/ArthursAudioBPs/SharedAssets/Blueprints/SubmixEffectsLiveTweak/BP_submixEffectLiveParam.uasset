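; Demo actor for live-tweaking a submix filter effect while a sound plays.
; On BeginPlay it routes the example sound to a submix, a change that persists on the asset after PIE, and plays it.
; It then spawns a BP_SubmixEffectsLiveTweaker just above itself, passing itself as reference.
; Every tick it copies the tweaker's filter frequency onto the submix filter effect's cutoff.
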(event `self.ReceiveBeginPlay`
  (bind (_returnvalue_x _returnvalue_y _returnvalue_z) (`KismetMathLibrary.BreakVector` (`SceneComponent.K2_GetComponentLocation` (`self.DefaultSceneRoot`))))
  ;[1 0.9607 0.4655] this change to the sound asset STAYS after simulating in editor(PIE).
  ; Can be removed again if you want.
  (set `SoundBase.SoundSubmixObject` (`self.SubmixRef`) (`self.SoundToPlay`))
  ;[1 1 1] making the example sound play
  (`AudioComponent.SetSound` (`self.Audio`) (`self.SoundToPlay`))
  (`AudioComponent.Play` (`self.Audio`) 0.0)
  ;[1 1 1] spawn submix tweaker
  (bind _returnvalue (`|SpawnActorFromClass` "/Game/ArthursAudioBPs/SharedAssets/Blueprints/SubmixEffectsLiveTweak/BP_SubmixEffectsLiveTweaker.BP_SubmixEffectsLiveTweaker_C" (`KismetMathLibrary.MakeTransform` (`KismetMathLibrary.MakeVector` _returnvalue_x _returnvalue_y (+ _returnvalue_z 50.0)) (struct) (0.4 0.4 0.4)) "Undefined" "OverrideRootScale" null self null))
  (set `self.SubmixTweakerBp` _returnvalue))

(event `self.ReceiveTick`
  (params (DeltaSeconds :type "Float (single-precision)"))
  ;[1 1 1] change filter effect frequency
  (`SubmixEffectFilterPreset.SetFilterCutoffFrequency` (`self.SubmixFilterEffectRef`) (`/Game/ArthursAudioBPs/SharedAssets/Blueprints/SubmixEffectsLiveTweak/BP_SubmixEffectsLiveTweaker.SubmixFilterFreq` (`self.SubmixTweakerBp`))))

(fn `UserConstructionScript`)