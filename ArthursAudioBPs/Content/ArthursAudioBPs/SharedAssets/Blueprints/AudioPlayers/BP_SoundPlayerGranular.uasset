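; Sound player Blueprint that plays a sound wave through a granular synth component.
; The construction script applies attenuation, volume and bus routing to the synth.
; On BeginPlay it applies a granular preset, assigns the sound, then starts the synth after a short delay.
; The synth's envelope callback caches the latest amplitude value in LatestEnvelope.
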(event `self.ReceiveBeginPlay`
  (`|ExecutionSequence`
    (:`then_0`
      (`/Game/ArthursAudioBPs/SharedAssets/FunctionLibraries/GranularSynthFunctionLibrary.UpdateGranular` (`self.GranularSynth`) (`self.GranularPreset`)))
    (:`then_1`
      (`GranularSynth.SetSoundWave` (`self.GranularSynth`) (`self.Sound`)))
    (:`then_2`
      (`KismetSystemLibrary.Delay` 0.2)
      (`/Game/ArthursAudioBPs/SharedAssets/FunctionLibraries/GranularSynthFunctionLibrary.StartGranular` (`self.GranularSynth`)))))

(event `self.GranularSynth.OnAudioEnvelopeValue`
  (params (EnvelopeValue :type "Float (single-precision)"))
  (set `self.LatestEnvelope` EnvelopeValue))

(fn `UserConstructionScript`
  (set `SynthComponent.AttenuationSettings` (`self.Attenuation`) (`self.GranularSynth`))
  (`SynthComponent.SetVolumeMultiplier` (`self.GranularSynth`) (`self.VolumeMP`))
  (set `SynthComponent.bOutputToBusOnly` (`self.OutputToBusOnly`) (`self.GranularSynth`))
  (set `SynthComponent.BusSends` (`self.SourceBusSends`) (`self.GranularSynth`)))