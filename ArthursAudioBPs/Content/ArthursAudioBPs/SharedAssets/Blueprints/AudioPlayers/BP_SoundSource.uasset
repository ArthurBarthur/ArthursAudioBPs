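; BP_SoundSource is a placeable audio player that plays a configurable sound after an optional start delay.
; The construction script applies attenuation and spatialization to its AudioComponent, and BeginPlay sets sound, volume and pitch.
; Looping replays from StartTime using a Delay of the sound's remaining duration.
; Audio component events cache the latest envelope value and playback percent in variables.
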(event `self.ReceiveBeginPlay`
  (`KismetSystemLibrary.Delay` (`self.DelayedStartInSeconds`))
  ;[1 1 1] init sound
  (`AudioComponent.SetSound` (`self.AudioComponent`) (`self.SoundToPlay`))
  (set `AudioComponent.VolumeMultiplier` (`self.VolumeMP`) (`self.AudioComponent`))
  (`AudioComponent.SetPitchMultiplier` (`self.AudioComponent`) (`self.PitchMultiplier`))
  (`AudioComponent.Play` (`self.AudioComponent`) (`self.StartTime`) :!label _label)
  ;[1 1 1] loop?
  (if (`self.Loop`)
    (`KismetSystemLibrary.Delay` (- (`SoundBase.Duration` (`self.SoundToPlay`)) (`self.StartTime`)))
    (goto _label)))

(event `self.AudioComponent.OnAudioSingleEnvelopeValue`
  (params (PlayingSoundWave :type "SoundWave Object Reference") (EnvelopeValue :type "Float (single-precision)"))
  ;[1 1 1] Store latest envelope value
  (set `self.LatestEnvelopeValue` EnvelopeValue))

(event `self.AudioComponent.OnAudioPlaybackPercent`
  (params (PlayingSoundWave :type "SoundWave Object Reference") (PlaybackPercent :type "Float (single-precision)"))
  ;[1 1 1] Store latest playback percent value
  (set `self.AudioPlaybackPercent` PlaybackPercent))

(fn `UserConstructionScript`
  (set `AudioComponent.AttenuationSettings` (`self.AttenuationSettings`) (`self.AudioComponent`))
  (set `AudioComponent.bAllowSpatialization` (`self.AllowSpatialization`) (`self.AudioComponent`)))