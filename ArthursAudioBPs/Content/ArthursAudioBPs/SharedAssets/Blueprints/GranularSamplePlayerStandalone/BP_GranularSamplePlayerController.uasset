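; Controller actor that spawns a separate granular sample player and plays a sound wave through its granular synth, with adjustable speed and pitch.
; BeginPlay replaces any existing player, loads the sound and preset, then starts playback.
; Each Tick derives grains per second from a curve, using whichever of speed or pitch deviates most from 1.
; Grain duration follows at just under twice the grain interval, then the updated preset is applied and debug-printed.
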(event `self.ReceiveBeginPlay`
  ;[1 1 1] spawn separate actor containing just a granular synth
  (`/Engine/EditorBlueprintResources/StandardMacros.IsValid` (`self.GranularSamplePlayerRef`)
    (:`Is Valid`
      ;[1 1 1] delete old if respawning
      (`self.K2_DestroyActor` (`self.GranularSamplePlayerRef`))
      (set `self.GranularSamplePlayerRef` null))
    (:`Is Not Valid`
      _))
  (bind _returnvalue (`|SpawnActorFromClass` "/Game/ArthursAudioBPs/SharedAssets/Blueprints/GranularSamplePlayerStandalone/BP_GranularSamplePlayer.BP_GranularSamplePlayer_C" (`SceneComponent.K2_GetComponentToWorld` (`self.DefaultSceneRoot`)) "Undefined" "OverrideRootScale" null null))
  (bind _output_get (set `self.GranularSamplePlayerRef` _returnvalue))
  (set `self.GranularSynthRef` (`/Game/ArthursAudioBPs/SharedAssets/Blueprints/GranularSamplePlayerStandalone/BP_GranularSamplePlayer.GranularSynth` _output_get))
  ;[1 1 1] init preset
  (`GranularSynth.SetSoundWave` (`self.GranularSynthRef`) (`self.SoundToPlay`))
  (`/Game/ArthursAudioBPs/SharedAssets/FunctionLibraries/GranularSynthFunctionLibrary.UpdateGranular` (`self.GranularSynthRef`) (`self.GranularPreset`))
  ;[1 1 1] start it
  (`/Game/ArthursAudioBPs/SharedAssets/FunctionLibraries/GranularSynthFunctionLibrary.StartGranular` (`self.GranularSynthRef`) 69.0))

(event `self.ReceiveTick`
  (params (DeltaSeconds :type "Float (single-precision)"))
  (bind _pitch (`self.Pitch`))
  (bind ((`GrainsPerSecond_28_FB913A6443DB4978747958AE9B07E7B1` _grainspersecond) (`DurationBaseMsec_55_629930E44F1507F01122F697D24D492F` _durationbasemsec)) (break `/Game/ArthursAudioBPs/SharedAssets/Blueprints/GranularSynth/FGranularPreset` (`self.GranularPreset`)))
  (bind _returnvalue (`KismetMathLibrary.Abs` (`self.PlaySpeed`)))
  (bind _returnvalue_2 (`KismetMathLibrary.SelectFloat` (/ 1.0 _pitch) _pitch (> _pitch 1.0)))
  (bind _returnvalue_3 (`KismetMathLibrary.SelectFloat` (/ 1.0 _returnvalue) _returnvalue (> _returnvalue 1.0)))
  (set `self.LatestDelta` DeltaSeconds)
  ;[1 1 1] update playspeed and pitch
  (setmembers `/Game/ArthursAudioBPs/SharedAssets/Blueprints/GranularSynth/FGranularPreset` :`StructRef` (`self.GranularPreset`) :`PlayheadSpeed/Rate` (`self.PlaySpeed`) :`PitchBase` (`self.Pitch`))
  ;[1 1 1] auto GPS from playspeed+pitch against curve
  (setmembers `/Game/ArthursAudioBPs/SharedAssets/Blueprints/GranularSynth/FGranularPreset` :`StructRef` (`self.GranularPreset`) :`GrainsPerSecond` (`CurveFloat.GetFloatValue` (`self.Curve`) (`KismetMathLibrary.SelectFloat` _returnvalue_3 _returnvalue_2 (< _returnvalue_3 _returnvalue_2))))
  ;[1 1 1] auto GPS to duration
  (setmembers `/Game/ArthursAudioBPs/SharedAssets/Blueprints/GranularSynth/FGranularPreset` :`StructRef` (`self.GranularPreset`) :`DurationBaseMsec` (- (* (/ 1.0 (/ (`.GrainsPerSecond_28_FB913A6443DB4978747958AE9B07E7B1` (break `/Game/ArthursAudioBPs/SharedAssets/Blueprints/GranularSynth/FGranularPreset` (`self.GranularPreset`))) 1000.0)) 2.0) 1.0))
  ;[1 1 1] update granular
  (`/Game/ArthursAudioBPs/SharedAssets/FunctionLibraries/GranularSynthFunctionLibrary.UpdateGranular` (`self.GranularSynthRef`) (`self.GranularPreset`))
  ;[0.9978 1 0.1834] debug current preset
  (`KismetSystemLibrary.PrintString` (`KismetStringLibrary.Concat_StrStr` "GPS: " (`KismetStringLibrary.Conv_DoubleToString` _grainspersecond) " Duration: " (`KismetStringLibrary.Conv_DoubleToString` _durationbasemsec)) true true (struct :`G` 0.66 :`B` 1.0 :`A` 1.0) (`self.LatestDelta`)))

(fn `UserConstructionScript`)