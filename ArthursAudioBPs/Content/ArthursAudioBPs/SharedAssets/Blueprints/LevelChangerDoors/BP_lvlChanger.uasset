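; BP_lvlChanger is a level-changer trigger that opens the level named in LevelToLoad.
; Its box overlap requires the other actor's LevelChanger tag and one of two sphere component names, matched by string, for first-person and sedan characters.
; An OpenLevel event triggers the same load directly, bypassing those checks.
; The construction script writes LevelToLoad onto a TextRender, labelling the destination.
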(event `self.ReceiveBeginPlay`)

(event `self.Box.OnComponentBeginOverlap`
  (params (OverlappedComponent :type "PrimitiveComponent Object Reference") (OtherActor :type "Actor Object Reference") (OtherComp :type "PrimitiveComponent Object Reference") (OtherBodyIndex :type Integer) (bFromSweep :type Boolean) (SweepResult :type "HitResult Structure (by ref)"))
  (bind _returnvalue (`KismetSystemLibrary.GetObjectName` OtherComp))
  (if (and (`self.ActorHasTag` OtherActor "LevelChanger") (or (`KismetStringLibrary.EqualEqual_StrStr` _returnvalue "FPSphereCollision1ForSedanChar") (`KismetStringLibrary.EqualEqual_StrStr` _returnvalue "SedanSphereCollision1ForFirstPersonChar")))
    (`GameplayStatics.OpenLevel` (`self.LevelToLoad`) :!label _label)))

(event `OpenLevel`
  (goto _label))

(fn `UpdateText`
  (`TextRenderComponent.K2_SetText` (`self.TextRender`) (`KismetTextLibrary.Conv_NameToText` (`self.LevelToLoad`))))

(fn `UserConstructionScript`
  (`self.UpdateText`))