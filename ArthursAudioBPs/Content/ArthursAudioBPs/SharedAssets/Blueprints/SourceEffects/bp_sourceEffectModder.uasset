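; Blueprint that live-controls a source effect preset chain, exposing bypass flags and settings for its audio effects.
; Every Tick, a Sequence sets each entry's bypass state and pushes settings into the matching preset, covering delays, modulation, distortion, filtering, EQ, dynamics and spatial effects.
; Chain entries are addressed by hard-coded index, which differs from the Sequence order for the wave shaper and dynamics processor.
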(event `self.ReceiveTick`
  (params (DeltaSeconds :type "Float (single-precision)"))
  (`|ExecutionSequence`
    (:`then_0`
      ;[1 1 1] bypass?
      (`AudioMixerBlueprintLibrary.SetBypassSourceEffectChainEntry` (`self.SourceEffectChain`) 0 (`self.BypassSimpleDelay`))
      ;[1 1 1] Simple Delay
      (`SourceEffectSimpleDelayPreset.SetSettings` (`self.SourceEffectSimpleDelay`) (`self.SimpleDelaySettings`)))
    (:`then_1`
      (`AudioMixerBlueprintLibrary.SetBypassSourceEffectChainEntry` (`self.SourceEffectChain`) 12 (`self.BypassWaveShaper`))
      ;[1 1 1] waveshaper(volume)
      (`SourceEffectWaveShaperPreset.SetSettings` (`self.SourceEffectWaveShaper`) (`self.WaveShaperSettings`)))
    (:`then_2`
      (`AudioMixerBlueprintLibrary.SetBypassSourceEffectChainEntry` (`self.SourceEffectChain`) 1 (`self.BypassBitCrusher`))
      ;[1 1 1] Bitcrusher
      (`SourceEffectBitCrusherPreset.SetSettings` (`self.SourceEffectBitCrusher`) (`self.BitCrusherSettings`)))
    (:`then_3`
      (`AudioMixerBlueprintLibrary.SetBypassSourceEffectChainEntry` (`self.SourceEffectChain`) 2 (`self.BypassFilter`))
      ;[1 1 1] Filter
      (`SourceEffectFilterPreset.SetSettings` (`self.SourceEffectFilter`) (`self.FilterSettings`)))
    (:`then_4`
      (`AudioMixerBlueprintLibrary.SetBypassSourceEffectChainEntry` (`self.SourceEffectChain`) 3 (`self.BypassPhaser`))
      ;[1 1 1] Phaser
      (`SourceEffectPhaserPreset.SetSettings` (`self.SourceEffectPhaser`) (`self.PhaserSettings`)))
    (:`then_5`
      (`AudioMixerBlueprintLibrary.SetBypassSourceEffectChainEntry` (`self.SourceEffectChain`) 4 (`self.BypassStereoDelay`))
      ;[1 1 1] Stereo Delay
      (`SourceEffectStereoDelayPreset.SetSettings` (`self.SourceEffectStereoDelay`) (`self.StereoDelaySettings`)))
    (:`then_6`
      (`AudioMixerBlueprintLibrary.SetBypassSourceEffectChainEntry` (`self.SourceEffectChain`) 5 (`self.BypassChorus`))
      ;[1 1 1] chorus
      (`SourceEffectChorusPreset.SetSettings` (`self.SourceEffectChorus`) (`self.ChorusSettings`)))
    (:`then_7`
      (`AudioMixerBlueprintLibrary.SetBypassSourceEffectChainEntry` (`self.SourceEffectChain`) 11 (`self.BypassDynamicsProcessor`))
      ;[1 1 1] dynamicsProcessor
      (`SourceEffectDynamicsProcessorPreset.SetSettings` (`self.SourceEffectDynamicsProcessor`) (`self.DynamicsProcessorSettings`)))
    (:`then_8`
      (`AudioMixerBlueprintLibrary.SetBypassSourceEffectChainEntry` (`self.SourceEffectChain`) 6 (`self.BypassEQ`))
      ;[1 1 1] EQ
      (`SourceEffectEQPreset.SetSettings` (`self.SourceEffectEQ`) (`self.EQSettings`)))
    (:`then_9`
      (`AudioMixerBlueprintLibrary.SetBypassSourceEffectChainEntry` (`self.SourceEffectChain`) 7 (`self.BypassFoldbackDistortion`))
      ;[1 1 1] FoldbackDistortion
      (`SourceEffectFoldbackDistortionPreset.SetSettings` (`self.SourceEffectFoldbackDistortion`) (`self.FoldbackDistortionSettings`)))
    (:`then_10`
      (`AudioMixerBlueprintLibrary.SetBypassSourceEffectChainEntry` (`self.SourceEffectChain`) 8 (`self.BypassMidSideSpreader`))
      ;[1 1 1] MidSideSpreader
      (`SourceEffectMidSideSpreaderPreset.SetSettings` (`self.SourceEffectMidSideSpreader`) (`self.MidSideSpreaderSettings`)))
    (:`then_11`
      (`AudioMixerBlueprintLibrary.SetBypassSourceEffectChainEntry` (`self.SourceEffectChain`) 9 (`self.BypassPanner`))
      ;[1 1 1] Panner
      (`SourceEffectPannerPreset.SetSettings` (`self.SourceEffectPanner`) (`self.PannerSettings`)))
    (:`then_12`
      (`AudioMixerBlueprintLibrary.SetBypassSourceEffectChainEntry` (`self.SourceEffectChain`) 10 (`self.BypassRingModulation`))
      ;[1 1 1] RingModulation
      (`SourceEffectRingModulationPreset.SetSettings` (`self.SourceEffectRingModulation`) (`self.RingModulationSettings`)))))

(fn `UserConstructionScript`)