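; Note plate actor for the bounce music setup that plays a synth note and flashes when something hits it.
; On BeginPlay it creates a dynamic material, loads an override or bank preset into its modular synth and computes the MIDI note from Note and Octave.
; Hit impulse strength maps to note velocity.
; A timeline, rate-scaled by note length, drives the emissive fade so the glow matches the note's duration.
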(event `self.ReceiveBeginPlay`
  ;[1 1 1] create dynamic material(MID)
  (bind _returnvalue (`PrimitiveComponent.CreateDynamicMaterialInstance` (`self.StaticMesh`) 0 "/Game/ArthursAudioBPs/SharedAssets/Visuals/Materials/MI_SimpleMat_Inst7.MI_SimpleMat_Inst7" "None"))
  (set `self.MID` _returnvalue)
  ;[1 1 1] Init synth settings
  (`ModularSynthComponent.SetSynthPreset` (`self.ModularSynth`) (select `bool` (`self.OverridePreset`) :`false` (`.Preset` (break `ModularSynthPresetBankEntry` (`|GetArrayItem` (`ModularSynthPresetBank.Presets` (`self.PresetBank`)) (`self.CurrentBankPreset`)))) :`true` (`self.SynthPresetOverride`)))
  (`self.SetMidiNote`))

(event `self.StaticMesh.OnComponentHit`
  (params (HitComponent :type "PrimitiveComponent Object Reference") (OtherActor :type "Actor Object Reference") (OtherComp :type "PrimitiveComponent Object Reference") (NormalImpulse :type "Vector Structure") (Hit :type "HitResult Structure (by ref)"))
  (`self.MidOnAndFadeOut`)
  ;[1 1 1] Note on
  (`ModularSynthComponent.NoteOn` (`self.ModularSynth`) (`self.MidiNote`) (`KismetMathLibrary.FTrunc` (`KismetMathLibrary.MapRangeClamped` (`KismetMathLibrary.FClamp` (`KismetMathLibrary.VSize` NormalImpulse) 1000.0 15000.0) 1000.0 15000.0 30.0 127.0)) (`self.NoteLength`)))

(event `MidOnAndFadeOut`
  ;[1 1 1] fadeOut emissive
  (`TimelineComponent.SetPlayRate` (`self.Timeline_0`) (/ 1.0 (`self.NoteLength`)))
  (bind (_direction _1_0smoothly1sec) (`Timeline|Timeline_0` :!via `PlayFromStart`)
    (:`Update`
      (`MaterialInstanceDynamic.SetScalarParameterValue` (`self.MID`) "Emissive Multiplier" (* _1_0smoothly1sec 30.0)))))

(fn `SetMidiNote`
  (set `self.MidiNote` (`KismetMathLibrary.FClamp` (`KismetMathLibrary.Conv_IntToDouble` (+ (* 12 (`self.Octave`)) (select `/Game/ArthursAudioBPs/SharedAssets/Components/ChordComponent/ERootNotes` (`self.Note`) :`NewEnumerator1` 1 :`NewEnumerator2` 2 :`NewEnumerator3` 3 :`NewEnumerator4` 4 :`NewEnumerator5` 5 :`NewEnumerator6` 6 :`NewEnumerator7` 7 :`NewEnumerator8` 8 :`NewEnumerator9` 9 :`NewEnumerator10` 10 :`NewEnumerator11` 11))) 0.0 127.0)))

(fn `UserConstructionScript`)