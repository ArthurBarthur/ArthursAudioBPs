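; BP_Launcher is a physics launcher actor that periodically spawns a configurable class at its own transform, scaled down, and fires it along its up vector.
; After an initial delay, a looping timer drives launches; a gate shuts them off once a spawn is invalid, such as when blocked by collision.
; Each spawn's static mesh gets CCD, physics and a randomized velocity-change impulse, then a self-destruct component limits its lifetime.
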(event `self.ReceiveBeginPlay`
  (`KismetSystemLibrary.Delay` (`self.InitialDelay`))
  ;[1 1 1] LaunchTimer
  (`KismetSystemLibrary.K2_SetTimerDelegate` (`|CreateDelegate` :!event `Launch`) (`self.LaunchInterval`) true)
  (`self.Launch`))

(event `Launch`
  (`/Engine/EditorBlueprintResources/StandardMacros.Gate` false :!label _label
    (:`Exit`
      ;[1 1 1] Spawn thing to be launched
      (bind _returnvalue (`|SpawnActorFromClass` (`self.ClassToSpawn`) (`KismetMathLibrary.MakeTransform` (.location (`self.GetTransform`)) (.rotation (`self.GetTransform`)) (/ (.scale (`self.GetTransform`)) 5.0)) "DontSpawnIfColliding" "OverrideRootScale" null null))
      (bind _output_get (set `self.LatestSpawnedActor` _returnvalue))
      ;[1 1 1] stop if invalid
      (`/Engine/EditorBlueprintResources/StandardMacros.IsValid` _output_get
        (:`Is Valid`
          (`KismetSystemLibrary.Delay` 0.2)
          ;[1 1 1] add impulse to launched obj
          (`self.AddImpulse`)
          ;[1 1 1] add time to live selfdestruct component to actor
          (`AddComponent|NODE_Addbpc_timeToLive-2` :`self` (`self.LatestSpawnedActor`) :`TimeToLive` (select `bool` (`self.OverrideBallTTL`) :`false` (`self.LaunchInterval`) :`true` (`self.TTL`)))
          (goto _label :!via `Open`))
        (:`Is Not Valid`
          (goto _label :!via `Close`))))))

(fn `AddImpulse`
  (locals (_MeshComponent :type "StaticMeshComponent Object Reference"))
  ;[1 1 1] Add impulse to first mesh in launchd obj
  (set `local._MeshComponent` (`self.GetComponentByClass` (`self.LatestSpawnedActor`) "/Script/Engine.StaticMeshComponent"))
  (`PrimitiveComponent.SetUseCCD` (`local._MeshComponent`) true "None")
  (`PrimitiveComponent.SetEnableGravity` (`local._MeshComponent`) true)
  (`PrimitiveComponent.SetSimulatePhysics` (`local._MeshComponent`) true)
  (`PrimitiveComponent.AddImpulse` (`local._MeshComponent`) (* (+ (`self.GetActorUpVector`) (* (`KismetMathLibrary.RandomUnitVector`) (/ (`self.ImpulseRandomnessPercent`) 100.0))) (`self.LaunchImpulseMP`)) "None" true))

(fn `UserConstructionScript`)