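; BP_BoxDeliverer is a spawner actor that keeps delivering BP_box actors with a set mass and scale.
; On BeginPlay it removes its preview cube, spawns a box immediately, then repeats on a looping one-second timer, with actor tick disabled in construction.
; Each box spawns at the Cube component's location minus a SpawnLocation offset, and is skipped if that spot would collide.
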(event `self.ReceiveBeginPlay`
  ;[1 1 1] destroy pre-viz cube
  (`ActorComponent.K2_DestroyComponent` (`self.Cube1`))
  ;[1 1 1] add cubes on timer
  (`KismetSystemLibrary.K2_SetTimerDelegate` (delegate `TryToAddCube`) 1.0 true)
  (`self.AddCube` :!label _label))

(event `TryToAddCube`
  ;[1 1 1] add cubes on timer
  (goto _label))

(fn `AddCube`
  (bind _returnvalue_location (`KismetMathLibrary.BreakTransform` (`SceneComponent.K2_GetComponentToWorld` (`self.Cube`))))
  (`|SpawnActorFromClass` "/Game/ArthursAudioBPs/SharedAssets/Blueprints/SpringKeys/BP_box.BP_box_C" (`KismetMathLibrary.MakeTransform` (- _returnvalue_location (`self.SpawnLocation`)) (struct) (`self.BoxScaleMultiplier`)) "DontSpawnIfColliding" "OverrideRootScale" null (`self.BoxWeightInKg`) null))

(fn `UserConstructionScript`
  (`self.SetActorTickEnabled` false))