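; Physics spring pad that measures its own motion as normalized travel, velocity and acceleration values, with an optional debug text readout.
; The construction script configures the constraint's linear drive and Z limit from the spring settings, then positions and scales the pad.
; Each tick derives push direction and motion from the pad's Z offset, with acceleration computed simply as velocity over delta time.
; Velocity and acceleration normalize against running maxima, which a timer decays every second to recover from spikes.
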(event `self.ReceiveBeginPlay`
  (bind (_relativelocation_x _relativelocation_y _relativelocation_z) (`KismetMathLibrary.BreakVector` (`SceneComponent.RelativeLocation` (`self.Pad`))))
  ;[1 1 1] beginPlay
  (`|ExecutionSequence`
    (:`then_0`
      ;[1 1 1] store starting location('zero')
      (set `self.LocationStart` _relativelocation_z))
    (:`then_1`
      ;[1 1 1] destroy debugtext
      (if (not (`self.ShowDebug`))
        (`ActorComponent.K2_DestroyComponent` (`self.TextRender`))))
    (:`then_2`
      (`KismetSystemLibrary.K2_SetTimerDelegate` (delegate `DecreaseHistoricMaxValuesForNormalizing`) 1.0 true 1.0))))

(event `DecreaseHistoricMaxValuesForNormalizing`
  ;[1 1 1] decrease historic max values(for calming down normalizing if it ever goes crazy)
  (bind _output_get (set `self.VelocityMax` (* (stale _output_get) 0.9)))
  (bind _output_get_2 (set `self.AccelerationMax` (* (stale _output_get_2) 0.9))))

(event `self.ReceiveTick`
  (params (DeltaSeconds :type "Float (single-precision)"))
  (bind (_relativelocation_x _relativelocation_y _relativelocation_z) (`KismetMathLibrary.BreakVector` (`SceneComponent.RelativeLocation` (`self.Pad`))))
  (bind _returnvalue (- _relativelocation_z (`self.LocationStart`)))
  ;[1 1 1] tick
  (set `self.deltaTick` DeltaSeconds)
  (`|ExecutionSequence`
    (:`then_0`
      ;[1 1 1] pushed up or down?
      (`/Engine/EditorBlueprintResources/StandardMacros.CompareFloat` _returnvalue
        (:`>`
          (set `self.PushedUp` true))
        (:`<`
          (set `self.PushedUp` false))))
    (:`then_1`
      ;[1 1 1] store current loc
      (set `self.CurrentLoc` (`KismetMathLibrary.Abs` _returnvalue))
      ;[1 1 1] normalize loc
      (set `self.TravelNormalized` (`KismetMathLibrary.MapRangeClamped` (`self.CurrentLoc`) 0.0 (`self.SpringLimit`) 0.0 1.0))
      ;[1 1 1] calc velocity
      (set `self.Velocity` (/ (`KismetMathLibrary.Abs` (- (`self.PreviousLoc`) (`self.CurrentLoc`))) (`self.deltaTick`)))
      ;;[1 1 1] Store Max
      (set `self.VelocityMax` (`KismetMathLibrary.SelectFloat` (`self.Velocity`) (`self.VelocityMax`) (> (`self.Velocity`) (`self.VelocityMax`))))
      ;;[1 1 1] normalize velocity
      (set `self.VelocityNormalized` (`KismetMathLibrary.MapRangeClamped` (`self.Velocity`) 0.0 (`self.VelocityMax`) 0.0 1.0))
      ;[1 1 1] calc acceleration
      (set `self.Acceleration` (/ (`self.Velocity`) (`self.deltaTick`)))
      ;;[1 1 1] Store Max
      (set `self.AccelerationMax` (`KismetMathLibrary.SelectFloat` (`self.Acceleration`) (`self.AccelerationMax`) (> (`self.Acceleration`) (`self.AccelerationMax`))))
      ;;[1 1 1] normalize acceleration
      (set `self.AccelerationNormalized` (`KismetMathLibrary.MapRangeClamped` (`self.Acceleration`) 0.0 (`self.AccelerationMax`) 0.0 1.0))
      ;[1 1 1] store current location as 'previous' location for next time
      (set `self.PreviousLoc` (`self.CurrentLoc`)))
    (:`then_2`
      ;[1 1 1] update text info
      (`self.UpdateText`))))

(fn `UpdateText`
  ;[1 1 1] update text contents
  (if (`self.ShowDebug`)
    (`TextRenderComponent.K2_SetText` (`self.TextRender`) (`KismetTextLibrary.Conv_StringToText` (`KismetStringLibrary.Concat_StrStr` "Velocity: " (`KismetStringLibrary.Conv_DoubleToString` (`KismetMathLibrary.GridSnap_Float` (`self.VelocityNormalized`) 0.1)) " \n" "Acceleration: " (`KismetStringLibrary.Conv_DoubleToString` (`KismetMathLibrary.GridSnap_Float` (`self.AccelerationNormalized`) 0.1)) " \n" "Spring Travel: " (`KismetStringLibrary.Conv_DoubleToString` (`KismetMathLibrary.GridSnap_Float` (`self.TravelNormalized`) 0.1)))))))

(fn `UserConstructionScript`
  (`|ExecutionSequence`
    (:`then_0`
      ;[1 1 1] set pad location according to spring limit
      (`SceneComponent.K2_SetRelativeLocation` (`self.Pad`) (`KismetMathLibrary.MakeVector` 0.0 0.0 (+ (`self.SpringLimit`) 10.0)) false true))
    (:`then_1`
      ;[1 1 1] set up spring physics
      (`PhysicsConstraintComponent.SetLinearDriveParams` (`self.Spring`) (`self.SpringStrength`) (`self.SpringDampening`) 0.0))
    (:`then_2`
      (`PhysicsConstraintComponent.SetLinearZLimit` (`self.Spring`) "LCM_Limited" (`self.SpringLimit`)))
    (:`then_3`
      ;[1 1 1] update text
      (`self.UpdateText`))
    (:`then_4`
      ;[1 1 1] update scale
      (`SceneComponent.SetRelativeScale3D` (`self.Pad`) (`self.PadScale`)))))