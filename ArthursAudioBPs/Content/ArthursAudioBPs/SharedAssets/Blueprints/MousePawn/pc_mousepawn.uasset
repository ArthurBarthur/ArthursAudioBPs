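; pc_mousepawn lets the player drag Movable scene components with the mouse in a grab mode, toggled with the cursor on BeginPlay and G.
; Left click traces from the deprojected cursor, storing hit distance and relative grab point until release.
; Tick projects the cursor at that distance, pulling physics bodies or skeletal bones via PhysicsHandle with a debug line.
; Non-physics components move directly, offset by the grab point.
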(event `self.ReceiveBeginPlay`
  (bind _returnvalue (`GameplayStatics.GetPlayerController` 0))
  ;[1 1 1] Toggle mouse mode
  (set `self.GrabMode` (not (`self.GrabMode`)) :!label _label)
  (set `PlayerController.bShowMouseCursor` (not (`PlayerController.bShowMouseCursor` _returnvalue)) _returnvalue))

(event `Key|G`
  (params (Key :type "Key Structure"))
  ;[1 1 1] Toggle mouse mode
  (:`Pressed`
    (goto _label)))

(event `Key|LeftMouseButton`
  (params (Key :type "Key Structure"))
  (bind _grabmode (`self.GrabMode`))
  (bind (_worldlocation _worlddirection) (`PlayerController.DeprojectMousePositionToWorld` (`GameplayStatics.GetPlayerController` 0)))
  (bind (_bblockinghit _binitialoverlap _time _distance _location _impactpoint _normal _impactnormal _physmat _hitactor _hitcomponent) (`GameplayStatics.BreakHitResult` (`self.TraceHitResult`)))
  ;[1 1 1] click mouse button
  (:`Pressed`
    (if _grabmode
      ;[1 1 1] trace from mouse position to world
      (bind (_outhit _returnvalue) (`KismetSystemLibrary.LineTraceSingle` :`Start` _worldlocation :`End` (+ _worldlocation (* _worlddirection 10000000.0)) :`TraceChannel` "TraceTypeQuery1" :`bTraceComplex` true :`DrawDebugType` "ForDuration"))
      (set `self.TraceHitResult` _outhit)
      ;[1 1 1] validate result
      (if _returnvalue
        (set `self.ValidComponent` true)
        ;;[1 1 1] extraValidate
        (`/Engine/EditorBlueprintResources/StandardMacros.IsValid` (`.HitComponent` (`GameplayStatics.BreakHitResult` (`self.TraceHitResult`)))
          (:`Is Valid`
            ;;[1 1 1] movable?
            (if (== (enumliteral `EComponentMobility` "Movable") (`SceneComponent.Mobility` (`.HitComponent` (`GameplayStatics.BreakHitResult` (`self.TraceHitResult`)))))
              (bind _output_get (set `self.GrabbedComponent` (`.HitComponent` (`GameplayStatics.BreakHitResult` (`self.TraceHitResult`)))))
              ;[1 1 1] store O.G. distance
              (set `self.OriginalDistanceToObject` (`.Distance` (`GameplayStatics.BreakHitResult` (`self.TraceHitResult`))))
              ;[1 1 1] physics?
              (if (`SceneComponent.IsSimulatingPhysics` _output_get "None")
                ;[1 1 1] skelmesh?
                (cast `SkeletalMeshComponent` (`self.GrabbedComponent`)
                  (:`then`
                    (set `self.SkeletalMesh` true)
                    (set `self.BoneName` (`.HitBoneName` (`GameplayStatics.BreakHitResult` (`self.TraceHitResult`)))))
                  (:`CastFailed`
                    (set `self.SkeletalMesh` false)))
                ;[1 1 1] grab physics component where we pointed
                (`PhysicsHandleComponent.GrabComponentAtLocation` (`self.PhysicsHandle`) (`self.GrabbedComponent`) (`self.BoneName`) (`.Location` (`GameplayStatics.BreakHitResult` (`self.TraceHitResult`))))
                ;[1 1 1] calc grab location of physics mesh relative to center
                (set `self.RelativeGrabLocation` (`KismetMathLibrary.InverseTransformLocation` (select `bool` (`self.SkeletalMesh`) :`false` (`SceneComponent.K2_GetComponentToWorld` (`self.GrabbedComponent`)) :`true` (`SceneComponent.GetSocketTransform` (`self.GrabbedComponent`) (`self.BoneName`) "RTS_World")) (`.Location` (`GameplayStatics.BreakHitResult` (`self.TraceHitResult`)))))
                (else
                  ;[1 1 1] calculate grab location of non-physics mesh relative to center
                  (set `self.RelativeGrabLocation` (`KismetMathLibrary.InverseTransformLocation` (`KismetMathLibrary.Conv_VectorToTransform` (`SceneComponent.K2_GetComponentLocation` _hitcomponent)) _location))))))
          (:`Is Not Valid`
            (set `self.ValidComponent` false)))
        (else
          (set `self.ValidComponent` false)))))
  (:`Released`
    (if _grabmode
      (set `self.ValidComponent` false)
      (`PhysicsHandleComponent.ReleaseComponent` (`self.PhysicsHandle`))
      (set `self.GrabbedComponent` null))))

(event `self.ReceiveTick`
  (params (DeltaSeconds :type "Float (single-precision)"))
  (bind (_worldlocation _worlddirection) (`PlayerController.DeprojectMousePositionToWorld` (`GameplayStatics.GetPlayerController` 0)))
  ;[1 1 1] tick
  (set `self.deltaTick` DeltaSeconds)
  ;[1 1 1] grabMode on
  (if (and (`self.GrabMode`) (`self.ValidComponent`))
    (`/Engine/EditorBlueprintResources/StandardMacros.IsValid` (`self.GrabbedComponent`)
      (:`Is Valid`
        ;[1 1 1] ConvertMouseScreenLocationToWorldSpace
        (bind _output_get (set `self.MouseScreenLocToWorldSpace` (+ _worldlocation (* _worlddirection (`self.OriginalDistanceToObject`)))))
        ;[1 1 1] physics?
        (if (`SceneComponent.IsSimulatingPhysics` (`self.GrabbedComponent`) "None")
          ;[1 1 1] move physicsHandle in camera relative plane
          (`PhysicsHandleComponent.SetTargetLocation` (`self.PhysicsHandle`) _output_get)
          ;[1 1 1] draw debug-line
          (`KismetSystemLibrary.DrawDebugLine` _output_get (`KismetMathLibrary.TransformLocation` (select `bool` (`self.SkeletalMesh`) :`false` (`SceneComponent.K2_GetComponentToWorld` (`self.GrabbedComponent`)) :`true` (`SceneComponent.GetSocketTransform` (`self.GrabbedComponent`) (`self.BoneName`) "RTS_World")) (`self.RelativeGrabLocation`)) (struct :`R` 0.813436 :`G` 0.087154 :`B` 0.904514 :`A` 1.0) 0.0 5.0)
          (else
            ;[1 1 1] move non-physics object
            (`SceneComponent.K2_SetWorldLocation` (`self.GrabbedComponent`) (`KismetMathLibrary.InverseTransformLocation` (`KismetMathLibrary.Conv_VectorToTransform` (`self.RelativeGrabLocation`)) _output_get) false false)))))))

(fn `UserConstructionScript`)