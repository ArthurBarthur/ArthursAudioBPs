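; Synth ball actor that plays a sustained chord through a modular synth, with pitch driven by the ball's height.
; BeginPlay optionally randomizes the preset, builds the chord via ChordComponent, starts the selected notes, creates a dynamic material and enables Tick.
; Tick maps world Z to oscillator semitones.
; The synth's audio envelope, normalized against its historic peak, drives emissive brightness so the ball lights up with volume.
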(event `self.ReceiveBeginPlay`
  ;[1 1 1] beginplay
  (`KismetSystemLibrary.Delay` 0.25)
  (`|ExecutionSequence`
    (:`then_0`
      ;[1 1 1] init setup
      (`PrimitiveComponent.SetPhysMaterialOverride` (`self.BallMesh`) (`self.PhysMatOverride`)))
    (:`then_1`
      (if (`self.RandomizeSynthPreset`)
        ;[1 1 1] random preset override
        (if (`self.RandomizeSeedAsWell`)
          (bind _synthpresetfinal (`/Game/ArthursAudioBPs/SharedAssets/DataAssets/BP_DataPrimary_RandomPresets.RandomizePresetFull` (`self.RandomSynthPresetType`) (`KismetMathLibrary.RandomIntegerInRange` -666 214748364)))
          (set `self.BaseSynthPreset` _synthpresetfinal)
          (else
            (bind _synthpresetfinal_2 (`/Game/ArthursAudioBPs/SharedAssets/DataAssets/BP_DataPrimary_RandomPresets.RandomizePresetFull` (`self.RandomSynthPresetType`) (`self.RandomSeed`)))
            (set `self.BaseSynthPreset` _synthpresetfinal_2)))))
    (:`then_2`
      (`ModularSynthComponent.SetSynthPreset` (`self.ModularSynth`) (`self.BaseSynthPreset`)))
    (:`then_3`
      (bind _midinotes (`/Game/ArthursAudioBPs/SharedAssets/Components/ChordComponent/BP_ChordComponent.BuildChord` (`self.ChordComponent`) (`self.ChordSettings`)))
      (set `self.MidiNotes` _midinotes))
    (:`then_4`
      ;[1 1 1] note(s) on
      (if (`self.PlayBaseNote`)
        (`ModularSynthComponent.NoteOn` (`self.ModularSynth`) (`|GetArrayItem` (`self.MidiNotes`)) 100 -1.0)))
    (:`then_5`
      (if (`self.PlayRestOfChord`)
        (for _index (range 1 (+ (`KismetArrayLibrary.Array_LastIndex` (`self.MidiNotes`)) 1))
          (`ModularSynthComponent.NoteOn` (`self.ModularSynth`) (`|GetArrayItem` (`self.MidiNotes`) _index) 90 -1.0))))
    (:`then_6`
      ;[1 1 1] create dynamic material
      (bind _returnvalue (`KismetMaterialLibrary.CreateDynamicMaterialInstance` "/Game/ArthursAudioBPs/SharedAssets/Visuals/Materials/MI_SimpleMat_Inst1.MI_SimpleMat_Inst1"))
      (set `self.MID` _returnvalue)
      (`PrimitiveComponent.SetMaterial` (`self.BallMesh`) 0 (`self.MID`)))
    (:`then_7`
      ;[1 1 1] enable tick
      (`self.SetActorTickEnabled` true))))

(event `self.ReceiveTick`
  (params (DeltaSeconds :type "Float (single-precision)"))
  ;[1 1 1] tick
  (set `self.DeltaTick` DeltaSeconds)
  ;[1 1 1] world-loc to seminote
  (`self.WorldPosToSynthSeminote` (`self.WorldZRangeA`) (`self.WorldZRangeB`) (`self.SeminoteRangeA`) (`self.SemitoneRangeB`))
  ;[1 1 1] Change synth seminotes
  (for _index (range 2)
    (`ModularSynthComponent.SetOscSemitones` (`self.ModularSynth`) _index (`self.LatestSemitone`))
    ;[1 1 1] envelope(light up by volume)
    (set `self.EnvLatest` (stale `self.ModularSynth.OnAudioEnvelopeValue` EnvelopeValue))
    ;;[1 1 1] store max env ever
    (bind _output_get (set `self.EnvMaxHistoric` (`KismetMathLibrary.SelectFloat` (`self.EnvLatest`) (stale _output_get) (> (`self.EnvLatest`) (`self.EnvMaxHistoric`)))))
    (`MaterialInstanceDynamic.SetScalarParameterValue` (`self.MID`) "Emissive Multiplier" (`KismetMathLibrary.MapRangeClamped` (`KismetMathLibrary.MapRangeClamped` (`self.EnvLatest`) 0.0 (`self.EnvMaxHistoric`) 0.0 1.0) (`self.LowerThreshold`) 1.0 0.0 (`self.EmissiveStrength`)))))

(event `self.ModularSynth.OnAudioEnvelopeValue`
  (params (EnvelopeValue :type "Float (single-precision)"))
  ;[1 1 1] envelope(light up by volume)
)

(fn `UserConstructionScript`
  (set `SynthComponent.AttenuationSettings` (`self.AttenuationSettings`) (`self.ModularSynth`)))

(fn `WorldPosToSynthSeminote`
  (params (WorldZRangeA :type "Float (double-precision)") (WorldZRangeB :type "Float (double-precision)") (SeminoteRangeA :type "Float (double-precision)") (SeminoteRangeB :type "Float (double-precision)"))
  (returns (Seminote :type "Float (double-precision)"))
  (bind _output_get (set `self.LatestSemitone` (`KismetMathLibrary.MapRangeClamped` (.z (`SceneComponent.K2_GetComponentLocation` (`self.BallMesh`))) WorldZRangeA WorldZRangeB SeminoteRangeA SeminoteRangeB)))
  (return _output_get))