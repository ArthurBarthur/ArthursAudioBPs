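; Spawner actor that repeatedly drops BP_SynthBall actors on a looping timer, passing each its chord, synth preset, attenuation and physical material settings.
; Unless the floor Z is overridden, it line-traces down before each drop to find the floor.
; Drop and floor heights feed each ball's Z range, paired with semitone bend values for both ends.
; A seeded random stream seeds each ball, which receives a timed self-destruct component.
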(event `self.ReceiveBeginPlay`
  ;[1 1 1] init random stream
  (`KismetMathLibrary.SetRandomStreamSeed` (`self.RandomStream`) (`self.RandomOverrideSeed`))
  ;[1 1 1] repeating loop
  (`KismetSystemLibrary.K2_SetTimerDelegate` (`|CreateDelegate` :!event `dropppp`) (`self.DropTimer`) true)
  (if (not (`self.OverrideFloorZlvl`)) :!label _label
    ;[1 1 1] find distance to ground
    (`self.FindDistanceToGround`))
  ;[1 1 1] drop ball
  (`self.DropBall`))

(event `dropppp`
  (goto _label))

(fn `DropBall`
  (bind (_returnvalue_x _returnvalue_y _returnvalue_z) (`KismetMathLibrary.BreakVector` (`SceneComponent.K2_GetComponentLocation` (`self.DefaultSceneRoot`))))
  ;[1 1 1] drop ball
  (bind _returnvalue (`|SpawnActorFromClass` "/Game/ArthursAudioBPs/SharedAssets/Blueprints/ModSynth/bp_SynthBall.BP_SynthBall_C" (`SceneComponent.K2_GetComponentToWorld` (`self.DefaultSceneRoot`)) "Undefined" "OverrideRootScale" null (`self.ChordSettings`) (`self.PlayBaseNote`) (`self.PlayRestOfChord`) (`self.PhysMatOverride`) (`KismetMathLibrary.SelectFloat` (`self.DistanceToFloorOverride`) (- _returnvalue_z (`self.FloorZlvlOverride`)) (`self.OverrideFloorZlvl`)) (+ (`self.FloorZlvlOverride`) 50.0) (`self.SemitoneBendAtDropPoint`) (`self.SemitoneBendAtFloor`) (`self.BaseSynthPreset`) (`self.RandomPresetOverride`) false (`KismetMathLibrary.RandomIntegerInRangeFromStream` 0 1000000 (`self.RandomStream`)) (`self.RandomSynthPresetType`) (`self.AttenuationSettings`) null))
  (`AddComponent|NODE_AddSelfDestructComponent-1` :`self` _returnvalue :`TimeToLive` (`self.TimeToLive`)))

(fn `FindDistanceToGround`
  (returns (Distance :type "Float (double-precision)"))
  (locals (_hitResult :type "HitResult Structure"))
  (bind _returnvalue (`SceneComponent.K2_GetComponentLocation` (`self.DefaultSceneRoot`)))
  ;[1 1 1] trace down to get distance to ground
  (bind (_outhit _returnvalue_2) (`KismetSystemLibrary.LineTraceSingleForObjects` :`Start` _returnvalue :`End` (- _returnvalue (0.0 0.0 10000.0)) :`ObjectTypes` (`|MakeArray` "ObjectTypeQuery1" :!type "EObjectTypeQuery Enum") :`DrawDebugType` "ForDuration"))
  (set `local._hitResult` _outhit)
  (if _returnvalue_2
    ;[1 1 1] store floor Z lvl at drop
    (set `self.FloorZlvlOverride` (.z (`.Location` (`GameplayStatics.BreakHitResult` (`local._hitResult`)))))
    ;[1 1 1] return distance to floor
    (bind _output_get (set `self.DistanceToFloorOverride` (`.Distance` (`GameplayStatics.BreakHitResult` (`local._hitResult`)))))
    (return _output_get)))

(fn `UserConstructionScript`)