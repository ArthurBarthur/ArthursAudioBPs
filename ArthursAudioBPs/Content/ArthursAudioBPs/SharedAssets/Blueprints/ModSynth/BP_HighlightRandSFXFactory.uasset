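; BP_HighlightRandSFXFactory is a placement actor that scatters musical BP_HighlightRandSFX instances, referred to as plants, over a random area.
; Its construction script clears previous spawns, then adds the requested number of child actor components at random flat XY offsets within the spawn range.
; It casts each child actor into the Highlighters array and passes on the shared chord settings and note length.
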(fn `SpawnActors`
  (locals (ChildActorComponents :type "Array of ChildActorComponent Object Reference"))
  (bind _childactorcomponents (`local.ChildActorComponents`))
  (bind _highlighters (`self.Highlighters`))
  (for _array_element _highlighters
    (`/Engine/EditorBlueprintResources/StandardMacros.IsValid` _array_element
      (:`Is Valid`
        (`self.K2_DestroyActor` _array_element))))
  (`KismetArrayLibrary.Array_Clear` _highlighters)
  (for _array_element_2 _childactorcomponents
    (`ActorComponent.K2_DestroyComponent` _array_element_2))
  (`KismetArrayLibrary.Array_Clear` _childactorcomponents)
  (for _ (range (`self.NumberOfSpawns`))
    (bind _returnvalue (`AddComponent|NODE_AddChildActorComponent-0` :`RelativeTransform` (`KismetMathLibrary.MakeTransform` (`KismetMathLibrary.MakeVector` (`KismetMathLibrary.RandomFloatInRange` (`self.SpawnAreaRange1`) (`self.SpawnAreaRange2`)) (`KismetMathLibrary.RandomFloatInRange` (`self.SpawnAreaRange1`) (`self.SpawnAreaRange2`))))))
    (`KismetArrayLibrary.Array_Add` (`local.ChildActorComponents`) _returnvalue))
  ;[1 1 1] convert to Highlighters actor ref array
  (for _array_element_3 (`local.ChildActorComponents`)
    (`ChildActorComponent.SetChildActorClass` _array_element_3 "/Game/ArthursAudioBPs/SharedAssets/Blueprints/ModSynth/BP_HighlightRandSFX.BP_HighlightRandSFX_C"))
  (for _array_element_4 (`local.ChildActorComponents`)
    (bind _asbp_highlight_rand_sfx (cast `/Game/ArthursAudioBPs/SharedAssets/Blueprints/ModSynth/BP_HighlightRandSFX` (`ChildActorComponent.ChildActor` _array_element_4))
      (:`then`
        (`KismetArrayLibrary.Array_Add` (`self.Highlighters`) _asbp_highlight_rand_sfx))
      (:`CastFailed`
        (`KismetSystemLibrary.PrintString` "this should never happen"))))
  ;[1 1 1] set up musicality in plants
  (for _array_element_5 (`self.Highlighters`)
    (set `/Game/ArthursAudioBPs/SharedAssets/Blueprints/ModSynth/BP_HighlightRandSFX.ChordSettings` (`self.ChordSettings`) _array_element_5)
    (set `/Game/ArthursAudioBPs/SharedAssets/Blueprints/ModSynth/BP_HighlightRandSFX.NoteLength` (`self.NoteLengthPerTrigger`) _array_element_5)))

(fn `UserConstructionScript`
  (`self.SpawnActors`))