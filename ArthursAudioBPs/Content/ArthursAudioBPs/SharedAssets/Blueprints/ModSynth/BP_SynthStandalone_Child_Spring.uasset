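; Standalone modular synth child whose sound is driven live by the travel of a linked spring Blueprint.
; With AttachToSpring set, its ball mesh snaps to the spring's pad at construction and BeginPlay.
; Each tick, normalized travel sets both oscillators' opposing detune, gain and pulsewidth, with pulsewidth direction following whether the spring is pushed up.
; Travel also drives filter frequency through a curve, with an option to invert the response.
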(event `self.ReceiveBeginPlay`
  ;[1 1 1] beginPlay
  (`parent.ReceiveBeginPlay`)
  ;[1 1 1] attach to spring
  (if (`self.AttachToSpring`)
    (`SceneComponent.K2_AttachToComponent` (`self.BallMesh`) (`/Game/ArthursAudioBPs/SharedAssets/Blueprints/SpringKeys/BP_Spring.Pad` (`self.bp_springRef`)) "None" "SnapToTarget" "SnapToTarget" "KeepWorld" true)))

(event `self.ReceiveTick`
  (params (DeltaSeconds :type "Float (single-precision)"))
  (bind _travelnormalized (`/Game/ArthursAudioBPs/SharedAssets/Blueprints/SpringKeys/BP_Spring.TravelNormalized` (`self.bp_springRef`)))
  (bind _returnvalue (`KismetMathLibrary.MapRangeClamped` (`/Game/ArthursAudioBPs/SharedAssets/Blueprints/SpringKeys/BP_Spring.TravelNormalized` (`self.bp_springRef`)) 0.0 1.0 0.0 5.0))
  ;[1 1 1] tick
  (`parent.ReceiveTick` DeltaSeconds)
  (`|ExecutionSequence`
    (:`then_0`
      ;[1 1 1] Loop over Oscillators
      (for _index (range 2)
        (`|ExecutionSequence`
          (:`then_0`
            ;[1 1 1] Detune Oscillators
            (`ModularSynthComponent.SetOscCents` (`self.ModularSynth`) _index (select `int` _index :`0` _returnvalue :`1` (* _returnvalue -1.0))))
          (:`then_1`
            ;[1 1 1] Control Gain on Oscillators
            (`ModularSynthComponent.SetOscGain` (`self.ModularSynth`) _index (`KismetMathLibrary.MapRangeClamped` (`/Game/ArthursAudioBPs/SharedAssets/Blueprints/SpringKeys/BP_Spring.TravelNormalized` (`self.bp_springRef`)) 0.05 1.0 0.001 1.0)))
          (:`then_2`
            ;[1 1 1] Control Oscillators Pulsewidth
            (`ModularSynthComponent.SetOscPulsewidth` (`self.ModularSynth`) _index (select `bool` (`/Game/ArthursAudioBPs/SharedAssets/Blueprints/SpringKeys/BP_Spring.PushedUp` (`self.bp_springRef`)) :`false` (`KismetMathLibrary.MapRangeClamped` (`/Game/ArthursAudioBPs/SharedAssets/Blueprints/SpringKeys/BP_Spring.TravelNormalized` (`self.bp_springRef`)) 0.0 1.0 0.5 0.0) :`true` (`KismetMathLibrary.MapRangeClamped` (`/Game/ArthursAudioBPs/SharedAssets/Blueprints/SpringKeys/BP_Spring.TravelNormalized` (`self.bp_springRef`)) 0.0 1.0 0.5 1.0)))))))
    (:`then_1`
      ;[1 1 1] Control Filter Freq
      (`ModularSynthComponent.SetFilterFrequency` (`self.ModularSynth`) (`CurveFloat.GetFloatValue` (`self.CurveFilter`) (`KismetMathLibrary.SelectFloat` (`KismetMathLibrary.MapRangeClamped` _travelnormalized 0.0 1.0 0.5 1.0) (`KismetMathLibrary.MapRangeClamped` _travelnormalized 0.0 1.0 1.0 0.5) (`self.InvertSpringResponse`)))))))

(fn `UserConstructionScript`
  (`parent.UserConstructionScript`)
  (`PrimitiveComponent.SetSimulatePhysics` (`self.BallMesh`) (`self.SimulatePhysics`))
  (`/Engine/EditorBlueprintResources/StandardMacros.IsValid` (`self.bp_springRef`)
    (:`Is Valid`
      (if (`self.AttachToSpring`)
        (`PrimitiveComponent.SetCollisionEnabled` (`self.BallMesh`) "NoCollision")
        (`SceneComponent.K2_AttachToComponent` (`self.BallMesh`) (`/Game/ArthursAudioBPs/SharedAssets/Blueprints/SpringKeys/BP_Spring.Pad` (`self.bp_springRef`)) "None" "SnapToTarget" "SnapToTarget" "KeepWorld" true)))))