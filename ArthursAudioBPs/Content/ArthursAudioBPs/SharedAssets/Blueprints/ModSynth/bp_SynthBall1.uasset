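; A synth ball actor that plays a sustained Modular Synth note whose pitch follows the height of its mesh.
; After a short BeginPlay delay it applies a physical material override, loads a base or randomized preset, builds a chord and holds one random note from it.
; It then swaps the ball material and enables Tick, which maps world Z to semitones on both oscillators.
; The construction script applies the synth's attenuation settings.
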(event `self.ReceiveBeginPlay`
  (bind _midinotes (`self.MidiNotes`))
  ;[1 1 1] beginplay
  (`KismetSystemLibrary.Delay` 0.25)
  (`|ExecutionSequence`
    (:`then_0`
      ;[1 1 1] init setup
      (`PrimitiveComponent.SetPhysMaterialOverride` (`self.BallMesh`) (`self.PhysMatOverride`)))
    (:`then_1`
      ;;[1 1 1] random preset override?
      (if (`self.RandomPresetOverride`)
        (bind _synthpresetfinal (`/Game/ArthursAudioBPs/SharedAssets/DataAssets/DataPrimary_RandomPresets.RandomizePresetFull` (`self.RandomSynthPresetType`) (`self.RandomPresetOverrideSeed`)))
        (set `self.BaseSynthPreset` _synthpresetfinal)))
    (:`then_2`
      (`ModularSynthComponent.SetSynthPreset` (`self.ModularSynth`) (`self.BaseSynthPreset`)))
    (:`then_3`
      (bind _midinotes_2 (`/Game/ArthursAudioBPs/SharedAssets/Components/ChordComponent/ChordComponent.BuildChord` (`self.ChordComponent`) (`self.ChordSettings`)))
      (set `self.MidiNotes` _midinotes_2))
    (:`then_4`
      ;[1 1 1] note(s) on
      (`ModularSynthComponent.NoteOn` (`self.ModularSynth`) (`|GetArrayItem` _midinotes (`KismetMathLibrary.RandomIntegerInRangeFromStream` 0 (`KismetArrayLibrary.Array_LastIndex` _midinotes) (`self.RandomStream`))) 100 -1.0))
    (:`then_5`
      ;[1 1 1] change material
      (`KismetSystemLibrary.Delay` 0.2)
      (`PrimitiveComponent.SetMaterial` (`self.BallMesh`) 0 "/Game/ArthursAudioBPs/SharedAssets/Visuals/Materials/m_SimpleMat_Inst5.m_SimpleMat_Inst5"))
    (:`then_6`
      ;[1 1 1] enable tick
      (`self.SetActorTickEnabled` true))))

(event `self.ReceiveTick`
  (params (DeltaSeconds :type "Float (single-precision)"))
  ;[1 1 1] tick
  (set `self.DeltaTick` DeltaSeconds)
  ;[1 1 1] world-loc to seminote
  (`self.WorldPosToSynthSeminote` (`self.WorldZRangeA`) (`self.WorldZRangeB`) (`self.SeminoteRangeA`) (`self.SemitoneRangeB`))
  ;[1 1 1] Change synth seminotes
  (for _index (range 2)
    (`ModularSynthComponent.SetOscSemitones` (`self.ModularSynth`) _index (`self.LatestSemitone`))))

(fn `UserConstructionScript`
  (set `SynthComponent.AttenuationSettings` (`self.AttenuationSettings`) (`self.ModularSynth`)))

(fn `WorldPosToSynthSeminote`
  (params (WorldZRangeA :type "Float (double-precision)") (WorldZRangeB :type "Float (double-precision)") (SeminoteRangeA :type "Float (double-precision)") (SeminoteRangeB :type "Float (double-precision)"))
  (returns (Seminote :type "Float (double-precision)"))
  (bind _output_get (set `self.LatestSemitone` (`KismetMathLibrary.MapRangeClamped` (.z (`SceneComponent.K2_GetComponentLocation` (`self.BallMesh`))) WorldZRangeA WorldZRangeB SeminoteRangeA SeminoteRangeB)))
  (return _output_get))