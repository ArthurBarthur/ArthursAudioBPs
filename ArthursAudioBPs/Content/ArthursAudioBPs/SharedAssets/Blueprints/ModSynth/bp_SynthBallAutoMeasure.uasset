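; Synth ball actor that plays a sustained random chord note on a ModularSynth and bends its pitch by the ball's height.
; On BeginPlay it applies a base or randomized preset, picks the note with a seeded stream, and traces down to measure the floor automatically.
; Tick maps the mesh's Z between spawn and floor to oscillator semitones.
; The synth's smoothed audio envelope drives the material's emissive glow.
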(event `self.ReceiveBeginPlay`
  (bind _midinotes (`self.MidiNotes`))
  (bind (_returnvalue_x _returnvalue_y _returnvalue_z) (`KismetMathLibrary.BreakVector` (`SceneComponent.K2_GetComponentLocation` (`self.RootComponent`))))
  ;[1 1 1] beginplay
  (`KismetSystemLibrary.Delay` 0.25)
  (`|ExecutionSequence`
    (:`then_0`
      ;[1 1 1] init setup
      (`KismetMathLibrary.SetRandomStreamSeed` (`self.RandomStream`) (`self.RandomOverrideSeed`)))
    (:`then_1`
      (`PrimitiveComponent.SetPhysMaterialOverride` (`self.BallMesh`) (`self.PhysMatOverride`)))
    (:`then_2`
      ;;[1 1 1] random preset override?
      (if (`self.RandomPresetOverride`)
        (bind _synthpresetfinal (`/Game/ArthursAudioBPs/SharedAssets/DataAssets/DataPrimary_RandomPresets.RandomizePresetFull` (`self.RandomSynthPresetType`) (`self.RandomOverrideSeed`)))
        (set `self.BaseSynthPreset` _synthpresetfinal)))
    (:`then_3`
      (`ModularSynthComponent.SetSynthPreset` (`self.ModularSynth`) (`self.BaseSynthPreset`)))
    (:`then_4`
      (bind _midinotes_2 (`/Game/ArthursAudioBPs/SharedAssets/Components/ChordComponent/ChordComponent.BuildChord` (`self.ChordComponent`) (`self.ChordSettings`)))
      (set `self.MidiNotes` _midinotes_2))
    (:`then_5`
      ;[1 1 1] note(s) on
      (`ModularSynthComponent.NoteOn` (`self.ModularSynth`) (`|GetArrayItem` _midinotes (`KismetMathLibrary.RandomIntegerInRangeFromStream` 0 (`KismetArrayLibrary.Array_LastIndex` _midinotes) (`self.RandomStream`))) 100 -1.0))
    (:`then_6`
      ;[1 1 1] create dynamic material
      (bind _returnvalue (`PrimitiveComponent.CreateDynamicMaterialInstance` (`self.BallMesh`) 0 "/Game/ArthursAudioBPs/SharedAssets/Visuals/Materials/m_SimpleMat_Inst1.m_SimpleMat_Inst1" "None"))
      (set `self.MID` _returnvalue))
    (:`then_7`
      ;[1 1 1] measure height
      (`self.FindDistanceToGround`)
      (set `self.WorldZRangeA` _returnvalue_z)
      (set `self.WorldZRangeB` (+ (`self.FloorZlvlOverride`) 50.0)))
    (:`then_8`
      ;[1 1 1] enable tick
      (`self.SetActorTickEnabled` true))))

(event `self.ReceiveTick`
  (params (DeltaSeconds :type "Float (single-precision)"))
  ;[1 1 1] tick
  (set `self.DeltaTick` DeltaSeconds)
  ;[1 1 1] world-loc to seminote
  (`self.WorldPosToSynthSeminote` (`self.WorldZRangeA`) (`self.WorldZRangeB`) (`self.SeminoteBendAtSpawnHeight`) (`self.SemitoneRangeAtGroundBelow`))
  ;[1 1 1] Change synth oscs seminotes
  (for _index (range 2)
    (`ModularSynthComponent.SetOscSemitones` (`self.ModularSynth`) _index (`self.LatestSemitone`))))

(event `self.ModularSynth.OnAudioEnvelopeValue`
  (params (EnvelopeValue :type "Float (single-precision)"))
  ;[1 1 1] envelope
  (bind _envsmoothed (`/Game/ArthursAudioBPs/SharedAssets/Components/NormalizingAndSmoothingComponent.Beautify` (`self.NormalizingAndSmoothingComponnent`) EnvelopeValue 100.0 500.0))
  (`MaterialInstanceDynamic.SetScalarParameterValue` (`self.MID`) "Emissive Multiplier" (* _envsmoothed 20.0)))

(fn `FindDistanceToGround`
  (returns (Output_Get :type "Float (double-precision)"))
  (locals (_hitResult :type "HitResult Structure"))
  (bind _returnvalue (`SceneComponent.K2_GetComponentLocation` (`self.RootComponent`)))
  ;[1 1 1] trace down to get distance to ground
  (bind (_outhit _returnvalue_2) (`KismetSystemLibrary.LineTraceSingleForObjects` :`Start` _returnvalue :`End` (- _returnvalue (0.0 0.0 100000000.0)) :`ObjectTypes` (`|MakeArray` "ObjectTypeQuery1" :!type "EObjectTypeQuery Enum") :`DrawDebugType` "ForDuration"))
  (set `local._hitResult` _outhit)
  (if _returnvalue_2
    ;[1 1 1] store floor Z lvl at drop
    (set `self.FloorZlvlOverride` (.z (`.Location` (`GameplayStatics.BreakHitResult` (`local._hitResult`)))))
    (return 0.0)))

(fn `UserConstructionScript`
  (set `SynthComponent.AttenuationSettings` (`self.AttenuationSettings`) (`self.ModularSynth`)))

(fn `WorldPosToSynthSeminote`
  (params (WorldZRangeA :type "Float (double-precision)") (WorldZRangeB :type "Float (double-precision)") (SeminoteRangeA :type "Float (double-precision)") (SeminoteRangeB :type "Float (double-precision)"))
  (returns (Seminote :type "Float (double-precision)"))
  (bind _output_get (set `self.LatestSemitone` (`KismetMathLibrary.MapRangeClamped` (.z (`SceneComponent.K2_GetComponentLocation` (`self.BallMesh`))) WorldZRangeA WorldZRangeB SeminoteRangeA SeminoteRangeB)))
  (return _output_get))