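; Spatialized synth prop that plays notes with a randomized preset and pulses a randomly colored mesh to its sound.
; BeginPlay randomizes the ModularSynth preset, builds a chord and picks one special note from it.
; NotePlay triggers that note or loops over the chord, with timed note-off and gated deactivation after inactivity.
; The envelope follower, normalized against a decaying peak, drives emissive, color brightness and mesh height.
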(event `self.ReceiveBeginPlay`
  (bind _currentnotes (`self.CurrentNotes`))
  (`|ExecutionSequence`
    (:`then_0`
      ;[1 1 1] randomized synth preset
      (`self.RandomizePreset`)
      (`ModularSynthComponent.SetSynthPreset` (`self.ModularSynth`) (`self.SynthBasePreset`))
      ;[1 1 1] get chord
      (bind _midinotes (`/Game/ArthursAudioBPs/SharedAssets/Components/ChordComponent/BP_ChordComponent.BuildChord` (`self.BP_ChordComponent`) (`self.ChordSettings`)))
      (set `self.CurrentNotes` _midinotes)
      ;[1 1 1] make special random note
      (set `self.SpecialRandomNote` (`|GetArrayItem` _currentnotes (`KismetMathLibrary.RandomIntegerInRange` 0 (`KismetArrayLibrary.Array_LastIndex` _currentnotes)))))
    (:`then_1`
      ;[1 1 1] dynamic material MID
      (bind _returnvalue (`PrimitiveComponent.CreateDynamicMaterialInstance` (`self.StaticMesh`) 0 "/Game/ArthursAudioBPs/SharedAssets/Visuals/Materials/MAT_SimpleMat.MAT_SimpleMat" "None"))
      (set `self.MID` _returnvalue)
      (set `self.Color` (`KismetMathLibrary.HSVToRGB` (`KismetMathLibrary.RandomFloatInRange` 0.0 360.0) (`KismetMathLibrary.RandomFloat`) (`KismetMathLibrary.RandomFloat`))))
    (:`then_2`
      ;[1 1 1] decrease max historic vol
      (`KismetSystemLibrary.K2_SetTimerDelegate` (delegate `DecreaseHistoricMaxEnv`) 0.5 true))))

(event `DecreaseHistoricMaxEnv`
  ;[1 1 1] decrease max historic vol
  (bind _output_get (set `self.EnvMax` (* (stale _output_get) 0.9))))

(event `/Game/ArthursAudioBPs/SharedAssets/Interfaces/MidiNoteSendingInterface.NotePlay`
  (params (Note :type "Float (single-precision)") (Velocity :type Integer) (Duration :type "Float (single-precision)"))
  (`|ExecutionSequence`
    (:`then_0`
      (`ActorComponent.Activate` (`self.ModularSynth`) false)
      (`|ExecutionSequence`
        (:`then_0`
          (if (`self.PlayOnlyOneUniqueNote`)
            ;[1 1 1] play one unique note
            (`ModularSynthComponent.NoteOn` (`self.ModularSynth`) (`self.SpecialRandomNote`) 100 -1.0)
            (else
              ;[1 1 1] play all notes in chord
              (for _ (`self.CurrentNotes`)
                (`ModularSynthComponent.NoteOn` (`self.ModularSynth`) 0.0 100 -1.0)))))
        (:`then_1`
          ;[1 1 1] turn off note after some time
          (`KismetSystemLibrary.RetriggerableDelay` (`self.NoteLength`))
          (`ModularSynthComponent.NoteOff` (`self.ModularSynth`) 0.0 true false))))
    (:`then_1`
      (goto _label :!via `Close`))))

(event `/Game/ArthursAudioBPs/SharedAssets/Interfaces/MidiNoteSendingInterface.NoteStop`
  (params (Note :type "Float (single-precision)") (StopAll :type Boolean))
  (`|ExecutionSequence`
    (:`then_0`
      (`ModularSynthComponent.NoteOff` (`self.ModularSynth`) 0.0 true false)
      ;[1 1 1] deactivate after 10 seconds of inactivity
      (`KismetSystemLibrary.RetriggerableDelay` 10.0)
      (`/Engine/EditorBlueprintResources/StandardMacros.Gate` false :!label _label
        (:`Exit`
          (`ActorComponent.Deactivate` (`self.ModularSynth`)))))
    (:`then_1`
      (goto _label :!via `Open`))))

(event `self.ModularSynth.OnAudioEnvelopeValue`
  (params (EnvelopeValue :type "Float (single-precision)"))
  (bind (_h _s _v _a) (`KismetMathLibrary.RGBToHSV` (`self.Color`)))
  (bind (_h_2 _s_2 _v_2 _a_2) (`KismetMathLibrary.RGBToHSV` (`self.Color`)))
  ;[1 1 1] normalize
  (set `self.EnvLatest` EnvelopeValue)
  (if (> (`self.EnvLatest`) (`self.EnvMax`))
    (set `self.EnvMax` (`self.EnvLatest`)))
  (set `self.Vol0-1` (`KismetMathLibrary.MapRangeClamped` (`self.EnvLatest`) 0.0 (`self.EnvMax`) 0.0 1.0))
  ;[1 1 1] mod material
  (`MaterialInstanceDynamic.SetScalarParameterValue` (`self.MID`) "Emissive Multiplier" (* (+ (`self.Vol0-1`) 0.5) (`self.EmissiveMultiplier`)))
  (`MaterialInstanceDynamic.SetVectorParameterValue` (`self.MID`) "Base Color" (`KismetMathLibrary.LinearColorLerp` (`KismetMathLibrary.HSVToRGB` _h_2 _s_2 0.5 _a_2) (`KismetMathLibrary.HSVToRGB` _h _s 1.0 _a) (`self.Vol0-1`)))
  ;[1 1 1] move mesh up and down
  (`SceneComponent.K2_SetRelativeLocation` (`self.StaticMesh`) (`KismetMathLibrary.MakeVector` 0.0 0.0 (* (`self.Vol0-1`) 50.0)) false false))

(fn `RandomizePreset`
  (bind _synthpresetfinal (`/Game/ArthursAudioBPs/SharedAssets/DataAssets/BP_DataPrimary_RandomPresets.RandomizePresetFull` (`self.PresetGeneratorRandom`) (+ (`KismetMathLibrary.RandomIntegerInRange` -1000000 1000000) (`KismetMathLibrary.FTrunc` (* (`.PartialSeconds` (`GameplayStatics.GetAccurateRealTime`)) 100000.0)))))
  (set `self.SynthBasePreset` _synthpresetfinal))

(fn `UserConstructionScript`
  (bind _modularsynth (`self.ModularSynth`))
  (`|ExecutionSequence`
    (:`then_0`
      (bind _returnvalue (`AddComponent|NODE_AddStaticMeshComponent-0`))
      (set `self.StaticMesh` _returnvalue)
      (`StaticMeshComponent.SetStaticMesh` (`self.StaticMesh`) (`self.MeshToUse`)))
    (:`then_1`
      (bind _returnvalue_2 (`AddComponent|NODE_AddModularSynthComponent-0`))
      (set `self.ModularSynth` _returnvalue_2)
      (set `SynthComponent.AttenuationSettings` "/Game/ArthursAudioBPs/SharedAssets/Audio/Attenuation/ATT_HighlightRandSFX.ATT_HighlightRandSFX" (`self.ModularSynth`))
      (set `SynthComponent.bAllowSpatialization` true (`self.ModularSynth`))
      (set `SynthComponent.EnvelopeFollowerAttackTime` 300 _modularsynth)
      (set `SynthComponent.EnvelopeFollowerReleaseTime` 2000 _modularsynth))))