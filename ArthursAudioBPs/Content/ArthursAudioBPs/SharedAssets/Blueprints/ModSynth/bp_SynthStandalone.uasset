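; Standalone synth actor with a ball mesh that plays notes received through a note interface and glows in response to its own audio.
; On BeginPlay, after a short delay, it applies a physical material, loads the base or randomized preset into ModularSynth and creates a dynamic material.
; Tick normalizes the synth's audio envelope against its historic peak to drive emissive strength, so the glow self-calibrates to loudness.
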(event `self.ReceiveBeginPlay`
  ;[1 1 1] beginplay
  (`KismetSystemLibrary.Delay` 0.25)
  (`|ExecutionSequence`
    (:`then_0`
      ;[1 1 1] init setup
      (`PrimitiveComponent.SetPhysMaterialOverride` (`self.BallMesh`) (`self.PhysMatOverride`)))
    (:`then_1`
      ;;[1 1 1] random preset override?
      (if (`self.RandomPresetOverride`)
        (bind _synthpresetfinal (`/Game/ArthursAudioBPs/SharedAssets/DataAssets/DataPrimary_RandomPresets.RandomizePresetFull` (`self.RandomSynthPresetType`) (`self.RandomOverrideSeed`)))
        (set `self.BaseSynthPreset` _synthpresetfinal)))
    (:`then_2`
      (`ModularSynthComponent.SetSynthPreset` (`self.ModularSynth`) (`self.BaseSynthPreset`)))
    (:`then_3`
      ;[1 1 1] init dynamic material
      (bind _returnvalue (`KismetMaterialLibrary.CreateDynamicMaterialInstance` "/Game/ArthursAudioBPs/SharedAssets/Visuals/Materials/m_SimpleMat_Inst1.m_SimpleMat_Inst1"))
      (bind _output_get (set `self.MID` _returnvalue))
      (`PrimitiveComponent.SetMaterial` (`self.BallMesh`) 0 _output_get))
    (:`then_6`
      ;[1 1 1] enable tick
      (`self.SetActorTickEnabled` true))))

(event `/Game/ArthursAudioBPs/SharedAssets/Interfaces/NoteInterface.NotePlay`
  (params (Note :type "Float (single-precision)") (Velocity :type Integer) (Duration :type "Float (single-precision)"))
  ;[1 1 1] note interface
  ;[1 1 1] receive note-interface here in this actor
  (`ModularSynthComponent.NoteOn` (`self.ModularSynth`) Note Velocity -1.0))

(event `/Game/ArthursAudioBPs/SharedAssets/Interfaces/NoteInterface.NoteStop`
  (params (Note :type "Float (single-precision)") (StopAll :type Boolean))
  ;[1 1 1] note interface
  ;[1 1 1] receive note-interface here in this actor
  (`ModularSynthComponent.NoteOff` (`self.ModularSynth`) Note StopAll false))

(event `self.ReceiveTick`
  (params (DeltaSeconds :type "Float (single-precision)"))
  ;[1 1 1] tick
  (set `self.DeltaTick` DeltaSeconds)
  (set `self.EnvLatest` (stale `self.ModularSynth.OnAudioEnvelopeValue` EnvelopeValue))
  ;[1 1 1] store max env ever
  (bind _output_get (set `self.EnvMaxHistoric` (`KismetMathLibrary.SelectFloat` (`self.EnvLatest`) (stale _output_get) (> (`self.EnvLatest`) (`self.EnvMaxHistoric`)))))
  ;[1 1 1] mod material emissive
  (`MaterialInstanceDynamic.SetScalarParameterValue` (`self.MID`) "Emissive Multiplier" (`KismetMathLibrary.MapRangeClamped` (`KismetMathLibrary.MapRangeClamped` (`self.EnvLatest`) 0.0 (`self.EnvMaxHistoric`) 0.0 1.0) 0.3 1.0 0.0 (`self.EmissiveStrength`))))

(event `self.ModularSynth.OnAudioEnvelopeValue`
  (params (EnvelopeValue :type "Float (single-precision)")))

(fn `PlayNote`
  (params (Note :type "Float (double-precision)") (Velocity :type Integer)))

(fn `UserConstructionScript`
  (set `SynthComponent.AttenuationSettings` (`self.AttenuationSettings`) (`self.ModularSynth`)))