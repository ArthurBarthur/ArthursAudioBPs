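; Music conductor actor that spawns a 3D grid of BP_granular synths and plays them as one chordal instrument.
; Chord events, fired directly or by the song timeline, give each synth a random chord note and octave, then trigger a volume envelope timeline.
; Tick normalizes the SoundPlayer drum envelope against a decaying peak to drive the mesh's color and glow and sidechain the synths' volume.
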(event `self.ReceiveBeginPlay`
  ;[1 1 1] beginplay
  (`|ExecutionSequence`
    (:`then_0`
      ;[1 1 1] spawn granulars
      (`self.SpawnGranularArray`))
    (:`then_1`
      ;[1 1 1] create  floor drum MID
      (bind _returnvalue (`KismetMaterialLibrary.CreateDynamicMaterialInstance` "/Game/ArthursAudioBPs/SharedAssets/Visuals/Materials/MI_SimpleMat_Inst1.MI_SimpleMat_Inst1"))
      (bind _output_get (set `self.MID` _returnvalue))
      (`PrimitiveComponent.SetMaterial` (`self.StaticMesh`) 0 _output_get))
    (:`then_2`
      ;[1 1 1] timer for decreasing max recorded env
      (`KismetSystemLibrary.K2_SetTimerDelegate` (`|CreateDelegate` :!event `DecreaseHistoricMaxEnv`) 0.5 true))))

(event `Oct+`
  ;[1 1 1] oct +/-
  (for _array_element (`self.SpwndGranulars`)
    (`/Game/ArthursAudioBPs/SharedAssets/Blueprints/GranularSynth/GranularMusic/BP_granular.Octave+` _array_element)))

(event `ResetAllNotes`
  ;[1 1 1] reset notes
  (for _array_element (`self.SpwndGranulars`)
    (set `/Game/ArthursAudioBPs/SharedAssets/Blueprints/GranularSynth/GranularMusic/BP_granular.Note` 0 _array_element)
    (set `/Game/ArthursAudioBPs/SharedAssets/Blueprints/GranularSynth/GranularMusic/BP_granular.Octave` 4 _array_element)))

(event `Oct-`
  ;[1 1 1] oct +/-
  (for _array_element (`self.SpwndGranulars`)
    (`/Game/ArthursAudioBPs/SharedAssets/Blueprints/GranularSynth/GranularMusic/BP_granular.Octave-` _array_element)))

(event `Start`
  ;[1 1 1] start
  (for _array_element (`self.SpwndGranulars`)
    (`GranularSynth.NoteOn` (`/Game/ArthursAudioBPs/SharedAssets/Blueprints/GranularSynth/GranularMusic/BP_granular.GranularSynth` _array_element) 60.0 100 -1.0)))

(event `Stop`
  ;[1 1 1] stop
  (for _array_element (`self.SpwndGranulars`)
    (`GranularSynth.NoteOff` (`/Game/ArthursAudioBPs/SharedAssets/Blueprints/GranularSynth/GranularMusic/BP_granular.GranularSynth` _array_element) 60.0 false)))

(event `Randomize Source samples`
  ;[1 1 1] randomize source sounds
  (for _array_element (`self.SpwndGranulars`)
    (`/Game/ArthursAudioBPs/SharedAssets/Blueprints/GranularSynth/GranularMusic/BP_granular.ChangeRandomActiveSound` _array_element)))

(event `AMaj`
  ;[1 1 1] chords
  (`self.ChordSwitch` (`self.ArrChordAmaj`)))

(event `RandomPlayheadTimes`
  ;[1 1 1] Random playhead time
  (for _array_element (`self.SpwndGranulars`)
    (`/Game/ArthursAudioBPs/SharedAssets/Blueprints/GranularSynth/GranularMusic/BP_granular.RandomPlayheadTime` _array_element)))

(event `Playsong`
  ;[1 1 1] play song
  (`Timeline|Timeline_0` :!via `PlayFromStart`
    (:`F`
      (`self.FMaj`))
    (:`G`
      (`self.GMaj`))
    (:`Am`
      (`self.AMin`))))

(event `AMin`
  ;[1 1 1] chords
  (`self.ChordSwitch` (`self.ArrChordAmin`)))

(event `BMin`
  ;[1 1 1] chords
  (`self.ChordSwitch` (`self.ArrChordBMin`)))

(event `FMaj`
  ;[1 1 1] chords
  (`self.ChordSwitch` (`self.ArrChordFmaj`)))

(event `AllRandOctave`
  ;[1 1 1] RandOct
  (for _array_element (`self.SpwndGranulars`)
    (set `/Game/ArthursAudioBPs/SharedAssets/Blueprints/GranularSynth/GranularMusic/BP_granular.Octave` (`KismetMathLibrary.RandomIntegerInRange` (`self.OctaveRangeMin`) (`self.OctaveRangeMax`)) _array_element))
  ;[1 1 1] extra ADSR
  (`TimelineComponent.SetPlayRate` (`self.Timeline_1`) 0.25)
  (bind (_direction _volume1_0) (`Timeline|Timeline_1` :!via `PlayFromStart`)
    (:`Update`
      (set `self.GranularVolumeMP` _volume1_0))))

(event `GMaj`
  ;[1 1 1] chords
  (`self.ChordSwitch` (`self.ArrChordGmaj`)))

(event `CMaj`
  ;[1 1 1] chords
  (`self.ChordSwitch` (`self.ArrChordCmaj`)))

(event `DMin`
  ;[1 1 1] chords
  (`self.ChordSwitch` (`self.ArrChordDmin`)))

(event `self.ReceiveTick`
  (params (DeltaSeconds :type "Float (single-precision)"))
  (bind _mid (`self.MID`))
  (bind _soundplayer (`self.SoundPlayer`))
  (bind (_inrangea _inrangeb _outrangea _outrangeb) (break `/Game/ArthursAudioBPs/SharedAssets/VariousHelpers/FMapRange` (`self.MapRangeNormalizedVolume`)))
  ;[1 1 1] tick
  (set `self.LatestTickDellta` DeltaSeconds)
  (`|ExecutionSequence`
    (:`then_0`
      ;[1 1 1] drum beat normalized volume
      (`/Engine/EditorBlueprintResources/StandardMacros.IsValid` _soundplayer
        (:`Is Valid`
          (bind _output_get (set `self.LatstDrumEnv` (`/Game/ArthursAudioBPs/SharedAssets/Blueprints/AudioPlayers/BP_SoundPlayerGranular.LatestEnvelope` _soundplayer)))
          (if (> _output_get (`self.MaxDrumEnv`))
            (set `self.MaxDrumEnv` (`self.LatstDrumEnv`)))
          (set `self.EnvNormalized` (`KismetMathLibrary.MapRangeClamped` (`self.LatstDrumEnv`) 0.0 (`self.MaxDrumEnv`) 0.0 1.0))
          ;[1 1 1] mod MID
          (`MaterialInstanceDynamic.SetScalarParameterValue` _mid "Emissive Multiplier" (* (`self.EnvNormalized`) (`self.EmissiveMultiplier`)))
          (`MaterialInstanceDynamic.SetVectorParameterValue` _mid "Base Color" (`KismetMathLibrary.LinearColorLerp` (struct :`R` 0.692062 :`B` 1.0 :`A` 1.0) (struct :`G` 1.0 :`B` 0.536032 :`A` 1.0) (`self.EnvNormalized`))))))
    (:`then_1`
      ;[1 1 1] set granular volume
      (for _array_element (`self.SpwndGranulars`)
        (`SynthComponent.SetVolumeMultiplier` (`/Game/ArthursAudioBPs/SharedAssets/Blueprints/GranularSynth/GranularMusic/BP_granular.DerGranular` _array_element) (* (`KismetMathLibrary.MapRangeClamped` (`self.EnvNormalized`) _inrangea _inrangeb _outrangea _outrangeb) (`self.GranularVolumeMP`)))))))

(event `DMaj`
  ;[1 1 1] chords
  (`self.ChordSwitch` (`self.ArrChordDmaj`)))

(event `DecreaseHistoricMaxEnv`
  ;[1 1 1] drum beat normalized volume
  ;;[1 1 1] decrease max recorded env
  (bind _output_get (set `self.MaxDrumEnv` (* (stale _output_get) 0.9))))

(event `EMaj`
  ;[1 1 1] chords
  (`self.ChordSwitch` (`self.ArrChordEmaj`)))

(event `EMin`
  ;[1 1 1] chords
  (`self.ChordSwitch` (`self.ArrChordEmin`)))

(fn `ChordSwitch`
  (params (Chord :type "Array of Integer"))
  (for _array_element (`self.SpwndGranulars`)
    (set `/Game/ArthursAudioBPs/SharedAssets/Blueprints/GranularSynth/GranularMusic/BP_granular.Note` (`|GetArrayItem` Chord (`KismetMathLibrary.RandomIntegerInRange` 0 2)) _array_element))
  (`self.AllRandOctave`))

(fn `SpawnGranular`
  (params (OffsetX :type "Float (double-precision)") (OffsetY :type "Float (double-precision)") (OffsetZ :type "Float (double-precision)"))
  (bind _returnvalue (`|SpawnActorFromClass` "/Game/ArthursAudioBPs/SharedAssets/Blueprints/GranularSynth/GranularMusic/BP_granular.BP_granular_C" (`self.OffsetWorldTransform` (`SceneComponent.K2_GetComponentToWorld` (`self.DefaultSceneRoot`)) OffsetX OffsetY OffsetZ) "Undefined" "OverrideRootScale" null (`self.GranularBasePreset`) (`self.SamplePool`) null))
  (`KismetArrayLibrary.Array_Add` (`self.SpwndGranulars`) _returnvalue))

(fn `SpawnGranularArray`
  (locals (_offsetXLocal :type "Float (double-precision)" :default 0.0) (_offsetYLocal :type "Float (double-precision)" :default 0.0) (_offsetZLocal :type "Float (double-precision)" :default 0.0) (_spawnPositionsLocal :type "Array of Vector Structure"))
  ;[1 1 1] spawn granulars
  ;;[1 1 1] make grid
  (for _index (range (+ (`KismetMathLibrary.Clamp` (- (`self.RowsX`) 1) 0 1000) 1))
    (set `local._offsetXLocal` (* _index (`self.OffsetX`)))
    (for _index_2 (range (+ (`KismetMathLibrary.Clamp` (- (`self.RowsY`) 1) 0 1000) 1))
      (set `local._offsetYLocal` (* _index_2 (`self.OffsetY`)))
      (for _index_3 (range (+ (`KismetMathLibrary.Clamp` (- (`self.RowsZ`) 1) 0 1000) 1))
        (set `local._offsetZLocal` (* _index_3 (`self.OffsetZ`)))
        (`KismetArrayLibrary.Array_Add` (`local._spawnPositionsLocal`) (`KismetMathLibrary.MakeVector` (`local._offsetXLocal`) (`local._offsetYLocal`) (`local._offsetZLocal`)))
        ;;[1 1 1] spawn
        (`self.SpawnGranular` (`local._offsetXLocal`) (`local._offsetYLocal`) (`local._offsetZLocal`)))))
  (set `self.SpawnPositions` (`local._spawnPositionsLocal`))
  (return))

(fn `UserConstructionScript`)