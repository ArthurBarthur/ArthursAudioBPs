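; BP_granular is a musical granular synth actor whose pitch comes from grain rate, with start/stop, note and octave stepping events.
; Tick eases grains-per-second toward the selected octave and note frequency and pushes the preset to the GranularSynth component.
; The synth's audio envelope drives the mesh's horizontal scale and a dynamic material's colour and emissive glow.
; Source sample and playhead position can be randomized, both at BeginPlay and through events.
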(event `LLatestEnv`
  (params (EnvelopeValue :type "Float (double-precision)"))
  ;[1 1 1] init granular
  ;;[1 1 1] bind env event
  (set `self.LatestEnv` EnvelopeValue))

(event `self.ReceiveBeginPlay`
  (`|ExecutionSequence`
    (:`then_0`
      ;[1 1 1] init granular
      ;;[1 1 1] add gran
      (set `self.DerGranular` (`self.GranularSynth`))
      ;;[1 1 1] bind env event
      (add `SynthComponent.OnAudioEnvelopeValue` (`self.DerGranular`) (delegate `LLatestEnv`))
      ;;[1 1 1] propagation settings
      (set `SynthComponent.bAllowSpatialization` true (`self.DerGranular`))
      (set `SynthComponent.AttenuationSettings` "/Game/ArthursAudioBPs/SharedAssets/Audio/Attenuation/ATT_Gran.ATT_Gran" (`self.DerGranular`))
      ;;[1 1 1] update preset
      (`/Game/ArthursAudioBPs/SharedAssets/FunctionLibraries/GranularSynthFunctionLibrary.UpdateGranular` (`self.DerGranular`) (`self.GranularPreset`))
      ;;[1 1 1] change active sound
      (`self.ChangeRandomActiveSound`)
      ;;[1 1 1] random playhead time
      (`self.RandomPlayheadTime`)
      ;;[1 1 1] start
      (`KismetSystemLibrary.Delay` 0.5)
      (`self.startGran` (`self.DerGranular`)))
    (:`then_1`
      ;[1 1 1] create granular box MID
      (bind _returnvalue (`KismetMaterialLibrary.CreateDynamicMaterialInstance` "/Game/ArthursAudioBPs/SharedAssets/Visuals/Materials/MI_SimpleMat_Inst1.MI_SimpleMat_Inst1"))
      (bind _output_get (set `self.MID` _returnvalue))
      (`PrimitiveComponent.SetMaterial` (`self.StaticMesh`) 0 _output_get))))

(event `Note+`
  (bind _note (`self.Note`))
  ;[1 1 1] notes/octaves +- input
  (`/Engine/EditorBlueprintResources/StandardMacros.CompareInt` _note 11
    (:`<`
      (`/Engine/EditorBlueprintResources/StandardMacros.IncrementInt` _note))))

(event `self.ReceiveTick`
  (params (DeltaSeconds :type "Float (single-precision)"))
  (bind _latestenv (`self.LatestEnv`))
  (bind _mid (`self.MID`))
  (bind _output (`|GetArrayItem` (`self.OctaveArray`) (`self.Octave`)))
  (bind _returnvalue (`KismetMathLibrary.FClamp` (* _latestenv 50.0)))
  (bind _returnvalue_2 (`KismetMathLibrary.MapRangeUnclamped` (* _latestenv 50.0) 0.1 1.0 4.0 6.0))
  ;[1 1 1] tick
  (`|ExecutionSequence`
    (:`then_0`
      ;[1 1 1] interp to target note
      (bind _output_get (set `self.CurrentGPS` (`KismetMathLibrary.FInterpTo` (`self.CurrentGPS`) (* _output (`|GetArrayItem` (`self.NoteFloatArray`) (`self.Note`))) DeltaSeconds (+ (`KismetMathLibrary.Conv_IntToDouble` _output) 4.0))))
      ;[1 1 1] gran tick update
      (bind _structout (setmembers `/Game/ArthursAudioBPs/SharedAssets/Blueprints/GranularSynth/FGranularPreset` :`StructRef` (`self.GranularPreset`) :`GrainsPerSecond` _output_get))
      (`/Game/ArthursAudioBPs/SharedAssets/FunctionLibraries/GranularSynthFunctionLibrary.UpdateGranular` (`self.DerGranular`) _structout))
    (:`then_1`
      ;[1 1 1] env scale mesh
      (`SceneComponent.SetRelativeScale3D` (`self.StaticMesh`) (`KismetMathLibrary.MakeVector` _returnvalue_2 _returnvalue_2 4.0)))
    (:`then_2`
      ;[1 1 1] mod MID
      (`MaterialInstanceDynamic.SetScalarParameterValue` _mid "Emissive Multiplier" (* _returnvalue 200.0))
      (`MaterialInstanceDynamic.SetVectorParameterValue` _mid "Base Color" (`KismetMathLibrary.LinearColorLerp` (struct :`A` 1.0) (struct :`R` 1.0 :`G` 0.58409 :`A` 1.0) _returnvalue)))))

(event `Note-`
  (bind _note (`self.Note`))
  ;[1 1 1] notes/octaves +- input
  (`/Engine/EditorBlueprintResources/StandardMacros.CompareInt` _note
    (:`>`
      (`/Engine/EditorBlueprintResources/StandardMacros.DecrementInt` _note))))

(event `Octave+`
  (bind _octave (`self.Octave`))
  ;[1 1 1] notes/octaves +- input
  (`/Engine/EditorBlueprintResources/StandardMacros.CompareInt` _octave 8
    (:`<`
      (`/Engine/EditorBlueprintResources/StandardMacros.IncrementInt` _octave))))

(event `Octave-`
  (bind _octave (`self.Octave`))
  ;[1 1 1] notes/octaves +- input
  (`/Engine/EditorBlueprintResources/StandardMacros.CompareInt` _octave
    (:`>`
      (`/Engine/EditorBlueprintResources/StandardMacros.DecrementInt` _octave))))

(event `Start`
  ;[1 1 1] start
  (`GranularSynth.NoteOn` (`self.DerGranular`) 60.0 100 -1.0))

(event `Stop`
  ;[1 1 1] stop
  (`GranularSynth.NoteOff` (`self.DerGranular`) 60.0 false))

(event `RandomizeSourceSample`
  ;[1 1 1] RandomizeSound4Gran
  (`self.ChangeRandomActiveSound`))

(event `SetRandomPlayheadTime`
  ;[1 1 1] Random Playhead Time
  (`self.RandomPlayheadTime`))

(fn `ChangeRandomActiveSound`
  ;[1 1 1] SetActiveSound
  (bind _output_get (set `self.ActiveSound` (`self.GetRandSound`)))
  ;[1 1 1] set sound on gran + delays
  (`GranularSynth.SetSoundWave` (`self.DerGranular`) _output_get))

(fn `RandomPlayheadTime`
  (locals (_PlayheadPositionInSecWeWant :type "Float (double-precision)" :default 0.0))
  (set `local._PlayheadPositionInSecWeWant` (`KismetMathLibrary.RandomFloatInRange` 0.0 (`GranularSynth.GetSampleDuration` (`self.GranularSynth`))))
  (setmembers `/Game/ArthursAudioBPs/SharedAssets/Blueprints/GranularSynth/FGranularPreset` :`StructRef` (`self.GranularPreset`) :`PlayheadPosSec` (`local._PlayheadPositionInSecWeWant`)))

(fn `startGran`
  (params (Gransynth :type "GranularSynth Object Reference"))
  (`ActorComponent.Activate` Gransynth false)
  (`SynthComponent.Start` Gransynth))

(fn `UserConstructionScript`)