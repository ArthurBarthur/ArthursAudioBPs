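; Granular sound player actor that plays a Sound through a GranularSynth component, advancing the playhead with elapsed game time.
; BeginPlay applies the base preset and wave, then after a short delay starts the synth and opens a gate.
; While open, Tick sets playhead, pitch, grain duration and density from multipliers, restarting or closing at the sound's end per Loop.
; Construction applies attenuation and bus routing; envelope values are cached.
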(event `self.ReceiveBeginPlay`
  ;[1 1 1] beginPlay
  ;[1 1 1] boot up granular
  (`|ExecutionSequence`
    (:`then_0`
      (`/Game/ArthursAudioBPs/SharedAssets/FunctionLibraries/GranularSynthFunctionLibrary.UpdateGranular` (`self.GranularSynth`) (`self.GranularPresetBase`)))
    (:`then_1`
      (`GranularSynth.SetSoundWave` (`self.GranularSynth`) (`self.Sound`)))
    (:`then_2`
      (`KismetSystemLibrary.Delay` 0.2)
      (`/Game/ArthursAudioBPs/SharedAssets/FunctionLibraries/GranularSynthFunctionLibrary.StartGranular` (`self.GranularSynth`))
      ;[1 1 1] Open gate
      (`self.OpenGate`))))

(event `self.ReceiveTick`
  (params (DeltaSeconds :type "Float (single-precision)"))
  ;[1 1 1] tick
  (set `self.LatestDeltaTick` DeltaSeconds)
  ;[1 1 1] gate
  (`/Engine/EditorBlueprintResources/StandardMacros.Gate` true :!label _label
    (:`Exit`
      ;[1 1 1] store latest elapsed time
      (set `self.LatestElapsedTime` (- (`KismetSystemLibrary.GetGameTimeInSeconds`) (`self.StartTime`)))
      ;[1 1 1] gone through sample?
      (if (>= (`self.LatestElapsedTime`) (`SoundBase.Duration` (`self.Sound`)))
        ;[1 1 1] Finished
        ;;[1 1 1] loop?
        (if (`self.Loop`)
          ;;[1 1 1] Open Gate
          (`self.OpenGate`)
          (else
            ;;[1 1 1] close gate
            (`self.CloseGate`)))
        (else
          ;[1 1 1] Still playing
          ;;[1 1 1] update pitch
          (`GranularSynth.SetGrainPitch` (`self.GranularSynth`) (`self.PitchMP`) (0.0 0.0))
          ;;[1 1 1] update playhead time
          (`GranularSynth.SetPlayheadTime` (`self.GranularSynth`) (`self.LatestElapsedTime`) 0.0 "FromBeginning")
          ;;[1 1 1] grain duration
          (`GranularSynth.SetGrainDuration` (`self.GranularSynth`) (* (* (`.DurationBaseMsec_55_629930E44F1507F01122F697D24D492F` (break `/Game/ArthursAudioBPs/SharedAssets/Blueprints/GranularSynth/FGranularPreset` (`self.GranularPresetBase`))) (`self.GrainDurationMP_0`)) (`self.GrainDurationMP_1`)) (0.0 0.0))
          ;;[1 1 1] grainsPerSecond
          (`GranularSynth.SetGrainsPerSecond` (`self.GranularSynth`) (* (`.GrainsPerSecond_28_FB913A6443DB4978747958AE9B07E7B1` (break `/Game/ArthursAudioBPs/SharedAssets/Blueprints/GranularSynth/FGranularPreset` (`self.GranularPresetBase`))) (`self.GrainsPerSecond`))))))))

(event `self.GranularSynth.OnAudioEnvelopeValue`
  (params (EnvelopeValue :type "Float (single-precision)"))
  ;[1 1 1] Envelope
  (set `self.LatestEnvelope` EnvelopeValue))

(event `OpenGate`
  ;[1 1 1] gate
  ;;[1 1 1] store current time
  (set `self.StartTime` (`KismetSystemLibrary.GetGameTimeInSeconds`))
  (goto _label :!via `Open`))

(event `CloseGate`
  ;[1 1 1] gate
  (goto _label :!via `Close`))

(fn `UserConstructionScript`
  (set `SynthComponent.AttenuationSettings` (`self.Attenuation`) (`self.GranularSynth`))
  (set `SynthComponent.bOutputToBusOnly` (`self.OutputToBusOnly`) (`self.GranularSynth`))
  (set `SynthComponent.BusSends` (`self.SourceBusSends`) (`self.GranularSynth`)))