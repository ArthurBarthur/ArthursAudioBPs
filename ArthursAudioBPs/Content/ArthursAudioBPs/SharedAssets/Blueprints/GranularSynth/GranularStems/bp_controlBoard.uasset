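; Control board actor that drives a referenced granular synth and the game's global time dilation.
; On BeginPlay it enables tick only if the GranularSynthTime reference is valid, otherwise printing a warning.
; Each tick it applies clamped time dilation and pitch multipliers, then maps them through float curves to set the synth's two grain duration multipliers and grains-per-second.
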(event `self.ReceiveBeginPlay`
  ;[1 1 1] beginPlay
  ;[1 1 1] enable tick if safe
  (`/Engine/EditorBlueprintResources/StandardMacros.IsValid` (`self.GranularSynthTime`)
    (:`Is Valid`
      (`self.SetActorTickEnabled` true))
    (:`Is Not Valid`
      (`KismetSystemLibrary.PrintString` "BP_ControlBoard has Invalid GranularSynthTime-Reference"))))

(event `self.ReceiveTick`
  (params (DeltaSeconds :type "Float (single-precision)"))
  ;[1 1 1] tick
  ;[1 1 1] set global time dilation
  (`GameplayStatics.SetGlobalTimeDilation` (`KismetMathLibrary.FClamp` (`self.TimeDilationMP`) 0.1 9999999.0))
  ;[1 1 1] Pitch MP
  (set `/Game/ArthursAudioBPs/SharedAssets/Blueprints/GranularSynth/GranularStems/BP_SoundPlayerGranular_Time.PitchMP` (`KismetMathLibrary.FClamp` (`self.PitchMP`) 0.0 666.0) (`self.GranularSynthTime`))
  ;[1 1 1] pitch to grain duration MP_0
  (set `/Game/ArthursAudioBPs/SharedAssets/Blueprints/GranularSynth/GranularStems/BP_SoundPlayerGranular_Time.GrainDurationMP_0` (`CurveFloat.GetFloatValue` (`self.Curve_PitchMPToGrainDurationMP`) (`self.PitchMP`)) (`self.GranularSynthTime`))
  ;[1 1 1] timeDilation to grain duration MP_1
  (set `/Game/ArthursAudioBPs/SharedAssets/Blueprints/GranularSynth/GranularStems/BP_SoundPlayerGranular_Time.GrainDurationMP_1` (`CurveFloat.GetFloatValue` (`self.Curve_TimeDilationMpToGrainDurationMp`) (`self.TimeDilationMP`)) (`self.GranularSynthTime`))
  ;[1 1 1] timeDilation to grainsPerSecond
  (set `/Game/ArthursAudioBPs/SharedAssets/Blueprints/GranularSynth/GranularStems/BP_SoundPlayerGranular_Time.GrainsPerSecond` (`CurveFloat.GetFloatValue` (`self.Curve_GlobalTimeDilationMPToGrainsPerSecondMP`) (`self.TimeDilationMP`)) (`self.GranularSynthTime`)))

(fn `UserConstructionScript`)