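; Actor that tracks which Synesthesia onset a looping sound has reached and shows that count on its text renders.
; The construction script caches channel 0 timestamps and strengths from an OnsetNRT asset.
; Tick converts the audio component's reported playback percent to seconds, advances the onset index, and displays it alongside slower divided counts.
; Near the loop start, a briefly self-closing gate resets the index.
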(event `self.ReceiveBeginPlay`
  ;[1 1 1] beginplay
  (`KismetSystemLibrary.Delay` 0.5)
  (`|ExecutionSequence`
    (:`then_0`
      ;[1 1 1] set up custom event GetLatestPercentagePlayedFromAudioComp
      (add `AudioComponent.OnAudioPlaybackPercent` (`self.GetComponentByClass` (`self.ActorWithAudioComp`) "/Script/Engine.AudioComponent") (`|CreateDelegate` :!event `OnAudioPlaybackPercent_Event_0`)))
    (:`then_2`
      ;[1 1 1] enable tick
      (`self.SetActorTickEnabled` true))))

(event `ResetGateOpen`
  ;[1 1 1] gate
  (goto _label :!via `Open`))

(event `ResetGateClose`
  ;[1 1 1] gate
  (goto _label :!via `Close`))

(event `self.ReceiveTick`
  (params (DeltaSeconds :type "Float (single-precision)"))
  (bind _startindex (`self.StartIndex`))
  (bind _tickdelta (`self.tickDelta`))
  ;[1 1 1] tick
  (set `self.tickDelta` DeltaSeconds)
  ;[1 1 1] get current playback time
  (bind _output_get (set `self.CurrentPlaybackTime` (* (`SoundBase.Duration` (`AudioAnalyzerNRT.Sound` (`self.OnsetNRT`))) (mod (stale `OnAudioPlaybackPercent_Event_0` PlaybackPercent) 1.0))))
  ;[1 1 1] close to 0?
  (if (`KismetMathLibrary.NearlyEqual_FloatFloat` _output_get 0.0 (+ _tickdelta _tickdelta _tickdelta _tickdelta))
    ;[1 1 1] gate
    (`/Engine/EditorBlueprintResources/StandardMacros.Gate` false :!label _label
      (:`Exit`
        ;[1 1 1] reset around 0
        (set `self.OnsetTimestampsCopy` (`self.onsetTimestamps`))
        (set `self.TempStartIndex` 0)
        (set `self.StartIndex` 0)
        ;[1 1 1] shut gate for a short time
        (`self.ResetGateClose`)
        (`KismetSystemLibrary.Delay` 0.05)
        (`self.ResetGateOpen`)))
    (else
      ;[1 1 1] Find out which Onset timestamp index we are at, depending on current sample playback time.
      ;;[1 1 1] go through remaining timestamps
      (for _index (range (`self.StartIndex`) (+ (`KismetArrayLibrary.Array_LastIndex` (`self.OnsetTimestampsCopy`)) 1))
        ;;[1 1 1] Past current playback time?
        (if (< (`|GetArrayItem` (`self.OnsetTimestampsCopy`) _index) (`self.CurrentPlaybackTime`))
          ;;[1 1 1] Store most current index
          (set `self.TempStartIndex` _index)))
      ;[1 1 1] start on next index when looping again
      (set `self.StartIndex` (+ (`self.TempStartIndex`) 1))
      ;[1 1 1] display info stuff
      ;;[1 1 1] update texts
      (for _array_element (`self.TextDisplays`)
        (`TextRenderComponent.K2_SetText` _array_element (`KismetTextLibrary.Conv_StringToText` (`KismetStringLibrary.Concat_StrStr` (`KismetStringLibrary.Conv_IntToString` _startindex) " \n" (`KismetStringLibrary.Conv_IntToString` (+ (/ _startindex 2) 1)) " \n" (`KismetStringLibrary.Conv_IntToString` (+ (/ _startindex 4) 1)) " \n" (`KismetStringLibrary.Conv_IntToString` (+ (/ _startindex 8) 1)))))))))

(event `OnAudioPlaybackPercent_Event_0`
  (params (PlayingSoundWave :type "SoundWave Object Reference") (PlaybackPercent :type "Float (double-precision)"))
  ;[1 1 1] get current playback time
  ;;[1 1 1] 0-1
)

(fn `UserConstructionScript`
  (bind _onsetnrt (`self.OnsetNRT`))
  (bind (_outonsettimestamps _outonsetstrengths) (`OnsetNRT.GetNormalizedChannelOnsetsBetweenTimes` _onsetnrt 0.0 (`AudioAnalyzerNRT.DurationInSeconds` _onsetnrt) 0))
  ;[1 1 1] OnsetNRT get times and strengths
  (set `self.OnsetStrengths` _outonsetstrengths)
  (bind _output_get (set `self.onsetTimestamps` _outonsettimestamps))
  (set `self.OnsetTimestampsCopy` _output_get)
  ;[1 1 1] gather all text renders into array
  (set `self.TextDisplays` (`self.K2_GetComponentsByClass` self "/Script/Engine.TextRenderComponent")))