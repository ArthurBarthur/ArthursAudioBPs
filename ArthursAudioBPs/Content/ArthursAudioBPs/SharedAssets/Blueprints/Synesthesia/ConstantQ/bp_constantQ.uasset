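; Audio visualizer actor that draws a row of meshes scaled to the frequency bands of a pre-analyzed Synesthesia Constant-Q (NRT) asset.
; The construction script spawns one evenly spaced mesh per band.
; After a short delay it binds to another actor's audio playback percent, which Tick wraps and converts to time for sampling channel 0's normalized values.
; ResizeMeshes scales each mesh's Z by its band value, multiplier and minimum offset.
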(event `self.ReceiveBeginPlay`
  (`KismetSystemLibrary.Delay` 0.5)
  ;[1 1 1] get playback percent of audio component
  (add `AudioComponent.OnAudioPlaybackPercent` (`self.GetComponentByClass` (`self.ActorWithAudioComp`) "/Script/Engine.AudioComponent") (`|CreateDelegate` :!event `OnAudioPlaybackPercent_Event_0`))
  ;[1 1 1] enable tick
  (`self.SetActorTickEnabled` true))

(event `self.ReceiveTick`
  (params (DeltaSeconds :type "Float (single-precision)"))
  ;[1 1 1] Get Qs at time of frame
  (`/Engine/EditorBlueprintResources/StandardMacros.IsValid` (stale `OnAudioPlaybackPercent_Event_0` PlayingSoundWave)
    (:`Is Valid`
      (bind _output_get (set `self.OutConstantQs` (`ConstantQNRT.GetNormalizedChannelConstantQAtTime` (`self.ConstantQNRT`) (* (`SoundBase.Duration` (stale `OnAudioPlaybackPercent_Event_0` PlayingSoundWave)) (mod (stale `OnAudioPlaybackPercent_Event_0` PlaybackPercent) 1.0)) 0)))
      ;[1 1 1] resize all the meshes
      (`self.ResizeMeshes` _output_get))))

(event `OnAudioPlaybackPercent_Event_0`
  (params (PlayingSoundWave :type "SoundWave Object Reference") (PlaybackPercent :type "Float (double-precision)"))
  ;[1 1 1] Get Qs at time of frame
)

(fn `ResizeMeshes`
  (params (Array :type "Array of Float (double-precision)"))
  (locals (_currentIndex :type Integer) (_currentQ :type "Float (double-precision)"))
  ;[1 1 1] loop through
  (for (_array_element _array_index) Array
    (set `local._currentQ` _array_element)
    (set `local._currentIndex` _array_index)
    ;[1 1 1] resize
    (`SceneComponent.K2_SetRelativeTransform` (`|GetArrayItem` (`self.Meshes`) (`local._currentIndex`)) (`KismetMathLibrary.MakeTransform` (.location (`|GetArrayItem` (`self.MeshStartTransforms`) (`local._currentIndex`))) (.rotation (`|GetArrayItem` (`self.MeshStartTransforms`) (`local._currentIndex`))) (`KismetMathLibrary.MakeVector` (.x (.scale (`|GetArrayItem` (`self.MeshStartTransforms`) (`local._currentIndex`)))) (.y (.scale (`|GetArrayItem` (`self.MeshStartTransforms`) (`local._currentIndex`)))) (+ (* (.z (.scale (`|GetArrayItem` (`self.MeshStartTransforms`) (`local._currentIndex`)))) (* (`local._currentQ`) (`self.QMultiplier`))) (`self.MinimumScaleZ`)))) false false)))

(fn `UserConstructionScript`
  ;[1 1 1] make mesh transform for each band
  (for _index (range (`ConstantQNRTSettings.NumBands` (`ConstantQNRT.Settings` (`self.ConstantQNRT`))))
    (`KismetArrayLibrary.Array_Add` (`self.MeshStartTransforms`) (`KismetMathLibrary.MakeTransform` (* (`self.MeshSpacing`) (`KismetMathLibrary.Conv_IntToDouble` _index)) (struct) (`self.MeshStartingScale`))))
  ;[1 1 1] spawn mesh for each band
  (for _array_element (`self.MeshStartTransforms`)
    (bind _returnvalue (`AddComponent|NODE_AddStaticMeshComponent-0` :`RelativeTransform` _array_element))
    (`KismetArrayLibrary.Array_Add` (`self.Meshes`) _returnvalue))
  ;[1 1 1] set static mesh to use
  (for _array_element_2 (`self.Meshes`)
    (`StaticMeshComponent.SetStaticMesh` _array_element_2 (`self.MeshType`))))