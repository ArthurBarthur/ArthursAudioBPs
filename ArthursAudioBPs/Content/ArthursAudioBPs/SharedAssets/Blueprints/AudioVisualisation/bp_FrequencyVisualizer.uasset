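; Audio frequency visualizer actor that shows submix analysis as a row of meshes that stretch and glow with each band.
; The construction script spawns one mesh per frequency from the SubmixAnalyzer, assigns dynamic materials with optional random colors, and randomizes scale and emissive as an editor preview.
; After a short delay, BeginPlay validates the analyzer and beautifier references and enables Tick, which drives Z scale and emissive strength from the beautifier's smoothed values.
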(event `self.ReceiveBeginPlay`
  ;[1 1 1] beginplay
  (`KismetSystemLibrary.Delay` 0.5)
  (`/Engine/EditorBlueprintResources/StandardMacros.IsValid` (`self.SubmixAnalyzerRef`)
    (:`Is Valid`
      (`/Engine/EditorBlueprintResources/StandardMacros.IsValid` (`self.SubmixBeautifierRef`)
        (:`Is Valid`
          (`|ExecutionSequence`
            (:`then_4`
              ;[1 1 1] Enable Tick
              (`self.SetActorTickEnabled` true))))))))

(event `self.ReceiveTick`
  (params (DeltaSeconds :type "Float (single-precision)"))
  ;[1 1 1] Tick
  (set `self.DeltaTick` DeltaSeconds)
  (`|ExecutionSequence`
    (:`then_0`
      ;[1 1 1] get latest beautified analysis
      (set `self.LatestSmoothValues` (`/Game/ArthursAudioBPs/SharedAssets/Blueprints/AudioVisualisation/BP_AnalysisBeautifier.FinalOutputValuesFromAnalysis` (`self.SubmixBeautifierRef`))))
    (:`then_1`
      ;[1 1 1] Update mesh scales
      (`self.ScaleMeshes`))
    (:`then_2`
      ;[1 1 1] Update dynamic material emissive strength
      (`self.UpdateMaterialEmissive`))))

(fn `ConstructionPreVizMeshes`
  (locals (_currentIndex :type Integer) (_currentMesh :type "StaticMeshComponent Object Reference") (CurrentValue :type "Float (double-precision)" :default 0.0))
  ;[1 1 1] loop through meshes
  (for (_array_element _array_index) (`self.VizMeshes`)
    (set `local._currentMesh` _array_element)
    (set `local._currentIndex` _array_index)
    (bind _output_get (set `local.CurrentValue` (+ (* (`KismetMathLibrary.SelectFloat` (`KismetMathLibrary.RandomFloatInRange` 0.0 0.5) (`KismetMathLibrary.RandomFloatInRange` 0.5 1.0) (`KismetMathLibrary.RandomBoolWithWeight` 0.7)) (`self.MeshScaleMultiplier`)) (`self.MinimumSize`))))
    ;[1 1 1] set new mesh scale
    (`SceneComponent.SetRelativeScale3D` (`local._currentMesh`) (`KismetMathLibrary.MakeVector` 1.0 1.0 _output_get))
    ;[1 1 1] modify MID emissive multiplier value
    (`MaterialInstanceDynamic.SetScalarParameterValue` (`|GetArrayItem` (`self.MIDs`) (`local._currentIndex`)) "Emissive Multiplier" (* (`local.CurrentValue`) (`self.MaterialEmissiveMultiplier`)))))

(fn `InitializeDynamicMaterials`
  (locals (_currentIndex :type Integer) (_currentMesh :type "StaticMeshComponent Object Reference") (_latestRandomColor :type "LinearColor Structure"))
  (`KismetArrayLibrary.Array_Clear` (`self.MIDs`))
  ;[1 1 1] loop through meshes
  (for (_array_element _array_index) (`self.VizMeshes`)
    (`|ExecutionSequence`
      (:`then_0`
        ;[1 1 1] store local variables
        (set `local._currentMesh` _array_element)
        (set `local._currentIndex` _array_index))
      (:`then_1`
        ;[1 1 1] create dynamic materials(MIDs)
        (bind _returnvalue (`KismetMaterialLibrary.CreateDynamicMaterialInstance` (`self.BaseMaterial`)))
        (`KismetArrayLibrary.Array_Set` (`self.MIDs`) (`local._currentIndex`) _returnvalue true))
      (:`then_2`
        ;[1 1 1] put MIDs on meshes
        (`PrimitiveComponent.SetMaterial` (`local._currentMesh`) 0 (`|GetArrayItem` (`self.MIDs`) (`local._currentIndex`))))
      (:`then_3`
        ;[1 1 1] random color?
        (if (`self.RandomColors?`)
          ;[1 1 1] make color
          (bind _linearcolor (`self.MakeRandomColor`))
          (set `local._latestRandomColor` _linearcolor)
          ;[1 1 1] set colors on materials
          (`MaterialInstanceDynamic.SetVectorParameterValue` (`|GetArrayItem` (`self.MIDs`) (`local._currentIndex`)) "Base Color" (`local._latestRandomColor`)))))))

(fn `MakeRandomColor`
  (returns (LinearColor :type "LinearColor Structure"))
  (bind (_bvalue_x _bvalue_y) (`KismetMathLibrary.BreakVector2D` (`self.bValue`)))
  (bind (_rvalue_x _rvalue_y) (`KismetMathLibrary.BreakVector2D` (`self.rValue`)))
  (bind (_gvalue_x _gvalue_y) (`KismetMathLibrary.BreakVector2D` (`self.gValue`)))
  (return (make `LinearColor` (`KismetMathLibrary.RandomFloatInRange` _rvalue_x _rvalue_y) (`KismetMathLibrary.RandomFloatInRange` _gvalue_x _gvalue_y) (`KismetMathLibrary.RandomFloatInRange` _bvalue_x _bvalue_y))))

(fn `ScaleMeshes`
  (locals (_currentIndex :type Integer) (_currentMesh :type "StaticMeshComponent Object Reference"))
  ;[1 1 1] loop through meshes
  (for (_array_element _array_index) (`self.VizMeshes`)
    (set `local._currentMesh` _array_element)
    (set `local._currentIndex` _array_index)
    ;[1 1 1] set new mesh scale
    (`SceneComponent.SetRelativeScale3D` (`local._currentMesh`) (`KismetMathLibrary.MakeVector` 1.0 1.0 (+ (* (`|GetArrayItem` (`self.LatestSmoothValues`) (`local._currentIndex`)) (`self.MeshScaleMultiplier`)) (`self.MinimumSize`))))))

(fn `SpawnVisualizerMeshes`
  (locals (_currentIndex :type Integer))
  (bind _vizmeshes (`self.VizMeshes`))
  ;[1 1 1] clear out old existing meshes if any
  (for _array_element _vizmeshes
    (`ActorComponent.K2_DestroyComponent` _array_element))
  (`KismetArrayLibrary.Array_Clear` _vizmeshes)
  ;[1 1 1] loop through frequencies
  (for (_ _array_index) (`self.FrequenciesToAnalyze`)
    ;[1 1 1] spawn visualizer meshes in a row
    (set `local._currentIndex` _array_index)
    (bind _returnvalue (`AddComponent|NODE_AddStaticMeshComponent-0` :`RelativeTransform` (`KismetMathLibrary.MakeTransform` (`KismetMathLibrary.MakeVector` 0.0 (* (`local._currentIndex`) (`self.MeshRowDistanceOffset`))))))
    ;[1 1 1] store mesh references
    (`KismetArrayLibrary.Array_Set` (`self.VizMeshes`) (`local._currentIndex`) _returnvalue true))
  ;[1 1 1] attach to rootmesh
  (for _array_element_2 (`self.VizMeshes`)
    (`SceneComponent.K2_AttachToComponent` _array_element_2 (`self.StaticNoMesh`) "None" "KeepRelative" "KeepRelative" "KeepRelative" true)))

(fn `UpdateMaterialEmissive`
  ;[1 1 1] modify MID emissive multiplier value
  (for (_array_element _array_index) (`self.MIDs`)
    (`MaterialInstanceDynamic.SetScalarParameterValue` _array_element "Emissive Multiplier" (* (`|GetArrayItem` (`self.LatestSmoothValues`) _array_index) (`self.MaterialEmissiveMultiplier`)))))

(fn `UserConstructionScript`
  (`|ExecutionSequence`
    (:`then_0`
      ;[1 1 1] get frequencies to analyze from SubmixAnalyzer
      (set `self.FrequenciesToAnalyze` (`/Game/ArthursAudioBPs/SharedAssets/Blueprints/AudioVisualisation/BP_SubmixAnalyzer.FrequenciesToAnalyze` (`self.SubmixAnalyzerRef`)))
      ;[1 1 1] spawn visualizing meshes
      (`self.SpawnVisualizerMeshes`)
      ;[1 1 1] initialize dynamic materials(MIDs)
      (`self.InitializeDynamicMaterials`)
      ;[1 1 1] pre-viz scaling of meshes
      (`self.ConstructionPreVizMeshes`))))