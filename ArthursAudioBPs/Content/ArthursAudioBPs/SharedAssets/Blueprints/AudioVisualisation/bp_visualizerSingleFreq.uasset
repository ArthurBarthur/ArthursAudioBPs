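; Audio visualizer actor that makes a cube and optional point light react to a single frequency band.
; Each tick it reads one envelope value from the referenced analysis beautifier's output array, selected by slot index.
; That envelope drives light intensity and color, the dynamic material's emissive and base color, and cube scale.
; The construction script can randomize the color pair, with black as the low end, and removes the light when disabled.
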(event `self.ReceiveBeginPlay`
  ;[1 1 1] set up MID(material instance dynamic)
  (bind _returnvalue (`KismetMaterialLibrary.CreateDynamicMaterialInstance` "/Game/ArthursAudioBPs/SharedAssets/Visuals/Materials/MAT_SimpleMat.MAT_SimpleMat"))
  (set `self.MID` _returnvalue)
  (`PrimitiveComponent.SetMaterial` (`self.Cube`) 0 (`self.MID`)))

(event `self.ReceiveTick`
  (params (DeltaSeconds :type "Float (single-precision)"))
  ;[1 1 1] tick
  (set `self.TickDelta` DeltaSeconds)
  ;[1 1 1] store latest env
  (set `self.Envelope0-1Live` (`|GetArrayItem` (`/Game/ArthursAudioBPs/SharedAssets/Blueprints/AudioVisualisation/bp_AnalysisBeautifier.FinalOutputValuesFromAnalysis` (`self.AnalysisBeautifierRef`)) (`self.FreqSlot(from submix analyzers array of freqs)`)))
  (`|ExecutionSequence`
    (:`then_0`
      ;[1 1 1] mod LIGHT
      (if (`self.HaveLight`)
        (`LightComponent.SetIntensity` (`self.PointLight`) (* (`self.Envelope0-1Live`) 100.0))
        (`LightComponent.SetLightColor` (`self.PointLight`) (`KismetMathLibrary.LinearColorLerp` (`self.ColorLow`) (`self.ColorHigh`) (`self.Envelope0-1Live`)) true)))
    (:`then_1`
      ;[1 1 1] mod material
      ;;[1 1 1] emissive
      (`MaterialInstanceDynamic.SetScalarParameterValue` (`self.MID`) "Emissive Multiplier" (* (`self.Envelope0-1Live`) 500.0))
      ;;[1 1 1] color
      (`MaterialInstanceDynamic.SetVectorParameterValue` (`self.MID`) "Base Color" (`KismetMathLibrary.LinearColorLerp` (`self.ColorLow`) (`self.ColorHigh`) (`self.Envelope0-1Live`))))
    (:`then_2`
      ;[1 1 1] mod mesh
      (`SceneComponent.SetRelativeScale3D` (`self.Cube`) (`KismetMathLibrary.Conv_DoubleToVector` (+ (`self.Envelope0-1Live`) 0.5))))))

(fn `ModLights`
  (params (LightRef :type "LightComponent Object Reference") (`Envelope0-1` :type "Float (double-precision)"))
  ;[1 1 1] mod LIGHT
  (`LightComponent.SetIntensity` LightRef (* `Envelope0-1` 100.0))
  (`LightComponent.SetLightColor` LightRef (`KismetMathLibrary.LinearColorLerp` (`self.ColorLow`) (`self.ColorHigh`) `Envelope0-1`) true))

(fn `RandomColors`
  (if (`self.RandomColors?`)
    (set `self.ColorLow` (`KismetMathLibrary.HSVToRGB` (`KismetMathLibrary.RandomFloatInRange` 0.0 360.0) (`KismetMathLibrary.RandomFloatInRange` 0.3 1.0) 0.0))
    (set `self.ColorHigh` (`KismetMathLibrary.HSVToRGB` (`KismetMathLibrary.RandomFloatInRange` 0.0 360.0) (`KismetMathLibrary.RandomFloatInRange` 0.3 1.0) (`KismetMathLibrary.RandomFloatInRange` 0.5 1.0)))))

(fn `UserConstructionScript`
  (`self.RandomColors`)
  (if (not (`self.HaveLight`))
    (`ActorComponent.K2_DestroyComponent` (`self.PointLight`))))