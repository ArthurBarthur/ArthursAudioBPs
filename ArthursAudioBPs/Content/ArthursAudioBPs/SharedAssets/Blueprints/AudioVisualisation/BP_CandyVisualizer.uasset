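; Audio visualizer that leaves a trail of randomly colored candy meshes driven by the music's volume envelope.
; A looping timer, used instead of Tick, normalizes the envelope against the running peak to set a leading mesh's offset and scale.
; Each update also rotates and advances the central mesh, then adds a static mesh component at the leading mesh's transform.
; The construction script pregenerates the pool of colored dynamic materials.
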(event `self.ReceiveBeginPlay`
  (bind _latestvolumetreated (`self.LatestVolumeTreated`))
  (bind _latestvolumeraw (`self.LatestVolumeRaw`))
  ;[1 1 1] looping timer instead of tick
  (`KismetSystemLibrary.K2_SetTimerDelegate` (`|CreateDelegate` :!event `SpawnMesh`) (`self.UpdateIntervalInSeconds`) true)
  (set `self.LatestVolumeRaw` (stale `self.AudioComponentMusic.OnAudioSingleEnvelopeValue` EnvelopeValue) :!label _label)
  ;[1 1 1] if max volume ever, store the peak
  (if (> _latestvolumeraw (`self.MaxVolumeRecorded`))
    (set `self.MaxVolumeRecorded` _latestvolumeraw))
  ;[1 1 1] normalize volume 0-1
  (set `self.LatestVolumeTreated` (`KismetMathLibrary.MapRangeClamped` (`self.LatestVolumeRaw`) 0.0 (`self.MaxVolumeRecorded`) 0.0 1.0))
  (`|ExecutionSequence`
    (:`then_0`
      ;[1 1 1] move spawnpoint out from center
      (`SceneComponent.K2_SetRelativeLocation` (`self.LeadingStaticMesh`) (`KismetMathLibrary.MakeVector` 0.0 0.0 (* (`self.LatestVolumeTreated`) (`self.DistanceToBounceFromCenter`))) false true))
    (:`then_1`
      ;[1 1 1] update spawn scale
      (`SceneComponent.SetRelativeScale3D` (`self.LeadingStaticMesh`) (`KismetMathLibrary.MakeVector` 4.0 _latestvolumetreated _latestvolumetreated)))
    (:`then_2`
      ;[1 1 1] rotate it
      (`SceneComponent.K2_AddRelativeRotation` (`self.CentralStaticMesh`) (`self.RotationalSpeed`) false true))
    (:`then_3`
      ;[1 1 1] Move whole thing in direction
      (`SceneComponent.K2_AddLocalOffset` (`self.CentralStaticMesh`) (`self.MovementSpeed`) false true))
    (:`then_4`
      ;[1 1 1] spawn viz mesh
      (`self.SpawnNewVizMesh`))))

(event `SpawnMesh`
  (goto _label))

(event `self.AudioComponentMusic.OnAudioSingleEnvelopeValue`
  (params (PlayingSoundWave :type "SoundWave Object Reference") (EnvelopeValue :type "Float (single-precision)"))
  ;[1 1 1] get latest raw volume
)

(fn `SpawnNewVizMesh`
  (locals (LatestMesh :type "StaticMeshComponent Object Reference"))
  (bind _materials (`self.Materials`))
  (bind _leadingstaticmesh (`self.LeadingStaticMesh`))
  (bind _returnvalue (`SceneComponent.GetRelativeTransform` (`self.CentralStaticMesh`)))
  ;[1 1 1] spawn mesh
  (bind _returnvalue_2 (`AddComponent|NODE_AddStaticMeshComponent-0` :`RelativeTransform` (`KismetMathLibrary.MakeTransform` (`KismetMathLibrary.TransformLocation` _returnvalue (`SceneComponent.RelativeLocation` _leadingstaticmesh)) (`KismetMathLibrary.TransformRotation` _returnvalue (`SceneComponent.RelativeRotation` _leadingstaticmesh)) (`SceneComponent.RelativeScale3D` _leadingstaticmesh))))
  (set `local.LatestMesh` _returnvalue_2)
  ;[1 1 1] store mesh
  (`KismetArrayLibrary.Array_Add` (`self.AllSpawnedCandies`) (`local.LatestMesh`))
  ;[1 1 1] set 3d mesh
  (`StaticMeshComponent.SetStaticMesh` (`local.LatestMesh`) (`self.MeshToUseForViz`))
  ;[1 1 1] set random material
  (`PrimitiveComponent.SetMaterial` (`local.LatestMesh`) 0 (`|GetArrayItem` _materials (`KismetMathLibrary.RandomIntegerInRange` 0 (`KismetArrayLibrary.Array_LastIndex` _materials)))))

(fn `UserConstructionScript`
  (bind _availablecolors (`self.AvailableColors`))
  (bind (_h _s _v _a) (`KismetMathLibrary.RGBToHSV` (`self.AutoColorSpanEnd`)))
  (bind (_h_2 _s_2 _v_2 _a_2) (`KismetMathLibrary.RGBToHSV` (`self.AutoColorSpanStart`)))
  ;[1 1 1] clear old variables
  (`KismetArrayLibrary.Array_Clear` (`self.AllSpawnedCandies`))
  (`KismetArrayLibrary.Array_Clear` (`self.Materials`))
  (`KismetArrayLibrary.Array_Clear` (`self.AvailableColors`))
  ;[1 1 1] create material instances
  (for _ (range 1 (+ (`self.NumberOfRandomColorsToPre-generate`) 1))
    (bind _returnvalue (`KismetMaterialLibrary.CreateDynamicMaterialInstance` "/Game/ArthursAudioBPs/SharedAssets/Visuals/Materials/MAT_SimpleMat.MAT_SimpleMat"))
    (`KismetArrayLibrary.Array_Add` (`self.Materials`) _returnvalue))
  ;[1 1 1] init material colors
  ;;[1 1 1] auto-colors?
  (if (`self.Auto-GenerateColors`)
    ;;[1 1 1] random color generator
    (for _ (`self.Materials`)
      (`KismetArrayLibrary.Array_Add` (`self.AvailableColors`) (`KismetMathLibrary.HSVToRGB` (`KismetMathLibrary.RandomFloatInRange` _h_2 _h) (`KismetMathLibrary.RandomFloatInRange` _s_2 _s) (`KismetMathLibrary.RandomFloatInRange` _v_2 _v) (`KismetMathLibrary.RandomFloatInRange` _a_2 _a))))
    ;;[1 1 1] apply colors to material instances
    (for (_array_element _array_index) (`self.Materials`)
      (`MaterialInstanceDynamic.SetVectorParameterValue` _array_element "Base Color" (`|GetArrayItem` (`self.AvailableColors`) _array_index)))
    (else
      ;;[1 1 1] pick random materials from user-defined list
      (for _array_element_2 (`self.Materials`)
        (`MaterialInstanceDynamic.SetVectorParameterValue` _array_element_2 "Base Color" (`|GetArrayItem` _availablecolors (`KismetMathLibrary.RandomIntegerInRange` 0 (`KismetArrayLibrary.Array_LastIndex` _availablecolors))))))))