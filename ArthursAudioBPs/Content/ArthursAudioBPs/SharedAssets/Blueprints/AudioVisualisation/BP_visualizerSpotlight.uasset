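; BP_visualizerSpotlight is an audio-reactive spotlight for audio visualisation.
; Each tick it averages three adjacent frequency slots from the referenced analysis beautifier's output into a live envelope.
; That envelope drives the light's intensity, blends its colour from low to high, and pitches it away from its starting rotation.
; A ModLights helper applies similar intensity and colour changes at a much lower scale but is not called here.
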(event `self.ReceiveBeginPlay`
  (set `self.StartingRelativeRot` (`SceneComponent.RelativeRotation` (`self.SpotLight`))))

(event `self.ReceiveTick`
  (params (DeltaSeconds :type "Float (single-precision)"))
  (bind _freqslot_from_submix_analyzers_array_of_freqs_ (`self.FreqSlot(from submix analyzers array of freqs)`))
  (bind _finaloutputvaluesfromanalysis (`/Game/ArthursAudioBPs/SharedAssets/Blueprints/AudioVisualisation/bp_AnalysisBeautifier.FinalOutputValuesFromAnalysis` (`self.AnalysisBeautifierRef`)))
  ;[1 1 1] tick
  (set `self.TickDelta` DeltaSeconds)
  ;[1 1 1] store latest env
  (set `self.Envelope0-1Live` (/ (+ (`|GetArrayItem` _finaloutputvaluesfromanalysis _freqslot_from_submix_analyzers_array_of_freqs_) (`|GetArrayItem` _finaloutputvaluesfromanalysis (- _freqslot_from_submix_analyzers_array_of_freqs_ 1)) (`|GetArrayItem` _finaloutputvaluesfromanalysis (+ _freqslot_from_submix_analyzers_array_of_freqs_ 1))) 3.0))
  (`|ExecutionSequence`
    (:`then_0`
      ;[1 1 1] mod LIGHT
      (`LightComponent.SetIntensity` (`self.SpotLight`) (* (`self.Envelope0-1Live`) 10000000.0))
      (`LightComponent.SetLightColor` (`self.SpotLight`) (`KismetMathLibrary.LinearColorLerp` (`self.ColorLow`) (`self.ColorHigh`) (`self.Envelope0-1Live`)) true))
    (:`then_1`
      ;[1 1 1] rotate spotlight to vol
      (`SceneComponent.K2_SetRelativeRotation` (`self.SpotLight`) (`KismetMathLibrary.ComposeRotators` (`self.StartingRelativeRot`) (`KismetMathLibrary.MakeRotator` 0.0 (`KismetMathLibrary.MapRangeClamped` (`self.Envelope0-1Live`) 0.0 1.0 0.0 45.0))) false false))))

(fn `ModLights`
  (params (LightRef :type "LightComponent Object Reference") (`Envelope0-1` :type "Float (double-precision)"))
  ;[1 1 1] mod LIGHT
  (`LightComponent.SetIntensity` LightRef (* `Envelope0-1` 100.0))
  (`LightComponent.SetLightColor` LightRef (`KismetMathLibrary.LinearColorLerp` (`self.ColorLow`) (`self.ColorHigh`) `Envelope0-1`) true))

(fn `UserConstructionScript`)