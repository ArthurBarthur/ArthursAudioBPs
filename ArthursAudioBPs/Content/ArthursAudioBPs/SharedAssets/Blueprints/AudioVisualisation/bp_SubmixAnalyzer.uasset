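; Blueprint that runs real-time spectral analysis on an audio submix, in a shared audio visualisation folder.
; BeginPlay prefills LatestMagnitudes with a small value for each entry in FrequenciesToAnalyze and starts FFT output analysis on SubmixToAnalyze from inside that loop.
; Tick queries the magnitudes at those frequencies and stores them in LatestMagnitudes.
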(event `self.ReceiveBeginPlay`
  ;[1 1 1] beginplay
  ;[1 1 1] prefill magnitudes array with zeroes
  (for (_ _array_index) (`self.FrequenciesToAnalyze`)
    (`KismetArrayLibrary.Array_Set` (`self.LatestMagnitudes`) _array_index 0.01 true)
    ;[1 1 1] start analyzing submix output
    (`AudioMixerBlueprintLibrary.StartAnalyzingOutput` (`self.SubmixToAnalyze`) "Large")))

(event `self.ReceiveTick`
  (params (DeltaSeconds :type "Float (single-precision)"))
  ;[1 1 1] tick
  ;[1 1 1] get latest magnitudes
  (bind _magnitudes (`AudioMixerBlueprintLibrary.GetMagnitudeForFrequencies` (`self.FrequenciesToAnalyze`) (`self.SubmixToAnalyze`)))
  (set `self.LatestMagnitudes` _magnitudes))

(fn `UserConstructionScript`)