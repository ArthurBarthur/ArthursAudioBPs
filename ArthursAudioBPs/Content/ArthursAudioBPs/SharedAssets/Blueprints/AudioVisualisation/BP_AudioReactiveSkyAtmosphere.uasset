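; Audio-reactive actor that drives a referenced sun-sky actor's atmosphere from audio analysis.
; Each Tick it reads the smoothed, normalized envelope value for a chosen frequency slot from a Beautifier reference.
; That value is remapped with a clamped range to set the SkyAtmosphere's Mie absorption scale, and also shows its Sphere mesh only above a volume threshold.
; BeginPlay caches the SkyAtmosphere component, but Tick accesses it directly through the sun-sky reference.
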(event `self.ReceiveBeginPlay`
  (set `self.Atmospheric foc component reference` (`self.GetComponentByClass` (`self.SunSkyThingReference`) "/Script/Engine.SkyAtmosphereComponent")))

(event `self.ReceiveTick`
  (params (DeltaSeconds :type "Float (single-precision)"))
  (bind _output_get (set `self.LatestVolumeThing` (`|GetArrayItem` (`/Game/ArthursAudioBPs/SharedAssets/Blueprints/AudioVisualisation/bp_AnalysisBeautifier.FinalEnvelopeSmoothedNormalizedOutputValuesFromAnalysis` (`self.BeautifierReference`)) (`self.FreqSlotToListenTo`))))
  ;[1 1 1] Turn mesh visibility off
  ; if UNDER 0.2 volume)
  (`SceneComponent.SetVisibility` (`self.Sphere`) (> _output_get 0.2) false)
  (`SkyAtmosphereComponent.SetMieAbsorptionScale` (`/SunPosition/SunSky.SkyAtmosphere` (`self.SunSkyThingReference`)) (`KismetMathLibrary.MapRangeClamped` (`self.LatestVolumeThing`) 0.0 1.0 0.000444 0.5)))

(fn `UserConstructionScript`)