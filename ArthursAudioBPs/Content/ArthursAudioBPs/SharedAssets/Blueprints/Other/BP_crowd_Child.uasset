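; A child crowd Blueprint that bobs its crowd meshes up and down in response to audio analysis.
; On BeginPlay it takes the MeshesFinal list and caches each mesh's relative location as a rest position.
; Each Tick it offsets every mesh's Z from that origin by one chosen frequency slot of the Beautifier's analysis output, scaled by a reactivity multiplier, so the crowd moves in unison.
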(event `self.ReceiveBeginPlay`
  (`parent.ReceiveBeginPlay`)
  (set `self.AllCrowdMeshes` (`self.meshesFinal`))
  ;[1 1 1] store origin positions of crowd
  (for _array_element (`self.AllCrowdMeshes`)
    (`KismetArrayLibrary.Array_Add` (`self.array`) (`SceneComponent.RelativeLocation` _array_element))))

(event `self.ReceiveTick`
  (params (DeltaSeconds :type "Float (single-precision)"))
  (`parent.ReceiveTick` DeltaSeconds)
  ;[1 1 1] update positions of crowd to music or whatevs
  (for (_array_element _array_index) (`self.AllCrowdMeshes`)
    (`SceneComponent.K2_SetRelativeLocation` _array_element (`KismetMathLibrary.MakeVector` (.x (`|GetArrayItem` (`self.array`) _array_index)) (.y (`|GetArrayItem` (`self.array`) _array_index)) (+ (.z (`|GetArrayItem` (`self.array`) _array_index)) (* (`|GetArrayItem` (`/Game/ArthursAudioBPs/SharedAssets/Blueprints/AudioVisualisation/BP_AnalysisBeautifier.FinalOutputValuesFromAnalysis` (`self.Beautifier`)) (`self.FreqSlot(from submix analyzers array of freqs)`)) (`self.ReactivityMP`)))) false false)))

(fn `UserConstructionScript`
  (`parent.UserConstructionScript`))