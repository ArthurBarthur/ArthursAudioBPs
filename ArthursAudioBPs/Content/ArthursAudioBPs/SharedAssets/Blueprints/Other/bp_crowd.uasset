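; Crowd actor that procedurally scatters static-mesh people in its construction script, with no runtime logic.
; It adds a configurable number of mesh components at random location, yaw and non-uniform scale within exposed ranges, each given a random mesh from MeshTemplates.
; An overlap pass then destroys any member touching more than one WorldStatic or WorldDynamic component and prints how many were deleted.
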(fn `MakeRandomTransform`
  (returns (ReturnValue :type "Transform Structure"))
  (bind (_personscalerangewidth_x _personscalerangewidth_y) (`KismetMathLibrary.BreakVector2D` (`self.PersonScaleRangeWidth`)))
  (bind (_personscalerangethickness_x _personscalerangethickness_y) (`KismetMathLibrary.BreakVector2D` (`self.PersonScaleRangeThickness`)))
  (bind (_personscalerangeheight_x _personscalerangeheight_y) (`KismetMathLibrary.BreakVector2D` (`self.PersonScaleRangeHeight`)))
  (bind (_personrotationrange_x _personrotationrange_y) (`KismetMathLibrary.BreakVector2D` (`self.PersonRotationRange`)))
  (bind (_personlocationsrangex_x _personlocationsrangex_y) (`KismetMathLibrary.BreakVector2D` (`self.PersonLocationsRangeX`)))
  (bind (_personlocationsrangey_x _personlocationsrangey_y) (`KismetMathLibrary.BreakVector2D` (`self.PersonLocationsRangeY`)))
  (bind (_personlocationsrangez_x _personlocationsrangez_y) (`KismetMathLibrary.BreakVector2D` (`self.PersonLocationsRangeZ`)))
  (return (`KismetMathLibrary.MakeTransform` (`KismetMathLibrary.MakeVector` (`KismetMathLibrary.RandomFloatInRange` _personlocationsrangex_x _personlocationsrangex_y) (`KismetMathLibrary.RandomFloatInRange` _personlocationsrangey_x _personlocationsrangey_y) (`KismetMathLibrary.RandomFloatInRange` _personlocationsrangez_x _personlocationsrangez_y)) (`KismetMathLibrary.MakeRotator` 0.0 0.0 (`KismetMathLibrary.RandomFloatInRange` _personrotationrange_x _personrotationrange_y)) (`KismetMathLibrary.MakeVector` (`KismetMathLibrary.RandomFloatInRange` _personscalerangewidth_x _personscalerangewidth_y) (`KismetMathLibrary.RandomFloatInRange` _personscalerangethickness_x _personscalerangethickness_y) (`KismetMathLibrary.RandomFloatInRange` _personscalerangeheight_x _personscalerangeheight_y)))))

(fn `UserConstructionScript`
  (bind _meshtemplates (`self.meshTemplates`))
  (bind _deletedpeeps (`self.DeletedPeeps`))
  ;[1 1 1] add all people(meshes)
  (if (> (`self.NumberOfPeople`) 0)
    (for _ (range (`self.NumberOfPeople`))
      (bind _returnvalue (`self.MakeRandomTransform`))
      (bind _returnvalue_2 (`AddComponent|NODE_AddStaticMeshComponent-1` :`RelativeTransform` _returnvalue))
      (`KismetArrayLibrary.Array_Add` (`self.meshesCreated`) _returnvalue_2))
    ;[1 1 1] set which meshes to use for crowd
    (for _array_element (`self.meshesCreated`)
      (`StaticMeshComponent.SetStaticMesh` _array_element (`|GetArrayItem` _meshtemplates (`KismetMathLibrary.RandomIntegerInRange` 0 (`KismetArrayLibrary.Array_LastIndex` _meshtemplates)))))
    ;[1 1 1] delete any crowd members that overlap worldDynamic or worldStatic objects.
    (for _array_element_2 (`self.meshesCreated`)
      (bind _outcomponents (`KismetSystemLibrary.ComponentOverlapComponents` _array_element_2 (`SceneComponent.K2_GetComponentToWorld` _array_element_2) (`|MakeArray` "ObjectTypeQuery2" "ObjectTypeQuery1" :!type "EObjectTypeQuery Enum")))
      (if (> (`KismetArrayLibrary.Array_Length` _outcomponents) 1)
        (`ActorComponent.K2_DestroyComponent` _array_element_2)
        (`/Engine/EditorBlueprintResources/StandardMacros.IncrementInt` (`self.DeletedPeeps`))))
    (if (> _deletedpeeps 0)
      (`KismetSystemLibrary.PrintString` (`KismetStringLibrary.Concat_StrStr` "Deleted overlappers: " (`KismetStringLibrary.Conv_IntToString` _deletedpeeps))))))