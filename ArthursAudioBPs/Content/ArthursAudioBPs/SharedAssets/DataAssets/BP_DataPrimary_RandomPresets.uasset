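; Data asset that generates random modular synth presets from a seed, meant to be called by a parent actor through RandomizePresetFull.
; Each parameter has its own macro drawing from a shared seeded random stream, mostly using min/max or chance variables.
; Stage 1 builds the base preset; stage 2 refines values depending on earlier rolls: noise oscillator gain, one-shot LFO rates and filter frequency per filter type.
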(fn `RandomizePresetFull`
  (params (NewSeed :type Integer))
  (returns (SynthPresetFinal :type "ModularSynthPreset Structure"))
  ;[1 1 1] set random seed
  (`KismetMathLibrary.SetRandomStreamSeed` (`self.RandomStream`) NewSeed)
  ;[1 1 1] randomize stage 1
  (`self.RandomizeStage1`)
  ;[1 1 1] randomize stage 2
  (`self.RandomizeStage2`)
  (return (`self.SynthPresetFinal`)))

(fn `RandomizeStage1`
  ;[1 1 1] stage 1 random base preset
  (set `self.SynthPresetStage1` (make `ModularSynthPreset` (`self.PolyphonyOnOff`) (`self.OscTypeNoNoise`) (`self.OscGain`) (`self.OscOctave`) 0.0 (`self.OscCents(detune)`) (`self.OscPulseWidth`) (`self.OscType`) (`self.OscGain`) (`self.OscOctave`) 0.0 (`self.OscCents(detune)`) (`self.OscPulseWidth`) (`self.PortamentoOnOff`) (`self.UnisonOnOff`) (`self.OscSyncOnOff`) (`self.StereoSpread`) 0.0 (`self.LFO1Freq`) (`self.LFO1Gain`) (`self.LFO Type`) (`self.LFO Mode`) (`self.LFO1 Patch`) (`self.LFO2Freq`) (`self.LFO2Gain`) (`self.LFO Type`) (`self.LFO Mode`) (`self.LFO2 Patch`) -3.0 (`self.Attack`) (`self.Decay`) (`self.Sustain`) (`self.Release`) (`self.ModEnvPatchType`) (`self.ModEnvBiasPatchType`) (`self.ModEnvInvert`) (`self.ModEnvInvertBias`) (`self.ModEnvDepth`) (`self.ModEnvAttack`) (`self.ModEnvDecay`) (`self.ModEnvSustain`) (`self.ModEnvRelease`) (`self.LegatoOnOff`) (`self.RetriggerOnOff`) 2000.0 (`self.FilterQ`) (`self.FilterType`) (`self.FilterAlgorithm`) (`self.StereoDelayOnOff`) (`self.StereoDelayMode`) (`self.StereoDelayTime`) (`self.StereoDelayFeedback`) (`self.StereoDelayWetlevel`) (`self.StereoDelayWidenessRatio`) (`self.Chorus`) (`self.ChorusDepth`) (`self.ChorusFeedback`) (`self.ChorusFreq`) (`|MakeArray` (struct) :!type "EpicSynth1Patch Structure"))))

(fn `RandomizeStage2`
  (bind ((`Osc2Type` _osc2type) (`Osc2Gain` _osc2gain)) (break `ModularSynthPreset` (`self.SynthPresetStage1`)))
  (bind ((`LFO1Frequency` _lfo1frequency) (`LFO1Mode` _lfo1mode)) (break `ModularSynthPreset` (`self.SynthPresetStage1`)))
  (bind ((`LFO2Frequency` _lfo2frequency) (`LFO2Mode` _lfo2mode)) (break `ModularSynthPreset` (`self.SynthPresetStage1`)))
  ;[1 1 1] stage 2 now that some things are set in stone
  (set `self.SynthPresetStage2` (`self.SynthPresetStage1`))
  (bind _structout (setmembers `ModularSynthPreset` :`StructRef` (`self.SynthPresetStage2`) :`Osc2Gain` (select `bool` (`|EnumEquality` _osc2type "Noise") :`false` _osc2gain :`true` (`self.NoiseGain`)) :`LFO1Frequency` (select `bool` (`|EnumEquality` _lfo1mode "OneShot") :`false` _lfo1frequency :`true` (`self.LFO Oneshot Freq`)) :`LFO2Frequency` (select `bool` (`|EnumEquality` _lfo2mode "OneShot") :`false` _lfo2frequency :`true` (`self.LFO Oneshot Freq`)) :`FilterFrequency` (select `ESynthFilterType` (`.FilterType` (break `ModularSynthPreset` (`self.SynthPresetStage1`))) :`LowPass` (`self.FilterFreqLowpass`) :`HighPass` (`self.FilterFreqHighpass`) :`BandPass` (`self.FilterFreqBandpass`) :`BandStop` (`self.FilterFreqBandstop`))))
  (set `self.SynthPresetFinal` _structout))