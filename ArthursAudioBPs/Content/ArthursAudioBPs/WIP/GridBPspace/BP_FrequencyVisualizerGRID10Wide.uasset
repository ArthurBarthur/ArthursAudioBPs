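; Audio frequency visualizer actor that renders smoothed submix analysis as a grid of height-scaled meshes.
; Construction spawns a center row with one mesh per analyzer frequency, adds dynamic materials with optional random colors, previews random heights, and adds five rows on either side.
; After validating analyzer and beautifier references, Tick reads the beautifier's smoothed values to drive center-row height and emissive strength.
; Side rows copy center heights, divided progressively more with distance.
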(event `self.ReceiveBeginPlay`
  ;[1 1 1] beginplay
  ;[1 1 1] init
  (`KismetSystemLibrary.Delay` 0.5)
  (`/Engine/EditorBlueprintResources/StandardMacros.IsValid` (`self.SubmixAnalyzerRef`)
    (:`Is Valid`
      (`/Engine/EditorBlueprintResources/StandardMacros.IsValid` (`self.SubmixBeautifierRef`)
        (:`Is Valid`
          ;;[1 1 1] Enable Tick
          (`self.SetActorTickEnabled` true))
        (:`Is Not Valid`
          (`self.DebugPrint` (`KismetSystemLibrary.GetDisplayName` self) " does not have valid beautifier-ref"))))
    (:`Is Not Valid`
      (`self.DebugPrint` (`KismetSystemLibrary.GetDisplayName` self) " does not have valid analyzer-ref"))))

(event `self.ReceiveTick`
  (params (DeltaSeconds :type "Float (single-precision)"))
  (bind (__5 __4 __3 __2 __1 _1 _2 _3 _4 _5) (break `/Game/ArthursAudioBPs/WIP/GridBPspace/GridStruct10wide` (`self.GridStruct`)))
  ;[1 1 1] Tick
  (set `self.DeltaTick` DeltaSeconds)
  (`|ExecutionSequence`
    (:`then_0`
      ;[1 1 1] get latest beautified analysis
      (set `self.LatestSmoothValues` (`/ArthursAudioVisualToolkit/Blueprints/AudioViz/BP_AnalysisBeautifier.FinalEnvelopeSmoothedNormalizedOutputValuesFromAnalysis` (`self.SubmixBeautifierRef`))))
    (:`then_1`
      ;[1 1 1] Update mesh scales
      (`self.ScaleMeshes`))
    (:`then_2`
      ;[1 1 1] Update dynamic material emissive strength
      (`self.UpdateMaterialEmissive`))
    (:`then_3`
      ;[1 1 1] rescale all rows
      (`self.ScaleARow` __5 6.0)
      (`self.ScaleARow` __4 5.0)
      (`self.ScaleARow` __3 4.0)
      (`self.ScaleARow` __2 3.0)
      (`self.ScaleARow` __1 2.0)
      (`self.ScaleARow` _1 2.0)
      (`self.ScaleARow` _2 3.0)
      (`self.ScaleARow` _3 4.0)
      (`self.ScaleARow` _4 5.0)
      (`self.ScaleARow` _5 6.0))))

(fn `AddRowsOnEitherSide`
  (bind (__5 __4 __3 __2 __1 _1 _2 _3 _4 _5) (break `/Game/ArthursAudioBPs/WIP/GridBPspace/GridStruct10wide` (`self.GridStruct`)))
  (bind (__5_2 __4_2 __3_2 __2_2 __1_2 _1_2 _2_2 _3_2 _4_2 _5_2) (break `/Game/ArthursAudioBPs/WIP/GridBPspace/GridStruct10wide` (`self.GridStruct`)))
  (`KismetArrayLibrary.Array_Clear` __5)
  (`KismetArrayLibrary.Array_Clear` __4)
  (`KismetArrayLibrary.Array_Clear` __3)
  (`KismetArrayLibrary.Array_Clear` __2)
  (`KismetArrayLibrary.Array_Clear` __1)
  (`KismetArrayLibrary.Array_Clear` _1)
  (`KismetArrayLibrary.Array_Clear` _2)
  (`KismetArrayLibrary.Array_Clear` _3)
  (`KismetArrayLibrary.Array_Clear` _4)
  (`KismetArrayLibrary.Array_Clear` _5)
  ;[1 1 1] Add rows on either side
  (for _index (range -5 6)
    (if (!= _index 0)
      (for _array_element (`self.VizMeshes`)
        (bind _returnvalue (`AddComponent|NODE_AddStaticMeshComponent-2` :`RelativeTransform` (`KismetMathLibrary.MakeTransform` (`KismetMathLibrary.MakeVector` (+ (.x (.location (`SceneComponent.GetRelativeTransform` _array_element))) (* _index (`self.MeshRowDistanceOffset`))) (.y (.location (`SceneComponent.GetRelativeTransform` _array_element))) (.z (.location (`SceneComponent.GetRelativeTransform` _array_element)))) (.rotation (`SceneComponent.GetRelativeTransform` _array_element)) (.scale (`SceneComponent.GetRelativeTransform` _array_element)))))
        (switch `int` (+ _index 5)
          (:`0`
            (`KismetArrayLibrary.Array_Add` __5_2 _returnvalue))
          (:`1`
            (`KismetArrayLibrary.Array_Add` __4_2 _returnvalue))
          (:`2`
            (`KismetArrayLibrary.Array_Add` __3_2 _returnvalue))
          (:`3`
            (`KismetArrayLibrary.Array_Add` __2_2 _returnvalue))
          (:`4`
            (`KismetArrayLibrary.Array_Add` __1_2 _returnvalue))
          (:`6`
            (`KismetArrayLibrary.Array_Add` _1_2 _returnvalue))
          (:`7`
            (`KismetArrayLibrary.Array_Add` _2_2 _returnvalue))
          (:`8`
            (`KismetArrayLibrary.Array_Add` _3_2 _returnvalue))
          (:`9`
            (`KismetArrayLibrary.Array_Add` _4_2 _returnvalue))
          (:`10`
            (`KismetArrayLibrary.Array_Add` _5_2 _returnvalue)))))))

(fn `ConstructionPreVizMeshes`
  (locals (_currentIndex :type Integer) (_currentMesh :type "StaticMeshComponent Object Reference") (CurrentValue :type "Float (double-precision)" :default 0.0))
  ;[1 1 1] loop through meshes
  (for (_array_element _array_index) (`self.VizMeshes`)
    (set `local._currentMesh` _array_element)
    (set `local._currentIndex` _array_index)
    (bind _output_get (set `local.CurrentValue` (+ (* (`KismetMathLibrary.SelectFloat` (`KismetMathLibrary.RandomFloatInRange` 0.0 0.5) (`KismetMathLibrary.RandomFloatInRange` 0.5 1.0) (`KismetMathLibrary.RandomBoolWithWeight` 0.7)) (`self.MeshScaleMultiplier`)) (`self.MinimumSize`))))
    ;[1 1 1] set new mesh scale
    (`SceneComponent.SetRelativeScale3D` (`local._currentMesh`) (`KismetMathLibrary.MakeVector` 1.0 1.0 _output_get))
    ;[1 1 1] modify MID emissive multiplier value
    (`MaterialInstanceDynamic.SetScalarParameterValue` (`|GetArrayItem` (`self.MIDs`) (`local._currentIndex`)) (`self.MaterialParameterEmissiveMultiplier`) (* (`local.CurrentValue`) (`self.MaterialEmissiveMultiplier`)))))

(fn `DebugPrint`
  (params (`String part 1` :type String) (`String part 2` :type String) (`String part 3` :type String))
  (`KismetSystemLibrary.PrintString` (`KismetStringLibrary.Concat_StrStr` `String part 1` `String part 2` `String part 3`)))

(fn `InitializeDynamicMaterials`
  (locals (_currentIndex :type Integer) (_currentMesh :type "StaticMeshComponent Object Reference") (_latestRandomColor :type "LinearColor Structure"))
  (`KismetArrayLibrary.Array_Clear` (`self.MIDs`))
  ;[1 1 1] loop through meshes
  (for (_array_element _array_index) (`self.VizMeshes`)
    (`|ExecutionSequence`
      (:`then_0`
        ;[1 1 1] store local variables
        (set `local._currentMesh` _array_element)
        (set `local._currentIndex` _array_index))
      (:`then_1`
        ;[1 1 1] create dynamic materials(MIDs)
        (bind _returnvalue (`KismetMaterialLibrary.CreateDynamicMaterialInstance` (`self.BaseMaterial`)))
        (`KismetArrayLibrary.Array_Set` (`self.MIDs`) (`local._currentIndex`) _returnvalue true))
      (:`then_2`
        ;[1 1 1] put MIDs on meshes
        (`PrimitiveComponent.SetMaterial` (`local._currentMesh`) 0 (`|GetArrayItem` (`self.MIDs`) (`local._currentIndex`))))
      (:`then_3`
        ;[1 1 1] random color?
        (if (`self.RandomColors?`)
          ;[1 1 1] make color
          (bind _linearcolor (`self.MakeRandomColor`))
          (set `local._latestRandomColor` _linearcolor)
          ;[1 1 1] set colors on materials
          (`MaterialInstanceDynamic.SetVectorParameterValue` (`|GetArrayItem` (`self.MIDs`) (`local._currentIndex`)) (`self.MaterialParameterBaseColor`) (`local._latestRandomColor`)))))))

(fn `MakeRandomColor`
  (returns (LinearColor :type "LinearColor Structure"))
  (bind (_bvalue_x _bvalue_y) (`KismetMathLibrary.BreakVector2D` (`self.bValue`)))
  (bind (_rvalue_x _rvalue_y) (`KismetMathLibrary.BreakVector2D` (`self.rValue`)))
  (bind (_gvalue_x _gvalue_y) (`KismetMathLibrary.BreakVector2D` (`self.gValue`)))
  (return (make `LinearColor` (`KismetMathLibrary.RandomFloatInRange` _rvalue_x _rvalue_y) (`KismetMathLibrary.RandomFloatInRange` _gvalue_x _gvalue_y) (`KismetMathLibrary.RandomFloatInRange` _bvalue_x _bvalue_y))))

(fn `ScaleARow`
  (params (MeshArray :type "Array of StaticMeshComponent Object Reference") (DivideScaleBy :type "Float (double-precision)"))
  (for (_array_element _array_index) MeshArray
    (`SceneComponent.SetRelativeScale3D` _array_element (`KismetMathLibrary.MakeVector` (.x (`SceneComponent.RelativeScale3D` (`|GetArrayItem` (`self.VizMeshes`) _array_index))) (.y (`SceneComponent.RelativeScale3D` (`|GetArrayItem` (`self.VizMeshes`) _array_index))) (/ (.z (`SceneComponent.RelativeScale3D` (`|GetArrayItem` (`self.VizMeshes`) _array_index))) DivideScaleBy)))))

(fn `ScaleMeshes`
  (locals (_currentIndex :type Integer) (_currentMesh :type "StaticMeshComponent Object Reference"))
  ;[1 1 1] loop through meshes
  (for (_array_element _array_index) (`self.VizMeshes`)
    (set `local._currentMesh` _array_element)
    (set `local._currentIndex` _array_index)
    ;[1 1 1] set new mesh scale
    (`SceneComponent.SetRelativeScale3D` (`local._currentMesh`) (`KismetMathLibrary.MakeVector` 1.0 1.0 (+ (* (`|GetArrayItem` (`self.LatestSmoothValues`) (`local._currentIndex`)) (`self.MeshScaleMultiplier`)) (`self.MinimumSize`))))))

(fn `SpawnVisualizerMeshes`
  (locals (_currentIndex :type Integer))
  (bind _vizmeshes (`self.VizMeshes`))
  ;[1 1 1] clear out old existing meshes if any
  (for _array_element _vizmeshes
    (`ActorComponent.K2_DestroyComponent` _array_element))
  (`KismetArrayLibrary.Array_Clear` _vizmeshes)
  ;[1 1 1] loop through frequencies
  (for (_ _array_index) (`self.FrequenciesToAnalyze`)
    ;[1 1 1] spawn visualizer meshes in a row
    (set `local._currentIndex` _array_index)
    (bind _returnvalue (`AddComponent|NODE_AddStaticMeshComponent-0` :`RelativeTransform` (`KismetMathLibrary.MakeTransform` (`KismetMathLibrary.MakeVector` 0.0 (* (`local._currentIndex`) (`self.MeshRowDistanceOffset`))))))
    ;[1 1 1] store mesh references
    (`KismetArrayLibrary.Array_Set` (`self.VizMeshes`) (`local._currentIndex`) _returnvalue true))
  ;[1 1 1] attach to rootmesh
  (for _array_element_2 (`self.VizMeshes`)
    (`SceneComponent.K2_AttachToComponent` _array_element_2 (`self.StaticNoMesh`) "None" "KeepRelative" "KeepRelative" "KeepRelative" true)))

(fn `UpdateMaterialEmissive`
  ;[1 1 1] modify MID emissive multiplier value
  (for (_array_element _array_index) (`self.MIDs`)
    (`MaterialInstanceDynamic.SetScalarParameterValue` _array_element (`self.MaterialParameterEmissiveMultiplier`) (* (+ (`|GetArrayItem` (`self.LatestSmoothValues`) _array_index) (`self.MinimumEmissiveStrength`)) (`self.MaterialEmissiveMultiplier`)))))

(fn `UserConstructionScript`
  ;[1 1 1] get frequencies to analyze from SubmixAnalyzer
  (set `self.FrequenciesToAnalyze` (`/ArthursAudioVisualToolkit/Blueprints/AudioViz/BP_SubmixAnalyzer.FrequenciesToAnalyze` (`self.SubmixAnalyzerRef`)))
  ;[1 1 1] spawn visualizing meshes
  (`self.SpawnVisualizerMeshes`)
  ;[1 1 1] initialize dynamic materials(MIDs)
  (`self.InitializeDynamicMaterials`)
  ;[1 1 1] pre-viz scaling of meshes
  (`self.ConstructionPreVizMeshes`)
  ;[1 1 1] add rows on either side
  (`self.AddRowsOnEitherSide`))