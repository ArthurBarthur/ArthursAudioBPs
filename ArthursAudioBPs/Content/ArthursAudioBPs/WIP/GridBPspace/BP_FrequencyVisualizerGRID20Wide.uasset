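; Audio-reactive frequency visualizer actor that displays submix analysis as a wide grid of height-scaled, glowing meshes.
; Construction spawns one mesh per analyzed frequency with dynamic materials and a random preview, then copies that row ten times to either side.
; Each Tick, smoothed values from the submix beautifier drive center-row height and emissive strength.
; Side rows divide those heights by growing amounts outward and take emissive values from center materials through a modulo index.
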(event `self.ReceiveBeginPlay`
  ;[1 1 1] beginplay
  ;[1 1 1] init
  (`KismetSystemLibrary.Delay` 0.5)
  (`/Engine/EditorBlueprintResources/StandardMacros.IsValid` (`self.SubmixAnalyzerRef`)
    (:`Is Valid`
      (`/Engine/EditorBlueprintResources/StandardMacros.IsValid` (`self.SubmixBeautifierRef`)
        (:`Is Valid`
          ;;[1 1 1] Enable Tick
          (`self.SetActorTickEnabled` true))
        (:`Is Not Valid`
          (`self.DebugPrint` (`KismetSystemLibrary.GetDisplayName` self) " does not have valid beautifier-ref"))))
    (:`Is Not Valid`
      (`self.DebugPrint` (`KismetSystemLibrary.GetDisplayName` self) " does not have valid analyzer-ref"))))

(event `self.ReceiveTick`
  (params (DeltaSeconds :type "Float (single-precision)"))
  (bind _mids (`self.MIDs`))
  ;[1 1 1] Tick
  (set `self.DeltaTick` DeltaSeconds)
  (`|ExecutionSequence`
    (:`then_0`
      ;[1 1 1] get latest beautified analysis
      (set `self.LatestSmoothValues` (`/ArthursAudioVisualToolkit/Blueprints/AudioViz/BP_AnalysisBeautifier.FinalEnvelopeSmoothedNormalizedOutputValuesFromAnalysis` (`self.SubmixBeautifierRef`))))
    (:`then_1`
      ;[1 1 1] Update mesh scales
      (`self.ScaleMeshes`))
    (:`then_2`
      ;[1 1 1] Update dynamic material emissive strength
      (`self.UpdateMaterialEmissive`))
    (:`then_3`
      ;[1 1 1] rescale all extra rows
      (`self.RescaleAllExtraRows`))
    (:`then_4`
      (for (_array_element _array_index) (`self.ExtraGridMIDs`)
        (bind _returnvalue (`MaterialInstanceDynamic.K2_GetScalarParameterValue` (`|GetArrayItem` _mids (mod _array_index (`KismetArrayLibrary.Array_LastIndex` _mids))) (`self.MaterialParameterEmissiveMultiplier`)))
        (`MaterialInstanceDynamic.SetScalarParameterValue` _array_element (`self.MaterialParameterEmissiveMultiplier`) _returnvalue)))))

(fn `AddRowsOnEitherSide`
  (bind (__10 __9 __8 __7 __6 __5 __4 __3 __2 __1 _1 _2 _3 _4 _5 _6 _7 _8 _9 _10) (break `/Game/ArthursAudioBPs/WIP/GridBPspace/GridStruct20wide` (`self.GridStruct20`)))
  (bind (__10_2 __9_2 __8_2 __7_2 __6_2 __5_2 __4_2 __3_2 __2_2 __1_2 _1_2 _2_2 _3_2 _4_2 _5_2 _6_2 _7_2 _8_2 _9_2 _10_2) (break `/Game/ArthursAudioBPs/WIP/GridBPspace/GridStruct20wide` (`self.GridStruct20`)))
  (bind (__10_3 __9_3 __8_3 __7_3 __6_3 __5_3 __4_3 __3_3 __2_3 __1_3 _1_3 _2_3 _3_3 _4_3 _5_3 _6_3 _7_3 _8_3 _9_3 _10_3) (break `/Game/ArthursAudioBPs/WIP/GridBPspace/GridStruct20wide` (`self.GridStruct20`)))
  (`KismetArrayLibrary.Array_Clear` __10_2)
  (`KismetArrayLibrary.Array_Clear` __9_2)
  (`KismetArrayLibrary.Array_Clear` __8_2)
  (`KismetArrayLibrary.Array_Clear` __7_2)
  (`KismetArrayLibrary.Array_Clear` __6_2)
  (`KismetArrayLibrary.Array_Clear` __5_2)
  (`KismetArrayLibrary.Array_Clear` __4_2)
  (`KismetArrayLibrary.Array_Clear` __3_2)
  (`KismetArrayLibrary.Array_Clear` __2_2)
  (`KismetArrayLibrary.Array_Clear` __1_2)
  (`KismetArrayLibrary.Array_Clear` _1_2)
  (`KismetArrayLibrary.Array_Clear` _2_2)
  (`KismetArrayLibrary.Array_Clear` _3_2)
  (`KismetArrayLibrary.Array_Clear` _4_2)
  (`KismetArrayLibrary.Array_Clear` _5_2)
  (`KismetArrayLibrary.Array_Clear` _6_2)
  (`KismetArrayLibrary.Array_Clear` _7_2)
  (`KismetArrayLibrary.Array_Clear` _8_2)
  (`KismetArrayLibrary.Array_Clear` _9_2)
  (`KismetArrayLibrary.Array_Clear` _10_2)
  ;[1 1 1] Add rows on either side
  (for _index (range -10 11)
    (if (!= _index 0)
      (for _array_element (`self.VizMeshes`)
        (bind _returnvalue (`AddComponent|NODE_AddStaticMeshComponent-2` :`RelativeTransform` (`KismetMathLibrary.MakeTransform` (`KismetMathLibrary.MakeVector` (+ (.x (.location (`SceneComponent.GetRelativeTransform` _array_element))) (* _index (`self.MeshRowDistanceOffset`))) (.y (.location (`SceneComponent.GetRelativeTransform` _array_element))) (.z (.location (`SceneComponent.GetRelativeTransform` _array_element)))) (.rotation (`SceneComponent.GetRelativeTransform` _array_element)) (.scale (`SceneComponent.GetRelativeTransform` _array_element)))))
        (switch `int` (+ _index 10)
          (:`0`
            (`KismetArrayLibrary.Array_Add` __10_3 _returnvalue))
          (:`1`
            (`KismetArrayLibrary.Array_Add` __9_3 _returnvalue))
          (:`2`
            (`KismetArrayLibrary.Array_Add` __8_3 _returnvalue))
          (:`3`
            (`KismetArrayLibrary.Array_Add` __7_3 _returnvalue))
          (:`4`
            (`KismetArrayLibrary.Array_Add` __6_3 _returnvalue))
          (:`5`
            (`KismetArrayLibrary.Array_Add` __5_3 _returnvalue))
          (:`6`
            (`KismetArrayLibrary.Array_Add` __4_3 _returnvalue))
          (:`7`
            (`KismetArrayLibrary.Array_Add` __3_3 _returnvalue))
          (:`8`
            (`KismetArrayLibrary.Array_Add` __2_3 _returnvalue))
          (:`9`
            (`KismetArrayLibrary.Array_Add` __1_3 _returnvalue))
          (:`11`
            (`KismetArrayLibrary.Array_Add` _1_3 _returnvalue))
          (:`12`
            (`KismetArrayLibrary.Array_Add` _2_3 _returnvalue))
          (:`13`
            (`KismetArrayLibrary.Array_Add` _3_3 _returnvalue))
          (:`14`
            (`KismetArrayLibrary.Array_Add` _4_3 _returnvalue))
          (:`15`
            (`KismetArrayLibrary.Array_Add` _5_3 _returnvalue))
          (:`16`
            (`KismetArrayLibrary.Array_Add` _6_3 _returnvalue))
          (:`17`
            (`KismetArrayLibrary.Array_Add` _7_3 _returnvalue))
          (:`18`
            (`KismetArrayLibrary.Array_Add` _8_3 _returnvalue))
          (:`19`
            (`KismetArrayLibrary.Array_Add` _9_3 _returnvalue))
          (:`20`
            (`KismetArrayLibrary.Array_Add` _10_3 _returnvalue))))))
  ;[1 1 1] add all meshes to master list
  (for _array_element_2 __10
    (`KismetArrayLibrary.Array_Add` (`self.AllExtraGridMeshes`) _array_element_2))
  (for _array_element_3 __9
    (`KismetArrayLibrary.Array_Add` (`self.AllExtraGridMeshes`) _array_element_3))
  (for _array_element_4 __8
    (`KismetArrayLibrary.Array_Add` (`self.AllExtraGridMeshes`) _array_element_4))
  (for _array_element_5 __7
    (`KismetArrayLibrary.Array_Add` (`self.AllExtraGridMeshes`) _array_element_5))
  (for _array_element_6 __6
    (`KismetArrayLibrary.Array_Add` (`self.AllExtraGridMeshes`) _array_element_6))
  (for _array_element_7 __5
    (`KismetArrayLibrary.Array_Add` (`self.AllExtraGridMeshes`) _array_element_7))
  (for _array_element_8 __4
    (`KismetArrayLibrary.Array_Add` (`self.AllExtraGridMeshes`) _array_element_8))
  (for _array_element_9 __3
    (`KismetArrayLibrary.Array_Add` (`self.AllExtraGridMeshes`) _array_element_9))
  (for _array_element_10 __2
    (`KismetArrayLibrary.Array_Add` (`self.AllExtraGridMeshes`) _array_element_10))
  (for _array_element_11 __1
    (`KismetArrayLibrary.Array_Add` (`self.AllExtraGridMeshes`) _array_element_11))
  (for _array_element_12 _1
    (`KismetArrayLibrary.Array_Add` (`self.AllExtraGridMeshes`) _array_element_12))
  (for _array_element_13 _2
    (`KismetArrayLibrary.Array_Add` (`self.AllExtraGridMeshes`) _array_element_13))
  (for _array_element_14 _3
    (`KismetArrayLibrary.Array_Add` (`self.AllExtraGridMeshes`) _array_element_14))
  (for _array_element_15 _4
    (`KismetArrayLibrary.Array_Add` (`self.AllExtraGridMeshes`) _array_element_15))
  (for _array_element_16 _5
    (`KismetArrayLibrary.Array_Add` (`self.AllExtraGridMeshes`) _array_element_16))
  (for _array_element_17 _6
    (`KismetArrayLibrary.Array_Add` (`self.AllExtraGridMeshes`) _array_element_17))
  (for _array_element_18 _7
    (`KismetArrayLibrary.Array_Add` (`self.AllExtraGridMeshes`) _array_element_18))
  (for _array_element_19 _8
    (`KismetArrayLibrary.Array_Add` (`self.AllExtraGridMeshes`) _array_element_19))
  (for _array_element_20 _9
    (`KismetArrayLibrary.Array_Add` (`self.AllExtraGridMeshes`) _array_element_20))
  (for _array_element_21 _10
    (`KismetArrayLibrary.Array_Add` (`self.AllExtraGridMeshes`) _array_element_21)))

(fn `ConstructionPreVizMeshes`
  (locals (_currentIndex :type Integer) (_currentMesh :type "StaticMeshComponent Object Reference") (CurrentValue :type "Float (double-precision)" :default 0.0))
  ;[1 1 1] loop through meshes
  (for (_array_element _array_index) (`self.VizMeshes`)
    (set `local._currentMesh` _array_element)
    (set `local._currentIndex` _array_index)
    (bind _output_get (set `local.CurrentValue` (+ (* (`KismetMathLibrary.SelectFloat` (`KismetMathLibrary.RandomFloatInRange` 0.0 0.5) (`KismetMathLibrary.RandomFloatInRange` 0.5 1.0) (`KismetMathLibrary.RandomBoolWithWeight` 0.7)) (`self.MeshScaleMultiplier`)) (`self.MinimumSize`))))
    ;[1 1 1] set new mesh scale
    (`SceneComponent.SetRelativeScale3D` (`local._currentMesh`) (`KismetMathLibrary.MakeVector` 1.0 1.0 _output_get))
    ;[1 1 1] modify MID emissive multiplier value
    (`MaterialInstanceDynamic.SetScalarParameterValue` (`|GetArrayItem` (`self.MIDs`) (`local._currentIndex`)) (`self.MaterialParameterEmissiveMultiplier`) (* (`local.CurrentValue`) (`self.MaterialEmissiveMultiplier`)))))

(fn `DebugPrint`
  (params (`String part 1` :type String) (`String part 2` :type String) (`String part 3` :type String))
  (`KismetSystemLibrary.PrintString` (`KismetStringLibrary.Concat_StrStr` `String part 1` `String part 2` `String part 3`)))

(fn `InitializeDynamicMaterials`
  (locals (_currentIndex :type Integer) (_currentMesh :type "StaticMeshComponent Object Reference") (_latestRandomColor :type "LinearColor Structure"))
  (`KismetArrayLibrary.Array_Clear` (`self.MIDs`))
  ;[1 1 1] loop through meshes
  (for (_array_element _array_index) (`self.VizMeshes`)
    (`|ExecutionSequence`
      (:`then_0`
        ;[1 1 1] store local variables
        (set `local._currentMesh` _array_element)
        (set `local._currentIndex` _array_index))
      (:`then_1`
        ;[1 1 1] create dynamic materials(MIDs)
        (bind _returnvalue (`KismetMaterialLibrary.CreateDynamicMaterialInstance` (`self.BaseMaterial`)))
        (`KismetArrayLibrary.Array_Set` (`self.MIDs`) (`local._currentIndex`) _returnvalue true))
      (:`then_2`
        ;[1 1 1] put MIDs on meshes
        (`PrimitiveComponent.SetMaterial` (`local._currentMesh`) 0 (`|GetArrayItem` (`self.MIDs`) (`local._currentIndex`))))
      (:`then_3`
        ;[1 1 1] random color?
        (if (`self.RandomColors?`)
          ;[1 1 1] make color
          (bind _linearcolor (`self.MakeRandomColor`))
          (set `local._latestRandomColor` _linearcolor)
          ;[1 1 1] set colors on materials
          (`MaterialInstanceDynamic.SetVectorParameterValue` (`|GetArrayItem` (`self.MIDs`) (`local._currentIndex`)) (`self.MaterialParameterBaseColor`) (`local._latestRandomColor`)))))))

(fn `MakeRandomColor`
  (returns (LinearColor :type "LinearColor Structure"))
  (bind (_bvalue_x _bvalue_y) (`KismetMathLibrary.BreakVector2D` (`self.bValue`)))
  (bind (_rvalue_x _rvalue_y) (`KismetMathLibrary.BreakVector2D` (`self.rValue`)))
  (bind (_gvalue_x _gvalue_y) (`KismetMathLibrary.BreakVector2D` (`self.gValue`)))
  (return (make `LinearColor` (`KismetMathLibrary.RandomFloatInRange` _rvalue_x _rvalue_y) (`KismetMathLibrary.RandomFloatInRange` _gvalue_x _gvalue_y) (`KismetMathLibrary.RandomFloatInRange` _bvalue_x _bvalue_y))))

(fn `RescaleAllExtraRows`
  (bind _gridscaledividerstart (`self.GridScaleDividerStart`))
  (bind (__10 __9 __8 __7 __6 __5 __4 __3 __2 __1 _1 _2 _3 _4 _5 _6 _7 _8 _9 _10) (break `/Game/ArthursAudioBPs/WIP/GridBPspace/GridStruct20wide` (`self.GridStruct20`)))
  (bind _returnvalue (+ _gridscaledividerstart (`self.GridScaleDividerChangeVal`)))
  (bind _returnvalue_2 (+ _gridscaledividerstart (`self.GridScaleDividerChangeVal`)))
  (bind _returnvalue_3 (+ _returnvalue_2 (`self.GridScaleDividerChangeVal`)))
  (bind _returnvalue_4 (+ _returnvalue (`self.GridScaleDividerChangeVal`)))
  (bind _returnvalue_5 (+ _returnvalue_3 (`self.GridScaleDividerChangeVal`)))
  (bind _returnvalue_6 (+ _returnvalue_4 (`self.GridScaleDividerChangeVal`)))
  (bind _returnvalue_7 (+ _returnvalue_5 (`self.GridScaleDividerChangeVal`)))
  (bind _returnvalue_8 (+ _returnvalue_6 (`self.GridScaleDividerChangeVal`)))
  (bind _returnvalue_9 (+ _returnvalue_8 (`self.GridScaleDividerChangeVal`)))
  (bind _returnvalue_10 (+ _returnvalue_7 (`self.GridScaleDividerChangeVal`)))
  (bind _returnvalue_11 (+ _returnvalue_9 (`self.GridScaleDividerChangeVal`)))
  (bind _returnvalue_12 (+ _returnvalue_10 (`self.GridScaleDividerChangeVal`)))
  (bind _returnvalue_13 (+ _returnvalue_12 (`self.GridScaleDividerChangeVal`)))
  (bind _returnvalue_14 (+ _returnvalue_11 (`self.GridScaleDividerChangeVal`)))
  (bind _returnvalue_15 (+ _returnvalue_13 (`self.GridScaleDividerChangeVal`)))
  (bind _returnvalue_16 (+ _returnvalue_14 (`self.GridScaleDividerChangeVal`)))
  (bind _returnvalue_17 (+ _returnvalue_16 (`self.GridScaleDividerChangeVal`)))
  ;[1 1 1] rescale all rows
  (`self.ScaleARow` __10 (+ _returnvalue_17 (`self.GridScaleDividerChangeVal`)))
  (`self.ScaleARow` __9 _returnvalue_17)
  (`self.ScaleARow` __8 _returnvalue_16)
  (`self.ScaleARow` __7 _returnvalue_14)
  (`self.ScaleARow` __6 _returnvalue_11)
  (`self.ScaleARow` __5 _returnvalue_9)
  (`self.ScaleARow` __4 _returnvalue_8)
  (`self.ScaleARow` __3 _returnvalue_6)
  (`self.ScaleARow` __2 _returnvalue_4)
  (`self.ScaleARow` __1 _returnvalue)
  (`self.ScaleARow` _1 _gridscaledividerstart)
  (`self.ScaleARow` _2 _returnvalue_2)
  (`self.ScaleARow` _3 _returnvalue_3)
  (`self.ScaleARow` _4 _returnvalue_5)
  (`self.ScaleARow` _5 _returnvalue_7)
  (`self.ScaleARow` _6 _returnvalue_10)
  (`self.ScaleARow` _7 _returnvalue_12)
  (`self.ScaleARow` _8 _returnvalue_13)
  (`self.ScaleARow` _9 _returnvalue_15)
  (`self.ScaleARow` _10 (+ _returnvalue_15 (`self.GridScaleDividerChangeVal`))))

(fn `ScaleARow`
  (params (MeshArray :type "Array of StaticMeshComponent Object Reference") (DivideScaleBy :type "Float (double-precision)"))
  (for (_array_element _array_index) MeshArray
    (`SceneComponent.SetRelativeScale3D` _array_element (`KismetMathLibrary.MakeVector` (.x (`SceneComponent.RelativeScale3D` (`|GetArrayItem` (`self.VizMeshes`) _array_index))) (.y (`SceneComponent.RelativeScale3D` (`|GetArrayItem` (`self.VizMeshes`) _array_index))) (/ (.z (`SceneComponent.RelativeScale3D` (`|GetArrayItem` (`self.VizMeshes`) _array_index))) DivideScaleBy)))))

(fn `ScaleMeshes`
  (locals (_currentIndex :type Integer) (_currentMesh :type "StaticMeshComponent Object Reference"))
  ;[1 1 1] loop through meshes
  (for (_array_element _array_index) (`self.VizMeshes`)
    (set `local._currentMesh` _array_element)
    (set `local._currentIndex` _array_index)
    ;[1 1 1] set new mesh scale
    (`SceneComponent.SetRelativeScale3D` (`local._currentMesh`) (`KismetMathLibrary.MakeVector` 1.0 1.0 (+ (* (`|GetArrayItem` (`self.LatestSmoothValues`) (`local._currentIndex`)) (`self.MeshScaleMultiplier`)) (`self.MinimumSize`))))))

(fn `SpawnVisualizerMeshes`
  (locals (_currentIndex :type Integer))
  (bind _vizmeshes (`self.VizMeshes`))
  ;[1 1 1] clear out old existing meshes if any
  (for _array_element _vizmeshes
    (`ActorComponent.K2_DestroyComponent` _array_element))
  (`KismetArrayLibrary.Array_Clear` _vizmeshes)
  ;[1 1 1] loop through frequencies
  (for (_ _array_index) (`self.FrequenciesToAnalyze`)
    ;[1 1 1] spawn visualizer meshes in a row
    (set `local._currentIndex` _array_index)
    (bind _returnvalue (`AddComponent|NODE_AddStaticMeshComponent-0` :`RelativeTransform` (`KismetMathLibrary.MakeTransform` (`KismetMathLibrary.MakeVector` 0.0 (* (`local._currentIndex`) (`self.MeshRowDistanceOffset`))))))
    ;[1 1 1] store mesh references
    (`KismetArrayLibrary.Array_Set` (`self.VizMeshes`) (`local._currentIndex`) _returnvalue true))
  ;[1 1 1] attach to rootmesh
  (for _array_element_2 (`self.VizMeshes`)
    (`SceneComponent.K2_AttachToComponent` _array_element_2 (`self.StaticNoMesh`) "None" "KeepRelative" "KeepRelative" "KeepRelative" true)))

(fn `UpdateMaterialEmissive`
  ;[1 1 1] modify MID emissive multiplier value
  (for (_array_element _array_index) (`self.MIDs`)
    (`MaterialInstanceDynamic.SetScalarParameterValue` _array_element (`self.MaterialParameterEmissiveMultiplier`) (* (+ (`|GetArrayItem` (`self.LatestSmoothValues`) _array_index) (`self.MinimumEmissiveStrength`)) (`self.MaterialEmissiveMultiplier`)))))

(fn `UserConstructionScript`
  (bind _mids (`self.MIDs`))
  ;[1 1 1] get frequencies to analyze from SubmixAnalyzer
  (set `self.FrequenciesToAnalyze` (`/ArthursAudioVisualToolkit/Blueprints/AudioViz/BP_SubmixAnalyzer.FrequenciesToAnalyze` (`self.SubmixAnalyzerRef`)))
  ;[1 1 1] spawn visualizing meshes
  (`self.SpawnVisualizerMeshes`)
  ;[1 1 1] initialize dynamic materials(MIDs)
  (`self.InitializeDynamicMaterials`)
  ;[1 1 1] pre-viz scaling of meshes
  (`self.ConstructionPreVizMeshes`)
  ;[1 1 1] add rows on either side
  (`self.AddRowsOnEitherSide`)
  ;[1 1 1] create extra grid MIDs
  (for (_ _array_index) (`self.AllExtraGridMeshes`)
    (bind _returnvalue (`KismetMaterialLibrary.CreateDynamicMaterialInstance` (`self.BaseMaterial`)))
    (`KismetArrayLibrary.Array_Set` (`self.ExtraGridMIDs`) _array_index _returnvalue true))
  ;[1 1 1] copy colors over
  (for (_array_element _array_index_2) (`self.ExtraGridMIDs`)
    (bind _returnvalue_2 (`MaterialInstanceDynamic.K2_GetScalarParameterValue` (`|GetArrayItem` _mids (mod _array_index_2 (`KismetArrayLibrary.Array_LastIndex` _mids))) (`self.MaterialParameterBaseColor`)))
    (`MaterialInstanceDynamic.SetScalarParameterValue` _array_element (`self.MaterialParameterBaseColor`) _returnvalue_2))
  ;[1 1 1] put gridmaterials on grid
  (for (_array_element_2 _array_index_3) (`self.AllExtraGridMeshes`)
    (`PrimitiveComponent.SetMaterial` _array_element_2 0 (`|GetArrayItem` (`self.ExtraGridMIDs`) _array_index_3))))