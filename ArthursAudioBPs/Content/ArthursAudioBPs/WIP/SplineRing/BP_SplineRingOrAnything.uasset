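; Audio visualizer actor that animates a ring of meshes along a spline from a linked Beautifier's frequency analysis.
; The construction script spaces one spline point per analyzed frequency around a circle of Radius and spawns a mesh at each.
; Every tick, each band's smoothed, normalized value blends MeshBase toward MeshMax, displacing its spline point.
; Meshes then follow the reshaped spline, with the blended location, rotation and scale applied on top.
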(event `self.ReceiveBeginPlay`
  (`KismetArrayLibrary.Array_Clear` (`self.SpawnPointsVisualized`)))

(event `self.ReceiveTick`
  (params (DeltaSeconds :type "Float (single-precision)"))
  (`|ExecutionSequence`
    (:`then_0`
      (`self.SetSplinePoints`))
    (:`then_1`
      (`self.UpdateTransforms`))))

(fn `SetSplinePoints`
  (locals (SpawnPointsLocal :type "Array of Vector Structure"))
  (for (_array_element _array_index) (`self.SpawnPointsBase`)
    (`KismetArrayLibrary.Array_Add` (`local.SpawnPointsLocal`) (+ _array_element (.location (`KismetMathLibrary.TLerp` (`self.MeshBase`) (`self.MeshMax`) (`|GetArrayItem` (`/ArthursAudioVisualToolkit/Blueprints/AudioViz/BP_AnalysisBeautifier.FinalEnvelopeSmoothedNormalizedOutputValuesFromAnalysis` (`self.Beautifier`)) _array_index))))))
  (set `self.SpawnPointsVisualized` (`local.SpawnPointsLocal`))
  (`SplineComponent.SetSplinePoints` (`self.Spline`) (`self.SpawnPointsVisualized`) "Local" true))

(fn `UpdateTransforms`
  ;[1 1 1] UpdateTransforms
  (for (_array_element _array_index) (`self.VizMeshes`)
    (bind (_returnvalue_location _returnvalue_rotation _returnvalue_scale) (`KismetMathLibrary.BreakTransform` (`SplineComponent.GetTransformAtSplinePoint` (`self.Spline`) _array_index "Local" false)))
    (bind (_returnvalue_location_2 _returnvalue_rotation_2 _returnvalue_scale_2) (`KismetMathLibrary.BreakTransform` (`KismetMathLibrary.TLerp` (`self.MeshBase`) (`self.MeshMax`) (`|GetArrayItem` (`/ArthursAudioVisualToolkit/Blueprints/AudioViz/BP_AnalysisBeautifier.FinalEnvelopeSmoothedNormalizedOutputValuesFromAnalysis` (`self.Beautifier`)) _array_index))))
    (`SceneComponent.K2_SetRelativeTransform` _array_element (`KismetMathLibrary.MakeTransform` (+ _returnvalue_location _returnvalue_location_2) (`KismetMathLibrary.ComposeRotators` _returnvalue_rotation _returnvalue_rotation_2) (* _returnvalue_scale _returnvalue_scale_2)) false false)))

(fn `UserConstructionScript`
  (bind _frequenciestoanalyze (`/ArthursAudioVisualToolkit/Blueprints/AudioViz/BP_AnalysisBeautifier.FrequenciesToAnalyze` (`self.Beautifier`)))
  ;[1 1 1] valid beautifier?
  (`/Engine/EditorBlueprintResources/StandardMacros.IsValid` (`self.Beautifier`)
    (:`Is Valid`
      (`|ExecutionSequence`
        (:`then_0`
          ;[1 1 1 0.17] circlespawner
          (`SplineComponent.ClearSplinePoints` (`self.Spline`) false)
          (`KismetArrayLibrary.Array_Clear` (`self.SpawnPointsBase`))
          (for (_ _array_index) _frequenciestoanalyze
            (`KismetArrayLibrary.Array_Set` (`self.SpawnPointsBase`) _array_index (* (`KismetMathLibrary.GetForwardVector` (`KismetMathLibrary.MakeRotator` 0.0 0.0 (* (+ _array_index 1) (/ 360.0 (`KismetMathLibrary.Conv_IntToDouble` (`KismetArrayLibrary.Array_Length` _frequenciestoanalyze)))))) (`self.Radius`)) true))
          (for (_array_element _array_index_2) (`self.SpawnPointsBase`)
            (`SplineComponent.AddSplinePointAtIndex` (`self.Spline`) _array_element _array_index_2 "Local" false))
          (`SplineComponent.UpdateSpline` (`self.Spline`)))
        (:`then_1`
          ;[1 1 1] add meshes at spline points
          (`KismetArrayLibrary.Array_Clear` (`self.VizMeshes`))
          (for (_array_element_2 _array_index_3) (`self.SpawnPointsBase`)
            (bind _returnvalue (`AddComponent|NODE_AddStaticMeshComponent-0` :`RelativeTransform` (`KismetMathLibrary.MakeTransform` (+ _array_element_2 (.location (`self.MeshBase`))) (`KismetMathLibrary.ComposeRotators` (.rotation (`SplineComponent.GetTransformAtSplinePoint` (`self.Spline`) _array_index_3 "Local" false)) (.rotation (`self.MeshBase`))) (.scale (`self.MeshBase`)))))
            (`KismetArrayLibrary.Array_Set` (`self.VizMeshes`) _array_index_3 _returnvalue true)))
        (:`then_2`
          ;[1 1 1] set mesh models
          (for _array_element_3 (`self.VizMeshes`)
            (`StaticMeshComponent.SetStaticMesh` _array_element_3 (`self.MeshToUseForViz`))))))
    (:`Is Not Valid`
      (`KismetSystemLibrary.PrintString` (`KismetStringLibrary.Concat_StrStr` (`KismetSystemLibrary.GetDisplayName` self) " needs to be connected to a beautifier")))))