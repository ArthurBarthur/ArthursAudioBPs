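; BP_MusicMover is an audio-reactive prop with a moving head, driven by the average volume read from a referenced Beautifier.
; Each tick maps that volume to pan yaw, mover location, head scale and emissive glow.
; Tilt is gated instead: a timeline plays while volume is above zero and reverses otherwise, its rate set from a tilt duration.
; The construction script creates the head's tinted dynamic material.
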(event `self.ReceiveBeginPlay`
  (`TimelineComponent.SetPlayRate` (`self.Tilter`) (/ 1.0 (`self.TiltTimeInSec`))))

(event `self.ReceiveTick`
  (params (DeltaSeconds :type "Float (single-precision)"))
  (`|ExecutionSequence`
    (:`then_0`
      ;[1 1 1] get latest average vol from beautifier
      (if (> (`/ArthursAudioVisualToolkit/Blueprints/AudioViz/BP_AnalysisBeautifier.CurrentAverageVol01` (`self.BeautifierRef`)) 0.0)
        ;[1 1 1] tilt
        (bind (_direction _tilt) (`Timeline|Tilter` :!label _label)
          (:`Update`
            (`SceneComponent.K2_SetRelativeRotation` (`self.Tilt`) (`KismetMathLibrary.MakeRotator` _tilt) false false)))
        (else
          (goto _label :!via `Reverse`))))
    (:`then_1`
      ;[1 1 1] pan
      (`SceneComponent.K2_SetRelativeRotation` (`self.Pan`) (`KismetMathLibrary.MakeRotator` 0.0 0.0 (`KismetMathLibrary.MapRangeClamped` (`/ArthursAudioVisualToolkit/Blueprints/AudioViz/BP_AnalysisBeautifier.CurrentAverageVol01` (`self.BeautifierRef`)) 0.0 1.0 (`self.PanVolMin`) (`self.PanVolMax`))) false false))
    (:`then_2`
      ;[1 1 1] Move
      (`SceneComponent.K2_SetRelativeLocation` (`self.Move`) (`KismetMathLibrary.VLerp` (`self.MoverLocationVolMin`) (`self.MoverLocationVolMax`) (`/ArthursAudioVisualToolkit/Blueprints/AudioViz/BP_AnalysisBeautifier.CurrentAverageVol01` (`self.BeautifierRef`))) false false))
    (:`then_3`
      ;[1 1 1] Glow
      (`MaterialInstanceDynamic.SetScalarParameterValue` (`self.MID`) "Emissive Multiplier" (`KismetMathLibrary.MapRangeClamped` (`/ArthursAudioVisualToolkit/Blueprints/AudioViz/BP_AnalysisBeautifier.CurrentAverageVol01` (`self.BeautifierRef`)) 0.0 1.0 (`self.GlowMin`) (`self.GlowMax`))))
    (:`then_4`
      (`SceneComponent.SetRelativeScale3D` (`self.StaticMeshMove(head)`) (`KismetMathLibrary.VLerp` (`self.HeadScaleMin`) (`self.HeadScaleMax`) (`/ArthursAudioVisualToolkit/Blueprints/AudioViz/BP_AnalysisBeautifier.CurrentAverageVol01` (`self.BeautifierRef`)))))))

(fn `UserConstructionScript`
  (bind _returnvalue (`PrimitiveComponent.CreateDynamicMaterialInstance` (`self.StaticMeshMove(head)`) 0 (`self.BaseForMID`) "None"))
  (bind _output_get (set `self.MID` _returnvalue))
  (`MaterialInstanceDynamic.SetVectorParameterValue` _output_get "Base Color" (`self.MIDcolor`)))