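; BP_MusicMover2 is an audio-reactive actor that moves and glows with the volume reported by a referenced Beautifier.
; Each tick, the Beautifier's current normalized average volume serves as the time along a spline to set the mesh's relative location.
; The same value drives the emissive multiplier between GlowMin and GlowMax.
; The construction script creates the mesh's dynamic material instance and applies its base color.
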(event `self.ReceiveTick`
  (params (DeltaSeconds :type "Float (single-precision)"))
  (`|ExecutionSequence`
    (:`then_0`
      ;[1 1 1] transform along spline
      (`SceneComponent.K2_SetRelativeTransform` (`self.StaticMeshTilt(body)`) (`KismetMathLibrary.MakeTransform` (`SplineComponent.GetLocationAtTime` (`self.Spline`) (`/ArthursAudioVisualToolkit/Blueprints/AudioViz/BP_AnalysisBeautifier.CurrentAverageVol01` (`self.BeautifierRef`)) "Local" false)) false false))
    (:`then_1`
      ;[1 1 1] Glow
      (`MaterialInstanceDynamic.SetScalarParameterValue` (`self.MID`) "Emissive Multiplier" (`KismetMathLibrary.MapRangeClamped` (`/ArthursAudioVisualToolkit/Blueprints/AudioViz/BP_AnalysisBeautifier.CurrentAverageVol01` (`self.BeautifierRef`)) 0.0 1.0 (`self.GlowMin`) (`self.GlowMax`))))))

(fn `UserConstructionScript`
  (bind _returnvalue (`PrimitiveComponent.CreateDynamicMaterialInstance` (`self.StaticMeshTilt(body)`) 0 (`self.BaseForMID`) "None"))
  (bind _output_get (set `self.MID` _returnvalue))
  (`MaterialInstanceDynamic.SetVectorParameterValue` _output_get "Base Color" (`self.MIDcolor`)))