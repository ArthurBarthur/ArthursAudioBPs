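; BP_MidiInput is an actor that routes external MIDI keyboard input to instruments placed in the level.
; On BeginPlay it finds a MIDI input device by name, binds note on/off events and caches every actor implementing AabpsMidiInterface.
; Notes are forwarded to those actors as play and stop interface messages, with note-on also printed.
; The R key re-initializes any cached BP_modularSynth to change its preset.
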(event `self.ReceiveBeginPlay`
  ;[1 1 1] set up default midi device
  (bind (_foundvalidmidiinputdevice _midideviceinputcontroller) (`/Game/ArthursAudioBPs/Core/FunctionLibraries/AabpsMidiDeviceFinder.FindMidiDevices` (`self.Midi Device Input Name Contains`) (`self.Midi Device Output Name Contains`) (`self.Print Debug Info`)))
  (if _foundvalidmidiinputdevice
    (bind _output_get (set `self.MidiController` _midideviceinputcontroller))
    ;[1 1 1] set up midi events
    (add `MIDIDeviceInputController.OnMIDINoteOn` _output_get (delegate `OnMIDINoteOn_Event_0`))
    (add `MIDIDeviceInputController.OnMIDINoteOff` _output_get (delegate `OnMIDINoteOff_Event_0`))
    ;[1 1 1] find all actors in level with midi interface
    (bind _outactors (`GameplayStatics.GetAllActorsWithInterface` "/Game/ArthursAudioBPs/Core/Interfaces/AabpsMidiInterface.AabpsMidiInterface_C"))
    (set `self.ActorsInLevelWithMidiInterface` _outactors)
    ;[1 1 1] enable input "R" to change preset
    (`self.EnableInput` (`GameplayStatics.GetPlayerController` 0))))

(event `Key|R`
  (params (Key :type "Key Structure"))
  ;[1 1 1] enable input "R" to change preset
  (:`Pressed`
    (for _array_element (`self.ActorsInLevelWithMidiInterface`)
      (bind _asbp_modular_synth (cast `/Game/ArthursAudioBPs/Core/Blueprints/ModSynth/BP_modularSynth` _array_element))
      (`/Game/ArthursAudioBPs/Core/Blueprints/ModSynth/BP_modularSynth.InitSynth` _asbp_modular_synth))))

(event `OnMIDINoteOn_Event_0`
  (params (MIDIDeviceController :type "MIDIDeviceInputController Object Reference") (Timestamp :type Integer) (Channel :type Integer) (Note :type Integer) (Velocity :type Integer))
  ;[1 1 1] midi events
  ;[1 1 1] note on
  (`KismetSystemLibrary.PrintString` (`KismetStringLibrary.Concat_StrStr` "Note: " (`KismetStringLibrary.Conv_IntToString` Note) " Velocity: " (`KismetStringLibrary.Conv_IntToString` Velocity)))
  (for _array_element (`self.ActorsInLevelWithMidiInterface`)
    (message `/Game/ArthursAudioBPs/Core/Interfaces/AabpsMidiInterface.NotePlay` _array_element (`KismetMathLibrary.Conv_IntToDouble` Note) Velocity -1.0 Channel)))

(event `OnMIDINoteOff_Event_0`
  (params (MIDIDeviceController :type "MIDIDeviceInputController Object Reference") (Timestamp :type Integer) (Channel :type Integer) (Note :type Integer) (Velocity :type Integer))
  ;[1 1 1] midi events
  ;[1 1 1] note off
  (for _array_element (`self.ActorsInLevelWithMidiInterface`)
    (message `/Game/ArthursAudioBPs/Core/Interfaces/AabpsMidiInterface.NoteStop` _array_element (`KismetMathLibrary.Conv_IntToDouble` Note) false Channel)))

(fn `UserConstructionScript`)