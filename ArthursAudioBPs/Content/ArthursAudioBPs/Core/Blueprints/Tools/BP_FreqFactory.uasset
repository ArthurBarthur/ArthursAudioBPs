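; BP_FreqFactory is a helper actor that generates a list of musically spaced audio frequencies, packed tightly at low Hz and spread out at high Hz.
; UpdateFrequenciesCalculation starts at the clamped high end of the range and repeatedly divides by a clamped spacing factor until reaching the low bound, giving geometric spacing.
; The Freqs array is then reversed into ascending order and printed as a joined string.
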(event `UpdateFrequenciesCalculation`
  ;[1 1 1] This is a helper actor that can generate a bunch of freqiecneis between 0-20000 hz, that make musical sense. We need space between freqs at high values, and we need very tight packing of freqs at low values(of hz), so this thing does that. Generates as many freqs as we want, at the scaling we want.
  (`self.MakeABunchOfFrequencies`))

(fn `MakeABunchOfFrequencies`
  ;[1 1 1] prepare
  (`KismetArrayLibrary.Array_Clear` (`self.Freqs`))
  (set `self.latest` (`KismetMathLibrary.FClamp` (`self.FreqRangeHigh`) (`self.FreqRangeLow`) 20000.0))
  ;[1 1 1] add latest
  (`KismetArrayLibrary.Array_Add` (`self.Freqs`) (`self.latest`) :!label _label)
  ;[1 1 1] decrease it
  (bind _output_get (set `self.latest` (/ (stale _output_get) (`KismetMathLibrary.FClamp` (`self.FactorOfSpacing`) 1.005 32.0))))
  ;[1 1 1] are we through yet?
  (if (> (`self.latest`) (`KismetMathLibrary.FClamp` (`self.FreqRangeLow`) 20.0 (`self.FreqRangeHigh`)))
    (goto _label)
    (else
      (`self.ReverseArray`)
      ;[1 1 1] print list of freqs
      (`KismetArrayLibrary.Array_Clear` (`self.StringArray`))
      (for _array_element (`self.Freqs`)
        (`KismetArrayLibrary.Array_Add` (`self.StringArray`) (`KismetStringLibrary.Conv_DoubleToString` _array_element)))
      (`KismetSystemLibrary.PrintString` (`KismetStringLibrary.JoinStringArray` (`self.StringArray`) " \n")))))

(fn `ReverseArray`
  (locals (_freqs :type "Array of Float (double-precision)") (_freqsReversed :type "Array of Float (double-precision)"))
  (bind _output_get (set `local._freqs` (`self.Freqs`)))
  (bind (_arrayindex _arrayelement) (`/Engine/EditorBlueprintResources/StandardMacros.ReverseForEachLoop` _output_get)
    (:`LoopBody`
      (`KismetArrayLibrary.Array_Add` (`local._freqsReversed`) _arrayelement))
    (:`Completed`
      (set `self.Freqs` (`local._freqsReversed`)))))

(fn `UserConstructionScript`)