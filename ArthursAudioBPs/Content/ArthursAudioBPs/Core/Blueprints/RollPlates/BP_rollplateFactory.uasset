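; BP_rollplateFactory builds a row of musical rollplates and assigns each a note from a chord.
; The construction script spawns evenly spaced BP_rollplate child actors and passes them the note-interfaced actor reference, color, emissive maximum and physical material override.
; Shortly after BeginPlay, it builds MIDI notes from the chord settings.
; Plates receive either random notes or sequential ones that wrap around the list, optionally in reversed plate order.
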(event `self.ReceiveBeginPlay`
  ;[1 1 1] beginplay
  (`KismetSystemLibrary.Delay` 0.5)
  ;[1 1 1] shuffle?
  (if (`self.ShuffledNotes`)
    ;[1 1 1] shuffle.
    (`self.SetRandomNoteOnPlates`)
    (else
      ;[1 1 1] in orderly fashion
      (`self.SetScaleNoteOnPlates`))))

(fn `SetRandomNoteOnPlates`
  (locals (_latestRollplate :type "/Game/ArthursAudioBPs/Core/Blueprints/RollPlates/BP_rollplate Object Reference") (ChordNotes :type "Array of Float (double-precision)"))
  ;[1 1 1] get list of notes
  (set `local.ChordNotes` (`/ArthursAudioVisualToolkit/FunctionLibraries/AabpsMidiChordGenerator/AabpsMidiChordGenerator.BuildMusicalMidiChord` (`self.ChordSettings`)))
  ;[1 1 1] choose random notes and put on plates
  (for _array_element (`self.RollPlates`)
    (set `local._latestRollplate` _array_element)
    (set `/Game/ArthursAudioBPs/Core/Blueprints/RollPlates/BP_rollplate.NoteToPlay` (`|GetArrayItem` (`local.ChordNotes`) (`KismetMathLibrary.RandomIntegerInRange` 0 (`KismetArrayLibrary.Array_LastIndex` (`local.ChordNotes`)))) (`local._latestRollplate`))))

(fn `SetScaleNoteOnPlates`
  (locals (_latestRollplate :type "/Game/ArthursAudioBPs/Core/Blueprints/RollPlates/BP_rollplate Object Reference") (_CurrentNoteIndex :type Integer :default 0) (ChordNotes :type "Array of Float (double-precision)"))
  (bind _rollplates (`self.RollPlates`))
  ;[1 1 1] get list of notes
  (set `local.ChordNotes` (`/ArthursAudioVisualToolkit/FunctionLibraries/AabpsMidiChordGenerator/AabpsMidiChordGenerator.BuildMusicalMidiChord` (`self.ChordSettings`)))
  ;[1 1 1] reverse?
  (if (`self.ReverseNoteOrder`)
    (bind (_arrayindex _arrayelement) (`/Engine/EditorBlueprintResources/StandardMacros.ReverseForEachLoop` _rollplates)
      (:`LoopBody`
        (set `local._latestRollplate` _arrayelement)
        ;[1 1 1] set note on plate
        (set `/Game/ArthursAudioBPs/Core/Blueprints/RollPlates/BP_rollplate.NoteToPlay` (`|GetArrayItem` (`local.ChordNotes`) (`local._CurrentNoteIndex`)) (`local._latestRollplate`) :!label _label)
        ;[1 1 1] start from beginning of notelist again if we run out of notes
        (bind _result (`/Engine/EditorBlueprintResources/StandardMacros.IncrementInt` (`local._CurrentNoteIndex`))
          (:`  `
            (if (> _result (`KismetArrayLibrary.Array_LastIndex` (`local.ChordNotes`)))
              (set `local._CurrentNoteIndex` 0))))))
    (else
      (for _array_element _rollplates
        (set `local._latestRollplate` _array_element)
        (goto _label)))))

(fn `UserConstructionScript`
  ;[1 1 1] spawn child actors(to be rollplates)
  (`KismetArrayLibrary.Array_Clear` (`self.ChildActors`))
  (for _index (range 1 (+ (`self.NumberOfRollplates`) 1))
    (bind _returnvalue (`AddComponent|NODE_AddChildActorComponent-2` :`RelativeTransform` (`KismetMathLibrary.MakeTransform` (`KismetMathLibrary.MakeVector` (* _index (`self.Spacing`))))))
    (`KismetArrayLibrary.Array_Add` (`self.ChildActors`) _returnvalue))
  ;[1 1 1] turn them into rollplates and store them
  (for _array_element (`self.ChildActors`)
    (`ChildActorComponent.SetChildActorClass` _array_element "/Game/ArthursAudioBPs/Core/Blueprints/RollPlates/BP_rollplate.BP_rollplate_C"))
  (for _array_element_2 (`self.ChildActors`)
    (bind _asbp_rollplate (cast `/Game/ArthursAudioBPs/Core/Blueprints/RollPlates/BP_rollplate` (`ChildActorComponent.ChildActor` _array_element_2)))
    (`KismetArrayLibrary.Array_Add` (`self.RollPlates`) _asbp_rollplate))
  ;[1 1 1] do stuff to our rollplates
  (for _array_element_3 (`self.RollPlates`)
    (set `/Game/ArthursAudioBPs/Core/Blueprints/RollPlates/BP_rollplate.NoteInterfacedActorRef` (`self.NoteInterfacedActorRef`) _array_element_3))
  (for _array_element_4 (`self.RollPlates`)
    (`/Game/ArthursAudioBPs/Core/Blueprints/RollPlates/BP_rollplate.SetMIDColor` _array_element_4 (`self.Color`)))
  (for _array_element_5 (`self.RollPlates`)
    (set `/Game/ArthursAudioBPs/Core/Blueprints/RollPlates/BP_rollplate.EmissiveMax` (`self.EmissiveMax`) _array_element_5))
  (for _array_element_6 (`self.RollPlates`)
    (`PrimitiveComponent.SetPhysMaterialOverride` (`/Game/ArthursAudioBPs/Core/Blueprints/RollPlates/BP_rollplate.StaticMesh` _array_element_6) (`self.PhysMatOverride`))))