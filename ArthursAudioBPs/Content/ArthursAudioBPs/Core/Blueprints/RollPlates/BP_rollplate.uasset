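; Roll plate actor that plays a MIDI note and glows when a non-plate object overlaps its box.
; The object's peak-axis speed maps to note velocity, using custom bounds or an auto-tracked maximum, then goes to a note-interface actor, with a short retrigger debounce.
; Velocity drives dynamic material emissive, which jumps on hit and interpolates down on Tick after end overlap stops the note.
; Optional text components display velocity debug values.
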(event `self.ReceiveBeginPlay`
  ;[1 1 1] beginPlay
  ;[1 1 1] set color on material
  (`self.SetMIDColor` (`self.Color`))
  ;[1 1 1] GetNoteToPlay
  (set `self.NoteToPlay` (`|GetArrayItem` (`/ArthursAudioVisualToolkit/FunctionLibraries/AabpsMidiChordGenerator/AabpsMidiChordGenerator.BuildMusicalMidiChord` (`self.NoteSettings`))))
  ;[1 0.5589 0.2618] debugstuff
  (if (`self.debug`)
    (`self.AddDebugTextComponents`)))

(event `self.ReceiveTick`
  (params (DeltaSeconds :type "Float (single-precision)"))
  ;[1 1 1] tick
  (set `self.LatestDelta` DeltaSeconds)
  ;[1 1 1] lerp emissive towards target
  (`self.LerpTowardsEmissiveTarget` (`self.MID`)))

(event `self.Box.OnComponentBeginOverlap`
  (params (OverlappedComponent :type "PrimitiveComponent Object Reference") (OtherActor :type "Actor Object Reference") (OtherComp :type "PrimitiveComponent Object Reference") (OtherBodyIndex :type Integer) (bFromSweep :type Boolean) (SweepResult :type "HitResult Structure (by ref)"))
  (bind _maxdetectedphysvelocity (`self.MaxDetectedPhysVelocity`))
  (bind _latestphysvelocity (`self.latestPhysVelocity`))
  ;[1 1 1] begin overlap
  ;[1 1 1] proceed if its not another roll-plate
  (if (!= OtherActor "BP_rollplate")
    (`/Engine/EditorBlueprintResources/StandardMacros.DoOnce` false :!label _label
      (:`Completed`
        (`|ExecutionSequence`
          (:`then_0`
            ;[1 1 1] get phys
            (set `self.latestPhysVelocity` (`KismetMathLibrary.Vector_GetAbsMax` (`SceneComponent.GetComponentVelocity` OtherComp)))
            ;[1 1 1] store max velocity
            (set `self.MaxDetectedPhysVelocity` (select `bool` (< _latestphysvelocity _maxdetectedphysvelocity) :`false` _latestphysvelocity :`true` _maxdetectedphysvelocity))
            (if (`self.CustomPhysToMidiVelocityMapping`)
              ;[1 1 1] CUSTOM Phys to Midi Velocity mapping
              (set `self.FinalVelocity` (`KismetMathLibrary.Round` (`KismetMathLibrary.FClamp` (`KismetMathLibrary.MapRangeClamped` (`self.latestPhysVelocity`) (`self.CustomMinPhysVelocity`) (`self.CustomMaxPhysVelocity`) (`self.NoteVelocityMin`) (`self.NoteVelocityMax`)) 0.0 127.0)))
              (else
                ;[1 1 1] AUTO Phys to Midi Velocity mapping
                (set `self.FinalVelocity` (`KismetMathLibrary.Round` (`KismetMathLibrary.FClamp` (`KismetMathLibrary.MapRangeClamped` (`self.latestPhysVelocity`) 0.0 (`self.MaxDetectedPhysVelocity`) (`self.NoteVelocityMin`) (`self.NoteVelocityMax`)) 0.0 127.0)))))
            ;[1 1 1] call note interface
            (message `/ArthursAudioVisualToolkit/Interfaces/AabpsMidiInterface.NotePlay` (`self.NoteInterfacedActorRef`) (`self.NoteToPlay`) (`self.FinalVelocity`) -1.0 0)
            ;[1 1 1] calc final emissive
            (`self.CalcFinalEmissive`)
            (`|ExecutionSequence`
              (:`then_0`
                ;[1 1 1] enable lerping
                (`/Engine/EditorBlueprintResources/StandardMacros.DoOnce` false
                  (:`Completed`
                    (`self.SetActorTickEnabled` true))))
              (:`then_1`
                ;[1 1 1] straight to max emissive
                (bind _output_get (set `self.EmissiveCurrent` (`self.EmissiveFinal`)))
                (`MaterialInstanceDynamic.SetScalarParameterValue` (`self.MID`) "Emissive Multiplier" _output_get)
                (`self.UpdateDebug`))))
          (:`then_1`
            (`KismetSystemLibrary.Delay` 0.1)
            (goto _label :!via `Reset`)))))))

(event `self.Box.OnComponentEndOverlap`
  (params (OverlappedComponent :type "PrimitiveComponent Object Reference") (OtherActor :type "Actor Object Reference") (OtherComp :type "PrimitiveComponent Object Reference") (OtherBodyIndex :type Integer))
  ;[1 1 1] end overlap
  ;[1 1 1] proceed if its not another roll-plate
  (if (!= null "BP_rollplate")
    (set `self.latestPhysVelocity` 0.0)
    ;[1 1 1] call note interface
    (message `/ArthursAudioVisualToolkit/Interfaces/AabpsMidiInterface.NoteStop` (`self.NoteInterfacedActorRef`) (`self.NoteToPlay`) false 0)
    (set `self.FinalVelocity` 0)
    ;[1 1 1] calc final emissive
    (`self.CalcFinalEmissive`)
    ;[1 1 1] slowly to min emissive
    (set `self.EmissiveInterpSpeed` (/ (`self.EmissiveMax`) 2.0))
    (`self.UpdateDebug`)))

(fn `AddDebugTextComponents`
  (locals (_currentIndex :type Integer) (_currentTextComp :type "TextRenderComponent Object Reference"))
  (for (_ _array_index) (`self.DebugInfos`)
    (bind _output_get (set `local._currentIndex` _array_index))
    (bind _returnvalue (`AddComponent|NODE_AddTextRenderComponent-1` :`RelativeTransform` (`KismetMathLibrary.MakeTransform` (`KismetMathLibrary.MakeVector` 0.0 0.0 (+ (* _output_get 30.0) 30.0)) (struct) (0.25 0.25 0.25))))
    (bind _output_get_2 (set `local._currentTextComp` _returnvalue))
    (`TextRenderComponent.K2_SetText` _output_get_2 (`KismetTextLibrary.Conv_StringToText` (`|GetArrayItem` (`self.DebugInfos`) (`local._currentIndex`))))
    (`KismetArrayLibrary.Array_Set` (`self.DebugTexts`) (`local._currentIndex`) (`local._currentTextComp`) true)))

(fn `CalcFinalEmissive`
  ;[1 1 1] calcFinalEmissive
  (set `self.EmissiveFinal` (`KismetMathLibrary.MapRangeClamped` (`KismetMathLibrary.Conv_IntToDouble` (`self.FinalVelocity`)) 0.0 127.0 (`self.EmissiveMin`) (`self.EmissiveMax`))))

(fn `LerpTowardsEmissiveTarget`
  (params (Target :type "MaterialInstanceDynamic Object Reference"))
  (set `self.EmissiveCurrent` (`KismetMathLibrary.FInterpTo_Constant` (`self.EmissiveCurrent`) (`self.EmissiveFinal`) (`self.LatestDelta`) (`self.EmissiveInterpSpeed`)))
  (`MaterialInstanceDynamic.SetScalarParameterValue` Target "Emissive Multiplier" (`self.EmissiveCurrent`)))

(fn `SetMIDColor`
  (params (Color :type "LinearColor Structure"))
  ;[1 1 1] set material Color
  (bind _output_get (set `self.Color` Color))
  (`MaterialInstanceDynamic.SetVectorParameterValue` (`self.MID`) "Base Color" _output_get))

(fn `UpdateDebug`
  ;[1 1 1] UpdateDebug
  (`self.UpdateDebugTextEntries`)
  (`self.UpdateDebugTextComps`))

(fn `UpdateDebugTextComps`
  (for (_array_element _array_index) (`self.DebugTexts`)
    (`TextRenderComponent.K2_SetText` _array_element (`KismetTextLibrary.Conv_StringToText` (`|GetArrayItem` (`self.DebugInfos`) _array_index)))))

(fn `UpdateDebugTextEntries`
  ;[1 0.5589 0.2618] debugstuff
  (if (`self.debug`)
    (`KismetArrayLibrary.Array_Set` (`self.DebugInfos`) 0 (`KismetStringLibrary.Concat_StrStr` "MaxRecordedPhysVelocity " (`KismetStringLibrary.Conv_DoubleToString` (`self.MaxDetectedPhysVelocity`))))
    (`KismetArrayLibrary.Array_Set` (`self.DebugInfos`) 1 (`KismetStringLibrary.Concat_StrStr` "CurrentPhysVelocity " (`KismetStringLibrary.Conv_DoubleToString` (`self.latestPhysVelocity`))))
    (`KismetArrayLibrary.Array_Set` (`self.DebugInfos`) 2 (`KismetStringLibrary.Concat_StrStr` "CurrentMidiVelocity" (`KismetStringLibrary.Conv_IntToString` (`self.FinalVelocity`))))
    (`self.UpdateDebugTextComps`)))

(fn `UserConstructionScript`
  ;[1 1 1] create material
  (bind _returnvalue (`KismetMaterialLibrary.CreateDynamicMaterialInstance` "/Game/ArthursAudioBPs/MaterialLibrary/Simple/MI_SimpleMat_Inst1.MI_SimpleMat_Inst1"))
  (set `self.MID` _returnvalue)
  ;[1 1 1] set material Color
  (`self.SetMIDColor` (`self.Color`))
  ;[1 1 1] set material
  (`PrimitiveComponent.SetMaterial` (`self.StaticMesh`) 0 (`self.MID`))
  ;[1 1 1] set physMat
  (`PrimitiveComponent.SetPhysMaterialOverride` (`self.StaticMesh`) (`self.PhysMat`)))