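; Garden spawner actor that scatters BP_SynthPlant instances around itself and manages their lifetime.
; The spawnerButton event spawns a set number at random XY offsets, passing shared chord, note length, attenuation and sound propagation settings plus a random velocity.
; Spawned plants are tracked in an array, pruned of invalid references before each spawn or DespawnAll, which destroys them all.
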(event `spawnerButton`
  ;[1 1 1] spawn plants
  (`|ExecutionSequence`
    (:`then_0`
      (`self.ClearOldInvalidPlantsReferences`))
    (:`then_1`
      (for _ (range (`self.NumberOfSpawns`))
        (bind _returnvalue (`|SpawnActorFromClass` "/ArthursAudioVisualToolkit/Blueprints/SynthPlant/BP_SynthPlant.BP_SynthPlant_C" (`KismetMathLibrary.MakeTransform` (+ (`SceneComponent.K2_GetComponentLocation` (`self.DefaultSceneRoot`)) (`KismetMathLibrary.MakeVector` (`KismetMathLibrary.RandomFloatInRange` (`self.SpawnAreaRange1`) (`self.SpawnAreaRange2`)) (`KismetMathLibrary.RandomFloatInRange` (`self.SpawnAreaRange1`) (`self.SpawnAreaRange2`))))) "Undefined" "OverrideRootScale" null "/Engine/BasicShapes/Cone.Cone" (`self.RandomPresetType`) (`self.ChordSettings`) (`self.PlaySingleRandomNotePerPlant`) (`self.UseRootNoteOnly`) (`KismetMathLibrary.RandomIntegerInRange` (`self.VelocityMin`) (`self.VelocityMax`)) (`self.NoteLengthPerTrigger`) (`self.AttenuationSettings`) (`self.SimulateSoundPropagation`) 30.0 "0.000000,0.000000,50.000000|0.000000,0.000000,0.000000|1.000000,1.000000,1.000000" "0.000000,0.000000,75.000000|0.000000,0.000000,0.000000|1.500000,1.500000,1.500000" "ECR_Overlap" null))
        (`KismetArrayLibrary.Array_Add` (`self.Plants`) _returnvalue)))))

(event `DespawnAll`
  (bind _plants (`self.Plants`))
  ;[1 1 1] despawn plants
  (`self.ClearOldInvalidPlantsReferences`)
  (for _array_element _plants
    (`self.K2_DestroyActor` _array_element))
  (`KismetArrayLibrary.Array_Clear` _plants))

(fn `ClearOldInvalidPlantsReferences`
  (locals (ValidRefs :type "Array of Integer") (ValidPlants :type "Array of /ArthursAudioVisualToolkit/Blueprints/SynthPlant/BP_SynthPlant Object Reference"))
  (for _array_element (`self.Plants`)
    (`/Engine/EditorBlueprintResources/StandardMacros.IsValid` _array_element
      (:`Is Valid`
        (`KismetArrayLibrary.Array_Add` (`local.ValidPlants`) _array_element))))
  (set `self.Plants` (`local.ValidPlants`)))

(fn `UserConstructionScript`)