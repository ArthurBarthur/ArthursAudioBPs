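; BP_synthBallFactoryTHX is a timed spawner that drops BP_SynthBallTHX synth balls from its location.
; It drops one shortly after BeginPlay, repeats on a looping timer, and expires after a set lifespan.
; Unless the floor height is overridden, a downward trace finds it before each drop.
; Each ball receives chord, preset, attenuation and height-to-semitone bend ranges, then gets its own lifespan.
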(event `self.ReceiveBeginPlay`
  (`KismetSystemLibrary.Delay` 0.2)
  (`|ExecutionSequence`
    (:`then_0`
      ;[1 1 1] repeating loop
      (`KismetSystemLibrary.K2_SetTimerDelegate` (`|CreateDelegate` :!event `dropppp`) (`self.DropTimer`) true))
    (:`then_1`
      (`self.SetLifeSpan` (`self.TimeBeforeStopping`)))
    (:`then_2`
      ;[1 1 1] override floor z lvl
      (if (not (`self.OverrideFloorZlvl`)) :!label _label
        ;[1 1 1] find distance to ground
        (`self.FindDistanceToGround`))
      ;[1 1 1] drop ball
      (bind _spawned (`self.DropBall`))
      (set `self.Latest` _spawned)
      ;[1 1 1] set ball to self-destruct later
      (`self.SetLifeSpan` (`self.Latest`) (`self.TimeToLive`)))))

(event `dropppp`
  (goto _label))

(fn `DropBall`
  (returns (Spawned :type "/Game/ArthursAudioBPs/Core/Blueprints/ModSynth/BP_SynthBallTHX Object Reference"))
  (bind (_returnvalue_x _returnvalue_y _returnvalue_z) (`KismetMathLibrary.BreakVector` (`SceneComponent.K2_GetComponentLocation` (`self.DefaultSceneRoot`))))
  ;[1 1 1] drop ball
  (bind _returnvalue (`|SpawnActorFromClass` "/Game/ArthursAudioBPs/Core/Blueprints/ModSynth/BP_SynthBallTHX.BP_SynthBallTHX_C" (`SceneComponent.K2_GetComponentToWorld` (`self.DefaultSceneRoot`)) "Undefined" "OverrideRootScale" null (`self.ChordSettings`) true false (`self.PhysMatOverride`) (`KismetMathLibrary.SelectFloat` (`self.DistanceToFloorOverride`) (- _returnvalue_z (`self.FloorZlvlOverride`)) (`self.OverrideFloorZlvl`)) (+ (`self.FloorZlvlOverride`) 50.0) (`self.SemitoneBendAtDropPoint`) (`self.SemitoneBendAtFloor`) (`self.BaseSynthPreset`) (`self.RandomPresetOverride`) 666 true (`self.RandomSynthPresetType`) (`self.AttenuationSettings`) null))
  (return _returnvalue))

(fn `FindDistanceToGround`
  (locals (_hitResult :type "HitResult Structure"))
  (bind _returnvalue (`SceneComponent.K2_GetComponentLocation` (`self.DefaultSceneRoot`)))
  ;[1 1 1] trace down to get distance to ground
  (bind (_outhit _returnvalue_2) (`KismetSystemLibrary.LineTraceSingleForObjects` :`Start` _returnvalue :`End` (- _returnvalue (0.0 0.0 100000000.0)) :`ObjectTypes` (`|MakeArray` "ObjectTypeQuery1" :!type "EObjectTypeQuery Enum") :`DrawDebugType` "ForDuration"))
  (set `local._hitResult` _outhit)
  (if _returnvalue_2
    ;[1 1 1] store floor Z lvl at drop
    (set `self.FloorZlvlOverride` (.z (`.Location` (`GameplayStatics.BreakHitResult` (`local._hitResult`)))))
    ;[1 1 1] store distance to floor
    (set `self.DistanceToFloorOverride` (`.Distance` (`GameplayStatics.BreakHitResult` (`local._hitResult`))))
    (return)))

(fn `UserConstructionScript`)