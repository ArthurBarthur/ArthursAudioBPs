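; BP_ChordPlate is a physical plate that plays a synthesized musical chord when struck.
; On begin play it sets its physical material, loads a ModularSynth preset from the bank or an override, and builds MIDI notes from the chord settings.
; Each hit plays every note with velocity mapped from impulse strength, while a timeline scaled to note duration drives an emissive fade on a dynamic material.
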(event `self.ReceiveBeginPlay`
  ;[1 1 1] set physMat
  (`PrimitiveComponent.SetPhysMaterialOverride` (`self.StaticMesh`) (`self.PhysicalMaterial`))
  ;[1 1 1] create dynamic material(MID)
  (bind _returnvalue (`PrimitiveComponent.CreateDynamicMaterialInstance` (`self.StaticMesh`) 0 "/Game/ArthursAudioBPs/MaterialLibrary/Simple/MI_SimpleMat_Inst7.MI_SimpleMat_Inst7" "None"))
  (set `self.MID` _returnvalue)
  ;[1 1 1] Init synth preset
  (bind _output_get (set `self.BankPresets` (`ModularSynthPresetBank.Presets` (`self.PresetBank`))))
  (`ModularSynthComponent.SetSynthPreset` (`self.ModularSynth`) (select `bool` (`self.OverridePreset`) :`false` (`.Preset` (break `ModularSynthPresetBankEntry` (`|GetArrayItem` _output_get (`self.CurrentBankPreset`)))) :`true` (`self.SynthPreset`)))
  ;[1 1 1] build chord
  (set `self.MidiNotes` (`/ArthursAudioVisualToolkit/FunctionLibraries/AabpsMidiChordGenerator/AabpsMidiChordGenerator.BuildMusicalMidiChord` (`self.ChordSettings`))))

(event `self.StaticMesh.OnComponentHit`
  (params (HitComponent :type "PrimitiveComponent Object Reference") (OtherActor :type "Actor Object Reference") (OtherComp :type "PrimitiveComponent Object Reference") (NormalImpulse :type "Vector Structure") (Hit :type "HitResult Structure (by ref)"))
  (`self.MidOnAndFadeOut`)
  ;[1 1 1] Notes on
  (for _array_element (`self.MidiNotes`)
    (`ModularSynthComponent.NoteOn` (`self.ModularSynth`) _array_element (`KismetMathLibrary.Round` (`KismetMathLibrary.MapRangeClamped` (`KismetMathLibrary.FClamp` (`KismetMathLibrary.VSize` NormalImpulse) 0.0 75000.0) 1000.0 15000.0 0.0 127.0)) (`self.NoteDuration`))))

(event `MidOnAndFadeOut`
  ;[1 1 1] fadeOut emissive
  (`TimelineComponent.SetPlayRate` (`self.Timeline_0`) (/ 1.0 (`self.NoteDuration`)))
  (bind (_direction _1_0smoothly1sec) (`Timeline|Timeline_0` :!via `PlayFromStart`)
    (:`Update`
      (`MaterialInstanceDynamic.SetScalarParameterValue` (`self.MID`) "Emissive Multiplier" (* _1_0smoothly1sec 30.0)))))

(fn `UserConstructionScript`)