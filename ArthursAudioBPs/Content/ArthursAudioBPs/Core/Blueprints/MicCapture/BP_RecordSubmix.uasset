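; BP_RecordSubmix is an actor that records an audio submix to a sound wave when play begins, then plays the result back.
; BeginPlay waits a predelay, starts recording the chosen submix for a set duration, then stops and exports it using configurable format, name, path and optional wave to overwrite.
; It stores the returned sound wave, prints status messages, and plays it in 2D after a short pause.
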(event `self.ReceiveBeginPlay`
  (`KismetSystemLibrary.Delay` (`self.RecordingStartPredelay`))
  (`AudioMixerBlueprintLibrary.StartRecordingOutput` (`self.DurationToRecord`) (`self.SubmixToRecord`))
  (`KismetSystemLibrary.Delay` (`self.DurationToRecord`))
  (bind _returnvalue (`AudioMixerBlueprintLibrary.StopRecordingOutput` (`self.RecordingExportType`) (`self.OutputFilename`) (`self.OutputPath`) (`self.SubmixToRecord`) (`self.(Optional)ExistingSoundwaveToOverwrite`)))
  (set `self.RecordedSoundWave` _returnvalue)
  (`KismetSystemLibrary.PrintString` "Finised recording")
  (`KismetSystemLibrary.Delay` 2.0)
  (`KismetSystemLibrary.PrintString` "Playing back Recording")
  (`GameplayStatics.PlaySound2D` (`self.RecordedSoundWave`) 1.0 1.0 0.0 null null))

(fn `UserConstructionScript`)