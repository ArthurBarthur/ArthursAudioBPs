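; Actor Blueprint that captures microphone audio through an AudioCapture component, named as an effects variant though its graphs show no effect logic.
; On BeginPlay it activates the component and then starts capture, with a short delay before each step.
; The component's envelope event prints the volume level as a debug readout, using the cached tick delta as display duration so each value lasts about one frame.
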(event `self.AudioCapture.OnAudioEnvelopeValue`
  (params (EnvelopeValue :type "Float (single-precision)"))
  ;[1 1 1] volume envelope
  ;[1 1 1] debugEnvelope
  (`KismetSystemLibrary.PrintString` (`KismetStringLibrary.Conv_DoubleToString` EnvelopeValue) true true (struct :`G` 0.66 :`B` 1.0 :`A` 1.0) (`self.deltaTick`)))

(event `self.ReceiveBeginPlay`
  (`KismetSystemLibrary.Delay` 0.2)
  (`ActorComponent.Activate` (`self.AudioCapture`) false)
  (`KismetSystemLibrary.Delay` 0.2)
  (`SynthComponent.Start` (`self.AudioCapture`)))

(event `self.ReceiveTick`
  (params (DeltaSeconds :type "Float (single-precision)"))
  ;[1 1 1] tick
  (set `self.deltaTick` DeltaSeconds))

(fn `UserConstructionScript`)