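; Audio visualizer Blueprint that draws a bar-graph spectrum of stacked blocks, one column per analyzed frequency, colored by height.
; Construction creates one instanced mesh component and dynamic material per color, computes height thresholds for each, and previews columns with random levels.
; Every Tick clears all instances and rebuilds the columns from AnalysisBeautifier's smoothed, normalized envelope values, adding each block to the component matching its height band.
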(event `self.ReceiveBeginPlay`)

(event `self.ReceiveTick`
  (params (DeltaSeconds :type "Float (single-precision)"))
  ;[1 1 1] add fresh meshes
  (`self.ManageAndAddInstancedMeshes`))

(fn `ConstructManageAndAddInstancedMeshes`
  (locals (_spacingX :type "Float (double-precision)" :default 0.0) (_spacingZ :type "Float (double-precision)" :default 0.0) (_latestValue :type "Float (double-precision)") (_resolutionIndex :type Integer) (_colorIndex :type Integer))
  ;[1 1 1] clear old mesh instances
  (for _array_element (`self.InstancedMeshComponents`)
    (`InstancedStaticMeshComponent.ClearInstances` _array_element))
  ;[1 1 1] go through latest values
  (for (_ _array_index) (`/ArthursAudioVisualToolkit/Blueprints/AudioViz/BP_AnalysisBeautifier.FrequenciesToAnalyze` (`self.AnalysisBeautifier`))
    (set `local._latestValue` (`KismetMathLibrary.RandomFloatInRange` 0.0 1.0))
    (set `local._spacingX` (* _array_index (`self.SpacingX`)))
    ;[1 1 1] Check value against height resolution and fill up from bottom
    (for _index (range (+ (`self.HeightResolution`) 1))
      (set `local._resolutionIndex` _index)
      (set `local._spacingZ` (* (`local._resolutionIndex`) (`self.SpacingZ`)))
      (if (<= (`local._spacingZ`) (* (`local._latestValue`) (* (`self.HeightResolution`) (`self.SpacingZ`))))
        ;[1 1 1] select instanced mesh of fitting color
        (for (_array_element_2 _array_index_2) (`self.ResolutionsColorDistribution`)
          (set `local._colorIndex` _array_index_2)
          (if (<= (`KismetMathLibrary.Conv_IntToDouble` (`local._resolutionIndex`)) _array_element_2)
            (`|ExecutionSequence`
              (:`then_0`
                ;[1 1 1] add an instance
                (`InstancedStaticMeshComponent.AddInstance` (`|GetArrayItem` (`self.InstancedMeshComponents`) (`local._colorIndex`)) (`KismetMathLibrary.MakeTransform` (`KismetMathLibrary.MakeVector` (`local._spacingX`) 0.0 (`local._spacingZ`)) (struct) (`self.BlockScale`))))
              (:`then_1`
                (break)))))))))

(fn `ManageAndAddInstancedMeshes`
  (locals (_spacingX :type "Float (double-precision)" :default 0.0) (_spacingZ :type "Float (double-precision)" :default 0.0) (_latestValue :type "Float (double-precision)") (_resolutionIndex :type Integer) (_colorIndex :type Integer))
  ;[1 1 1] clear old mesh instances
  (for _array_element (`self.InstancedMeshComponents`)
    (`InstancedStaticMeshComponent.ClearInstances` _array_element))
  ;[1 1 1] go through latest values
  (for (_array_element_2 _array_index) (`/ArthursAudioVisualToolkit/Blueprints/AudioViz/BP_AnalysisBeautifier.FinalEnvelopeSmoothedNormalizedOutputValuesFromAnalysis` (`self.AnalysisBeautifier`))
    (set `local._latestValue` _array_element_2)
    (set `local._spacingX` (* _array_index (`self.SpacingX`)))
    ;[1 1 1] Check value against height resolution and fill up from bottom
    (for _index (range (+ (`self.HeightResolution`) 1))
      (set `local._resolutionIndex` _index)
      (set `local._spacingZ` (* (`local._resolutionIndex`) (`self.SpacingZ`)))
      (if (<= (`local._spacingZ`) (* (`local._latestValue`) (* (`self.HeightResolution`) (`self.SpacingZ`))))
        ;[1 1 1] select instanced mesh of fitting color
        (for (_array_element_3 _array_index_2) (`self.ResolutionsColorDistribution`)
          (set `local._colorIndex` _array_index_2)
          (if (<= (`KismetMathLibrary.Conv_IntToDouble` (`local._resolutionIndex`)) _array_element_3)
            (`|ExecutionSequence`
              (:`then_0`
                ;[1 1 1] add an instance
                (`InstancedStaticMeshComponent.AddInstance` (`|GetArrayItem` (`self.InstancedMeshComponents`) (`local._colorIndex`)) (`KismetMathLibrary.MakeTransform` (`KismetMathLibrary.MakeVector` (`local._spacingX`) 0.0 (`local._spacingZ`)) (struct) (`self.BlockScale`))))
              (:`then_1`
                (break)))))))))

(fn `UserConstructionScript`
  (`|ExecutionSequence`
    (:`then_0`
      ;[1 1 1] clean up any mess
      (`KismetArrayLibrary.Array_Clear` (`self.MIDs`))
      (`KismetArrayLibrary.Array_Clear` (`self.InstancedMeshComponents`)))
    (:`then_1`
      ;[1 1 1] calculate color distribution
      (for (_ _array_index) (`self.ColorsToUse`)
        (`KismetArrayLibrary.Array_Set` (`self.ResolutionsColorDistribution`) _array_index (* (`self.HeightResolution`) (/ (`KismetMathLibrary.Conv_IntToDouble` (+ _array_index 1)) 10.0)) true)))
    (:`then_2`
      ;[1 1 1] Create InstancedMeshComponents
      (for _ (`self.ColorsToUse`)
        (bind _returnvalue (`AddComponent|NODE_AddInstancedStaticMeshComponent-1`))
        (`KismetArrayLibrary.Array_Add` (`self.InstancedMeshComponents`) _returnvalue)))
    (:`then_3`
      ;[1 1 1] set actual 3d mesh on instanced meshes
      (for _array_element (`self.InstancedMeshComponents`)
        (`StaticMeshComponent.SetStaticMesh` _array_element (`self.MeshToUse`))))
    (:`then_4`
      ;[1 1 1] create MIDs
      (for _ (`self.ColorsToUse`)
        (bind _returnvalue_2 (`KismetMaterialLibrary.CreateDynamicMaterialInstance` "/Game/ArthursAudioBPs/MaterialLibrary/Simple/MAT_SimpleMat.MAT_SimpleMat"))
        (`KismetArrayLibrary.Array_Add` (`self.MIDs`) _returnvalue_2)))
    (:`then_5`
      ;[1 1 1] set colors on MIDs
      (for (_array_element_2 _array_index_2) (`self.MIDs`)
        (`MaterialInstanceDynamic.SetVectorParameterValue` _array_element_2 "Base Color" (`|GetArrayItem` (`self.ColorsToUse`) _array_index_2))))
    (:`then_6`
      ;[1 1 1] put MIDs on instanced meshes
      (for (_array_element_3 _array_index_3) (`self.InstancedMeshComponents`)
        (`PrimitiveComponent.SetMaterial` _array_element_3 0 (`|GetArrayItem` (`self.MIDs`) _array_index_3))))
    (:`then_7`
      ;[1 1 1] construct temp mesh instances for pre-viz
      (`self.ConstructManageAndAddInstancedMeshes`))))