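; Audio visualizer Blueprint that leaves a trail of randomly colored "candy" meshes shaped by the music's volume.
; Each tick averages chosen frequency slots from BeautifierRef, lerping a component rig's movement, rotation, center offset and scale.
; A looping timer spawns meshes at that rig's transform, limited to once per tick, with optional collision and physics, deleting the oldest past a cap.
; The construction script pregenerates dynamic material instances using generated or user-listed colors.
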(event `self.ReceiveTick`
  (params (DeltaSeconds :type "Float (single-precision)"))
  (bind _relativelocation (`SceneComponent.RelativeLocation` (`self.ForwardMovingStaticMesh`)))
  (set `self.Delta Seconds` DeltaSeconds)
  ;[1 1 1] get average vol over freqs
  ;;[1 1 1] reset
  (set `self.LatestAverageFreqsVolume` 0.0)
  ;;[1 1 1] add together
  (for _array_element (`self.FreqSlotsToAnalyse`)
    (set `self.LatestAverageFreqsVolume` (+ (`self.LatestAverageFreqsVolume`) (`|GetArrayItem` (`/ArthursAudioVisualToolkit/Blueprints/AudioViz/BP_AnalysisBeautifier.FinalEnvelopeSmoothedNormalizedOutputValuesFromAnalysis` (`self.BeautifierRef`)) _array_element))))
  ;;[1 1 1] final average
  (bind _output_get (set `self.LatestAverageFreqsVolume` (/ (`self.LatestAverageFreqsVolume`) (`KismetMathLibrary.Conv_IntToDouble` (`KismetArrayLibrary.Array_Length` (`self.FreqSlotsToAnalyse`))))))
  (set `self.LatestVolume01` _output_get)
  (`|ExecutionSequence`
    (:`then_0`
      ;[1 1 1] Move whole thing in direction
      (`SceneComponent.K2_SetRelativeLocation` (`self.ForwardMovingStaticMesh`) (`KismetMathLibrary.VLerp` (+ _relativelocation (`self.MovementSpeedMinVol`)) (+ _relativelocation (`self.MovementSpeedMaxVol`)) (`self.LatestVolume01`)) false false))
    (:`then_1`
      ;[1 1 1] rotate
      (`SceneComponent.K2_AddRelativeRotation` (`self.RotatingStaticMesh`) (`KismetMathLibrary.RLerp` (`self.RotationalSpeedMinVol`) (`self.RotationalSpeedMaxVol`) (`self.LatestVolume01`)) false true))
    (:`then_2`
      ;[1 1 1] move spawnpoint out or in from center
      (`SceneComponent.K2_SetRelativeLocation` (`self.OutFromCenterMesh`) (`KismetMathLibrary.VLerp` (`self.LatestMeshLocationRelativeToCenterMinVol`) (`self.LatestMeshLocationRelativeToCenterMaxVol`) (`self.LatestVolume01`)) false true))
    (:`then_3`
      ;[1 1 1] update spawn scale
      (`SceneComponent.SetRelativeScale3D` (`self.SpawningScalingStaticMesh`) (`KismetMathLibrary.VLerp` (`self.MeshScaleMinVol`) (`self.MeshScaleMaxVol`) (`self.LatestVolume01`))))
    (:`then_4`
      (goto _label :!via `Reset`))))

(event `self.ReceiveBeginPlay`
  ;[1 1 1] looping timer instead of tick
  (`KismetSystemLibrary.K2_SetTimerDelegate` (delegate `SpawnMesh`) (`self.VizMeshSpawnIntervalInSeconds`) true))

(event `SpawnMesh`
  ;[1 1 1] dont do it more often than once per tick
  (`/Engine/EditorBlueprintResources/StandardMacros.DoOnce` true :!label _label
    (:`Completed`
      ;[1 1 1] spawn viz mesh
      (`self.SpawnNewVizMesh`)
      ;[1 1 1] remove old
      (`self.RemoveOldMeshesWhenTooMany`))))

(fn `RemoveOldMeshesWhenTooMany`
  (if (> (`KismetArrayLibrary.Array_LastIndex` (`self.AllSpawnedCandies`)) (- (`self.MaxNrOfMeshesBeforeDeletingOld`) 1))
    (`ActorComponent.K2_DestroyComponent` (`|GetArrayItem` (`self.AllSpawnedCandies`)))
    (`KismetArrayLibrary.Array_Remove` (`self.AllSpawnedCandies`))))

(fn `SpawnNewVizMesh`
  (locals (LatestMesh :type "StaticMeshComponent Object Reference"))
  (bind _materials (`self.Materials`))
  (bind (_minworldscaleperaxisbeforehidingvizmesh_x _minworldscaleperaxisbeforehidingvizmesh_y _minworldscaleperaxisbeforehidingvizmesh_z) (`KismetMathLibrary.BreakVector` (`self.MinWorldScalePerAxisBeforeHidingVizMesh`)))
  (bind (_returnvalue_location _returnvalue_rotation _returnvalue_scale) (`KismetMathLibrary.BreakTransform` (`SceneComponent.K2_GetComponentToWorld` (`self.SpawningScalingStaticMesh`))))
  ;[1 1 1] spawn mesh
  (bind _returnvalue (`AddComponent|NODE_AddStaticMeshComponent-0`))
  (set `local.LatestMesh` _returnvalue)
  ;[1 1 1] store mesh
  (`KismetArrayLibrary.Array_Add` (`self.AllSpawnedCandies`) (`local.LatestMesh`))
  ;[1 1 1] should be visible?
  (if (`KismetMathLibrary.BooleanNOR` (`KismetMathLibrary.BooleanNOR` (> (.x _returnvalue_scale) _minworldscaleperaxisbeforehidingvizmesh_x) (> (.y _returnvalue_scale) _minworldscaleperaxisbeforehidingvizmesh_y)) (> (.z _returnvalue_scale) _minworldscaleperaxisbeforehidingvizmesh_z))
    (`SceneComponent.SetVisibility` (`local.LatestMesh`) false false)
    (else
      ;[1 1 1] set world transform
      (`SceneComponent.K2_SetWorldTransform` (`local.LatestMesh`) (`SceneComponent.K2_GetComponentToWorld` (`self.SpawningScalingStaticMesh`)) false false)
      ;[1 1 1] attach?
      (if (not (`self.SimulatePhysics?`))
        (`SceneComponent.K2_AttachToComponent` (`local.LatestMesh`) (`self.CentralUnmovingStaticMesh`) "None" "KeepWorld" "KeepWorld" "KeepWorld" true))
      ;[1 1 1] set 3d mesh
      (`StaticMeshComponent.SetStaticMesh` (`local.LatestMesh`) (`self.MeshToUseForViz`))
      ;[1 1 1] collision?
      (if (`self.CollisionWithWorld`)
        (`PrimitiveComponent.SetCollisionEnabled` (`local.LatestMesh`) "QueryAndPhysics")
        (else
          (`PrimitiveComponent.SetCollisionEnabled` (`local.LatestMesh`) "NoCollision")))
      ;[1 1 1] physics?
      (if (`self.SimulatePhysics?`)
        (`PrimitiveComponent.SetSimulatePhysics` (`local.LatestMesh`) true)
        (`PrimitiveComponent.SetEnableGravity` (`local.LatestMesh`) (`self.GravityEnabled`)))
      ;[1 1 1] override physmat?
      (if (`self.OverridePhysMat`)
        (`PrimitiveComponent.SetPhysMaterialOverride` (`local.LatestMesh`) (`self.PhysMatOverride`)))
      ;[1 1 1] set random material
      (`PrimitiveComponent.SetMaterial` (`local.LatestMesh`) 0 (`|GetArrayItem` _materials (`KismetMathLibrary.RandomIntegerInRange` 0 (`KismetArrayLibrary.Array_LastIndex` _materials)))))))

(fn `UserConstructionScript`
  (bind _availablecolors (`self.AvailableColors`))
  (bind (_h _s _v _a) (`KismetMathLibrary.RGBToHSV` (`self.AutoColorSpanEnd`)))
  (bind (_h_2 _s_2 _v_2 _a_2) (`KismetMathLibrary.RGBToHSV` (`self.AutoColorSpanStart`)))
  ;[1 1 1] clear old variables
  (`KismetArrayLibrary.Array_Clear` (`self.AllSpawnedCandies`))
  (`KismetArrayLibrary.Array_Clear` (`self.Materials`))
  (`KismetArrayLibrary.Array_Clear` (`self.AvailableColors`))
  ;[1 1 1] create material instances
  (for _ (range 1 (+ (`self.NumberOfRandomColorsToPre-generate`) 1))
    (bind _returnvalue (`KismetMaterialLibrary.CreateDynamicMaterialInstance` (`self.BaseForMID`)))
    (`KismetArrayLibrary.Array_Add` (`self.Materials`) _returnvalue))
  ;[1 1 1] init material colors
  ;;[1 1 1] auto-colors?
  (if (`self.Auto-GenerateColors`)
    ;;[1 1 1] random color generator
    (for _ (`self.Materials`)
      (`KismetArrayLibrary.Array_Add` (`self.AvailableColors`) (`KismetMathLibrary.HSVToRGB` (`KismetMathLibrary.RandomFloatInRange` _h_2 _h) (`KismetMathLibrary.RandomFloatInRange` _s_2 _s) (`KismetMathLibrary.RandomFloatInRange` _v_2 _v) (`KismetMathLibrary.RandomFloatInRange` _a_2 _a))))
    ;;[1 1 1] apply colors to material instances
    (for (_array_element _array_index) (`self.Materials`)
      (`MaterialInstanceDynamic.SetVectorParameterValue` _array_element "Base Color" (`|GetArrayItem` (`self.AvailableColors`) _array_index)))
    (else
      ;;[1 1 1] pick random materials from user-defined list
      (for _array_element_2 (`self.Materials`)
        (`MaterialInstanceDynamic.SetVectorParameterValue` _array_element_2 "Base Color" (`|GetArrayItem` _availablecolors (`KismetMathLibrary.RandomIntegerInRange` 0 (`KismetArrayLibrary.Array_LastIndex` _availablecolors))))))))