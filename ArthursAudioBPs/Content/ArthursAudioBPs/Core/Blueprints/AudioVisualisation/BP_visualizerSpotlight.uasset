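; Audio visualizer spotlight that pulses, shifts color and tilts with one frequency band of analyzed audio.
; Each tick it reads the smoothed, normalized envelope for its frequency slot from the referenced analysis beautifier.
; That value scales intensity, blends between low and high colors, and pitches the light fixture relative to the spotlight's starting rotation.
; A separate ModLights function offers similar intensity and color modulation but is not called here.
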(event `self.ReceiveBeginPlay`
  (set `self.StartingRelativeRot` (`SceneComponent.RelativeRotation` (`self.SpotLight`))))

(event `self.ReceiveTick`
  (params (DeltaSeconds :type "Float (single-precision)"))
  ;[1 1 1] tick
  (set `self.TickDelta` DeltaSeconds)
  ;[1 1 1] store latest env
  (set `self.Envelope0-1Live` (`|GetArrayItem` (`/ArthursAudioVisualToolkit/Blueprints/AudioViz/BP_AnalysisBeautifier.FinalEnvelopeSmoothedNormalizedOutputValuesFromAnalysis` (`self.AnalysisBeautifierRef`)) (`self.FreqSlot(from submix analyzers array of freqs)`)))
  (`|ExecutionSequence`
    (:`then_0`
      ;[1 1 1] mod LIGHT (color and intensity)
      (`LightComponent.SetIntensity` (`self.SpotLight`) (* (`self.Envelope0-1Live`) 10000000.0))
      (`LightComponent.SetLightColor` (`self.SpotLight`) (`KismetMathLibrary.LinearColorLerp` (`self.ColorLow`) (`self.ColorHigh`) (`self.Envelope0-1Live`)) true))
    (:`then_1`
      ;[1 1 1] rotate spotlight to vol
      (`SceneComponent.K2_SetRelativeRotation` (`self.LightFixture`) (`KismetMathLibrary.ComposeRotators` (`self.StartingRelativeRot`) (`KismetMathLibrary.MakeRotator` 0.0 (`KismetMathLibrary.MapRangeClamped` (`self.Envelope0-1Live`) 0.0 1.0 90.0 45.0))) false false))))

(fn `ModLights`
  (params (LightRef :type "LightComponent Object Reference") (`Envelope0-1` :type "Float (double-precision)"))
  ;[1 1 1] mod LIGHT
  (`LightComponent.SetIntensity` LightRef (* `Envelope0-1` 100.0))
  (`LightComponent.SetLightColor` LightRef (`KismetMathLibrary.LinearColorLerp` (`self.ColorLow`) (`self.ColorHigh`) `Envelope0-1`) true))

(fn `UserConstructionScript`)