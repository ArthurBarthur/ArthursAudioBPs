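; Audio visualizer actor that plays a sound after a configurable delay and makes its mesh, material, spotlight and text react to the volume.
; Each tick, the latest envelope value is normalized against a recorded peak, which a looping timer slowly decays so the response adapts to quieter passages.
; Toggleable updates use that value to stretch mesh Z scale, drive dynamic material emissive, shift spotlight intensity and color, and show a volume percentage.
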(event `self.ReceiveBeginPlay`
  ;[1 1 1] beginplay
  (`|ExecutionSequence`
    (:`then_0`
      ;[1 1 1] Initialize dynamic material
      (bind _returnvalue (`KismetMaterialLibrary.CreateDynamicMaterialInstance` (`self.BaseMaterial`)))
      (set `self.MID` _returnvalue)
      (`PrimitiveComponent.SetMaterial` (`self.StaticMesh`) 0 (`self.MID`)))
    (:`then_1`
      ;[1 1 1] decreaseHistoricMaxVolume
      (`KismetSystemLibrary.K2_SetTimerDelegate` (delegate `LowerHistoricMaxRecordedVol`) 0.5 true))
    (:`then_2`
      (`KismetSystemLibrary.Delay` (`self.DelayedStartInSeconds`))
      ;[1 1 1] init sound
      (`AudioComponent.SetSound` (`self.AudioComponent`) (`self.SoundToPlay`))
      (set `AudioComponent.VolumeMultiplier` (`self.VolumeMP`) (`self.AudioComponent`))
      (`AudioComponent.SetPitchMultiplier` (`self.AudioComponent`) (`self.PitchMultiplier`))
      (`AudioComponent.Play` (`self.AudioComponent`) 0.0))))

(event `LowerHistoricMaxRecordedVol`
  ;[1 1 1] decreaseHistoricMaxVolume
  (bind _output_get (set `self.MaxRecordedVol` (* (stale _output_get) 0.95))))

(event `self.AudioComponent.OnAudioSingleEnvelopeValue`
  (params (PlayingSoundWave :type "SoundWave Object Reference") (EnvelopeValue :type "Float (single-precision)"))
  ;[1 1 1] Store latest envelope value
  (set `self.LatestEnvelopeValue` EnvelopeValue))

(event `self.AudioComponent.OnAudioPlaybackPercent`
  (params (PlayingSoundWave :type "SoundWave Object Reference") (PlaybackPercent :type "Float (single-precision)"))
  ;[1 1 1] Store latest playback percent value
  (set `self.AudioPlaybackPercent` PlaybackPercent))

(event `self.ReceiveTick`
  (params (DeltaSeconds :type "Float (single-precision)"))
  ;[1 1 1] tick
  (`|ExecutionSequence`
    (:`then_0`
      ;[1 1 1] Normalize volume output values to 0-1
      (`self.NormalizeVolume` (`self.LatestEnvelopeValue`)))
    (:`then_1`
      ;[1 1 1] visualize
      (if (`self.ScaleMeshToAudio`)
        ;;[1 1 1] Scale mesh
        (`self.UpdateMeshScale`)))
    (:`then_2`
      (if (`self.GlowMaterialToAudio`)
        ;;[1 1 1] Update dynamic material emissive strength
        (`self.UpdateMaterialEmissive`)))
    (:`then_3`
      ;;[1 1 1] update spotlight intensity and color
      (if (`self.DimSpotlightToAudio`)
        (`self.UpdateSpotlight`)))
    (:`then_4`
      ;;[1 1 1] update volume % text display
      (if (`self.ShowTextInfo`)
        (`self.UpdateText`)
        (else
          ;;[1 1 1] destroy text preview component
          (`/Engine/EditorBlueprintResources/StandardMacros.DoOnce` false
            (:`Completed`
              (`ActorComponent.K2_DestroyComponent` (`self.TextRenderVolumePercent`)))))))))

(fn `NormalizeVolume`
  (params (LatestEnvelopeValue :type "Float (double-precision)"))
  (returns (NormalizedVolume :type "Float (double-precision)"))
  (locals (_latestEnvelope :type "Float (double-precision)"))
  ;[1 1 1] Store latest value locally
  (set `local._latestEnvelope` LatestEnvelopeValue)
  (`|ExecutionSequence`
    (:`then_0`
      ;[1 1 1] Store maximum recorded volume
      (if (> (`local._latestEnvelope`) (`self.MaxRecordedVol`))
        (set `self.MaxRecordedVol` (`local._latestEnvelope`))))
    (:`then_1`
      ;[1 1 1] Normalize to range 0-1
      (set `self.NormalizedVolume` (`KismetMathLibrary.FClamp` (`KismetMathLibrary.NormalizeToRange` (`local._latestEnvelope`) 0.0 (`self.MaxRecordedVol`)))))
    (:`then_2`
      ;[1 1 1] Return
      (return (`self.NormalizedVolume`)))))

(fn `UpdateMaterialEmissive`
  (`MaterialInstanceDynamic.SetScalarParameterValue` (`self.MID`) "Emissive Multiplier" (* (`self.NormalizedVolume`) (`self.MaterialEmissiveStrength`))))

(fn `UpdateMeshScale`
  ;[1 1 1] Scale mesh with volume
  (`SceneComponent.SetRelativeScale3D` (`self.StaticMesh`) (`KismetMathLibrary.MakeVector` 1.0 1.0 (+ (* (`self.NormalizedVolume`) (`self.MeshScaleMultiplier`)) 1.0))))

(fn `UpdateSpotlight`
  (`LightComponent.SetIntensity` (`self.SpotLight`) (`KismetMathLibrary.MapRangeClamped` (`self.NormalizedVolume`) 0.0 1.0 15000.0 200000.0))
  (`LightComponent.SetLightColor` (`self.SpotLight`) (`KismetMathLibrary.LinearColorLerp` (struct :`R` 1.0 :`G` 0.090672 :`A` 1.0) (struct :`R` 1.0 :`G` 0.618977 :`B` 0.208333 :`A` 1.0) (`self.NormalizedVolume`)) true))

(fn `UpdateText`
  ;[1 1 1] update text content
  (`TextRenderComponent.K2_SetText` (`self.TextRenderVolumePercent`) (`KismetTextLibrary.Conv_StringToText` (`KismetStringLibrary.Concat_StrStr` "Volume: \n" (`KismetStringLibrary.Conv_IntToString` (`KismetMathLibrary.Round` (* (`self.NormalizedVolume`) 100.0))) "%")))
  ;[1 1 1] update text color
  (`TextRenderComponent.SetTextRenderColor` (`self.TextRenderVolumePercent`) (`KismetMathLibrary.Conv_LinearColorToColor` (`KismetMathLibrary.LinearColorLerp` (struct :`R` 0.34375 :`G` 0.34375 :`B` 0.34375 :`A` 1.0) (struct :`R` 0.005208 :`G` 0.005208 :`B` 0.005208 :`A` 1.0) (`self.NormalizedVolume`)) false)))

(fn `UserConstructionScript`)