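; Audio visualiser actor that bends a spline with smoothed, normalized frequency values read from a Beautifier.
; Construction builds one point per frequency with random preview offsets, optionally adding meshes with randomly tinted dynamic materials.
; Each tick offsets inner points from stored positions along a response vector, leaving the first and last fixed.
; Optional meshes follow point positions and tangents, and their emissive strength tracks each frequency value.
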(event `self.ReceiveBeginPlay`)

(event `self.ReceiveTick`
  (params (DeltaSeconds :type "Float (single-precision)"))
  ;[1 1 1] get latest freq vals
  (set `self.LatestFreqValues` (`/ArthursAudioVisualToolkit/Blueprints/AudioViz/BP_AnalysisBeautifier.FinalEnvelopeSmoothedNormalizedOutputValuesFromAnalysis` (`self.Beautifier`)))
  ;[1 1 1] update spline point locations
  (`self.ChangeSplinePoints`)
  (`self.UpdateMeshScales`)
  (if (`self.AddMeshesToSpline`)
    (`self.UpdateMIDsEmissiveMP`)))

(fn `ChangeSplinePoints`
  (locals (_currentIndex :type Integer))
  (bind _latestfreqvalues (`self.LatestFreqValues`))
  (bind __currentindex (`local._currentIndex`))
  ;[1 1 1] go through the spline points we are moving
  (for _index (range 1 (+ (`self.NrOfPoints`) 1))
    (set `local._currentIndex` _index)
    (if (`KismetArrayLibrary.Array_IsValidIndex` _latestfreqvalues __currentindex)
      ;[1 1 1] update point location
      (`SplineComponent.SetLocationAtSplinePoint` (`self.Spline`) (`local._currentIndex`) (+ (`|GetArrayItem` (`self.OriginalSplinePointLocations`) (`local._currentIndex`)) (* (`self.FreqResponseMP`) (`|GetArrayItem` _latestfreqvalues __currentindex))) "Local" false)))
  ;[1 1 1] update spline
  (`SplineComponent.UpdateSpline` (`self.Spline`)))

(fn `CreateMIDs`
  ;[1 1 1] create MIDs
  (for _array_element (`self.SplineMeshes`)
    (bind _returnvalue (`PrimitiveComponent.CreateDynamicMaterialInstance` _array_element 0 "/Game/ArthursAudioBPs/MaterialLibrary/Simple/MAT_SimpleMat.MAT_SimpleMat" "None"))
    (`KismetArrayLibrary.Array_Add` (`self.MIDs`) _returnvalue)))

(fn `SetMIDsBaseColor`
  (for _array_element (`self.MIDs`)
    (`MaterialInstanceDynamic.SetVectorParameterValue` _array_element "Base Color" (`KismetMathLibrary.HSVToRGB` (`KismetMathLibrary.SelectFloat` (`KismetMathLibrary.RandomFloatInRange` 290.0 360.0) (`KismetMathLibrary.RandomFloatInRange` 0.0 70.0) (`KismetMathLibrary.RandomBool`)) (`KismetMathLibrary.RandomFloatInRange` 0.5 0.7) (`KismetMathLibrary.RandomFloatInRange` 0.0 1.0)))))

(fn `SetUpSpline`
  (locals (_currentIndex :type Integer))
  ;[1 1 1] clear any old spline points
  (`SplineComponent.ClearSplinePoints` (`self.Spline`) true)
  (for (_ _array_index) (`self.LatestFreqValues`)
    (set `local._currentIndex` _array_index)
    ;[1 1 1] add points
    (`SplineComponent.AddPoint` (`self.Spline`) (make `SplinePoint` (`KismetMathLibrary.Conv_IntToDouble` (`local._currentIndex`)) (* (`self.Spacing`) (+ _array_index 1))) false))
  ;[1 1 1] update spline
  (`SplineComponent.UpdateSpline` (`self.Spline`))
  ;[1 1 1] store amount of spline points
  (set `self.NrOfPoints` (- (`SplineComponent.GetNumberOfSplinePoints` (`self.Spline`)) 2))
  ;[1 1 1] store original spline point locs
  (`self.StoreOriginalSplinePointLocations`))

(fn `SpawnMeshes`
  (bind _splinemeshes (`self.SplineMeshes`))
  ;[1 1 1] add meshes to spline
  (if (`self.AddMeshesToSpline`)
    (for _index (range (+ (`SplineComponent.GetNumberOfSplinePoints` (`self.Spline`)) 1))
      (bind (_location _tangent) (`SplineComponent.GetLocationAndTangentAtSplinePoint` (`self.Spline`) _index "Local"))
      (bind _returnvalue (`AddComponent|NODE_AddStaticMeshComponent-5` :`RelativeTransform` (`KismetMathLibrary.MakeTransform` _location (`KismetMathLibrary.Conv_VectorToRotator` _tangent) (`self.ScaleOfMeshes`))))
      (bind _returnvalue_2 (`KismetArrayLibrary.Array_Add` _splinemeshes _returnvalue))
      (`StaticMeshComponent.SetStaticMesh` (`|GetArrayItem` _splinemeshes _returnvalue_2) (`self.MeshToPutOnSpline`)))))

(fn `StoreOriginalSplinePointLocations`
  (locals (_currentIndex :type Integer))
  (for _index (range 1 (+ (`self.NrOfPoints`) 1))
    (set `local._currentIndex` _index)
    (`KismetArrayLibrary.Array_Set` (`self.OriginalSplinePointLocations`) (`local._currentIndex`) (`SplineComponent.GetLocationAtSplinePoint` (`self.Spline`) (`local._currentIndex`) "Local") true)))

(fn `UpdateMeshScales`
  (if (`self.AddMeshesToSpline`)
    (for _index (range (+ (`SplineComponent.GetNumberOfSplinePoints` (`self.Spline`)) 1))
      (bind (_location _tangent) (`SplineComponent.GetLocationAndTangentAtSplinePoint` (`self.Spline`) _index "Local"))
      (`SceneComponent.K2_SetRelativeTransform` (`|GetArrayItem` (`self.SplineMeshes`) _index) (`KismetMathLibrary.MakeTransform` _location (`KismetMathLibrary.Conv_VectorToRotator` _tangent) (`self.ScaleOfMeshes`)) false false))))

(fn `UpdateMIDsEmissiveMP`
  (bind _latestfreqvalues (`self.LatestFreqValues`))
  (for (_array_element _array_index) (`self.MIDs`)
    (if (`KismetArrayLibrary.Array_IsValidIndex` _latestfreqvalues _array_index)
      (`MaterialInstanceDynamic.SetScalarParameterValue` _array_element "Emissive Multiplier" (* (`|GetArrayItem` _latestfreqvalues _array_index) (`self.EmissiveMP`))))))

(fn `UserConstructionScript`
  ;[1 1 1] valid beautifier?
  (`/Engine/EditorBlueprintResources/StandardMacros.IsValid` (`self.Beautifier`)
    (:`Is Valid`
      ;[1 1 1] get latest freq vals
      (set `self.LatestFreqValues` (`/ArthursAudioVisualToolkit/Blueprints/AudioViz/BP_AnalysisBeautifier.FinalEnvelopeSmoothedNormalizedOutputValuesFromAnalysis` (`self.Beautifier`)))
      ;[1 1 1] randomize
      (for (_ _array_index) (`/ArthursAudioVisualToolkit/Blueprints/AudioViz/BP_AnalysisBeautifier.FrequenciesToAnalyze` (`self.Beautifier`))
        (`KismetArrayLibrary.Array_Set` (`self.LatestFreqValues`) _array_index (`KismetMathLibrary.RandomFloatInRange` 0.0 0.2) true))
      ;[1 1 1] set up spline according to beautifier freqs
      (`self.SetUpSpline`)
      (`self.ChangeSplinePoints`)
      (`self.SpawnMeshes`)
      (`self.CreateMIDs`)
      (`self.SetMIDsBaseColor`))
    (:`Is Not Valid`
      ;[1 1 1] no beautifier
      (`KismetSystemLibrary.PrintString` (`KismetStringLibrary.Concat_StrStr` (`KismetSystemLibrary.GetObjectName` self) " is not pointed to a valid beautifier")))))