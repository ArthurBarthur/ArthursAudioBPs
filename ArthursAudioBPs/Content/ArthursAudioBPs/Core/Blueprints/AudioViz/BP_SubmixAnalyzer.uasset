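; BP_SubmixAnalyzer is an actor that runs spectral analysis on an audio submix, apparently for audio visualization.
; BeginPlay prefills LatestAnalysis with near-zero values and starts submix analysis with configurable FFT and spectrum settings.
; Tick refreshes that array with the magnitudes of the chosen frequencies.
; The construction script gives its three static meshes a shared purple dynamic material, which the analysis does not drive here.
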(event `self.ReceiveBeginPlay`
  ;[1 1 1] beginplay
  ;[1 1 1] prefill magnitudes array with near-zeroes
  (for (_ _array_index) (`self.FrequenciesToAnalyze`)
    (`KismetArrayLibrary.Array_Set` (`self.LatestAnalysis`) _array_index 0.01 true)
    ;[1 1 1] start analyzing submix output
    (`AudioMixerBlueprintLibrary.StartAnalyzingOutput` (`self.SubmixToAnalyze`) (`self.FFT Size`) (`self.InterpolationMethod`) (`self.WindowType`) (`self.HopSize`) (`self.SpectrumType`))))

(event `self.ReceiveTick`
  (params (DeltaSeconds :type "Float (single-precision)"))
  ;[1 1 1] tick
  ;[1 1 1] get latest magnitudes
  (bind _magnitudes (`AudioMixerBlueprintLibrary.GetMagnitudeForFrequencies` (`self.FrequenciesToAnalyze`) (`self.SubmixToAnalyze`)))
  (set `self.LatestAnalysis` _magnitudes))

(fn `UserConstructionScript`
  ;[1 1 1] create dynamic material instance
  (bind _returnvalue (`KismetMaterialLibrary.CreateDynamicMaterialInstance` "/Engine/BasicShapes/BasicShapeMaterial.BasicShapeMaterial"))
  (set `self.MID` _returnvalue)
  (`PrimitiveComponent.SetMaterial` (`self.StaticMesh1`) 0 (`self.MID`))
  (`PrimitiveComponent.SetMaterial` (`self.StaticMesh2`) 0 (`self.MID`))
  (`PrimitiveComponent.SetMaterial` (`self.StaticMesh`) 0 (`self.MID`))
  (`MaterialInstanceDynamic.SetVectorParameterValue` (`self.MID`) "Color" (struct :`R` 0.2 :`G` 0.035294 :`B` 0.321569 :`A` 1.0)))