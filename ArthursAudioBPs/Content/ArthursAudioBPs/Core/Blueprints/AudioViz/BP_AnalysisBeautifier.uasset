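; Actor that turns raw per-frequency magnitudes from a SubmixAnalyzer into smoothed 0-1 envelopes and an overall average, apparently for audio visualization.
; Each tick it tracks historic maxima, normalizes against them per band or globally, applies attack/release smoothing, then remaps above a lower threshold.
; An optional looping timer re-arms a DoOnce that scales down maxima to regain sensitivity.
; Construction tints its cube and sphere through a dynamic material.
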(event `self.ReceiveBeginPlay`
  ;[1 1 1] beginplay
  (`|ExecutionSequence`
    (:`then_0`
      ;[1 1 1] get frequencies to analyze from SubmixAnalyzer
      (set `self.FrequenciesToAnalyze` (`/Game/ArthursAudioBPs/Core/Blueprints/AudioViz/BP_SubmixAnalyzer.FrequenciesToAnalyze` (`self.SubmixAnalyzerRef`))))
    (:`then_1`
      ;[1 1 1] initialize array of max magnitudes
      (if (`self.PreloadFrequencyMaxRecordedVol`)
        (set `self.MaxMagnitudes` (`self.MaxMagnitudesPreload(MustBeSameLengthAsFreqsInAnalyzer)`))
        (else
          (`KismetArrayLibrary.Array_Clear` (`self.MaxMagnitudes`))
          (for _ (`self.FrequenciesToAnalyze`)
            (`KismetArrayLibrary.Array_Add` (`self.MaxMagnitudes`) 1e-05)))))
    (:`then_2`
      ;[1 1 1] Enable Tick
      (`self.SetActorTickEnabled` true))
    (:`then_3`
      ;[1 1 1] Set up looping timer for DecreaseMaxValuesEvent
      (if (`self.RegularlyIncreaseSensitivity`)
        (`KismetSystemLibrary.K2_SetTimerDelegate` (`|CreateDelegate` :!event `DecreaseMaxValues`) (`self.Interval`) true)))))

(event `self.ReceiveTick`
  (params (DeltaSeconds :type "Float (single-precision)"))
  ;[1 1 1] Tick
  (set `self.DeltaTick` DeltaSeconds)
  (`|ExecutionSequence`
    (:`then_0`
      ;[1 1 1] get latest central analysis
      (set `self.LatestMagnitudes` (`/Game/ArthursAudioBPs/Core/Blueprints/AudioViz/BP_SubmixAnalyzer.LatestAnalysis` (`self.SubmixAnalyzerRef`))))
    (:`then_1`
      ;[1 1 1] store max recorded magnitudes
      (`self.StoreMaxMagnitudes`))
    (:`then_2`
      ;[1 1 1] normalize. (magnitudes to 0-1)
      (`self.NormalizeMagnitudes`))
    (:`then_3`
      ;[1 1 1] smoothing.
      (`|ExecutionSequence`
        (:`then_0`
          (`/Engine/EditorBlueprintResources/StandardMacros.DoOnce` false
            (:`Completed`
              (`self.InitSmoothing`))))
        (:`then_1`
          ;;[1 1 1] smoothen values
          (`self.Smoothing`))))
    (:`then_4`
      ;[1 1 1] Lower Threshold
      (`self.LowerThresholdNeedleEye`))
    (:`then_5`
      ;[1 1 1] DecreaseHistoricMaxValues
      (`/Engine/EditorBlueprintResources/StandardMacros.DoOnce` true :!label _label
        (:`Completed`
          (`self.DecreaseHistoricMaxMagnitudes`))))
    (:`then_6`
      (`self.Find Total Average(Allfreqs)`))))

(event `DecreaseMaxValues`
  ;[1 1 1] DecreaseHistoricMaxValues
  (goto _label :!via `Reset`))

(fn `DecreaseHistoricMaxMagnitudes`
  (locals (MaxMagnituedLocal :type "Array of Float (double-precision)"))
  (for _array_element (`self.MaxMagnitudes`)
    (`KismetArrayLibrary.Array_Add` (`local.MaxMagnituedLocal`) (`KismetMathLibrary.FClamp` (* _array_element (`KismetMathLibrary.MapRangeClamped` (`self.Aggresiveness`) 0.0 1.0 1.0)) 1e-05 9999.0)))
  (set `self.MaxMagnitudes` (`local.MaxMagnituedLocal`)))

(fn `Find Total Average(Allfreqs)`
  (bind _finalenvelopesmoothednormalizedoutputvaluesfromanalysis (`self.FinalEnvelopeSmoothedNormalizedOutputValuesFromAnalysis`))
  ;[1 1 1] find current average volume over all freqs
  (set `self.CurrentAverageVol01` 0.0)
  (for _array_element _finalenvelopesmoothednormalizedoutputvaluesfromanalysis
    (set `self.CurrentAverageVol01` (+ _array_element (`self.CurrentAverageVol01`))))
  (set `self.CurrentAverageVol01` (/ (`self.CurrentAverageVol01`) (`KismetMathLibrary.Conv_IntToDouble` (`KismetArrayLibrary.Array_Length` _finalenvelopesmoothednormalizedoutputvaluesfromanalysis)))))

(fn `InitSmoothing`
  ;[1 1 1] fill smoothed values array with the correct amount of zeroes
  (for (_ _array_index) (`self.NormalizedValues`)
    (`KismetArrayLibrary.Array_Set` (`self.SmoothedValues`) _array_index 0.0 true)))

(fn `LowerThresholdNeedleEye`
  (locals (TempArray :type "Array of Float (double-precision)"))
  (`KismetArrayLibrary.Array_Clear` (`local.TempArray`))
  (for _array_element (`self.SmoothedValues`)
    (`KismetArrayLibrary.Array_Add` (`local.TempArray`) (`KismetMathLibrary.MapRangeClamped` _array_element (`self.LowerThreshold`) 1.0 0.0 1.0)))
  (bind _output_get (set `self.ThresholdedValues` (`local.TempArray`)))
  (set `self.FinalEnvelopeSmoothedNormalizedOutputValuesFromAnalysis` _output_get))

(fn `NormalizeMagnitudes`
  (locals (_maxMagnitude :type "Float (double-precision)" :default 0.0) (NormalizedValuesLocalVar :type "Array of Float (double-precision)"))
  ;[1 0.3076 0.8269] fix changes are only here
  (set `local._maxMagnitude` (`.MaxValue` (`KismetMathLibrary.MaxOfFloatArray` (`self.MaxMagnitudes`))))
  ;[1 1 1] loop through latest magnitudes
  (for (_array_element _array_index) (`self.LatestMagnitudes`)
    ;[1 1 1] Store Normalized magnitudes
    (`KismetArrayLibrary.Array_Add` (`local.NormalizedValuesLocalVar`) (`KismetMathLibrary.MapRangeClamped` _array_element 0.0 (`KismetMathLibrary.SelectFloat` (`|GetArrayItem` (`self.MaxMagnitudes`) _array_index) (`local._maxMagnitude`) (`self.NormalizeEachFrequencyIndependently`)) 0.0 1.0)))
  (set `self.NormalizedValues` (`local.NormalizedValuesLocalVar`)))

(fn `Smoothing`
  (locals (_latestNormalizedValue :type "Float (double-precision)") (_latestSmoothValue :type "Float (double-precision)" :default 0.0) (SmoothedValuesLocal :type "Array of Float (double-precision)"))
  ;[1 1 1] loop through normalized values
  (for (_array_element _array_index) (`self.NormalizedValues`)
    ;[1 1 1] store smoothed values
    (`KismetArrayLibrary.Array_Add` (`local.SmoothedValuesLocal`) (`KismetMathLibrary.FInterpTo_Constant` (`|GetArrayItem` (`self.SmoothedValues`) _array_index) _array_element (`self.DeltaTick`) (select `bool` (> _array_element (`|GetArrayItem` (`self.SmoothedValues`) _array_index)) :`false` (/ 1.0 (/ (`self.Release(in milliseconds)`) 1000.0)) :`true` (/ 1.0 (/ (`self.Attack(in milliseconds)`) 1000.0))))))
  (set `self.SmoothedValues` (`local.SmoothedValuesLocal`)))

(fn `StoreMaxMagnitudes`
  (locals (_latestMagnitude :type "Float (double-precision)") (_currentIndex :type Integer) (MaxMagnitudesResultLocal :type "Array of Float (double-precision)"))
  (bind __latestmagnitude (`local._latestMagnitude`))
  (bind _output (`|GetArrayItem` (`self.MaxMagnitudes`) (`local._currentIndex`)))
  ;[1 1 1] loop through latest magnitudes
  (for (_array_element _array_index) (`self.LatestMagnitudes`)
    (set `local._latestMagnitude` _array_element)
    (set `local._currentIndex` _array_index)
    ;[1 1 1] store if current is an historic max value
    (`KismetArrayLibrary.Array_Add` (`local.MaxMagnitudesResultLocal`) (`KismetMathLibrary.SelectFloat` __latestmagnitude _output (> __latestmagnitude _output))))
  (set `self.MaxMagnitudes` (`local.MaxMagnitudesResultLocal`)))

(fn `UseOnlyTopMagnitudeForMax`
  (locals (_TopMagnitude :type "Float (double-precision)" :default 0.0) (MaxMagnitudesLocal :type "Array of Float (double-precision)"))
  ;[1 1 1] get top magnitude of all
  (set `local._TopMagnitude` (`.MaxValue` (`KismetMathLibrary.MaxOfFloatArray` (`self.MaxMagnitudes`))))
  ;[1 1 1] write top value to all records
  (for _ (`self.MaxMagnitudes`)
    (`KismetArrayLibrary.Array_Add` (`local.MaxMagnitudesLocal`) (`local._TopMagnitude`)))
  ;[1 1 1] output
  (set `self.MaxMagnitudes` (`local.MaxMagnitudesLocal`)))

(fn `UserConstructionScript`
  ;[1 1 1] get frequencies to analyze from SubmixAnalyzer
  (set `self.FrequenciesToAnalyze` (`/Game/ArthursAudioBPs/Core/Blueprints/AudioViz/BP_SubmixAnalyzer.FrequenciesToAnalyze` (`self.SubmixAnalyzerRef`)))
  (bind _returnvalue (`KismetMaterialLibrary.CreateDynamicMaterialInstance` "/Engine/BasicShapes/BasicShapeMaterial.BasicShapeMaterial"))
  (set `self.MID` _returnvalue)
  (`PrimitiveComponent.SetMaterial` (`self.Cube`) 0 (`self.MID`))
  (`PrimitiveComponent.SetMaterial` (`self.Sphere`) 0 (`self.MID`))
  (`MaterialInstanceDynamic.SetVectorParameterValue` (`self.MID`) "Color" (struct :`R` 0.2 :`G` 0.035294 :`B` 0.321569 :`A` 1.0)))