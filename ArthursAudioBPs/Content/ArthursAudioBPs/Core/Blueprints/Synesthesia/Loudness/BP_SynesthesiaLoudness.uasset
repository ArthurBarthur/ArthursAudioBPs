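; Actor that visualizes a sound's Loudness Synesthesia analysis as a row of instanced meshes with a playback cursor.
; The construction script samples normalized loudness every 0.01 seconds and scales one instance per sample.
; BeginPlay binds to a referenced actor's audio playback percentage, then enables Tick.
; Tick resets instance scales, enlarges the slice at the playback position and moves the Dial there, stretched by its loudness.
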(event `self.ReceiveBeginPlay`
  ;[1 1 1] beginplay
  (`KismetSystemLibrary.Delay` 0.5)
  (`|ExecutionSequence`
    (:`then_0`
      ;[1 1 1] store position dial starting transform position
      (set `self.DialStockTransform` (`SceneComponent.GetRelativeTransform` (`self.Dial`))))
    (:`then_1`
      ;[1 1 1] find out ca how many instances per percent
      (set `self.InstFractionalPos` (/ (`InstancedStaticMeshComponent.GetInstanceCount` (`self.InstMesh`)) 100)))
    (:`then_2`
      ;[1 1 1] set up custom event GetLatestPercentagePlayedFromAudioComp
      (add `AudioComponent.OnAudioPlaybackPercent` (`self.GetComponentByClass` (`self.ActorWithAudioComp`) "/Script/Engine.AudioComponent") (`|CreateDelegate` :!event `GetLatestPercentagePlayedFromAudioComp`)))
    (:`then_3`
      ;[1 1 1] enable tick
      (`self.SetActorTickEnabled` true))))

(event `self.ReceiveTick`
  (params (DeltaSeconds :type "Float (single-precision)"))
  (bind _highlightedtransform_location (`KismetMathLibrary.BreakTransform` (`self.HighlightedTransform`)))
  (bind _dialstocktransform (`self.DialStockTransform`))
  (bind _outinstancetransform (`InstancedStaticMeshComponent.GetInstanceTransform` (`self.InstMesh`) (`self.HighlightedInstanceIndex`) false))
  (bind _returnvalue_x (`KismetMathLibrary.BreakVector` (+ (.scale _outinstancetransform) 0.0)))
  (bind (_returnvalue_x_2 _returnvalue_y _returnvalue_z) (`KismetMathLibrary.BreakVector` (+ (* (.scale _outinstancetransform) (`self.HighlightMultiplier`)) 0.5)))
  ;[1 1 1] tick
  (set `self.TickDelta` DeltaSeconds)
  ;[1 1 1] get sample play position in percent
  (set `self.CurrentPlaybackPercent` (* (mod (stale `GetLatestPercentagePlayedFromAudioComp` PlaybackPercent) 1.0) 100.0))
  ;[1 1 1] make all instaces their right size(again)
  (for (_array_element _array_index) (`self.StoredLoudnesses`)
    (bind _returnvalue (* _array_element 10.0))
    (`InstancedStaticMeshComponent.UpdateInstanceTransform` (`self.InstMesh`) _array_index (`KismetMathLibrary.MakeTransform` (`KismetMathLibrary.MakeVector` (* (`KismetMathLibrary.Conv_IntToDouble` _array_index) (`self.Spacing`))) (struct) (`KismetMathLibrary.MakeVector` 0.1 _returnvalue _returnvalue)) false false false))
  ;[1 1 1] find current mesh slice instance (with regards to playback time)
  (set `self.HighlightedInstanceIndex` (`KismetMathLibrary.Round` (* (`self.InstFractionalPos`) (`self.CurrentPlaybackPercent`))))
  ;[1 1 1] create highlight transform
  (set `self.HighlightedTransform` (`KismetMathLibrary.MakeTransform` (.location _outinstancetransform) (.rotation _outinstancetransform) (`KismetMathLibrary.MakeVector` _returnvalue_x _returnvalue_y _returnvalue_z)))
  ;[1 1 1] highlight current instance
  (`InstancedStaticMeshComponent.UpdateInstanceTransform` (`self.InstMesh`) (`self.HighlightedInstanceIndex`) (`self.HighlightedTransform`) false true false)
  ;[1 1 1] make dial transform
  (set `self.BrightDialTransform` (`KismetMathLibrary.MakeTransform` _highlightedtransform_location (.rotation _dialstocktransform) (`KismetMathLibrary.MakeVector` (.x (.scale _dialstocktransform)) (.y (.scale _dialstocktransform)) (* (.z (.scale _dialstocktransform)) (+ (`|GetArrayItem` (`self.StoredLoudnesses`) (`self.HighlightedInstanceIndex`)) 1.0)))))
  ;[1 1 1] move dial
  (`SceneComponent.K2_SetRelativeTransform` (`self.Dial`) (`self.BrightDialTransform`) false false))

(event `GetLatestPercentagePlayedFromAudioComp`
  (params (PlayingSoundWave :type "SoundWave Object Reference") (PlaybackPercent :type "Float (double-precision)"))
  ;[1 1 1] get sample play position in percent
)

(fn `UserConstructionScript`
  (`|ExecutionSequence`
    (:`then_0`
      ;[1 1 1] store loudnesses for sample duration
      (`KismetArrayLibrary.Array_Clear` (`self.StoredLoudnesses`))
      (set `self.AnalysisDuration` (`AudioAnalyzerNRT.DurationInSeconds` (`self.LoudnessSynesthesia`)))
      (`KismetArrayLibrary.Array_Add` (`self.StoredLoudnesses`) (`LoudnessNRT.GetNormalizedLoudnessAtTime` (`self.LoudnessSynesthesia`) (`self.CurrentPosition`)) :!label _label)
      (bind _output_get (set `self.CurrentPosition` (+ (stale _output_get) 0.01)))
      (if (< (`self.CurrentPosition`) (`self.AnalysisDuration`))
        (goto _label)))
    (:`then_1`
      ;[1 1 1] spawn instanced meshes representing loudnesses
      (bind _returnvalue (`AddComponent|NODE_AddInstancedStaticMeshComponent-2`))
      (bind _output_get_2 (set `self.InstMesh` _returnvalue))
      (`StaticMeshComponent.SetStaticMesh` _output_get_2 (`self.MeshType`))
      (for (_array_element _array_index) (`self.StoredLoudnesses`)
        (bind _returnvalue_2 (* _array_element 10.0))
        (`InstancedStaticMeshComponent.AddInstance` (`self.InstMesh`) (`KismetMathLibrary.MakeTransform` (`KismetMathLibrary.MakeVector` (* (`KismetMathLibrary.Conv_IntToDouble` _array_index) (`self.Spacing`))) (struct) (`KismetMathLibrary.MakeVector` 0.1 _returnvalue_2 _returnvalue_2)))))))