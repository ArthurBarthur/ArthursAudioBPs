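; Crowd child Blueprint that bobs its crowd meshes up and down in reaction to analyzed audio.
; BeginPlay caches each mesh's relative location as a rest position.
; Each Tick, it offsets Z from that position by one smoothed, normalized Beautifier frequency band, scaled by a reactivity multiplier.
; The ListenToAllFreqs branch averages all bands, but as wired only the single-band branch sets mesh locations.
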(event `self.ReceiveBeginPlay`
  (`parent.ReceiveBeginPlay`)
  (set `self.AllCrowdMeshes` (`self.meshesFinal`))
  ;[1 1 1] store origin positions of crowd
  (for _array_element (`self.AllCrowdMeshes`)
    (`KismetArrayLibrary.Array_Add` (`self.array`) (`SceneComponent.RelativeLocation` _array_element))))

(event `self.ReceiveTick`
  (params (DeltaSeconds :type "Float (single-precision)"))
  (bind _freqslot_from_submix_analyzers_array_of_freqs_ (`self.FreqSlot(from submix analyzers array of freqs)`))
  (bind _finalenvelopesmoothednormalizedoutputvaluesfromanalysis (`/ArthursAudioVisualToolkit/Blueprints/AudioViz/BP_AnalysisBeautifier.FinalEnvelopeSmoothedNormalizedOutputValuesFromAnalysis` (`self.Beautifier`)))
  (bind _finalenvelopesmoothednormalizedoutputvaluesfromanalysis_2 (`/ArthursAudioVisualToolkit/Blueprints/AudioViz/BP_AnalysisBeautifier.FinalEnvelopeSmoothedNormalizedOutputValuesFromAnalysis` (`self.Beautifier`)))
  (`parent.ReceiveTick` DeltaSeconds)
  ;[1 1 1] update positions of crowd to music or whatevs
  (for (_array_element _array_index) (`self.AllCrowdMeshes`)
    (if (`self.ListenToAllFreqs`)
      ;;[1 1 1] get average of all freqs
      (set `self.AllFreqsAveraged` 0.0)
      (for _array_element_2 _finalenvelopesmoothednormalizedoutputvaluesfromanalysis
        (bind _output_get (set `self.AllFreqsAveraged` (+ (`self.AllFreqsAveraged`) _array_element_2))))
      (bind _output_get_2 (set `self.AllFreqsAveraged` (/ _output_get (`KismetMathLibrary.Conv_IntToDouble` (`KismetArrayLibrary.Array_Length` _finalenvelopesmoothednormalizedoutputvaluesfromanalysis)))))
      (else
        (`SceneComponent.K2_SetRelativeLocation` _array_element (`KismetMathLibrary.MakeVector` (.x (`|GetArrayItem` (`self.array`) _array_index)) (.y (`|GetArrayItem` (`self.array`) _array_index)) (+ (.z (`|GetArrayItem` (`self.array`) _array_index)) (`KismetMathLibrary.SelectFloat` _output_get_2 (`KismetMathLibrary.SelectFloat` (* (`|GetArrayItem` _finalenvelopesmoothednormalizedoutputvaluesfromanalysis_2 _freqslot_from_submix_analyzers_array_of_freqs_) (`self.ReactivityMP`)) 0.0 (`KismetArrayLibrary.Array_IsValidIndex` _finalenvelopesmoothednormalizedoutputvaluesfromanalysis_2 _freqslot_from_submix_analyzers_array_of_freqs_)) (`self.ListenToAllFreqs`)))) false false)))))

(fn `UserConstructionScript`
  (`parent.UserConstructionScript`))