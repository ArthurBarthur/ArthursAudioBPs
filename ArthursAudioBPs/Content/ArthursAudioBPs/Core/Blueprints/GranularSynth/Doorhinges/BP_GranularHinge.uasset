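; Granular synth actor that voices a door hinge from the motion of a referenced BP_door.
; Each tick, door rotation maps to the sample's scrub position, optionally reversed, and velocity sets volume, silencing a near-still door, before the granular preset is reapplied.
; The synth's envelope drives a debug-style box mesh's height, colour and glow.
; BeginPlay configures concurrency, attenuation and sound with staggered delays before ticking starts playback once.
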(event `self.ReceiveBeginPlay`
  ;[1 1 1] beginPlay
  (`KismetSystemLibrary.Delay` 0.5)
  ;[1 1 1] init granular
  ;;[1 1 1] bind event for latest envelope
  (add `SynthComponent.OnAudioEnvelopeValue` (`self.GranularSynth`) (`|CreateDelegate` :!event `EventLatestEnv`))
  ;;[1 1 1] set concurrency
  (set `SynthComponent.ConcurrencySet` (`|MakeSet` "/Game/ArthursAudioBPs/Core/Blueprints/GranularSynth/Doorhinges/SC_GranularSoundConcurrency.SC_GranularSoundConcurrency" :!type "SoundConcurrency Object Reference") (`self.GranularSynth`))
  ;;[1 1 1] propagation settings
  (set `SynthComponent.bAllowSpatialization` true (`self.GranularSynth`))
  (set `SynthComponent.AttenuationSettings` (`self.Attenuation`) (`self.GranularSynth`))
  ;;[1 1 1] update preset
  (`/ArthursAudioVisualToolkit/FunctionLibraries/AabpsGranularSynthHelpers.UpdateFullGranularPreset` (`self.GranularSynth`) (`self.GranularPreset`))
  ;;[1 1 1] set sound on gran
  (`KismetSystemLibrary.Delay` 1.0)
  (`GranularSynth.SetSoundWave` (`self.GranularSynth`) (`self.ActiveSound`))
  ;;[1 1 1] start
  (`KismetSystemLibrary.Delay` 1.0)
  ;[1 1 1] create and set MID
  (bind _returnvalue (`KismetMaterialLibrary.CreateDynamicMaterialInstance` "/Game/ArthursAudioBPs/MaterialLibrary/Simple/MI_SimpleMat_Inst1.MI_SimpleMat_Inst1"))
  (bind _output_get (set `self.granboxMID` _returnvalue))
  (`PrimitiveComponent.SetMaterial` (`self.StaticMesh`) 0 _output_get)
  ;[1 1 1] Enable Tick
  (`self.SetActorTickEnabled` true))

(event `EventLatestEnv`
  (params (EnvelopeValue :type "Float (double-precision)"))
  ;[1 1 1] latest envelope
  (set `self.LatestEnv` EnvelopeValue))

(event `self.ReceiveTick`
  (params (DeltaSeconds :type "Float (single-precision)"))
  ;[1 1 1] Tick
  (set `self.LatestTickDelta` DeltaSeconds)
  (`|ExecutionSequence`
    (:`then_0`
      ;[1 1 1] start granular
      ;;[1 1 1] once
      (`/Engine/EditorBlueprintResources/StandardMacros.DoOnce` false
        (:`Completed`
          (`/ArthursAudioVisualToolkit/FunctionLibraries/AabpsGranularSynthHelpers.StartGranular` (`self.GranularSynth`)))))
    (:`then_1`
      ;[1 1 1] scale mesh
      (`self.ScaleMesh`))
    (:`then_2`
      ;[1 1 1] mod MID
      (`self.ModMID`))
    (:`then_3`
      ;[1 1 1] RECEIVE DOOR STATE and update granular
      (`self.ReceiveDoorState`)
      ;[1 1 1] debug sample pos
      (`self.DebugSamplePlayPos`))))

(event `Start`
  ;[1 1 1] start
  (`GranularSynth.NoteOn` (`self.GranularSynth`) 60.0 100 -1.0))

(fn `DebugSamplePlayPos`
  (if (`self.Debug`)
    ;[1 1 1] print granular debug(current sample play position in percent)
    (if (> (`self.CopiedLatestVelocity`) 1.0)
      (`KismetSystemLibrary.PrintString` (`KismetStringLibrary.BuildString_Double` "" "SamplePositionInPercent:" (* (/ (`self.CurrentPlayheadScrubPosition`) (`SoundBase.Duration` (`self.ActiveSound`))) 100.0)) true true (struct :`G` 0.66 :`B` 1.0 :`A` 1.0) (`self.LatestTickDelta`)))))

(fn `ModMID`
  (locals (latestCalced :type "Float (double-precision)" :default 0.0))
  (bind _granboxmid (`self.granboxMID`))
  ;[1 1 1] mod MID
  (set `local.latestCalced` (`KismetMathLibrary.FClamp` (* (`self.LatestEnv`) 20.0)))
  (`MaterialInstanceDynamic.SetScalarParameterValue` _granboxmid "Emissive Multiplier" (* (`local.latestCalced`) 200.0))
  (`MaterialInstanceDynamic.SetVectorParameterValue` _granboxmid "Base Color" (`KismetMathLibrary.LinearColorLerp` (struct :`A` 1.0) (struct :`R` 1.0 :`G` 0.918136 :`A` 1.0) (`local.latestCalced`))))

(fn `ReceiveDoorState`
  (locals (Door :type "/Game/ArthursAudioBPs/Core/Blueprints/GranularSynth/Doorhinges/BP_door Object Reference"))
  (bind _activesoundduration (`self.ActiveSoundDuration`))
  ;[1 1 1] IF DOOR: get latest values once per tick
  (bind _asbp_door (cast `/Game/ArthursAudioBPs/Core/Blueprints/GranularSynth/Doorhinges/BP_door` (`self.ActualdoorRef`)))
  (bind _output_get (set `local.Door` _asbp_door))
  (set `self.CopiedLatestVelocity` (`/Game/ArthursAudioBPs/Core/Blueprints/GranularSynth/Doorhinges/BP_door.DoorVelocity0-2000` _output_get))
  (set `self.CopiedLatestPosition` (`/Game/ArthursAudioBPs/Core/Blueprints/GranularSynth/Doorhinges/BP_door.LatestDoorRot360-0` _output_get))
  (set `self.CopiedLatestMaxPosition` (`/Game/ArthursAudioBPs/Core/Blueprints/GranularSynth/Doorhinges/BP_door.DoorMaxSwingAngle` _output_get))
  (set `self.ActiveSoundDuration` (`SoundBase.Duration` (`self.ActiveSound`)))
  ;[1 1 1] live preset
  ;;[1 1 1] DoorRot2ScrubPos
  (bind _output_get_2 (set `self.RotMappedToDuration` (`KismetMathLibrary.FClamp` (`KismetMathLibrary.MapRangeClamped` (`KismetMathLibrary.MapRangeClamped` (`self.CopiedLatestPosition`) 360.0 0.0 0.0 360.0) 0.0 (`self.CopiedLatestMaxPosition`) 0.0 (- (`self.ActiveSoundDuration`) (/ (`.DurationBaseMsec_55_629930E44F1507F01122F697D24D492F` (break `/ArthursAudioVisualToolkit/FunctionLibraries/AabpsGranularPreset` (`self.GranularPreset`))) 1000.0))) 0.0 (`self.ActiveSoundDuration`))))
  ;[1 1 1] final playhead scrub position
  (set `self.CurrentPlayheadScrubPosition` (`KismetMathLibrary.SelectFloat` (`KismetMathLibrary.MapRangeClamped` _output_get_2 0.0 _activesoundduration _activesoundduration) _output_get_2 (`self.Reverse`)))
  ;[1 1 1] update granular
  (bind _structout (setmembers `/ArthursAudioVisualToolkit/FunctionLibraries/AabpsGranularPreset` :`StructRef` (`self.GranularPreset`) :`PlayheadPosSec` (`self.CurrentPlayheadScrubPosition`) :`VolumeBase` (* (`KismetMathLibrary.FClamp` (`KismetMathLibrary.MapRangeClamped` (`self.CopiedLatestVelocity`) 0.2 10.0 0.0 1.0)) (`self.GranVolMp`))))
  (`/ArthursAudioVisualToolkit/FunctionLibraries/AabpsGranularSynthHelpers.UpdateFullGranularPreset` (`self.GranularSynth`) _structout))

(fn `ScaleMesh`
  ;[1 1 1] env scale mesh
  (`SceneComponent.SetRelativeScale3D` (`self.StaticMesh`) (`KismetMathLibrary.MakeVector` 1.0 1.0 (`KismetMathLibrary.MapRangeUnclamped` (* (`self.LatestEnv`) 50.0) 0.0 1.0 1.0 10.0))))

(fn `UserConstructionScript`)