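; Control board actor that drives a list of synced granular music stem players, warping their playback with the player's movement speed.
; Each tick it derives a time-dilation multiplier from Sedan forward speed, averaged pawn velocity axes, or a manual override.
; It pushes that dilation and a pitch multiplier to every player, using curves to derive grain-duration multipliers and grains per second.
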(event `self.ReceiveBeginPlay`
  ;[1 1 1] beginPlay
  ;[1 1 1] enable tick if safe
  (for _array_element (`self.GranularSynthTime`)
    (`/Engine/EditorBlueprintResources/StandardMacros.IsValid` _array_element
      (:`Is Valid`
        (`self.SetActorTickEnabled` true))
      (:`Is Not Valid`
        (`KismetSystemLibrary.PrintString` "BP_ControlBoard has Invalid GranularSynthSuperTime-Reference")))))

(event `self.ReceiveTick`
  (params (DeltaSeconds :type "Float (single-precision)"))
  ;[1 1 1] tick
  (`self.UpdateGranular`))

(fn `UpdateGranular`
  (locals (LatestIndex :type "/Game/ArthursAudioBPs/Core/Blueprints/GranularSynth/GranularMusicStemsSyncedWarper/BP_GranularStems_SpatializedStem Object Reference"))
  (bind (_returnvalue_x _returnvalue_y _returnvalue_z) (`KismetMathLibrary.BreakVector` (`self.GetVelocity` (`GameplayStatics.GetPlayerPawn` 0))))
  (if (`self.OverrideTimeDilation`)
    ;[1 1 1] override
    (set `self.TimeDilationMP` (`self.TimeDilationOverride`))
    (else
      ;[1 1 1] Sedan forward speed = time dilation
      (bind _assedan (cast `/Game/ArthursAudioBPs/Core/PawnsAndGamemodes/Vehicle1/Sedan/Sedan` (`GameplayStatics.GetPlayerPawn` 0))
        (:`then`
          (set `self.TimeDilationMP` (`KismetMathLibrary.MapRangeUnclamped` (`KismetMathLibrary.Abs` (`WheeledVehicleMovementComponent.GetForwardSpeed` (`WheeledVehicle.VehicleMovement` _assedan))) 0.0 (`self.SedanSpeedWhereDilationIs1`) 0.05 1.0)))
        (:`CastFailed`
          ;[1 1 1] pawn velocity = time dilation
          (set `self.TimeDilationMP` (`KismetMathLibrary.MapRangeUnclamped` (/ (+ (`KismetMathLibrary.Abs` _returnvalue_x) (`KismetMathLibrary.Abs` _returnvalue_y) (`KismetMathLibrary.Abs` _returnvalue_z)) 3.0) 0.0 420.0 0.05 1.0))))))
  ;[1 1 1] loop through list of granular players
  (for _array_element (`self.GranularSynthTime`)
    (set `local.LatestIndex` _array_element)
    ;[1 1 1] set time dilation on granular player
    (set `Actor.CustomTimeDilation` (`KismetMathLibrary.FClamp` (`self.TimeDilationMP`) 0.0 9999999.0) (`local.LatestIndex`))
    ;[1 1 1] Pitch MP
    (set `/Game/ArthursAudioBPs/Core/Blueprints/GranularSynth/GranularMusicStemsSyncedWarper/BP_GranularStems_SpatializedStem.PitchMP` (`KismetMathLibrary.FClamp` (`self.PitchMP`) 0.0 666.0) (`local.LatestIndex`))
    ;[1 1 1] pitch to grain duration MP_0
    (set `/Game/ArthursAudioBPs/Core/Blueprints/GranularSynth/GranularMusicStemsSyncedWarper/BP_GranularStems_SpatializedStem.GrainDurationMP_0` (`CurveFloat.GetFloatValue` (`self.Curve_PitchMPToGrainDurationMP0`) (`self.PitchMP`)) (`local.LatestIndex`))
    ;[1 1 1] timeDilation to grain duration MP_1
    (set `/Game/ArthursAudioBPs/Core/Blueprints/GranularSynth/GranularMusicStemsSyncedWarper/BP_GranularStems_SpatializedStem.GrainDurationMP_1` (`CurveFloat.GetFloatValue` (`self.Curve_TimeDilationMpToGrainDurationMP1`) (`self.TimeDilationMP`)) (`local.LatestIndex`))
    ;[1 1 1] timeDilation to grainsPerSecond
    (set `/Game/ArthursAudioBPs/Core/Blueprints/GranularSynth/GranularMusicStemsSyncedWarper/BP_GranularStems_SpatializedStem.GrainsPerSecond` (`CurveFloat.GetFloatValue` (`self.Curve_GlobalTimeDilationMPToGrainsPerSecondMP`) (`self.TimeDilationMP`)) (`local.LatestIndex`))))

(fn `UserConstructionScript`)