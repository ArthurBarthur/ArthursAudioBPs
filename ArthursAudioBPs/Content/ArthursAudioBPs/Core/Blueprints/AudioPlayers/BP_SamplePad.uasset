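; BP_SamplePad is a configurable pad actor that plays an audio sample when its mesh is hit and glows with the sound.
; The construction script applies the mesh, sample, attenuation and glow color through a dynamic material instance.
; A gate blocks repeat hits until the sample's duration elapses, or only briefly if retriggering is allowed.
; The audio component's envelope value drives the material's emissive multiplier, making the glow follow loudness.
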(event `self.ReceiveBeginPlay`)

(event `self.StaticMesh.OnComponentHit`
  (params (HitComponent :type "PrimitiveComponent Object Reference") (OtherActor :type "Actor Object Reference") (OtherComp :type "PrimitiveComponent Object Reference") (NormalImpulse :type "Vector Structure") (Hit :type "HitResult Structure (by ref)"))
  ;[1 1 1] gate
  (`/Engine/EditorBlueprintResources/StandardMacros.Gate` false :!label _label
    (:`Exit`
      ;[1 1 1] close the gate
      (`|ExecutionSequence`
        (:`then_0`
          (goto _label :!via `Close`))
        (:`then_1`
          ;[1 1 1] play sound
          (`AudioComponent.Play` (`self.AudioComponent`) 0.0)
          (if (`self.AllowSampleRetrigger`)
            ;[1 1 1] open the gate almost immediately
            (`KismetSystemLibrary.Delay` 0.05)
            (goto _label :!via `Open`)
            (else
              ;[1 1 1] open the gate after sample is finished
              (`KismetSystemLibrary.Delay` (`SoundBase.Duration` (`AudioComponent.Sound` (`self.AudioComponent`))))
              (goto _label :!via `Open`))))))))

(event `self.StaticMesh.OnComponentBeginOverlap`
  (params (OverlappedComponent :type "PrimitiveComponent Object Reference") (OtherActor :type "Actor Object Reference") (OtherComp :type "PrimitiveComponent Object Reference") (OtherBodyIndex :type Integer) (bFromSweep :type Boolean) (SweepResult :type "HitResult Structure (by ref)")))

(event `self.AudioComponent.OnAudioSingleEnvelopeValue`
  (params (PlayingSoundWave :type "SoundWave Object Reference") (EnvelopeValue :type "Float (single-precision)"))
  (`MaterialInstanceDynamic.SetScalarParameterValue` (`self.MID`) "Emissive Multiplier" (* EnvelopeValue 100000.0)))

(fn `UserConstructionScript`
  (`StaticMeshComponent.SetStaticMesh` (`self.StaticMesh`) (`self.Mesh`))
  (bind _returnvalue (`PrimitiveComponent.CreateDynamicMaterialInstance` (`self.StaticMesh`) 0 "/Game/ArthursAudioBPs/MaterialLibrary/Simple/MAT_SimpleMat.MAT_SimpleMat" "None"))
  (bind _output_get (set `self.MID` _returnvalue))
  (`MaterialInstanceDynamic.SetVectorParameterValue` _output_get "Base Color" (`self.GlowColor`))
  (set `AudioComponent.AttenuationSettings` (`self.AttenuationSettings`) (`self.AudioComponent`))
  (`AudioComponent.SetSound` (`self.AudioComponent`) (`self.SampleToPlay`)))