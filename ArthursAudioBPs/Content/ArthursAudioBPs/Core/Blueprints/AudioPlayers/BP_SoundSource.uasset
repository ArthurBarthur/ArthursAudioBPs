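; BP_SoundSource is an audio player actor that plays a configured sound through its AudioComponent on BeginPlay, with volume, pitch, optional delay and start offset.
; Construction applies attenuation and spatialization, and a Blueprint-driven loop can replay the sound using timed delays.
; It caches the latest envelope and playback-percent values from component events.
; An InitSubmixSends helper routes to listed submixes but is not called here.
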(event `self.ReceiveBeginPlay`
  ;[1 1 1] init audioComp
  (set `AudioComponent.VolumeMultiplier` (`self.VolumeMP`) (`self.AudioComponent`))
  (`AudioComponent.SetPitchMultiplier` (`self.AudioComponent`) (`self.PitchMultiplier`))
  (`AudioComponent.SetSound` (`self.AudioComponent`) (`self.SoundToPlay`))
  ;[1 1 1] delayed start?
  (`KismetSystemLibrary.Delay` (`self.DelayedStartInSeconds`))
  ;[1 1 1] is start time set to something less than sample duration?
  (if (< (`self.StartTime`) (`SoundBase.Duration` (`self.SoundToPlay`)))
    ;[1 1 1] play
    (`AudioComponent.Play` (`self.AudioComponent`) (`self.StartTime`) :!label _label)
    ;;[1 1 1] bp assisted loop?
    (if (`self.LoopDoneByBp`)
      (`KismetSystemLibrary.Delay` (- (`SoundBase.Duration` (`self.SoundToPlay`)) (`self.StartTime`)))
      (goto _label))
    (else
      (`KismetSystemLibrary.PrintString` "bp_soundsource: start time must  \nbe something less than sample duration"))))

(event `self.AudioComponent.OnAudioSingleEnvelopeValue`
  (params (PlayingSoundWave :type "SoundWave Object Reference") (EnvelopeValue :type "Float (single-precision)"))
  ;[1 1 1] Store latest envelope value
  (set `self.LatestEnvelopeValue` EnvelopeValue))

(event `self.AudioComponent.OnAudioPlaybackPercent`
  (params (PlayingSoundWave :type "SoundWave Object Reference") (PlaybackPercent :type "Float (single-precision)"))
  ;[1 1 1] Store latest playback percent value
  (set `self.AudioPlaybackPercent` PlaybackPercent))

(fn `InitSubmixSends`
  (for _array_element (`self.SubmixSends`)
    (`AudioComponent.SetSubmixSend` (`self.AudioComponent`) (`.SoundSubmix` (break `SoundSubmixSendInfo` _array_element)) 1.0)))

(fn `UserConstructionScript`
  (set `AudioComponent.AttenuationSettings` (`self.AttenuationSettings`) (`self.AudioComponent`))
  (set `AudioComponent.bAllowSpatialization` (`self.AllowSpatialization`) (`self.AudioComponent`)))