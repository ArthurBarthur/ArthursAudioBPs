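; Box deliverer Blueprint that repeatedly spawns physics-configurable box meshes as components on itself.
; A preview cube shows the box scale in the editor and is destroyed on BeginPlay.
; AddCube runs at start and on a looping timer, pausing while the last spawned mesh still overlaps the Box volume.
; Each new mesh takes its configured mesh, material, scale, mass, collision type and physics setting.
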(event `self.ReceiveBeginPlay`
  ;[1 1 1] destroy pre-viz cube
  (`ActorComponent.K2_DestroyComponent` (`self.Cube1`))
  ;[1 1 1] add cubes on timer
  (`KismetSystemLibrary.K2_SetTimerDelegate` (delegate `TryToAddCube`) 1.0 true)
  (`self.AddCube` :!label _label))

(event `TryToAddCube`
  ;[1 1 1] add cubes on timer
  (goto _label))

(fn `AddCube`
  ;[1 1 1] pause spawning if space is occupied
  (if (not (`KismetArrayLibrary.Array_Contains` (`PrimitiveComponent.GetOverlappingComponents` (`self.Box`)) (`self.LastSpawnedMesh`)))
    ;[1 1 1] spawn mesh
    (bind _returnvalue (`AddComponent|NODE_AddStaticMeshComponent-2` :`RelativeTransform` (`KismetMathLibrary.MakeTransform` (- (`SceneComponent.RelativeLocation` (`self.Cube`)) (`self.SpawnLocation`)) (struct) (`self.BoxScaleMultiplier`))))
    (bind _output_get (set `self.LastSpawnedMesh` _returnvalue))
    ;[1 1 1] set up mesh
    (`StaticMeshComponent.SetStaticMesh` _output_get (`self.MeshToSpawn`))
    (`PrimitiveComponent.SetMaterial` _output_get 0 (`self.MaterialToUse`))
    (`PrimitiveComponent.SetMassOverrideInKg` _output_get "None" (`self.RootMeshWeightInKgOverride`) true)
    (`PrimitiveComponent.SetCollisionObjectType` _output_get (`self.ObjectType`))
    (`PrimitiveComponent.SetSimulatePhysics` _output_get (`self.SimulatePhysics`))))

(fn `UserConstructionScript`
  (`SceneComponent.SetRelativeScale3D` (`self.Cube1`) (`self.BoxScaleMultiplier`)))