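; A musical plant actor that gets a random color and synth preset, plays notes on demand and visualizes its own sound.
; Construction configures mesh, collision and a modular synth; NotePlay sounds a chord or one chosen chord note.
; After a squishy spawn bounce, the synth envelope, normalized against a decaying maximum, drives mesh movement, color and emissive glow.
; Retriggerable delays release notes and deactivate idle synths, sooner when frame time is high.
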(event `self.ReceiveBeginPlay`
  ;[1 1 1] beginPlay
  (`|ExecutionSequence`
    (:`then_0`
      ;[1 1 1] dynamic material MID
      (bind _returnvalue (`PrimitiveComponent.CreateDynamicMaterialInstance` (`self.StaticMesh`) 0 (`self.MatToUseForMid`) "None"))
      (set `self.MID` _returnvalue)
      ;[1 1 1] make random color
      (set `self.Color` (`KismetMathLibrary.HSVToRGB` (`KismetMathLibrary.RandomFloatInRange` 0.0 360.0) (`KismetMathLibrary.RandomFloat`) (`KismetMathLibrary.RandomFloat`))))
    (:`then_1`
      ;[1 1 1] decrease max historic vol
      (`KismetSystemLibrary.K2_SetTimerDelegate` (delegate `DecreaseHistoricMaxEnv`) 0.5 true))
    (:`then_2`
      ;[1 1 1] spawn-in squishyBounce
      (bind (_direction _0_1_0_over_1_sec) (`Timeline|SpawnBlob` :!via `PlayFromStart`)
        (:`Update`
          (`SceneComponent.K2_SetRelativeTransform` (`self.StaticMesh`) (`KismetMathLibrary.TLerp` (`self.MeshStartingTransform`) (`self.TransformSquished`) _0_1_0_over_1_sec) false false))
        (:`Finished`
          (`self.AllowVisualizing`))))))

(event `DecreaseHistoricMaxEnv`
  ;[1 1 1] decrease max historic vol
  (bind _output_get (set `self.EnvMax` (* (stale _output_get) 0.95))))

(event `/Game/ArthursAudioBPs/Core/Interfaces/AabpsMidiInterface.NotePlay`
  (params (Note :type "Float (single-precision)") (Velocity :type Integer) (Duration :type "Float (single-precision)") (Channel :type Integer))
  (bind _modularsynth (`self.ModularSynth`))
  ;[1 1 1] note in event
  (`|ExecutionSequence`
    (:`then_0`
      (`|ExecutionSequence`
        (:`then_0`
          ;[1 1 1] activate synth if we need to activate
          (if (not (`ActorComponent.IsActive` _modularsynth))
            (`ActorComponent.SetActive` _modularsynth true false)))
        (:`then_1`
          ;[1 1 1] play synth notes
          (if (`self.PlayOnlyOneRandomNoteFromChord`)
            ;;[1 1 1] play one unique note
            (`ModularSynthComponent.NoteOn` (`self.ModularSynth`) (`self.SelectedUniqueNote`) (`self.Velocity`) -1.0)
            (else
              ;;[1 1 1] play all notes in chord
              (for _array_element (`self.AllNotes`)
                (`ModularSynthComponent.NoteOn` (`self.ModularSynth`) _array_element (`self.Velocity`) -1.0)))))))
    (:`then_1`
      ;[1 1 1] deactivate after 10 seconds of inactivity
      (`KismetSystemLibrary.RetriggerableDelay` (`self.NoteLength`))
      (`ModularSynthComponent.NoteOff` (`self.ModularSynth`) 0.0 true false)
      (bind _output_get (set `self.Life` (`KismetMathLibrary.MapRangeClamped` (`GameplayStatics.GetWorldDeltaSeconds`) 0.02 0.009 1.0 8.0)))
      (`KismetSystemLibrary.RetriggerableDelay` _output_get)
      (`ActorComponent.Deactivate` (`self.ModularSynth`)))))

(event `self.ModularSynth.OnAudioEnvelopeValue`
  (params (EnvelopeValue :type "Float (single-precision)"))
  (bind (_h _s _v _a) (`KismetMathLibrary.RGBToHSV` (`self.Color`)))
  (bind (_h_2 _s_2 _v_2 _a_2) (`KismetMathLibrary.RGBToHSV` (`self.Color`)))
  ;[1 1 1] latest synth volume
  (set `self.EnvLatest` EnvelopeValue)
  ;[1 1 1] allow visualizing?
  (`/Engine/EditorBlueprintResources/StandardMacros.Gate` true :!label _label
    (:`Exit`
      ;[1 1 1] normalize
      (if (> (`self.EnvLatest`) (`self.EnvMax`))
        (set `self.EnvMax` (`self.EnvLatest`)))
      (set `self.Vol0-1` (`KismetMathLibrary.MapRangeClamped` (`self.EnvLatest`) 0.0 (`self.EnvMax`) 0.0 1.0))
      ;[1 1 1] mod material
      (`MaterialInstanceDynamic.SetScalarParameterValue` (`self.MID`) "Emissive Multiplier" (* (`self.Vol0-1`) (`self.EmissiveMultiplier`)))
      (`MaterialInstanceDynamic.SetVectorParameterValue` (`self.MID`) "Base Color" (`KismetMathLibrary.LinearColorLerp` (`KismetMathLibrary.HSVToRGB` _h_2 _s_2 0.5 _a_2) (`KismetMathLibrary.HSVToRGB` _h _s 1.0 _a) (`self.Vol0-1`)))
      ;[1 1 1] move mesh up and down
      (`SceneComponent.K2_SetRelativeTransform` (`self.StaticMesh`) (`|EaseFunction` "ExpoIn" (`self.Vol0-1`) (`self.MeshStartingTransform`) (`self.MeshVizMaxTransform`)) false false))))

(event `AllowVisualizing`
  ;[1 1 1] allow visualizing?
  (goto _label :!via `Open`))

(fn `Randomize Preset`
  (params (PresetType :type "PrimaryDataAsset Object Reference"))
  (returns (NewParam :type Boolean))
  (locals (SpicyRandomSeed :type Integer :default 0))
  (set `local.SpicyRandomSeed` (+ (`KismetMathLibrary.RandomIntegerInRange` -1000000 1000000) (`KismetMathLibrary.FTrunc` (* (`.PartialSeconds` (`GameplayStatics.GetAccurateRealTime`)) 100000.0))))
  ;[1 1 1] Find the right type of  data primary asset for randomizing
  (bind _asbasic (cast `/Game/ArthursAudioBPs/Core/FunctionLibraries/ModSynthPresetRandomizer/Types/Basic` PresetType)
    (:`then`
      (bind _synthpresetfinal (`/Game/ArthursAudioBPs/Core/FunctionLibraries/ModSynthPresetRandomizer/Types/Basic.RandomizePresetFull` _asbasic (`local.SpicyRandomSeed`)))
      (set `self.SynthBasePreset` _synthpresetfinal))
    (:`CastFailed`
      (bind _ascomplex (cast `/Game/ArthursAudioBPs/Core/FunctionLibraries/ModSynthPresetRandomizer/Types/Complex` PresetType))
      (bind _synthpresetfinal_2 (`/Game/ArthursAudioBPs/Core/FunctionLibraries/ModSynthPresetRandomizer/Types/Complex.RandomizePresetFull` _ascomplex (`local.SpicyRandomSeed`)))
      (set `self.SynthBasePreset` _synthpresetfinal_2)))
  (return false))

(fn `Re-randomize preset and re-init synth`
  (params (PresetType :type "PrimaryDataAsset Object Reference"))
  ;[1 1 1] randomized synth preset
  (`self.Randomize Preset` PresetType)
  (`ModularSynthComponent.SetSynthPreset` (`self.ModularSynth`) (`self.SynthBasePreset`)))

(fn `UserConstructionScript`
  (bind _allnotes (`self.AllNotes`))
  (bind _modularsynth (`self.ModularSynth`))
  (`|ExecutionSequence`
    (:`then_0`
      ;[1 1 1] set up mesh/visualizer
      (`SceneComponent.K2_SetRelativeTransform` (`self.StaticMesh`) (`self.MeshStartingTransform`) false false)
      (`StaticMeshComponent.SetStaticMesh` (`self.StaticMesh`) (`self.MeshToUse`)))
    (:`then_1`
      ;[1 1 1] set up synth
      ;;[1 1 1] spawn synth with or without source chain for doppler/speed of sound
      (if (`self.SimulateSoundPropagation`)
        (bind _returnvalue (`AddComponent|NODE_AddModularSynthComponent-0`))
        (set `self.ModularSynth` _returnvalue)
        (else
          (bind _returnvalue_2 (`AddComponent|NODE_AddModularSynthComponent-1`))
          (set `self.ModularSynth` _returnvalue_2)))
      (set `SynthComponent.AttenuationSettings` (`self.AttenuationSettings`) (`self.ModularSynth`))
      (set `SynthComponent.bAllowSpatialization` true (`self.ModularSynth`))
      (set `SynthComponent.EnvelopeFollowerAttackTime` 500 _modularsynth)
      (set `SynthComponent.EnvelopeFollowerReleaseTime` 2000 _modularsynth))
    (:`then_2`
      ;[1 1 1] find squish position
      (set `self.TransformSquished` (`KismetMathLibrary.MakeTransform` (+ (.location (`self.MeshStartingTransform`)) (.location (`self.TransformSquishFactor`))) (.rotation (`self.MeshStartingTransform`)) (* (.scale (`self.MeshStartingTransform`)) (.scale (`self.TransformSquishFactor`))))))
    (:`then_3`
      ;[1 1 1] random synth preset
      (bind _modularsynth_preset (`/Game/ArthursAudioBPs/Core/FunctionLibraries/ModSynthPresetRandomizer/SynthPresetRandomizerHelpers.GenerateRandomModularSynthPreset` (`self.PresetGeneratorRandom`)))
      (set `self.SynthBasePreset` _modularsynth_preset)
      (`ModularSynthComponent.SetSynthPreset` (`self.ModularSynth`) (`self.SynthBasePreset`))
      ;[1 1 1] get chord
      (set `self.AllNotes` (`/Game/ArthursAudioBPs/Core/FunctionLibraries/AabpsMidiChordGenerator/AabpsMidiChordGenerator.BuildMusicalMidiChord` (`self.ChordSettings`)))
      ;[1 1 1] make special random note
      (set `self.SelectedUniqueNote` (`KismetMathLibrary.SelectFloat` (`|GetArrayItem` _allnotes) (`|GetArrayItem` _allnotes (`KismetMathLibrary.RandomIntegerInRange` 0 (`KismetArrayLibrary.Array_LastIndex` _allnotes))) (`self.UseRootNoteOnly`))))
    (:`then_4`
      ;[1 1 1] set up collision
      (`PrimitiveComponent.SetCollisionObjectType` (`self.StaticMesh`) "ECC_GameTraceChannel1")
      (`PrimitiveComponent.SetCollisionResponseToAllChannels` (`self.StaticMesh`) (`self.PhysicsCollisionType`))
      ;;[1 1 1] always overlap plants-overlapper
      (`PrimitiveComponent.SetCollisionResponseToChannel` (`self.StaticMesh`) "ECC_GameTraceChannel1" "ECR_Overlap"))))