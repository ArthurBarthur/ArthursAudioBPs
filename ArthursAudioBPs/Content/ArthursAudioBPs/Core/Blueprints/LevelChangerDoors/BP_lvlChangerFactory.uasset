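; Construction-script factory that lays out a ring of BP_lvlChanger level-change doors, one per entry in the Levels list.
; It spawns each as a child actor at even angles on a set radius, with GapSize reserving empty slots in the circle.
; Doors share a scale and yaw offset and can optionally rotate with their angle around the center.
; A second pass assigns each door its level and refreshes its text.
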(fn `UserConstructionScript`
  (`KismetArrayLibrary.Array_Clear` (`self.lvlChangers`))
  ;[1 1 1] loop over list of levels
  (for (_ _array_index) (`self.Levels`)
    (bind _returnvalue (`KismetMathLibrary.MakeRotator` 0.0 0.0 (* (+ _array_index 1) (/ 360.0 (`KismetMathLibrary.Conv_IntToDouble` (+ (`KismetArrayLibrary.Array_Length` (`self.Levels`)) (`self.GapSize`)))))))
    ;[1 1 1] spawn lvlChangers
    (bind _returnvalue_2 (`AddComponent|NODE_AddChildActorComponent-0` :`RelativeTransform` (`KismetMathLibrary.MakeTransform` (`KismetMathLibrary.GreaterGreater_VectorRotator` (`KismetMathLibrary.MakeVector` (`self.Radius`)) _returnvalue) (`KismetMathLibrary.MakeRotator` (.roll (`KismetMathLibrary.SelectRotator` _returnvalue (struct) (`self.OrientToCenter`))) (.pitch (`KismetMathLibrary.SelectRotator` _returnvalue (struct) (`self.OrientToCenter`))) (+ (.yaw (`KismetMathLibrary.SelectRotator` _returnvalue (struct) (`self.OrientToCenter`))) (`self.YawOffset`))) (`self.DoorScale`))))
    (bind _asbp_lvl_changer (cast `/Game/ArthursAudioBPs/Core/Blueprints/LevelChangerDoors/BP_lvlChanger` (`ChildActorComponent.ChildActor` _returnvalue_2))
      (:`then`
        (`KismetArrayLibrary.Array_Add` (`self.lvlChangers`) _asbp_lvl_changer))
      (:`CastFailed`
        (`KismetSystemLibrary.PrintString` "child actor cast failed"))))
  (for (_array_element _array_index_2) (`self.lvlChangers`)
    (set `/Game/ArthursAudioBPs/Core/Blueprints/LevelChangerDoors/BP_lvlChanger.LevelToLoad` (`|GetArrayItem` (`self.Levels`) _array_index_2) _array_element)
    (`/Game/ArthursAudioBPs/Core/Blueprints/LevelChangerDoors/BP_lvlChanger.UpdateText` _array_element)))