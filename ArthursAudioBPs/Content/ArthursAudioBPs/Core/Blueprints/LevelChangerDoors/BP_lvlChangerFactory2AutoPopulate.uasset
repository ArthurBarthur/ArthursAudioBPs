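; Level-changer door factory that automatically builds a ring of BP_lvlChanger doors, one for each map in the Maps/Examples folder.
; The construction script and Refreshdoors event scan the Asset Registry, rebuilding only when map names or valid door count differ.
; SpawnDoors adds child actors around a configurable radius and gap, optionally oriented to center.
; Each door then receives its LevelToLoad and refreshes its text.
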(event `Refresh doors`
  (bind _different (`self.CheckIfLevelsHaveChanged` (`self.Levels`)))
  (if _different
    (`self.PopulateLevelList`)
    (`self.SpawnDoors`)))

(fn `CheckIfLevelsHaveChanged`
  (params (Levels :type "Array of Name (by ref)"))
  (returns (Different :type Boolean))
  (locals (FreshScannedLevels :type "Array of Name") (ExistingLevels :type "Array of Name") (ActualSpwndLevelDoors :type "Array of /Game/ArthursAudioBPs/Core/Blueprints/LevelChangerDoors/BP_lvlChanger Object Reference") (DiffFound :type Boolean :default false))
  (set `local.ExistingLevels` Levels)
  ;[1 1 1] do fresh scan of level assets
  (bind _outassetdata (`AssetRegistry.GetAllAssets` (`AssetRegistryHelpers.GetAssetRegistry`) false))
  (for _array_element _outassetdata
    (bind (_objectpath _packagename _packagepath _assetname _assetclass) (break `AssetData` _array_element))
    (if (`KismetStringLibrary.EqualEqual_StrStr` (`KismetStringLibrary.Conv_NameToString` _assetclass) "World")
      (if (`KismetStringLibrary.StartsWith` (`KismetStringLibrary.Conv_NameToString` _objectpath) "/Game/ArthursAudioBPs/Maps/Examples/")
        (`KismetArrayLibrary.Array_Add` (`local.FreshScannedLevels`) _assetname))))
  ;[1 1 1] look for any differences
  ;;[1 1 1] find existing valid doors
  (for _array_element_2 (`self.lvlChangers`)
    (if (`KismetStringLibrary.Contains` (`KismetSystemLibrary.GetDisplayName` _array_element_2) "lvlChanger")
      (if (not (`KismetStringLibrary.Contains` (`KismetSystemLibrary.GetObjectName` _array_element_2) "destroyed"))
        (`KismetArrayLibrary.Array_Add` (`local.ActualSpwndLevelDoors`) _array_element_2))))
  ;;[1 1 1] same amount of spawned doors as fresh levels?
  (if (== (`KismetArrayLibrary.Array_Length` (`local.ActualSpwndLevelDoors`)) (`KismetArrayLibrary.Array_Length` (`local.FreshScannedLevels`)))
    ;;[1 1 1] same amount of existing levels in list as in fresh scanned list?
    (if (== (`KismetArrayLibrary.Array_Length` (`local.ExistingLevels`)) (`KismetArrayLibrary.Array_Length` (`local.FreshScannedLevels`)))
      ;;[1 1 1] all the same entries?
      (for (_array_element_3 _array_index) (`local.FreshScannedLevels`)
        (if (< (`KismetArrayLibrary.Array_Find` (`local.ExistingLevels`) _array_element_3) 0)
          (set `local.DiffFound` true)))
      (else
        (set `local.DiffFound` true)))
    (else
      (set `local.DiffFound` true)))
  (return (`local.DiffFound`)))

(fn `PopulateLevelList`
  ;[1 1 1] create updated level list
  (`KismetArrayLibrary.Array_Clear` (`self.Levels`))
  (bind _outassetdata (`AssetRegistry.GetAllAssets` (`AssetRegistryHelpers.GetAssetRegistry`) false))
  (for _array_element _outassetdata
    (bind (_objectpath _packagename _packagepath _assetname _assetclass) (break `AssetData` _array_element))
    (if (`KismetStringLibrary.EqualEqual_StrStr` (`KismetStringLibrary.Conv_NameToString` _assetclass) "World")
      (if (`KismetStringLibrary.StartsWith` (`KismetStringLibrary.Conv_NameToString` _objectpath) "/Game/ArthursAudioBPs/Maps/Examples/")
        (`KismetArrayLibrary.Array_Add` (`self.Levels`) _assetname)))))

(fn `SpawnDoors`
  ;[1 1 1] spawn doors from level-list
  (`KismetArrayLibrary.Array_Clear` (`self.lvlChangers`))
  ;;[1 1 1] loop over list of levels
  (for (_ _array_index) (`self.Levels`)
    (bind _returnvalue (`KismetMathLibrary.MakeRotator` 0.0 0.0 (* (+ _array_index 1) (/ 360.0 (`KismetMathLibrary.Conv_IntToDouble` (+ (`KismetArrayLibrary.Array_Length` (`self.Levels`)) (`self.GapSize`)))))))
    ;;[1 1 1] spawn lvlChangers
    (bind _returnvalue_2 (`AddComponent|NODE_AddChildActorComponent-0` :`RelativeTransform` (`KismetMathLibrary.MakeTransform` (`KismetMathLibrary.GreaterGreater_VectorRotator` (`KismetMathLibrary.MakeVector` (`self.Radius`)) _returnvalue) (`KismetMathLibrary.MakeRotator` (.roll (`KismetMathLibrary.SelectRotator` _returnvalue (struct) (`self.OrientToCenter`))) (.pitch (`KismetMathLibrary.SelectRotator` _returnvalue (struct) (`self.OrientToCenter`))) (+ (.yaw (`KismetMathLibrary.SelectRotator` _returnvalue (struct) (`self.OrientToCenter`))) (`self.YawOffset`))) (`self.DoorScale`))))
    (bind _asbp_lvl_changer (cast `/Game/ArthursAudioBPs/Core/Blueprints/LevelChangerDoors/BP_lvlChanger` (`ChildActorComponent.ChildActor` _returnvalue_2))
      (:`then`
        (`KismetArrayLibrary.Array_Add` (`self.lvlChangers`) _asbp_lvl_changer))
      (:`CastFailed`
        (`KismetSystemLibrary.PrintString` "child actor cast failed"))))
  (for (_array_element _array_index_2) (`self.lvlChangers`)
    (set `/Game/ArthursAudioBPs/Core/Blueprints/LevelChangerDoors/BP_lvlChanger.LevelToLoad` (`|GetArrayItem` (`self.Levels`) _array_index_2) _array_element)
    (`/Game/ArthursAudioBPs/Core/Blueprints/LevelChangerDoors/BP_lvlChanger.UpdateText` _array_element)))

(fn `UserConstructionScript`
  (bind _different (`self.CheckIfLevelsHaveChanged` (`self.Levels`)))
  (if _different
    (`self.PopulateLevelList`)
    (`self.SpawnDoors`)))