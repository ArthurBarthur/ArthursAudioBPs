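; Audio-visualization actor that turns a door's hinge motion into spatialized granular synth sound when IsDoor is set.
; On BeginPlay it configures the synth from a preset in scrub mode, then opens a gated Tick that starts a sustained note.
; Each tick, door rotation scrubs the sample playhead, optionally reversed, and door velocity feeds volume and grain settings.
; The synth's audio envelope drives the mesh's Z scale, color and emissive glow.
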(event `self.ReceiveBeginPlay`
  ;[1 1 1] beginPlay
  (`KismetSystemLibrary.Delay` 1.0)
  ;[1 1 1] init granular
  ;;[1 1 1] init preset ref
  (set `self.GranularPreset` (make `/Game/AudioVisualization/Blueprints/GranularSynth/granularPreset` 10.0 10.0 30.0 0.7 0.0 0.0 "FromBeginning" 1.0 20.0 1.0 1.0 (0.0 0.0) 100.0 (0.0 0.0) 0.0 (0.0 0.0) 1.0 (0.0 0.0) true "Triangle"))
  ;;[1 1 1] add gran
  (set `self.DerGranular` (`self.GranularSynth`))
  ;;[1 1 1] bind env event
  (add `SynthComponent.OnAudioEnvelopeValue` (`self.DerGranular`) (delegate `EventLatestEnv`))
  ;;[1 1 1] set concurrency
  (set `SynthComponent.ConcurrencySet` (`|MakeSet` "/Game/AudioVisualization/Blueprints/GranularSynth/GranularSoundConcurrency.GranularSoundConcurrency" :!type "SoundConcurrency Object Reference") (`self.DerGranular`))
  ;;[1 1 1] propagation settings
  (set `SynthComponent.bAllowSpatialization` true (`self.DerGranular`))
  (set `SynthComponent.AttenuationSettings` "/Game/AudioVisualization/Blueprints/GranularSynth/GranularSoundAttenuation.GranularSoundAttenuation" (`self.DerGranular`))
  ;;[1 1 1] update preset
  (`self.UpdateGranSettings` (`self.DerGranular`) (`self.GranularPreset`))
  ;;[1 1 1] set sound on gran
  (`GranularSynth.SetSoundWave` (`self.DerGranular`) (`self.ActiveSound`))
  ;;[1 1 1] start
  (`KismetSystemLibrary.Delay` 0.5)
  (`self.startGran` (`self.DerGranular`))
  ;[1 1 1] create and set MID
  (bind _returnvalue (`KismetMaterialLibrary.CreateDynamicMaterialInstance` "/Game/AudioVisualization/Assets/Materials/m_SimpleMat_Inst1.m_SimpleMat_Inst1"))
  (bind _output_get (set `self.granboxMID` _returnvalue))
  (`PrimitiveComponent.SetMaterial` (`self.StaticMesh`) 0 _output_get)
  ;[1 1 1] open tick gate
  (`self.OpenTickGate`))

(event `EventLatestEnv`
  (params (EnvelopeValue :type "Float (double-precision)"))
  ;[1 1 1] init granular
  ;;[1 1 1] bind env event
  (set `self.LatestEnv` EnvelopeValue))

(event `self.ReceiveTick`
  (params (DeltaSeconds :type "Float (single-precision)"))
  (bind _latestenv (`self.LatestEnv`))
  (bind _granboxmid (`self.granboxMID`))
  (bind _returnvalue (`KismetMathLibrary.FClamp` (* _latestenv 20.0)))
  ;[1 1 1] tick
  (set `self.LatestTickDelta` DeltaSeconds)
  ;[1 1 1] tick gate
  (`/Engine/EditorBlueprintResources/StandardMacros.Gate` true :!label _label
    (:`Exit`
      (`|ExecutionSequence`
        (:`then_0`
          ;[1 1 1] start granular
          ;;[1 1 1] once
          (`/Engine/EditorBlueprintResources/StandardMacros.DoOnce` false
            (:`Completed`
              (`self.Start`))))
        (:`then_1`
          ;[1 1 1] env scale mesh
          (`SceneComponent.SetRelativeScale3D` (`self.StaticMesh`) (`KismetMathLibrary.MakeVector` 1.0 1.0 (`KismetMathLibrary.MapRangeUnclamped` (* _latestenv 50.0) 0.0 1.0 1.0 10.0))))
        (:`then_2`
          ;[1 1 1] mod MID
          (`MaterialInstanceDynamic.SetScalarParameterValue` _granboxmid "Emissive Multiplier" (* _returnvalue 200.0))
          (`MaterialInstanceDynamic.SetVectorParameterValue` _granboxmid "Base Color" (`KismetMathLibrary.LinearColorLerp` (struct :`A` 1.0) (struct :`R` 1.0 :`G` 0.918136 :`A` 1.0) _returnvalue)))
        (:`then_3`
          (if (`self.IsDoor`)
            ;[1 1 1] RECEIVE DOOR and update granular
            (`self.ReceiveDoor`)
            ;[1 1 1] print granular debug(current sample play position in percent)
            (if (> (`self.CopiedLatestVelocity`) 1.0)
              (`KismetSystemLibrary.PrintString` (`KismetStringLibrary.BuildString_Double` "" "SamplePositionInPercent:" (* (/ (`self.CurrentPlayheadScrubPosition`) (`SoundBase.Duration` (`self.ActiveSound`))) 100.0)) true true (struct :`G` 0.66 :`B` 1.0 :`A` 1.0) (`self.LatestTickDelta`)))))))))

(event `OpenTickGate`
  ;[1 1 1] tick gate
  (goto _label :!via `Open`))

(event `Start`
  ;[1 1 1] start
  (`GranularSynth.NoteOn` (`self.DerGranular`) 60.0 100 -1.0))

(event `Stop`
  ;[1 1 1] stop
  (`GranularSynth.NoteOff` (`self.DerGranular`) 60.0 false))

(fn `ReceiveDoor`
  (locals (Door :type "/Game/AudioVisualization/Blueprints/GranularSynth/bp_door Object Reference"))
  (bind _duration (`SoundBase.Duration` (`self.ActiveSound`)))
  (bind _returnvalue (`KismetMathLibrary.FClamp` (`KismetMathLibrary.MapRangeClamped` (`self.CopiedLatestVelocity`) 5.0 50.0 30.0 30.0) 10.0 50.0))
  (bind _returnvalue_2 (- _duration (/ (`.DurationBaseMsec_55_629930E44F1507F01122F697D24D492F` (break `/Game/AudioVisualization/Blueprints/GranularSynth/granularPreset` (`self.GranularPreset`))) 1000.0)))
  (bind _returnvalue_3 (`KismetMathLibrary.FClamp` (`KismetMathLibrary.MapRangeClamped` (`KismetMathLibrary.MapRangeClamped` (`self.CopiedLatestPosition`) 360.0 0.0 0.0 360.0) 0.0 (`self.CopiedLatestMaxPosition`) 0.0 _duration) 0.0 _returnvalue_2))
  ;[1 1 1] IF DOOR: get latest values once per tick
  (bind _asbp_door (cast `/Game/AudioVisualization/Blueprints/GranularSynth/bp_door` (`self.ActualdoorRef`)))
  (set `local.Door` _asbp_door)
  (set `self.CopiedLatestVelocity` (`/Game/AudioVisualization/Blueprints/GranularSynth/bp_door.DoorVelocity0-2000` _asbp_door))
  (set `self.CopiedLatestPosition` (`/Game/AudioVisualization/Blueprints/GranularSynth/bp_door.LatestDoorRot360-0` _asbp_door))
  (set `self.CopiedLatestMaxPosition` (`/Game/AudioVisualization/Blueprints/GranularSynth/bp_door.DoorMaxSwingAngle` _asbp_door))
  ;[1 1 1] live preset
  (set `self.CurrentPlayheadScrubPosition` (`KismetMathLibrary.SelectFloat` (`KismetMathLibrary.MapRangeClamped` _returnvalue_3 0.0 _returnvalue_2 _returnvalue_2) _returnvalue_3 (`self.Reverse`)))
  ;[1 1 1] update granular
  (bind _structout (setmembers `/Game/AudioVisualization/Blueprints/GranularSynth/granularPreset` :`StructRef` (`self.GranularPreset`) :`AttackMsec` _returnvalue :`ReleaseMsec` _returnvalue :`DecayMsec` _returnvalue :`PlayheadPosSec` (`self.CurrentPlayheadScrubPosition`) :`GrainsPerSecond` (`KismetMathLibrary.FClamp` (`KismetMathLibrary.MapRangeClamped` (`self.CopiedLatestVelocity`) 1.0 50.0 60.0 60.0) 0.0 60.0) :`GrainProbability` (select `bool` (`self.OverrideGrainProbability`) :`false` (`KismetMathLibrary.FClamp` (`KismetMathLibrary.MapRangeClamped` (`self.CopiedLatestVelocity`) 30.0 0.0 1.0)) :`true` (`self.GrainProbability0-1`)) :`VolumeBase` (`KismetMathLibrary.FClamp` (* (`KismetMathLibrary.MapRangeClamped` (`self.CopiedLatestVelocity`) 0.7 20.0 0.0 1.0) (`self.GranVolMp`))) :`DurationBaseMsec` (`KismetMathLibrary.FClamp` (`KismetMathLibrary.MapRangeClamped` (`self.CopiedLatestVelocity`) 1.0 50.0 50.0 50.0) 50.0 200.0)))
  (`self.UpdateGranSettings` (`self.DerGranular`) _structout))

(fn `startGran`
  (params (Gransynth :type "GranularSynth Object Reference"))
  (`ActorComponent.Activate` Gransynth false)
  (`SynthComponent.Start` Gransynth))

(fn `StopGran`
  (params (Gransynth :type "GranularSynth Object Reference"))
  (`SynthComponent.Stop` Gransynth)
  (`ActorComponent.Deactivate` Gransynth))

(fn `UpdateGranSettings`
  (params (GranSynth :type "GranularSynth Object Reference") (granularPreset :type "/Game/AudioVisualization/Blueprints/GranularSynth/granularPreset Structure (by ref)"))
  (bind (_attackmsec _releasemsec _decaymsec _sustaingain _playheadpossec _playheadlerpsec _playheadseektype _playheadspeedrate _grainspersecond _grainprobability _volumebase _volumerange _durationbasemsec _durationrange _panbase _panrange _pitchbase _pitchrange _scrubmode _envelopetype) (break `/Game/AudioVisualization/Blueprints/GranularSynth/granularPreset` granularPreset))
  (`|ExecutionSequence`
    (:`then_0`
      ;[1 1 1] ADSR
      (`GranularSynth.SetAttackTime` GranSynth _attackmsec))
    (:`then_1`
      (`GranularSynth.SetReleaseTimeMsec` GranSynth _releasemsec))
    (:`then_2`
      (`GranularSynth.SetDecayTime` GranSynth _decaymsec))
    (:`then_3`
      (`GranularSynth.SetSustainGain` GranSynth _sustaingain))
    (:`then_4`
      (`GranularSynth.SetPlayheadTime` GranSynth _playheadpossec _playheadlerpsec _playheadseektype))
    (:`then_5`
      (`GranularSynth.SetPlaybackSpeed` GranSynth _playheadspeedrate))
    (:`then_6`
      (`GranularSynth.SetGrainsPerSecond` GranSynth _grainspersecond))
    (:`then_7`
      (`GranularSynth.SetGrainProbability` GranSynth _grainprobability))
    (:`then_8`
      (`GranularSynth.SetGrainVolume` GranSynth _volumebase _volumerange))
    (:`then_9`
      (`GranularSynth.SetGrainDuration` GranSynth _durationbasemsec _durationrange))
    (:`then_10`
      (`GranularSynth.SetGrainPan` GranSynth _panbase _panrange))
    (:`then_11`
      (`GranularSynth.SetGrainPitch` GranSynth _pitchbase _pitchrange))
    (:`then_12`
      (`GranularSynth.SetScrubMode` GranSynth _scrubmode))
    (:`then_13`
      (`GranularSynth.SetGrainEnvelopeType` GranSynth _envelopetype))))

(fn `UserConstructionScript`)