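; Audio visualizer actor that shows submix frequency magnitudes as a row of meshes with Z scale and emissive glow following the sound.
; Finds a Bp_SubmixAnalyzer, retrying until valid, then spawns a mesh and dynamic material per analyzed frequency.
; Each tick normalizes the latest magnitudes against recorded peaks, per frequency or shared.
; Optional attack/release interpolation smooths the values before they drive scale and emissive strength.
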(event `self.ReceiveBeginPlay`
  ;[1 1 1] beginplay
  ;[1 1 1] don't proceed without a reference to SubmixAnalyzer
  (`/Engine/EditorBlueprintResources/StandardMacros.IsValid` (stale _output_get) :!label _label
    (:`Is Valid`
      _)
    (:`Is Not Valid`
      (bind _outactors (`GameplayStatics.GetAllActorsOfClass` "/Game/AudioVisualization/Blueprints/AudioViz/bp_SubmixAnalyzer.bp_SubmixAnalyzer_C"))
      (bind _output (`|GetArrayItem` _outactors))
      (`/Engine/EditorBlueprintResources/StandardMacros.IsValid` _output
        (:`Is Valid`
          (bind _output_get (set `self.SubmixAnalyzerRef` _output)))
        (:`Is Not Valid`
          (`KismetSystemLibrary.Delay` 2.0)
          (goto _label)))))
  (`|ExecutionSequence`
    (:`then_0`
      ;[1 1 1] get frequencies to analyze from SubmixAnalyzer
      (set `self.FrequenciesToAnalyze` (`/Game/AudioVisualization/Blueprints/AudioViz/bp_SubmixAnalyzer.FrequenciesToAnalyze` (`self.SubmixAnalyzerRef`))))
    (:`then_1`
      ;[1 1 1] spawn visualizing meshes
      (`self.SpawnVisualizerMeshes`))
    (:`then_2`
      ;[1 1 1] initialize array of max magnitudes
      (for (_ _array_index) (`self.FrequenciesToAnalyze`)
        (`KismetArrayLibrary.Array_Set` (`self.MaxMagnitudes`) _array_index 0.0 true)))
    (:`then_3`
      ;[1 1 1] initialize dynamic materials(MIDs)
      (`self.InitializeDynamicMaterials`))
    (:`then_4`
      ;[1 1 1] open tick gate
      (`self.OpenTickGate`))))

(event `self.ReceiveTick`
  (params (DeltaSeconds :type "Float (single-precision)"))
  ;[1 1 1] Tick
  (set `self.DeltaTick` DeltaSeconds)
  ;[1 1 1] Tick-Gate
  (`/Engine/EditorBlueprintResources/StandardMacros.Gate` true :!label _label_2
    (:`Exit`
      (`|ExecutionSequence`
        (:`then_0`
          ;[1 1 1] get latest central analysis
          (set `self.LatestMagnitudes` (`/Game/AudioVisualization/Blueprints/AudioViz/bp_SubmixAnalyzer.LatestMagnitudes` (`self.SubmixAnalyzerRef`))))
        (:`then_1`
          ;[1 1 1] store max recorded magnitudes
          (`self.StoreMaxMagnitudes`))
        (:`then_2`
          ;[1 1 1] normalize. (magnitudes to 0-1)
          (`self.NormalizeMagnitudes`))
        (:`then_3`
          ;[1 1 1] smoothing?
          (if (`self.SmoothInterpolation`)
            ;[1 1 1] smoothing.
            (`|ExecutionSequence`
              (:`then_0`
                (`/Engine/EditorBlueprintResources/StandardMacros.DoOnce` false
                  (:`Completed`
                    (`self.InitSmoothing`))))
              (:`then_1`
                ;;[1 1 1] smoothen values
                (`self.Smoothing`)))))
        (:`then_4`
          ;[1 1 1] Update mesh scales
          (`self.ScaleMeshes`))
        (:`then_5`
          ;[1 1 1] Update dynamic material emissive strength
          (`self.UpdateMaterialEmissive`))))))

(event `OpenTickGate`
  ;[1 1 1] Tick-Gate
  (goto _label_2 :!via `Open`))

(fn `InitializeDynamicMaterials`
  (locals (_currentIndex :type Integer) (_currentMesh :type "StaticMeshComponent Object Reference"))
  ;[1 1 1] loop through meshes
  (for (_array_element _array_index) (`self.VizMeshes`)
    (`|ExecutionSequence`
      (:`then_0`
        ;[1 1 1] store local variables
        (set `local._currentMesh` _array_element)
        (set `local._currentIndex` _array_index))
      (:`then_1`
        ;[1 1 1] create dynamic materials(MIDs)
        (bind _returnvalue (`KismetMaterialLibrary.CreateDynamicMaterialInstance` (`self.BaseMaterial`)))
        (`KismetArrayLibrary.Array_Set` (`self.MIDs`) (`local._currentIndex`) _returnvalue true))
      (:`then_2`
        ;[1 1 1] put MIDs on meshes
        (`PrimitiveComponent.SetMaterial` (`local._currentMesh`) 0 (`|GetArrayItem` (`self.MIDs`) (`local._currentIndex`)))))))

(fn `InitSmoothing`
  ;[1 1 1] fill smoothed values array with the correct amount of zeroes
  (for (_ _array_index) (`self.NormalizedValues`)
    (`KismetArrayLibrary.Array_Set` (`self.SmoothedValues`) _array_index 0.0 true)))

(fn `NormalizeMagnitudes`
  (locals (_currentIndex :type Integer))
  ;[1 1 1] Normalize all freqs independently?
  (if (not (`self.NormalizeEachFrequencyIndependently`))
    (`self.UseOnlyTopMagnitudeForMax`))
  ;[1 1 1] loop through latest magnitudes
  (for (_array_element _array_index) (`self.LatestMagnitudes`)
    (set `local._currentIndex` _array_index)
    ;[1 1 1] Store Normalized magnitudes
    (`KismetArrayLibrary.Array_Set` (`self.NormalizedValues`) (`local._currentIndex`) (`KismetMathLibrary.MapRangeClamped` _array_element 0.0 (`|GetArrayItem` (`self.MaxMagnitudes`) (`local._currentIndex`)) 0.0 1.0) true)))

(fn `ScaleMeshes`
  (locals (_currentIndex :type Integer) (_currentMesh :type "StaticMeshComponent Object Reference"))
  ;[1 1 1] loop through meshes
  (for (_array_element _array_index) (`self.VizMeshes`)
    (set `local._currentMesh` _array_element)
    (set `local._currentIndex` _array_index)
    ;[1 1 1] set new mesh scale
    (`SceneComponent.SetRelativeScale3D` (`local._currentMesh`) (`KismetMathLibrary.MakeVector` 1.0 1.0 (+ (* (`|GetArrayItem` (select `bool` (`self.SmoothInterpolation`) :`false` (`self.NormalizedValues`) :`true` (`self.SmoothedValues`)) (`local._currentIndex`)) (`self.MeshScaleMultiplier`)) 1.0)))))

(fn `Smoothing`
  (locals (_latestNormalizedValue :type "Float (double-precision)") (_currentIndex :type Integer) (_latestSmoothValue :type "Float (double-precision)" :default 0.0))
  ;[1 1 1] loop through normalized values
  (for (_array_element _array_index) (`self.NormalizedValues`)
    (set `local._latestNormalizedValue` _array_element)
    (set `local._currentIndex` _array_index)
    ;[1 1 1] store smoothed values
    (`KismetArrayLibrary.Array_Set` (`self.SmoothedValues`) (`local._currentIndex`) (`KismetMathLibrary.FInterpTo` (`|GetArrayItem` (`self.SmoothedValues`) (`local._currentIndex`)) (`local._latestNormalizedValue`) (`self.DeltaTick`) (select `bool` (> (`local._latestNormalizedValue`) (`|GetArrayItem` (`self.SmoothedValues`) (`local._currentIndex`))) :`false` (`self.Release`) :`true` (`self.Attack`))) true)))

(fn `SpawnVisualizerMeshes`
  (locals (_currentIndex :type Integer))
  (bind _vizmeshes (`self.VizMeshes`))
  ;[1 1 1] clear out old existing meshes if any
  (for _array_element _vizmeshes
    (`ActorComponent.K2_DestroyComponent` _array_element))
  (`KismetArrayLibrary.Array_Clear` _vizmeshes)
  ;[1 1 1] loop through frequencies
  (for (_ _array_index) (`self.FrequenciesToAnalyze`)
    ;[1 1 1] spawn visualizer meshes in a row
    (set `local._currentIndex` _array_index)
    (bind _returnvalue (`AddComponent|NODE_AddStaticMeshComponent-0` :`RelativeTransform` (`KismetMathLibrary.MakeTransform` (`KismetMathLibrary.MakeVector` 0.0 (* (`local._currentIndex`) (`self.MeshRowDistanceOffset`))))))
    ;[1 1 1] store mesh references
    (`KismetArrayLibrary.Array_Set` (`self.VizMeshes`) (`local._currentIndex`) _returnvalue true)))

(fn `StoreMaxMagnitudes`
  (locals (_latestMagnitude :type "Float (double-precision)") (_currentIndex :type Integer))
  ;[1 1 1] loop through latest magnitudes
  (for (_array_element _array_index) (`self.LatestMagnitudes`)
    (set `local._latestMagnitude` _array_element)
    (set `local._currentIndex` _array_index)
    ;[1 1 1] store if current is an historic max value
    (if (> (`local._latestMagnitude`) (`|GetArrayItem` (`self.MaxMagnitudes`) (`local._currentIndex`)))
      (`KismetArrayLibrary.Array_Set` (`self.MaxMagnitudes`) (`local._currentIndex`) (`local._latestMagnitude`) true))))

(fn `UpdateMaterialEmissive`
  ;[1 1 1] modify MID emissive multiplier value
  (for (_array_element _array_index) (`self.MIDs`)
    (`MaterialInstanceDynamic.SetScalarParameterValue` _array_element "Emissive Multiplier" (* (`|GetArrayItem` (select `bool` (`self.SmoothInterpolation`) :`false` (`self.NormalizedValues`) :`true` (`self.SmoothedValues`)) _array_index) (`self.MaterialEmissiveMultiplier`)))))

(fn `UseOnlyTopMagnitudeForMax`
  (locals (_TopMagnitude :type "Float (double-precision)" :default 0.0))
  ;[1 1 1] get top magnitude of all
  (set `local._TopMagnitude` (`.MaxValue` (`KismetMathLibrary.MaxOfFloatArray` (`self.MaxMagnitudes`))))
  ;[1 1 1] write top value to all records
  (for (_ _array_index) (`self.MaxMagnitudes`)
    (`KismetArrayLibrary.Array_Set` (`self.MaxMagnitudes`) _array_index (`local._TopMagnitude`) true)))

(fn `UserConstructionScript`)