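; Speaker actor that plays a configurable sound and moves its cone mesh in time with the audio amplitude.
; BeginPlay applies the sound source and volume multiplier to the audio component.
; The component's single envelope callback tracks a running peak to normalize each value, then maps it to the cone's local Y offset.
; An unconnected alternative that scales the cone instead is left in the graph.
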(event `self.ReceiveBeginPlay`
  (`AudioComponent.SetSound` (`self.AudioComp`) (`self.SoundSource`))
  (`AudioComponent.SetVolumeMultiplier` (`self.AudioComp`) (`self.VolumeMultiplier`)))

(event `self.AudioComp.OnAudioSingleEnvelopeValue`
  (params (PlayingSoundWave :type "SoundWave Object Reference") (EnvelopeValue :type "Float (single-precision)"))
  (set `self.latestEnv` EnvelopeValue)
  ;[1 1 1] normalize
  (if (> (`self.latestEnv`) (`self.MaxEnv`))
    (set `self.MaxEnv` (`self.latestEnv`)))
  ;[1 1 1] scale mesh
  (`SceneComponent.K2_SetRelativeLocation` (`self.Cone`) (`KismetMathLibrary.MakeVector` 0.0 (`KismetMathLibrary.MapRangeClamped` (`self.latestEnv`) 0.0 (`self.MaxEnv`) -20.0 -30.0)) false false))

(fn `UserConstructionScript`)