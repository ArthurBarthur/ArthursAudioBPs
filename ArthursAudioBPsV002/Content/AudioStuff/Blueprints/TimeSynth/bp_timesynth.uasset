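; TimeSynth actor that plays a clip-based drum pattern in time with musical quantization.
; On BeginPlay it configures a TimeSynth component, binds note-quantization events and spawns a bp_TimeSynthController linked to itself.
; Half- and sixteenth-note events trigger their own clips, quarter notes trigger one near beats 1 and 3, and eighth notes only update counters.
; Quantization settings are reapplied every Tick, and clip handles are stored for quantized stopping.
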(event `self.ReceiveBeginPlay`
  (set `self.BeginPlayCalled` true)
  (`|ExecutionSequence`
    (:`then_0`
      ;[1 1 1] initialize
      (`self.ConstructSynth`)
      (`self.UpdateQuantizationSettings`)
      ;[1 1 1] handle timesynth hits (ugly for now, sorry)
      (`TimeSynthComponent.AddQuantizationEventDelegate` (`self.TimeSynth`) "EighthNote" (delegate `QuantBeat1/8`))
      (`TimeSynthComponent.AddQuantizationEventDelegate` (`self.TimeSynth`) "QuarterNote" (delegate `QuantBeat1/4`))
      (`TimeSynthComponent.AddQuantizationEventDelegate` (`self.TimeSynth`) "HalfNote" (delegate `QuantBeat1/16`))
      (`TimeSynthComponent.AddQuantizationEventDelegate` (`self.TimeSynth`) "SixteenthNote" (delegate `QuantBeat1/8t`)))
    (:`then_1`
      ;[1 1 1] spawn bp_TimeSynthController
      (bind _returnvalue (`|SpawnActorFromClass` "/Game/AudioStuff/Blueprints/TimeSynth/bp_TimeSynthController.bp_TimeSynthController_C" (`KismetMathLibrary.MakeTransform` (`KismetMathLibrary.MakeVector` (+ (.x (`SceneComponent.K2_GetComponentLocation` (`self.DefaultSceneRoot`))) 400.0) (.y (`SceneComponent.K2_GetComponentLocation` (`self.DefaultSceneRoot`))) (.z (`SceneComponent.K2_GetComponentLocation` (`self.DefaultSceneRoot`))))) "Undefined" "OverrideRootScale" null self null))
      (set `self.TimeSynthControllerRef` _returnvalue))))

(event `QuantBeat1/16`
  (params (QuantizationType :type "ETimeSynthEventQuantization Enum" :default "None") (NumBars :type Integer) (Beat :type "Float (double-precision)"))
  ;[1 1 1] handle timesynth hits (ugly for now, sorry)
  (`self.ClipPlay` 4))

(event `QuantBeat1/8t`
  (params (QuantizationType :type "ETimeSynthEventQuantization Enum" :default "None") (NumBars :type Integer) (Beat :type "Float (double-precision)"))
  ;[1 1 1] handle timesynth hits (ugly for now, sorry)
  (`self.ClipPlay` 2))

(event `QuantBeat1/8`
  (params (QuantizationType :type "ETimeSynthEventQuantization Enum" :default "None") (NumBars :type Integer) (Beat :type "Float (double-precision)"))
  ;[1 1 1] handle timesynth hits (ugly for now, sorry)
  (`/Engine/EditorBlueprintResources/StandardMacros.IncrementInt` (`self.QuantBeat1/8Count`)
    (:`  `
      (set `self.numBars` NumBars)
      (set `self.beat` Beat)
      (`|ExecutionSequence`
        (:`then_0`
          (if (== (stale _output_get) 9)
            (bind _output_get (set `self.QuantBeat1/8Count` 1))))))))

(event `QuantBeat1/4`
  (params (QuantizationType :type "ETimeSynthEventQuantization Enum" :default "None") (NumBars :type Integer) (Beat :type "Float (double-precision)"))
  ;[1 1 1] handle timesynth hits (ugly for now, sorry)
  (if (`KismetMathLibrary.NearlyEqual_FloatFloat` Beat 1.0 0.5)
    (`self.ClipPlay` 1 :!label _label)
    (elif (`KismetMathLibrary.NearlyEqual_FloatFloat` Beat 3.0 0.5)
      (goto _label))))

(event `self.ReceiveTick`
  (params (DeltaSeconds :type "Float (single-precision)"))
  ;[1 1 1] update quantization settings
  (`self.UpdateQuantizationSettings`))

(fn `ClipPlay`
  (params (DrumClipSelection :type Integer))
  (locals (ClipSelection :type Integer))
  ;[1 1 1] play clip
  (bind _output_get (set `local.ClipSelection` DrumClipSelection))
  (bind _returnvalue (`TimeSynthComponent.PlayClip` (`self.TimeSynth`) (`|GetArrayItem` (`self.Clips`) _output_get) "/Game/AudioStuff/Blueprints/TimeSynth/NewTimeSynthVolumeGroup.NewTimeSynthVolumeGroup"))
  (`KismetArrayLibrary.Array_Set` (`self.PlayedClips`) _output_get _returnvalue true))

(fn `ClipStop`
  (params (ClipSelection :type Integer))
  ;[1 1 1] stop clip
  (`TimeSynthComponent.StopClip` (`self.TimeSynth`) (`|GetArrayItem` (`self.PlayedClips`) ClipSelection) (`self.drumSampleStopQuantization`)))

(fn `ConstructSynth`
  (`/Engine/EditorBlueprintResources/StandardMacros.IsValid` (`self.TimeSynth`)
    (:`Is Valid`
      _)
    (:`Is Not Valid`
      ;[1 1 1] add timesynth
      (bind _returnvalue (`AddComponent|NODE_AddTimeSynthComponent-1`))
      (set `self.TimeSynth` _returnvalue)))
  (`ActorComponent.SetAutoActivate` (`self.TimeSynth`) (`self.AutoActivate`))
  (if (`self.BeginPlayCalled`)
    (`ActorComponent.Activate` (`self.TimeSynth`) false))
  ;[1 1 1] envelope settings
  (set `TimeSynthComponent.bIsEnvelopeFollowerEnabled` (`self.EnvFollwrEnabled`) (`self.TimeSynth`))
  (set `SynthComponent.EnvelopeFollowerAttackTime` (`self.EnvAttack`) (`self.TimeSynth`))
  (set `SynthComponent.EnvelopeFollowerReleaseTime` (`self.EnvRelease`) (`self.TimeSynth`))
  ;[1 1 1] enable spatialization
  (set `SynthComponent.bAllowSpatialization` (`self.AllowSpatialization`) (`self.TimeSynth`))
  ;[1 1 1] setup attenuation
  (set `SynthComponent.AttenuationSettings` (`self.AttenuationSettings`) (`self.TimeSynth`)))

(fn `UpdateQuantizationSettings`
  ;[1 1 1] setup quantization settings
  (`TimeSynthComponent.SetQuantizationSettings` (`self.TimeSynth`) (`self.Quantization settingz`)))

(fn `UserConstructionScript`)