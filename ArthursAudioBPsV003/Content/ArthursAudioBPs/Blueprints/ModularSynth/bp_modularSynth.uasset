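; Demo actor that plays a self-running random melody on a modular synth and spins a cube from the sound.
; BeginPlay loads the first bank preset and starts a looping timer that plays random notes, re-rolling both oscillator waveforms each time.
; A slowed timeline is meant to sweep decay, release, filter and LFO settings.
; The synth's audio envelope callback drives the cube's rotation as a simple audio-reactive visual.
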(event `self.ReceiveBeginPlay`
  ;[1 1 1] init base preset
  (`ModularSynthComponent.SetSynthPreset` (`self.ModularSynth`) (`.Preset` (break `ModularSynthPresetBankEntry` (`|GetArrayItem` (`ModularSynthPresetBank.Presets` (`self.PresetBankRef`))))))
  ;[1 1 1] activate synth
  (`ActorComponent.Activate` (`self.ModularSynth`) false)
  ;[1 1 1] looping event
  (`KismetSystemLibrary.K2_SetTimerDelegate` (delegate `PlayRandomNote`) (`KismetMathLibrary.RandomFloatInRange` 0.25 0.3) true)
  ;[1 1 1] start timeline
  (`TimelineComponent.SetPlayRate` (`self.Timeline_0`) 0.1)
  (`TimelineComponent.PlayFromStart` (`self.Timeline_0`)))

(event `PlayRandomNote`
  ;[1 1 1] looping event
  ;[1 1 1] Play random note
  (`ModularSynthComponent.NoteOn` (`self.ModularSynth`) (`KismetMathLibrary.Conv_IntToDouble` (`KismetMathLibrary.RandomIntegerInRange` 24 92)) (`KismetMathLibrary.RandomIntegerInRange` 65 120) 0.2)
  ;[1 1 1] change to random osc type
  (`ModularSynthComponent.SetOscType` (`self.ModularSynth`) 0 (select `int` (`KismetMathLibrary.RandomIntegerInRange` 0 3) :`0` "Sine" :`1` "Saw" :`2` "Triangle" :`3` "Square" :!type "ESynth1OscType Enum"))
  (`ModularSynthComponent.SetOscType` (`self.ModularSynth`) 1 (select `int` (`KismetMathLibrary.RandomIntegerInRange` 0 3) :`0` "Sine" :`1` "Saw" :`2` "Triangle" :`3` "Square" :!type "ESynth1OscType Enum")))

(event `self.ModularSynth.OnAudioEnvelopeValue`
  (params (EnvelopeValue :type "Float (single-precision)"))
  (bind _returnvalue (* EnvelopeValue 500.0))
  ;[1 1 1] hacky envelope to cube-rotation
  (`SceneComponent.K2_SetRelativeRotation` (`self.Cube`) (`KismetMathLibrary.MakeRotator` _returnvalue _returnvalue _returnvalue) false false))

(fn `UserConstructionScript`)