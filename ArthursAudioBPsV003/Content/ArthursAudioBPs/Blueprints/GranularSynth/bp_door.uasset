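; Physics-simulated door actor that drives hinge and door-frame sounds, with configurable mesh, frame and optional auto-rotation.
; Construction applies layout and physics settings; BeginPlay can spawn a Bp_GranularHinge granular-synth actor referencing the door.
; Tick derives relative yaw and angular speed, adding impulses below a target speed when auto-rotating.
; Frame overlap boxes trigger big or small bangs gated by a speed threshold, with speed-scaled volume and pitch.
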(event `self.ReceiveBeginPlay`
  (bind _boxsmalll (`self.BoxSmalll`))
  (bind _boxbigback (`self.BoxBigBack`))
  (bind _boxsmallback (`self.BoxSmallBack`))
  (bind _boxbig (`self.BoxBig`))
  ;[1 1 1] beginPlay
  (`|ExecutionSequence`
    (:`then_0`
      ;[1 1 1] store starting world rotation
      (set `self.WorldRotationAtStart` (`SceneComponent.K2_GetComponentRotation` (`self.Door`))))
    (:`then_1`
      ;[1 1 1] spawn GranularHinge
      (if (`self.SpawnGranular`)
        (bind _returnvalue (`|SpawnActorFromClass` "/Game/ArthursAudioBPs/Blueprints/GranularSynth/bp_GranularHinge.bp_GranularHinge_C" (`SceneComponent.K2_GetComponentToWorld` (`self.GranularSpawnLocation`)) "Undefined" "OverrideRootScale" null (`self.SoundForGranular`) self (`self.Reverse`) (`self.GranVolMp`) (`self.OverrideGrainProbability`) (`self.GrainProbability0-1`) (`self.Debug?`) null))
        (set `self.GranularSynthSpwnd` _returnvalue)))
    (:`then_2`
      ;[1 1 1] doorframeBang
      ;;[1 1 1] init
      (`/Engine/EditorBlueprintResources/StandardMacros.IsValid` _boxbig
        (:`Is Valid`
          (add `PrimitiveComponent.OnComponentBeginOverlap` _boxbig (delegate `BoxBigOverlap`))
          (`/Engine/EditorBlueprintResources/StandardMacros.IsValid` _boxsmalll
            (:`Is Valid`
              (add `PrimitiveComponent.OnComponentBeginOverlap` _boxsmalll (delegate `BoxSmallOverlap`))
              (`/Engine/EditorBlueprintResources/StandardMacros.IsValid` _boxbigback
                (:`Is Valid`
                  (add `PrimitiveComponent.OnComponentBeginOverlap` _boxbigback (delegate `BoxBigBackOverllap`))
                  (`/Engine/EditorBlueprintResources/StandardMacros.IsValid` _boxsmallback
                    (:`Is Valid`
                      (add `PrimitiveComponent.OnComponentBeginOverlap` _boxsmallback (delegate `BoxBigBackOverlap`)))))))))))))

(event `BoxBigOverlap`
  (params (OverlappedComponent :type "PrimitiveComponent Object Reference") (OtherActor :type "Actor Object Reference") (OtherComp :type "PrimitiveComponent Object Reference") (OtherBodyIndex :type Integer) (bFromSweep :type Boolean) (SweepResult :type "HitResult Structure (by ref)"))
  ;[1 1 1] doorframeBang
  ;;[1 1 1] coll
  (`self.BigBang` (`self.BoxBig`)))

(event `BoxSmallOverlap`
  (params (OverlappedComponent :type "PrimitiveComponent Object Reference") (OtherActor :type "Actor Object Reference") (OtherComp :type "PrimitiveComponent Object Reference") (OtherBodyIndex :type Integer) (bFromSweep :type Boolean) (SweepResult :type "HitResult Structure (by ref)"))
  ;[1 1 1] doorframeBang
  ;;[1 1 1] coll
  (`self.SmallBang` (`self.BoxSmalll`)))

(event `BoxBigBackOverllap`
  (params (OverlappedComponent :type "PrimitiveComponent Object Reference") (OtherActor :type "Actor Object Reference") (OtherComp :type "PrimitiveComponent Object Reference") (OtherBodyIndex :type Integer) (bFromSweep :type Boolean) (SweepResult :type "HitResult Structure (by ref)"))
  ;[1 1 1] doorframeBang
  ;;[1 1 1] coll
  (`self.BigBang` (`self.BoxBigBack`)))

(event `self.ReceiveTick`
  (params (DeltaSeconds :type "Float (single-precision)"))
  ;[1 1 1] tick
  (`|ExecutionSequence`
    (:`then_0`
      ;[1 1 1] calc doorphysics
      (set `self.LatestDeltaTick` DeltaSeconds)
      (`self.GetDoorRot`)
      (`self.GetDoorVelocity`))
    (:`then_1`
      ;[1 1 1] rotate it
      (if (`self.AutoRotate`)
        (if (< (`self.DoorVelocity0-2000`) (`self.RotationRate`))
          (`PrimitiveComponent.AddAngularImpulseInDegrees` (`self.Door`) (`self.Acceleration`) "None" true))))))

(event `BoxBigBackOverlap`
  (params (OverlappedComponent :type "PrimitiveComponent Object Reference") (OtherActor :type "Actor Object Reference") (OtherComp :type "PrimitiveComponent Object Reference") (OtherBodyIndex :type Integer) (bFromSweep :type Boolean) (SweepResult :type "HitResult Structure (by ref)"))
  ;[1 1 1] doorframeBang
  ;;[1 1 1] coll
  (`self.SmallBang` (`self.BoxSmallBack`)))

(fn `BigBang`
  (params (CollBox :type "SceneComponent Object Reference"))
  (bind (_returnvalue_location _returnvalue_rotation) (`KismetMathLibrary.BreakTransform` (`SceneComponent.K2_GetComponentToWorld` CollBox)))
  (bind _returnvalue (`KismetMathLibrary.FClamp` (`KismetMathLibrary.MapRangeClamped` (`self.DoorVelocity0-2000`) 80.0 150.0 0.0 1.0)))
  (bind _returnvalue_2 (`KismetMathLibrary.Lerp` 0.9 1.1 _returnvalue))
  ;[1 1 1] BigBanglogic
  (if (> (`self.DoorVelocity0-2000`) 80.0)
    (`GameplayStatics.PlaySoundAtLocation` (`self.FrameBangBig`) _returnvalue_location _returnvalue_rotation _returnvalue _returnvalue_2 0.0 "/Game/ArthursAudioBPs/Blueprints/GranularSynth/GranularSoundAttenuation.GranularSoundAttenuation" null null)
    (`GameplayStatics.PlaySoundAtLocation` (`self.FrameBangSmall`) _returnvalue_location _returnvalue_rotation _returnvalue _returnvalue_2 0.0 "/Game/ArthursAudioBPs/Blueprints/GranularSynth/GranularSoundAttenuation.GranularSoundAttenuation" null null)))

(fn `GetDoorRot`
  (bind (_worldrotationatstart_roll _worldrotationatstart_pitch _worldrotationatstart_yaw) (`KismetMathLibrary.BreakRotator` (`self.WorldRotationAtStart`)))
  (bind (_returnvalue_roll _returnvalue_pitch _returnvalue_yaw) (`KismetMathLibrary.BreakRotator` (`SceneComponent.K2_GetComponentRotation` (`self.Door`))))
  ;[1 1 1] calc door rotation
  (bind _output_get (set `self.LatestDoorRot360-0` (mod (+ 360.0 (- _returnvalue_yaw _worldrotationatstart_yaw)) 360.0)))
  (if (`self.Debug?`)
    ;[1 1 1] print result when moving
    (if (> (`self.DoorVelocity0-2000`) 1.0)
      (`KismetSystemLibrary.PrintString` (`KismetStringLibrary.BuildString_Double` "" "DoorRelRot: " _output_get) true true (struct :`G` 0.66 :`B` 1.0 :`A` 1.0) (`self.LatestDeltaTick`)))))

(fn `GetDoorVelocity`
  ;[1 1 1] calc velocity
  (set `self.DoorVelocity0-2000` (/ (`KismetMathLibrary.Abs` (- (`self.PreviousLatestDoorRot360-0`) (`self.LatestDoorRot360-0`))) (`self.LatestDeltaTick`)))
  (set `self.PreviousLatestDoorRot360-0` (`self.LatestDoorRot360-0`))
  (if (`self.Debug?`)
    ;[1 1 1] print result when moving
    (if (> (`self.DoorVelocity0-2000`) 1.0)
      (`KismetSystemLibrary.PrintString` (`KismetStringLibrary.BuildString_Double` "" "DoorVelocity: " (`self.DoorVelocity0-2000`)) true true (struct :`G` 0.66 :`B` 1.0 :`A` 1.0) (`self.LatestDeltaTick`)))))

(fn `SetUpDoor`
  (`|ExecutionSequence`
    (:`then_0`
      ;[1 1 1] location
      (`SceneComponent.K2_SetRelativeLocation` (`self.Door`) (`self.DoorRelativeLocation`) false false)
      (`SceneComponent.K2_SetRelativeLocation` (`self.DoorStop0`) (`self.FrameClosedLoc`) false false)
      (`SceneComponent.K2_SetRelativeLocation` (`self.DoorStop1`) (`self.FrameOpenLoc`) false false))
    (:`then_1`
      ;[1 1 1] scale
      (`SceneComponent.SetRelativeScale3D` (`self.Door`) (`self.Scale`)))
    (:`then_2`
      ;[1 1 1] mesh
      (`StaticMeshComponent.SetStaticMesh` (`self.Door`) (`self.DoorMesh`)))
    (:`then_3`
      ;[1 1 1] FrameVisible?
      (if (not (`self.FrameVisible?`))
        (`SceneComponent.SetVisibility` (`self.DoorStop0`) false false)
        (`SceneComponent.SetVisibility` (`self.DoorStop1`) false false)
        (`SceneComponent.SetVisibility` (`self.BoxBig`) false false)
        (`SceneComponent.SetVisibility` (`self.BoxSmalll`) false false)))
    (:`then_4`
      ;[1 1 1] DoorframeAtAll?
      (if (not (`self.DoorFrame`))
        (`ActorComponent.K2_DestroyComponent` (`self.DoorStop0`))
        (`ActorComponent.K2_DestroyComponent` (`self.DoorStop1`))
        (`ActorComponent.K2_DestroyComponent` (`self.BoxBig`))
        (`ActorComponent.K2_DestroyComponent` (`self.BoxSmalll`))))
    (:`then_5`
      ;[1 1 1] physics
      (`PrimitiveComponent.SetAngularDamping` (`self.Door`) (`self.AnguarDamping`))
      (`PrimitiveComponent.SetLinearDamping` (`self.Door`) (`self.LinearDamping`))
      (`PrimitiveComponent.SetEnableGravity` (`self.Door`) false)
      (`PrimitiveComponent.SetCollisionObjectType` (`self.Door`) "ECC_PhysicsBody")
      (`PrimitiveComponent.SetCollisionResponseToAllChannels` (`self.Door`) "ECR_Block")
      (`PrimitiveComponent.SetSimulatePhysics` (`self.Door`) true))))

(fn `SmallBang`
  (params (CollBox :type "SceneComponent Object Reference"))
  (bind (_returnvalue_location _returnvalue_rotation) (`KismetMathLibrary.BreakTransform` (`SceneComponent.K2_GetComponentToWorld` CollBox)))
  (bind _returnvalue (`KismetMathLibrary.FClamp` (`KismetMathLibrary.MapRangeClamped` (`self.DoorVelocity0-2000`) 0.0 80.0 0.0 1.0)))
  ;[1 1 1] SmallBangLogic
  (if (< (`self.DoorVelocity0-2000`) 80.0)
    (`GameplayStatics.PlaySoundAtLocation` (`self.FrameBangSmall`) _returnvalue_location _returnvalue_rotation _returnvalue (`KismetMathLibrary.Lerp` 0.9 1.1 _returnvalue) 0.0 "/Game/ArthursAudioBPs/Blueprints/GranularSynth/GranularSoundAttenuation.GranularSoundAttenuation" null null)))

(fn `UserConstructionScript`
  (`self.SetUpDoor`))